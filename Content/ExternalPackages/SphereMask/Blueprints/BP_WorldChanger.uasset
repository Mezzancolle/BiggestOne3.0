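; Sphere-mask actor that switches tagged world objects between present and old-world states inside a scalable sphere.
; Timelines scale the sphere on enable, disable or resize, writing its location and scale to a Material Parameter Collection by sphere ID.
; BeginPlay and overlaps use mask tags to toggle objects' collision and shadows, notifying I_WorldChangable owners.
; An overlap count re-opens the sphere if objects still overlap when closing finishes.
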(event Custom|EnableSphereMask
  (params (Enable? :type Boolean) (CheckInside/Outside :type Boolean))
  ;[1 1 1] Spheremask enable/disable animation + tick enable/disable
  (Default|CallOnChangeState Enable?)
  (Variables|Default|SetIsEnabled? Enable?)
  (Variables|Default|SetShouldCheckCollisions? true)
  (if Enable?
    (bind _alpha (Timeline|TL_ScaleUp Play)
      (:Update
        (if CheckInside/Outside
          (Transformation|SetWorldScale3D (Variables|Default|GetBP_ExternalSphere) (Math|Conversions|ToVector(Float) (Math|Float|Lerp (Variables|Default|GetMinimumSphereScale) (Variables|Default|GetMaximumSphereScaleInside) _alpha)))
          (CallFunction|SetMaterialParameters)
          (else
            (Transformation|SetWorldScale3D (Variables|Default|GetBP_ExternalSphere) (Math|Conversions|ToVector(Float) (Math|Float|Lerp (Variables|Default|GetMinimumSphereScale) (Variables|Default|GetMaximumSphereScaleOutside) _alpha)))
            (CallFunction|SetMaterialParameters))))
      (:Finished
        (Variables|Default|SetShouldCheckCollisions? (Variables|Default|GetIsEnabled?))
        (if (not (Variables|Default|GetIsEnabled?))
          (if (> (Variables|Default|GetOvelappingObjectsAmount) 0)
            (CallFunction|EnableSphereMask true false)
            (else
              (Variables|Default|SetOvelappingObjectsAmount 0)
              (Transformation|SetWorldScale3D (Variables|Default|GetBP_ExternalSphere) "0, 0, 0")
              (CallFunction|SetMaterialParameters))))))
    (else
      (Timeline|TL_ScaleUp Reverse))))

(event Custom|ResizeScale
  (params (CheckInside/Outside :type Boolean))
  (if (Variables|Default|GetIsEnabled?)
    (bind _alpha (Timeline|TL_ScaleResize PlayFromStart)
      (:Update
        (if CheckInside/Outside
          (Transformation|SetWorldScale3D (Variables|Default|GetBP_ExternalSphere) (Math|Conversions|ToVector(Float) (Math|Float|Lerp (Variables|Default|GetMaximumSphereScaleOutside) (Variables|Default|GetMaximumSphereScaleInside) _alpha)))
          (CallFunction|SetMaterialParameters)
          (else
            (Transformation|SetWorldScale3D (Variables|Default|GetBP_ExternalSphere) (Math|Conversions|ToVector(Float) (Math|Float|Lerp (Variables|Default|GetMaximumSphereScaleInside) (Variables|Default|GetMaximumSphereScaleOutside) _alpha)))
            (CallFunction|SetMaterialParameters)))))))

(event EventBeginPlay
  ;[1 1 1] Setup collision into trigger when hidden ands outside of the sphere at the beginning
  (bind _outactors (Actor|GetAllActorswithTag (Variables|Default|GetWorldChangerTag)))
  (for _array_element _outactors
    (CallFunction|SetObjectVisibility (Actor|GetComponentsByClass _array_element "/Script/Engine.PrimitiveComponent") (Actor|ActorHasTag _array_element (Variables|Default|GetTagPresentMask)))))

(event Collision|EventActorBeginOverlap
  (params (OtherActor :type Actor%20Object%20Reference))
  ;[0.06447 0.1855 1 1 30] Start collision with a item affected by a Spheremask
  (if (Variables|Default|GetShouldCheckCollisions?)
    ;;[0.2031 0.2031 0.2031] Detect if the item is affected by a sphere
    (if (Actor|ActorHasTag OtherActor (Variables|Default|GetWorldChangerTag))
      (Math|Integer|IncrementInt (Variables|Default|GetOvelappingObjectsAmount)
        (:%20%20
          (CallFunction|SetObjectVisibility (Actor|GetComponentsByClass OtherActor "/Script/Engine.PrimitiveComponent") (Actor|ActorHasTag OtherActor (Variables|Default|GetTagOldMask))))))))

(event Collision|EventActorEndOverlap
  (params (OtherActor :type Actor%20Object%20Reference))
  ;[0.06447 0.1855 1] End collision with a item affected by a Spheremask
  (if (Variables|Default|GetShouldCheckCollisions?)
    ;;[0.2031 0.2031 0.2031] Detect if the item is affected by a sphere
    (if (Actor|ActorHasTag OtherActor (Variables|Default|GetWorldChangerTag))
      (Math|Integer|DecrementInt (Variables|Default|GetOvelappingObjectsAmount)
        (:%20%20
          ;;[0.2031 0.2031 0.2031] Detect if the item is affected by this sphere
          (CallFunction|SetObjectVisibility (Actor|GetComponentsByClass OtherActor "/Script/Engine.PrimitiveComponent") (not (Actor|ActorHasTag OtherActor (Variables|Default|GetTagOldMask)))))))))

(fn ConstructionScript)

(fn SetMaterialParameters
  (bind _worldspheredatas (Variables|Default|GetWorldSphereDatas))
  ;[0.1406 0.1406 0.1406] setup Material collection parametter Location Example : VariableName+idSphere = Location0
  (Rendering|Material|SetVectorParameterValue _worldspheredatas (Utilities|String|StringToName (Utilities|String|Append (Variables|Default|GetParameter%20Name%20Location) (Utilities|String|ToString(Integer) (Variables|Default|GetIDSphere)))) (Math|Conversions|ToLinearColor(Vector) (Transformation|GetActorLocation)) :!class /Script/Engine.KismetMaterialLibrary)
  ;[0.1406 0.1406 0.1406] setup Material collection parametter Scale Example : VariableName+idSphere = Scale0
  ;;[0.1406 0.1406 0.1406] setup Material collection parametter Scale Example : VariableName+idSphere = Scale0
  (Rendering|Material|SetVectorParameterValue _worldspheredatas (Utilities|String|StringToName (Utilities|String|Append (Variables|Default|GetParameter%20Name%20Scale) (Utilities|String|ToString(Integer) (Variables|Default|GetIDSphere)))) (Math|Conversions|ToLinearColor(Vector) (Transformation|GetWorldScale (Variables|Default|GetBP_ExternalSphere))) :!class /Script/Engine.KismetMaterialLibrary))

(fn SetObjectVisibility
  (params (Primitives :type Array%20of%20Primitive%20Component%20Object%20References) (Visible? :type Boolean))
  (if Visible?
    (for _array_element Primitives
      (Collision|SetCollisionResponsetoChannel _array_element "ECC_Pawn" "ECR_Block")
      (Collision|SetCollisionResponsetoChannel _array_element "ECC_Camera" "ECR_Block")
      (Collision|SetCollisionResponsetoChannel _array_element "ECC_PhysicsBody" "ECR_Block")
      (Rendering|SetCastShadow _array_element true)
      (if (not (Components|ComponentHasTag _array_element "NO!"))
        (Collision|SetCollisionResponsetoChannel _array_element "ECC_GameTraceChannel2" "ECR_Block")
        (if (Utilities|DoesObjectImplementInterface (Components|GetOwner _array_element) "/Game/Blueprint/Interfaces/I_WorldChangable.I_WorldChangable_C")
          (Class|IWorldChangable|OnOldWest(Message) (Components|GetOwner _array_element)))))
    (else
      (for _array_element_2 Primitives
        (Collision|SetCollisionResponsetoChannel _array_element_2 "ECC_Pawn" "ECR_Ignore")
        (Collision|SetCollisionResponsetoChannel _array_element_2 "ECC_Camera" "ECR_Ignore")
        (Collision|SetCollisionResponsetoChannel _array_element_2 "ECC_PhysicsBody" "ECR_Ignore")
        (Rendering|SetCastShadow _array_element_2 false)
        (Collision|SetCollisionResponsetoChannel _array_element_2 "ECC_GameTraceChannel2" "ECR_Ignore")
        (if (Utilities|DoesObjectImplementInterface (Components|GetOwner _array_element_2) "/Game/Blueprint/Interfaces/I_WorldChangable.I_WorldChangable_C")
          (Class|IWorldChangable|OnPresentWest(Message) (Components|GetOwner _array_element_2)))))))

(fn CheckforCollisions
  (params (IsClosing? :type Boolean))
  (bind _outhits (Collision|MultiSphereTraceByChannel (Transformation|GetActorLocation) (Transformation|GetActorLocation) 25.0 "TraceTypeQuery1" false 0 "Persistent"))
  (for _array_element _outhits
    (if (Actor|ActorHasTag (.HitActor (Collision|BreakHitResult _array_element)) "WC")
      (return false)))
  (return true))