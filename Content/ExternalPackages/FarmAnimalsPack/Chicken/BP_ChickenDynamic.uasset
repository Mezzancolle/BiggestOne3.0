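; Chicken actor that runs along one of two splines and destroys itself at the end.
; StartRunning sets IsRunning and uses FromPath to choose PathSpline or SchoolSpline, each driven by its own timeline.
; Timeline updates move the skeletal mesh along the spline with a 90-degree yaw offset.
; Play rate scales with spline length for constant speed, but is only set on MoveAlongSpline, even when the school route plays the other timeline.
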(event Custom|StartRunning
  (params (FromPath? :type Boolean))
  (if FromPath?
    (Variables|Default|SetIsRunning? true)
    (Variables|Default|SetSplineLength (Spline|GetSplineLength (Variables|Default|GetPathSpline)))
    (Components|Timeline|SetPlayRate (Variables|Default|GetMoveAlongSpline) (/ 1.0 (/ (Variables|Default|GetSplineLength) 402.0)))
    (bind _distance (Timeline|MoveAlongSpline PlayFromStart)
      (:Update
        (Transformation|SetWorldTransform (Variables|Default|GetSK_Chicken) (Math|Transform|MakeTransform (.location (Spline|GetTransformatDistanceAlongSpline (Variables|Default|GetPathSpline) (* _distance (Variables|Default|GetSplineLength)) "World" false)) (Math|Rotator|MakeRotator (.roll (.rotation (Spline|GetTransformatDistanceAlongSpline (Variables|Default|GetPathSpline) (* _distance (Variables|Default|GetSplineLength)) "World" false))) (.pitch (.rotation (Spline|GetTransformatDistanceAlongSpline (Variables|Default|GetPathSpline) (* _distance (Variables|Default|GetSplineLength)) "World" false))) (+ (.yaw (.rotation (Spline|GetTransformatDistanceAlongSpline (Variables|Default|GetPathSpline) (* _distance (Variables|Default|GetSplineLength)) "World" false))) 9e+01)) (.scale (Spline|GetTransformatDistanceAlongSpline (Variables|Default|GetPathSpline) (* _distance (Variables|Default|GetSplineLength)) "World" false))) false false))
      (:Finished
        (Actor|DestroyActor)))
    (else
      (Variables|Default|SetIsRunning? true)
      (Variables|Default|SetSplineLength (Spline|GetSplineLength (Variables|Default|GetSchoolSpline)))
      (Components|Timeline|SetPlayRate (Variables|Default|GetMoveAlongSpline) (/ 1.0 (/ (Variables|Default|GetSplineLength) 402.0)))
      (bind _distance_2 (Timeline|Timeline PlayFromStart)
        (:Update
          (Transformation|SetWorldTransform (Variables|Default|GetSK_Chicken) (Math|Transform|MakeTransform (.location (Spline|GetTransformatDistanceAlongSpline (Variables|Default|GetSchoolSpline) (* _distance_2 (Variables|Default|GetSplineLength)) "World" false)) (Math|Rotator|MakeRotator (.roll (.rotation (Spline|GetTransformatDistanceAlongSpline (Variables|Default|GetSchoolSpline) (* _distance_2 (Variables|Default|GetSplineLength)) "World" false))) (.pitch (.rotation (Spline|GetTransformatDistanceAlongSpline (Variables|Default|GetSchoolSpline) (* _distance_2 (Variables|Default|GetSplineLength)) "World" false))) (+ (.yaw (.rotation (Spline|GetTransformatDistanceAlongSpline (Variables|Default|GetSchoolSpline) (* _distance_2 (Variables|Default|GetSplineLength)) "World" false))) 9e+01)) (.scale (Spline|GetTransformatDistanceAlongSpline (Variables|Default|GetSchoolSpline) (* _distance_2 (Variables|Default|GetSplineLength)) "World" false))) false false))
        (:Finished
          (Actor|DestroyActor))))))

(fn ConstructionScript)