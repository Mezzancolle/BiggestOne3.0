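; BP_ChickenDynamicEvent is a trigger actor that sets a group of chickens running when the player first walks into its EventTrigger.
; A DoOnce gate limits the overlap response to the player character and a single firing.
; QueueChickens then calls StartRunning on each entry in the Chickens array one at a time, re-calling itself after a delay so the starts are spread evenly across TriggerDuration.
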(event OnComponentBeginOverlap(EventTrigger)
  (params (OverlappedComponent :type Primitive%20Component%20Object%20Reference) (OtherActor :type Actor%20Object%20Reference) (OtherComp :type Primitive%20Component%20Object%20Reference) (OtherBodyIndex :type Integer) (bFromSweep :type Boolean) (SweepResult :type Hit%20Result%20Structure%20%28by%20ref%29))
  (if (== OtherActor (Game|GetPlayerCharacter 0))
    (Utilities|FlowControl|DoOnce false
      (:Completed
        (CallFunction|QueueChickens)))))

(event Custom|QueueChickens
  (if (!= (Utilities|Array|Length (Variables|Default|GetChickens)) (Variables|Default|GetIndex))
    (Default|StartRunning (Utilities|Array|Get(acopy) (Variables|Default|GetChickens) (Variables|Default|GetIndex)))
    (Math|Integer|IncrementInt (Variables|Default|GetIndex)
      (:%20%20
        (Utilities|FlowControl|Delay (/ (Variables|Default|GetTriggerDuration) (Utilities|Array|Length (Variables|Default|GetChickens))))
        (CallFunction|QueueChickens)))))

(event EventBeginPlay)

(fn ConstructionScript)