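; Winter weather actor that drives autumn and snow amounts in the MPC_MW_Controller material parameter collection, with optional snow particles.
; The construction script and BeginPlay push the autumn amount, and BeginPlay either sets snow directly or starts a delayed accumulation timeline.
; SnowAnimation replays that timeline from zero up to the collection's current snow value.
; When particles are enabled, Tick smoothly interpolates the particle system toward the player pawn.
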(event EventBeginPlay
  (bind _snowamount (Variables|Snow|GetSnowAmount))
  (Rendering|Material|SetScalarParameterValue "/Game/ExternalPackages/MWCommon/_Legacy2/Materials/MASTER/Par/MPC_MW_Controller.MPC_MW_Controller" "MW_AutumnAmount" (Variables|Autumn|GetAutumnAmount) :!class /Script/Engine.KismetMaterialLibrary)
  (Components|Activation|SetActive (Variables|Default|GetParticleSystem) (Variables|Snow|GetSnowUseParticles) false)
  (if (Variables|Snow|GetSnowUseAnimation)
    (Utilities|FlowControl|Delay (Variables|Snow|GetSnowAccumulationDelay))
    (Components|Timeline|SetPlayRate (Variables|Default|GetSnowAccumulation) (/ 1.0 (Variables|Snow|GetSnowAccumulationTime)))
    (bind _snowamount_2 (Timeline|SnowAccumulation PlayFromStart)
      (:Update
        (Rendering|Material|SetScalarParameterValue "/Game/ExternalPackages/MWCommon/_Legacy2/Materials/MASTER/Par/MPC_MW_Controller.MPC_MW_Controller" "MW_SnowAmount" (Math|Float|Lerp 0.0 (Variables|Snow|GetSnowAmount) _snowamount_2) :!class /Script/Engine.KismetMaterialLibrary))
      (:Finished
        (Rendering|Material|SetScalarParameterValue "/Game/ExternalPackages/MWCommon/_Legacy2/Materials/MASTER/Par/MPC_MW_Controller.MPC_MW_Controller" "MW_SnowAmount" _snowamount :!class /Script/Engine.KismetMaterialLibrary)
        (Development|PrintString "Snow Animation Completed")))
    (else
      (Rendering|Material|SetScalarParameterValue "/Game/ExternalPackages/MWCommon/_Legacy2/Materials/MASTER/Par/MPC_MW_Controller.MPC_MW_Controller" "MW_SnowAmount" _snowamount :!class /Script/Engine.KismetMaterialLibrary))))

(event EventTick
  (params (DeltaSeconds :type Float%20%28single-precision%29))
  (bind _particlesystem (Variables|Default|GetParticleSystem))
  (if (Variables|Snow|GetSnowUseParticles)
    (Transformation|SetWorldLocation _particlesystem (Math|Interpolation|VInterpTo (Transformation|GetWorldLocation _particlesystem) (Transformation|GetActorLocation (Game|Player|GetPlayerPawn 0)) DeltaSeconds 1.0) false false)))

(event EventSnowAnimation
  (Development|PrintString "Running Snow Animation")
  (bind _returnvalue (Rendering|Material|GetScalarParameterValue "/Game/ExternalPackages/MWCommon/_Legacy2/Materials/MASTER/Par/MPC_MW_Controller.MPC_MW_Controller" "MW_SnowAmount" :!class /Script/Engine.KismetMaterialLibrary))
  (Variables|Snow|SetSnowAmount _returnvalue)
  (Rendering|Material|SetScalarParameterValue "/Game/ExternalPackages/MWCommon/_Legacy2/Materials/MASTER/Par/MPC_MW_Controller.MPC_MW_Controller" "MW_SnowAmount" 0.0 :!class /Script/Engine.KismetMaterialLibrary)
  (Components|Timeline|SetPlayRate (Variables|Default|GetSnowAccumulation) (/ 1.0 (Variables|Snow|GetSnowAccumulationTime)))
  (bind _snowamount (Timeline|SnowAccumulation PlayFromStart)
    (:Update
      (Rendering|Material|SetScalarParameterValue "/Game/ExternalPackages/MWCommon/_Legacy2/Materials/MASTER/Par/MPC_MW_Controller.MPC_MW_Controller" "MW_SnowAmount" (Math|Float|Lerp 0.0 (Variables|Snow|GetSnowAmount) _snowamount) :!class /Script/Engine.KismetMaterialLibrary))
    (:Finished
      (Rendering|Material|SetScalarParameterValue "/Game/ExternalPackages/MWCommon/_Legacy2/Materials/MASTER/Par/MPC_MW_Controller.MPC_MW_Controller" "MW_SnowAmount" (Variables|Snow|GetSnowAmount) :!class /Script/Engine.KismetMaterialLibrary)
      (Development|PrintString "Snow Animation Completed"))))

(fn ConstructionScript
  (Rendering|Material|SetScalarParameterValue "/Game/ExternalPackages/MWCommon/_Legacy2/Materials/MASTER/Par/MPC_MW_Controller.MPC_MW_Controller" "MW_AutumnAmount" (Variables|Autumn|GetAutumnAmount) :!class /Script/Engine.KismetMaterialLibrary))