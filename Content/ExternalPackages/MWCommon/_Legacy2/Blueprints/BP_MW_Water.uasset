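; BP_MW_Water is a water actor that sets up a water surface and a dirt mesh and publishes its height as the world water line.
; The construction script and BeginPlay run the same logic, assigning WaterMaterial and DirtMaterial to their meshes.
; Both also write the root's world Z to MW_WaterLine in the MPC_MW_Controller parameter collection, exposing the water height to materials that read it.
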(event EventBeginPlay
  (Rendering|Material|SetMaterial (Variables|Default|GetSM_Water) 0 (Variables|Water|GetWaterMaterial))
  (Rendering|Material|SetMaterial (Variables|Default|GetSM_Dirt) 0 (Variables|Water|GetDirt%20Material))
  (Rendering|Material|SetScalarParameterValue "/Game/ExternalPackages/MWCommon/_Legacy2/Materials/MASTER/Par/MPC_MW_Controller.MPC_MW_Controller" "MW_WaterLine" (.z (.location (Transformation|GetWorldTransform (Variables|Default|GetDefaultSceneRoot)))) :!class /Script/Engine.KismetMaterialLibrary))

(fn ConstructionScript
  (Rendering|Material|SetMaterial (Variables|Default|GetSM_Water) 0 (Variables|Water|GetWaterMaterial))
  (Rendering|Material|SetMaterial (Variables|Default|GetSM_Dirt) 0 (Variables|Water|GetDirt%20Material))
  (Rendering|Material|SetScalarParameterValue "/Game/ExternalPackages/MWCommon/_Legacy2/Materials/MASTER/Par/MPC_MW_Controller.MPC_MW_Controller" "MW_WaterLine" (.z (.location (Transformation|GetWorldTransform (Variables|Default|GetDefaultSceneRoot)))) :!class /Script/Engine.KismetMaterialLibrary))