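; Bird character that walks with foot IK and flies using physics.
; Tick eases turn and forward speeds, then runs foot traces while walking to set tarsus effector offsets and ground-aligned rotations.
; Soar clears behavior flags, enables capsule physics and launches into Flying mode, where Tick applies force and yaw torque.
; When flight inputs are near zero without upward motion, a downward trace triggers Landing, restoring walking and disabling physics.
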(event EventBeginPlay)

(event Collision|EventActorBeginOverlap
  (params (OtherActor :type Actor%20Object%20Reference)))

(event EventTick
  (params (DeltaSeconds :type Float%20%28single-precision%29))
  (bind _capsulecomponent (Variables|Collision|GetCapsuleComponent))
  (bind _capsulecomponent_2 (Variables|Collision|GetCapsuleComponent))
  (bind _capsulecomponent_3 (Variables|Collision|GetCapsuleComponent))
  (bind _capsulecomponent_4 (Variables|Collision|GetCapsuleComponent))
  (bind _capsulecomponent_5 (Variables|Collision|GetCapsuleComponent))
  (bind _returnvalue (Transformation|GetWorldLocation _capsulecomponent_2))
  (bind (_x _y _z) (Math|Vector|BreakVector _returnvalue))
  (Variables|デフォルト|SetDeltaSeconds DeltaSeconds)
  ;[1 1 1] Set the TurnSpeed.
  (Variables|Locomotion|SetTurnSpeed (Math|Interpolation|FInterpTo (Variables|Locomotion|GetTurnSpeed) (Variables|Locomotion|GetAimTurnSpeed) (Variables|デフォルト|GetDeltaSeconds) 1.0))
  ;[1 1 1] Set the ForwardSpeed
  (Variables|Locomotion|SetForwardSpeed (Math|Interpolation|FInterpTo (Variables|Locomotion|GetForwardSpeed) (Variables|Locomotion|GetAimForwardSpeed) (Variables|デフォルト|GetDeltaSeconds) 1.0))
  ;[1 1 1] IsWalking?
  (if (Pawn|Components|CharacterMovement|IsWalking (Variables|Character|GetCharacterMovement))
    (CallFunction|FootPlacement)
    (else
      ;[1 1 1] IsFalling?
      (if (not (AI|Components|NavMovement|IsFalling (Variables|Character|GetCharacterMovement)))
        ;[1 1 1] IsFlying?
        (if (Class|NavMovementComponent|IsFlying (Variables|Character|GetCharacterMovement))
          ;[1 1 1] Movement mode is Flying and IsTryLandPerch is false.
          (Physics|AddForce _capsulecomponent (+ (* (Math|Vector|GetForwardVector _capsulecomponent) (Variables|Locomotion|GetFlyForwardForce)) (* (Math|Vector|GetUpVector _capsulecomponent) (Variables|Locomotion|GetFlyUpForce))) "None" false)
          (Class|PrimitiveComponent|AddTorqueinDegrees _capsulecomponent_3 (* (Math|Vector|GetUpVector _capsulecomponent_3) (Variables|Locomotion|GetFlyYawTorque)) "None" false)
          (Variables|Locomotion|SetFlyForwardVelocity (Math|Vector|DotProduct (Transformation|GetComponentVelocity _capsulecomponent_4) (Math|Vector|GetForwardVector _capsulecomponent_4)))
          (Variables|Locomotion|SetFlyUpVelocity (Math|Vector|DotProduct (Transformation|GetComponentVelocity _capsulecomponent_5) (Math|Vector|GetUpVector _capsulecomponent_5)))
          (Variables|Locomotion|SetFlyYawVelocity (.Z (Math|Vector|BreakVector (Physics|GetPhysicsAngularVelocityinDegrees (Variables|Collision|GetCapsuleComponent) "None"))))
          (if (Math|Boolean|ANDBoolean (< (Math|Float|Absolute(Float) (Variables|Locomotion|GetFlyForwardForce)) 1.0) (< (Math|Float|Absolute(Float) (Variables|Locomotion|GetFlyUpForce)) 1.0) (< (Math|Float|Absolute(Float) (Variables|Locomotion|GetFlyYawTorque)) 1.0) (<= (Variables|Locomotion|GetFlyUpVelocity) 0.1))
            (Variables|Behavior|SetIsSoaring false)
            ;;[1 1 1] Determining whether the bird is close to the ground or not.
            (bind _returnvalue_2 (Collision|LineTraceByChannel (Transformation|GetWorldLocation (Variables|Collision|GetCapsuleComponent)) (Math|Vector|MakeVector _x _y (- _z (Variables|IK|GetIKTraceDistance))) "TraceTypeQuery1" false 0 "None"))
            (if _returnvalue_2
              (CallFunction|Landing))))))))

(fn ConstructionScript
  ;[1 1 1] Set the scale.
  (Variables|Default|SetScale (.Z (Math|Vector|BreakVector (.Scale (Math|Transform|BreakTransform (Transformation|GetActorTransform))))))
  ;[1 1 1] Set the scale dependent variables.
  (Variables|IK|SetMaxLegIKOffset (* (Variables|IK|GetMaxLegIKOffset) (Variables|Default|GetScale)))
  (Variables|IK|SetIKTraceDistance (* (Variables|IK|GetIKTraceDistance) (Variables|Default|GetScale))))

(fn FootPlacement
  ;[1 1 1] Calculate L_Tarsus_2 effector's transform.
  (bind (_ikheightoffsett _footisgrounded _footrot _grounddistance _ikeffectorloc) (CallFunction|TraceIKEffector (Variables|IK|GetL_FootName) (Variables|IK|GetIKTraceDistance) 0.0))
  (Variables|IK|SetL_Tarsus_2EffectorOffsetLoc _ikeffectorloc)
  (Variables|IK|SetL_Tarsus_2Rot _footrot)
  ;[1 1 1] Calculate R_Tarsus_2 effector's transform.
  (bind (_ikheightoffsett_2 _footisgrounded_2 _footrot_2 _grounddistance_2 _ikeffectorloc_2) (CallFunction|TraceIKEffector (Variables|IK|GetR_FootName) (Variables|IK|GetIKTraceDistance) 0.0))
  (Variables|IK|SetR_Tarsus_2EffectorOffsetLoc _ikeffectorloc_2)
  (Variables|IK|SetR_Tarsus_2Rot _footrot_2))

(fn TraceIKEffector
  (params (FootName :type Name) (TraceDistance :type Float%20%28double-precision%29) (HeightOffset :type Float%20%28double-precision%29))
  (bind _mesh (Variables|Character|GetMesh))
  (bind _forwardspeed (Variables|Locomotion|GetForwardSpeed))
  (bind _mesh_2 (Variables|Character|GetMesh))
  (bind _capsulecomponent (Variables|Collision|GetCapsuleComponent))
  (bind _capsulecomponent_2 (Variables|Collision|GetCapsuleComponent))
  (bind _forwardspeedmultiplier (Variables|IK|GetForwardSpeedMultiplier))
  (bind _returnvalue (Transformation|GetSocketRotation _mesh_2 FootName))
  (bind _returnvalue_2 (Transformation|GetSocketLocation _mesh FootName))
  (bind _returnvalue_3 (Math|Vector|GetUpVector _capsulecomponent))
  (bind _returnvalue_4 (Math|Vector|GetForwardVector _capsulecomponent_2))
  (bind _returnvalue_5 (* _forwardspeed _forwardspeedmultiplier))
  (bind (_x _y _z) (Math|Rotator|BreakRotIntoAxes _returnvalue))
  (bind _returnvalue_6 (* _returnvalue_3 TraceDistance))
  (bind _returnvalue_7 (* _returnvalue_5 -1.0))
  (bind _returnvalue_8 (* _returnvalue_4 _returnvalue_7))
  (bind _returnvalue_9 (+ _returnvalue_6 _returnvalue_8))
  ;[1 1 1] Trace from foot.
  (bind (_outhit _returnvalue_10) (Collision|LineTraceByChannel (+ _returnvalue_2 _returnvalue_9) (- _returnvalue_2 _returnvalue_9) "TraceTypeQuery1" true 0 "None"))
  (if _returnvalue_10
    ;[1 1 1] Calculate IKHeightOffset in Meshe's coordinate.
    (return (- (.z (Math|Transform|InverseTransformLocation (Transformation|GetWorldTransform (Variables|Character|GetMesh)) (.Location (Collision|BreakHitResult _outhit)))) HeightOffset) _returnvalue_10 (Math|Rotator|SelectRotator (Math|Rotator|MakeRotationfromAxes (Math|Vector|RotateVectorAroundAxis _x (Class|KismetMathLibrary|DegAsin (Math|Vector|VectorLength (Math|Vector|CrossProduct _y (.Normal (Collision|BreakHitResult _outhit))))) (Math|Vector|CrossProduct _y (.Normal (Collision|BreakHitResult _outhit)))) (.Normal (Collision|BreakHitResult _outhit)) (Math|Vector|RotateVectorAroundAxis _z (Class|KismetMathLibrary|DegAsin (Math|Vector|VectorLength (Math|Vector|CrossProduct _y (.Normal (Collision|BreakHitResult _outhit))))) (Math|Vector|CrossProduct _y (.Normal (Collision|BreakHitResult _outhit))))) _returnvalue _returnvalue_10) 0.0 (Math|Vector|MakeVector 0.0 (- (.z (Math|Transform|InverseTransformLocation (Transformation|GetWorldTransform (Variables|Character|GetMesh)) (.Location (Collision|BreakHitResult _outhit)))) HeightOffset) 0.0))
    (else
      (return (Variables|IK|GetMaxLegIKOffset) false "0, 0, 0" 0.0 "0, 0, 0"))))

(fn Soar
  (bind _capsulecomponent (Variables|Collision|GetCapsuleComponent))
  (if (and (Variables|Behavior|GetIsLived) (not (Math|Boolean|ORBoolean (Variables|Behavior|GetIsEating) (Variables|Behavior|GetIsCrying) (Variables|Behavior|GetIsAttacking) (Variables|Behavior|GetIsHitting) (Variables|Behavior|GetIsGrooming) (Variables|Behavior|GetIsHopping))))
    ;[1 1 1] Initialize variables for flight
    (Variables|IK|SetIKInterpSpeed 5e+01)
    (CallFunction|BehaviorOff)
    (Variables|Behavior|SetIsSoaring true)
    ;[1 1 1] Change the settings for flight
    (Pawn|Components|CharacterMovement|SetMovementMode (Variables|Character|GetCharacterMovement) "MOVE_Flying" 0)
    (Physics|SetSimulatePhysics (Variables|Collision|GetCapsuleComponent) true)
    (Components|Activation|Activate (Variables|Character|GetCharacterMovement) false)
    (Class|PrimitiveComponent|SetAllPhysicsLinearVelocity _capsulecomponent (* (+ (Math|Vector|GetForwardVector _capsulecomponent) (Math|Vector|GetUpVector _capsulecomponent)) (Variables|Locomotion|GetSoaringVelocity)) false)))

(fn Landing
  ;[1 1 1] Set movement mode, physics setting and  Initialize the variables.
  (Pawn|Components|CharacterMovement|SetMovementMode (Variables|Character|GetCharacterMovement) "MOVE_Walking" 0)
  (Physics|SetEnableGravity (Variables|Collision|GetCapsuleComponent) true)
  (Physics|SetSimulatePhysics (Variables|Collision|GetCapsuleComponent) false)
  (Variables|IK|SetIKInterpSpeed 1e+01)
  (CallFunction|BehaviorOff)
  (Variables|Locomotion|SetAimForwardSpeed 0.0)
  (Variables|Locomotion|SetAimTurnSpeed 0.0)
  (Variables|Locomotion|SetForwardSpeed 0.0)
  (Variables|Locomotion|SetTurnSpeed 0.0)
  (Variables|Locomotion|SetLandingStartTime 0.0))

(fn BehaviorOff
  ;[1 1 1] Turn off all actions.
  (Variables|Behavior|SetIsAttacking false)
  (Variables|Behavior|SetIsHitting false)
  (Variables|Behavior|SetIsCrying false)
  (Variables|Behavior|SetIsEating false)
  (Variables|Behavior|SetIsGrooming false)
  (Variables|Behavior|SetIsHopping false))