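; Lighting pole prop for the WesterTown building set, with a point light that can be switched on or off.
; The LightOn flag sets the PointLight's visibility in the construction script and again on BeginPlay.
; It has no other runtime logic, as the overlap event is an unused stub.
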(event EventBeginPlay
  (bind _pointlight (Variables|Default|GetPointLight))
  (if (Variables|Default|GetLightOn)
    (Rendering|SetVisibility _pointlight true false)
    (else
      (Rendering|SetVisibility _pointlight false false))))

(event Collision|EventActorBeginOverlap
  (params (OtherActor :type Actor%20Object%20Reference)))

(fn ConstructionScript
  (bind _pointlight (Variables|Default|GetPointLight))
  (if (Variables|Default|GetLightOn)
    (Rendering|SetVisibility _pointlight true false)
    (else
      (Rendering|SetVisibility _pointlight false false))))