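; BP_WallLantern is a wall lantern prop with a Niagara effect and a point light, switched by the LightOn flag.
; The construction script sets only the Niagara effect's visibility from LightOn.
; BeginPlay applies the flag to both the Niagara effect and the point light, so the script never updates the light's visibility before play starts.
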(event EventBeginPlay
  (bind _niagara (Variables|Default|GetNiagara))
  (if (Variables|Default|GetLightOn)
    (Rendering|SetVisibility _niagara true false)
    (else
      (Rendering|SetVisibility _niagara false false))))

(event Collision|EventActorBeginOverlap
  (params (OtherActor :type Actor%20Object%20Reference)))

(fn ConstructionScript
  (bind _niagara (Variables|Default|GetNiagara))
  (if (Variables|Default|GetLightOn)
    (Rendering|SetVisibility _niagara true false)
    (else
      (Rendering|SetVisibility _niagara false false))))