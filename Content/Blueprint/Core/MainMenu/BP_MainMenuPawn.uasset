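; BP_MainMenuPawn is the main menu pawn that sets up the menu's camera, UI and input when play begins.
; It switches player 0's view to the NewCamera target, adds WB_MainMenu to the viewport, shows the cursor and sets UI-only input.
; A short delay precedes giving focus to the New Game button.
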(event EventBeginPlay
  (bind _returnvalue (Game|GetPlayerController 0))
  (Game|Player|SetViewTargetwithBlend (Game|GetPlayerController 0) (Variables|Default|GetNewCamera) 0.0 "VTBlend_Linear" 0.0 false)
  (bind _returnvalue_2 (UserInterface|CreateWidget "/Game/UserInterfaces/WB_MainMenu.WB_MainMenu_C"))
  (bind _output_get (Variables|Default|SetWB_MainMenu _returnvalue_2))
  (UserInterface|Viewport|AddtoViewport _output_get 0)
  (Variables|/Script/Engine.PlayerController|SetbShowMouseCursor _returnvalue true)
  (Input|SetInputModeUIOnly _returnvalue _output_get "DoNotLock" false)
  (Utilities|FlowControl|Delay 0.2)
  (Widget|SetFocus (Variables|/Game/UserInterfaces/WB_MainMenu.WB_MainMenu_C|GetBTN_NewGame _output_get)))

(fn ConstructionScript)