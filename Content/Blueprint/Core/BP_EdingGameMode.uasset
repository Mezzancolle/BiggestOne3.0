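; BP_EdingGameMode is the game mode for the ending sequence that shows the credits.
; On BeginPlay it creates the WB_Credits widget, adds it to the viewport and makes it visible.
; Each Tick it polls the player controller for any key being held and opens Map_MainMenuNew to return to the main menu.
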(event EventBeginPlay
  (bind _returnvalue (UserInterface|CreateWidget "/Game/UserInterfaces/WB_Credits.WB_Credits_C"))
  (bind _output_get (Variables|Default|SetCredits _returnvalue))
  (UserInterface|Viewport|AddtoViewport _output_get 0)
  (Widget|SetVisibility _output_get "Visible"))

(event EventTick
  (params (DeltaSeconds :type Float%20%28single-precision%29))
  (if (Game|Player|IsInputKeyDown (Game|GetPlayerController 0) "AnyKey")
    (Game|OpenLevel(byObjectReference) "/Game/Maps/Map_MainMenuNew.Map_MainMenuNew")))

(fn ConstructionScript)