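; BP_SubtitlesManager is an actor that plays queued dialogue audio with timed, speaker-attributed subtitles.
; AddDialogueToPlay queues unique DT_Subtitles row names; PlayAudio blocking-loads the current clip and its timestamped lines, skipping missing rows.
; Tick feeds lines to a WB_Subtitles widget with DT_Speakers data, timing each against accumulated elapsed time.
; When lines run out, it fires OnEndDialogue, advances the queue, and disables Tick once empty.
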(event EventTick
  (params (DeltaSeconds :type Float%20%28single-precision%29))
  (bind _audiotoplay (Variables|Default|GetAudioToPlay))
  (bind _linestoshow (Variables|Default|GetLinesToShow))
  (bind _output (Utilities|Array|Get(acopy) _linestoshow))
  (Utilities|FlowControl|Sequence
    (:then_0
      ;[1 1 1] Check subtitle time is ended
      (bind _output_get (Variables|Default|SetRemaningTimeDialogueLine (- (Variables|Default|GetRemaningTimeDialogueLine) DeltaSeconds)))
      (if (<= _output_get 0.0)
        (if (Utilities|Array|IsNotEmpty _linestoshow)
          (bind _returnvalue (Utilities|GetDataTableRow "/Game/Other/DataTables/DT_Speakers.DT_Speakers" (.speakername _output))
            (:then
              (Variables|Default|SetRemaningTimeDialogueLine (- (.timestamp _output) (Variables|Default|GetElapsedTimeDialogueLine)))
              (Default|ShowSubtitlesforTime (Variables|Default|GetSubtitlesWidget) _returnvalue (.text _output)))
            (:RowNotFound
              (Development|PrintString "SPEAKER NOT FOUNDED")))
          (Utilities|Array|RemoveIndex (Variables|Default|GetLinesToShow))
          (else
            (if (> (Utilities|Array|Length _audiotoplay) 0)
              (Default|CallOnEndDialogue (Utilities|Array|Get(acopy) _audiotoplay))
              (Utilities|Array|RemoveIndex (Variables|Default|GetAudioToPlay)))
            (Default|OnEndAllCurrentDialogueLines (Variables|Default|GetSubtitlesWidget))
            (bind _alllinesended_ (CallFunction|PlayAudio))
            ;[1 1 1] If all lines are ended
            (if _alllinesended_
              (Actor|Tick|SetActorTickEnabled false))))))
    (:then_1
      ;[1 0 0] To fix in C++
      (Variables|Default|SetElapsedTimeDialogueLine (+ DeltaSeconds (Variables|Default|GetElapsedTimeDialogueLine))))))

(event EventBeginPlay
  (bind _returnvalue (UserInterface|CreateWidget "/Game/UserInterfaces/WB_Subtitles.WB_Subtitles_C"))
  (bind _output_get (Variables|Default|SetSubtitlesWidget _returnvalue))
  (UserInterface|Viewport|AddtoViewport _output_get 0))

(fn ConstructionScript)

(fn PlayAudio
  (bind _audiotoplay (Variables|Default|GetAudioToPlay))
  (bind _output (Utilities|Array|Get(acopy) _audiotoplay))
  (if (Utilities|Array|IsNotEmpty _audiotoplay)
    (Variables|Default|SetElapsedTimeDialogueLine 0.0)
    (bind _returnvalue (Utilities|GetDataTableRow "/Game/Other/DataTables/DT_Subtitles.DT_Subtitles" _output)
      (:then
        (Utilities|LoadAssetBlocking (.AudioClip (Utilities|Struct|BreakS_SubtitleKeyToTimeStamp _returnvalue)))
        (Audio|Components|Audio|SetSound (Variables|Default|GetAudioPlayer) (Utilities|ResolveSoftReference (.AudioClip (Utilities|Struct|BreakS_SubtitleKeyToTimeStamp _returnvalue))))
        (Variables|Default|SetLinesToShow (.TimeStamps (Utilities|Struct|BreakS_SubtitleKeyToTimeStamp _returnvalue)))
        (Audio|Components|Audio|Play (Variables|Default|GetAudioPlayer) 0.0)
        (Actor|Tick|SetActorTickEnabled true)
        (Variables|Default|SetInitialLinesToShow (Utilities|Array|Length (Variables|Default|GetLinesToShow)))
        (return false _returnvalue))
      (:RowNotFound
        ;[1 1 1] Try next audio
        (Development|PrintString (Utilities|String|Append "NOT FOUNDED " (Utilities|String|ToString(Name) _output) " CLIP"))
        (Utilities|Array|RemoveIndex (Variables|Default|GetAudioToPlay))
        (CallFunction|PlayAudio)))
    (else
      (return true ""))))

(fn AddDialoguetoPlay
  (params (AudioRowName :type Name))
  (bind _audiotoplay (Variables|Default|GetAudioToPlay))
  (if (not (== AudioRowName ""))
    (LocalVariables|SetIsNotPlayingAudio? (Utilities|Array|IsEmpty _audiotoplay))
    (if (not (Utilities|Array|ContainsItem _audiotoplay AudioRowName))
      (Utilities|Array|Add (Variables|Default|GetAudioToPlay) AudioRowName)
      (if (LocalVariables|GetIsNotPlayingAudio?)
        (bind _playedsubtitle (CallFunction|PlayAudio))
        (return _playedsubtitle)))))