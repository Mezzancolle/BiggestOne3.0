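; Box trigger actor that enqueues a dialogue from a data table when an actor tagged Player overlaps it, optionally stopping other dialogues.
; Non-repeatable triggers disable their collision, then on dialogue end record the row name in the saved map data asynchronously and destroy themselves.
; On BeginPlay it destroys itself if that row is already recorded, or prints a warning if the row name is invalid.
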(event OnComponentBeginOverlap(BoxTrigger)
  (params (OverlappedComponent :type Primitive%20Component%20Object%20Reference) (OtherActor :type Actor%20Object%20Reference) (OtherComp :type Primitive%20Component%20Object%20Reference) (OtherBodyIndex :type Integer) (bFromSweep :type Boolean) (SweepResult :type Hit%20Result%20Structure%20%28by%20ref%29))
  (if (Actor|ActorHasTag OtherActor "Player")
    (bind _returnvalue (Class|SNSNarrativeBlueprintFuncLib|EnqueueDialogue (Variables|Default|GetDialogues%20Data%20Table) (Variables|Default|GetAudio%20Row%20Name) (Variables|Default|GetStop%20All%20Other%20Dialogues?)))
    (if (not (Variables|Default|GetRepeatable?))
      (Class|SNSNarrativeBlueprintFuncLib|RegisterEventonEndDialogue _returnvalue false (delegate Custom|DestroyOnEndDialogue))
      (Collision|SetCollisionEnabled (Variables|Default|GetBoxTrigger) "NoCollision"))))

(event Custom|DestroyOnEndDialogue
  (bind _returnvalue (Game|GetGameInstance))
  (bind _saveddata (Class|ISaveGame|GetGameData(Message) _returnvalue))
  (Utilities|Array|Add (.triggereddialogues (Variables|/Game/Blueprint/SaveGame/BP_GameData.BP_GameData_C|GetMapData _saveddata)) (Variables|Default|GetAudio%20Row%20Name))
  (Class|ISaveGame|SaveMapData(Message) _returnvalue true (Variables|/Game/Blueprint/SaveGame/BP_GameData.BP_GameData_C|GetMapData _saveddata))
  (Actor|DestroyActor))

(event EventBeginPlay
  (bind _isvalid_ (CallFunction|CheckValidRowName (Variables|Default|GetAudio%20Row%20Name)))
  (if _isvalid_
    (bind _saveddata (Class|ISaveGame|GetGameData(Message) (Game|GetGameInstance)))
    (if (Utilities|Array|ContainsItem (.TriggeredDialogues (Utilities|Struct|BreakS_MapSaveData (Variables|/Game/Blueprint/SaveGame/BP_GameData.BP_GameData_C|GetMapData _saveddata))) (Variables|Default|GetAudio%20Row%20Name))
      (Actor|DestroyActor))
    (else
      (Development|PrintText (Utilities|Text|FormatText "Actor {name} has an invalid audio row name" (Utilities|GetDisplayName self))))))

(fn ConstructionScript)