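; Parent Blueprint for inspectable items, apparently meant to bring a picked-up item in front of the player's camera.
; BeginPlay caches the Pivot's world transform; PickUp registers the item on the player, removes the player input mapping context and stops the camera following control rotation.
; The camera-facing target calculation and the timeline that lerps Pivot toward it are disconnected, so the item never moves.
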(event EventPickUp
  (params (PlayerRef :type BP%20Main%20Character%20Object%20Reference))
  (bind _returnvalue (Game|GetPlayerController 0))
  (Variables|/Game/Blueprint/Player/BP_MainCharacter.BP_MainCharacter_C|SetItemInteractRef PlayerRef self)
  (Utilities|IsValid _returnvalue
    (:Is%20Valid
      (Input|RemoveMappingContext (PlayerController|LocalPlayerSubsystems|GetEnhancedInputLocalPlayerSubsystem _returnvalue) "/Game/Inputs/IMC_Player.IMC_Player" (Utilities|Struct|MakeModifyContextOptions false true false))
      (Variables|/Script/Engine.CameraComponent|SetbUsePawnControlRotation (Variables|/Game/Blueprint/Player/BP_MainCharacter.BP_MainCharacter_C|GetFirstPersonCamera PlayerRef) false))))

(event EventBeginPlay
  (bind _pivot (Variables|Default|GetPivot))
  (Variables|Default|SetStartPos (Transformation|GetWorldLocation _pivot))
  (Variables|Default|SetStartRot (Transformation|GetWorldRotation _pivot)))

(fn ConstructionScript)