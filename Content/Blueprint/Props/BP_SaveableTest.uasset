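; BP_SaveableTest is a test prop that exercises the saveable component by changing its look based on save state.
; The construction script has BPC_Saveable generate a random GUID, and interacting with the actor adds it to the saves.
; When the component reports the actor missing from saves it sets an Apple_quarter material; when found, it swaps the static mesh to a European hornbeam.
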(event OnNotinSaves(BPC_Saveable)
  (Rendering|Material|SetMaterial (Variables|Default|GetStaticMesh) 0 "/Game/Assets/Models/Zone1_shack_Andy/distiller/applebaskettextures/apples_textures/apple_quarter.apple_quarter"))

(event OnFoundinSaves(BPC_Saveable)
  (Components|StaticMesh|SetStaticMesh (Variables|Default|GetStaticMesh) "/Game/ExternalPackages/EuropeanHornbeam/Geometry/SimpleWind/SM_EuropeanHornbeam_Field_01.SM_EuropeanHornbeam_Field_01"))

(event Custom|OnInteract
  (Default|AddtoSaves (Variables|Default|GetBPC_Saveable)))

(event EventBeginPlay)

(event Collision|EventActorBeginOverlap
  (params (OtherActor :type Actor%20Object%20Reference)))

(event EventTick
  (params (DeltaSeconds :type Float%20%28single-precision%29)))

(fn ConstructionScript
  (Default|GenerateRandomGUID (Variables|Default|GetBPC_Saveable)))