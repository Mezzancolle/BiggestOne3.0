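; BP_LightingPole is an interactive street lamp that lights permanently, saving its state by ID in the game's map data.
; Interaction or a light-activation event disables its collision, swaps the lantern material, saves, and enables Tick.
; Tick lerps the smoke to the player's lantern, then notifies linked WarpBoxes and fades in fire and light via timeline.
; On BeginPlay, saved lamps skip the smoke travel and activation sounds.
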(event EventBeginPlay
  (bind _saveddata (Class|ISaveGame|GetGameData(Message) (Game|GetGameInstance)))
  (if (Utilities|Array|Get(acopy) (.lightonstreetlamps (Variables|/Game/Blueprint/SaveGame/BP_GameData.BP_GameData_C|GetMapData _saveddata)) (Variables|Default|GetID))
    (Variables|Default|SetIntensity (Variables|/Script/Engine.LightComponentBase|GetIntensity (Variables|Default|GetPointLight)))
    (Variables|Default|SetIsLightAlreadyVisible? true)
    (Collision|SetCollisionProfileName (Variables|Default|GetTriggerCollision) "NoCollision" true :!class /Script/Engine.PrimitiveComponent)
    (Collision|SetCollisionResponsetoChannel (Variables|Default|GetStaticMesh) "ECC_GameTraceChannel2" "ECR_Ignore")
    (Actor|Tick|SetActorTickEnabled true)
    (Rendering|Material|SetMaterial (Variables|Default|GetStaticMesh) 0 "/Game/ExternalPackages/WesterTown/Materials/Props/MI_Lantern.MI_Lantern")
    (else
      (CallFunction|SetLightVisibility false)
      (Variables|Default|SetIntensity (Variables|/Script/Engine.LightComponentBase|GetIntensity (Variables|Default|GetPointLight)))
      (Audio|Components|Audio|Stop (Variables|Default|GetCracklingAudio)))))

(event EventTick
  (params (DeltaSeconds :type Float%20%28single-precision%29))
  (if (Variables|Default|GetIsLightAlreadyVisible?)
    (Actor|Tick|SetActorTickEnabled false :!label _label)
    (Components|Activation|Deactivate (Variables|Default|GetSmoke))
    (for _array_element (Variables|Default|GetWarpBoxes)
      (Class|ILightningPole|OnLightActivation(Message) _array_element))
    (if (Variables|Default|GetIsLightAlreadyVisible?)
      _
      (else
        (Audio|PlaySoundatLocation "/Game/Audio/SFX/SFX_Misc/Lantern/SFX_Env_DarknessSucc.SFX_Env_DarknessSucc" (Transformation|GetWorldLocation (Variables|Default|GetSmoke)) "0, 0, 0" 1.0 1.0 0.0 "/Game/Audio/Settings/Attenuations/ATT_Audio3D.ATT_Audio3D" 0 0 0)
        (Audio|PlaySoundatLocation "/Game/Audio/SFX/SFX_Misc/Lantern/SFX_Env_FireStart_Cue.SFX_Env_FireStart_Cue" (Transformation|GetWorldLocation (Variables|Default|GetFire)) "0, 0, 0" 1.0 1.0 0.0 "/Game/Audio/Settings/Attenuations/ATT_Audio3D.ATT_Audio3D" 0 0 0)))
    (Rendering|Components|Light|SetIntensity (Variables|Default|GetPointLight) 0.0)
    (CallFunction|SetLightVisibility true)
    (bind _alpha (Timeline|TL_LanternLightOn PlayFromStart)
      (:Update
        (Rendering|Components|Light|SetIntensity (Variables|Default|GetPointLight) (* _alpha (Variables|Default|GetIntensity))))
      (:Finished
        (Components|DestroyComponent (Variables|Default|GetSmoke))))
    (else
      (bind _location (Class|IPlayerUtils|GetLanternActor(Message) (Game|Player|GetPlayerPawn 0)))
      (bind _output_get (Variables|Default|SetGoToPlayerCounter (+ DeltaSeconds (Variables|Default|GetGoToPlayerCounter))))
      (Transformation|SetWorldLocation (Variables|Default|GetSmoke) (Math|Vector|Lerp(Vector) (Transformation|GetWorldLocation (Variables|Default|GetPointLight)) (Transformation|GetWorldLocation _location) (/ _output_get (Variables|Default|GetGoToPlayerTimer))) false false)
      (if (> (Variables|Default|GetGoToPlayerCounter) (Variables|Default|GetGoToPlayerTimer))
        (goto _label)))))

(event EventOnLightActivation
  (Utilities|ActivateLightingPole))

(event EventInteract
  (params (LookingComponent :type Primitive%20Component%20Object%20Reference))
  (Utilities|ActivateLightingPole))

(fn ConstructionScript)

(fn SetLightVisibility
  (params (bNewVisibility :type Boolean))
  (Rendering|SetVisibility (Variables|Default|GetFire) bNewVisibility false)
  (Rendering|SetVisibility (Variables|Default|GetPointLight) bNewVisibility false))