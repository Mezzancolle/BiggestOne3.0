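; Interactable safe prop with a combination-dial minigame, viewed through a fixed camera with fade and zoom transitions.
; While interact is held, look input spins the wheel; drop exits to the player.
; RedArrow overlaps must match tagged number boxes in order, each held through a Tick countdown enabled only during overlap.
; Completion animates handle and door open; BeginPlay restores the open state if the inside item was already taken.
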(event OnComponentBeginOverlap(RedArrow)
  (params (OverlappedComponent :type Primitive%20Component%20Object%20Reference) (OtherActor :type Actor%20Object%20Reference) (OtherComp :type Primitive%20Component%20Object%20Reference) (OtherBodyIndex :type Integer) (bFromSweep :type Boolean) (SweepResult :type Hit%20Result%20Structure%20%28by%20ref%29))
  ;[1 1 1] CollisionCHeck
  (if (> (Utilities|Array|Length (Variables|Default|GetNumberBoxTags)) 0)
    (if (Components|ComponentHasTag OtherComp (Utilities|Array|Get(acopy) (Variables|Default|GetNumberBoxTags)))
      (Actor|Tick|SetActorTickEnabled true)
      (Variables|Default|SetCounterCheckCollision (Variables|Default|GetTimerCheckCollision)))))

(event OnComponentEndOverlap(RedArrow)
  (params (OverlappedComponent :type Primitive%20Component%20Object%20Reference) (OtherActor :type Actor%20Object%20Reference) (OtherComp :type Primitive%20Component%20Object%20Reference) (OtherBodyIndex :type Integer))
  ;[1 1 1] CollisionCHeck
  (Actor|Tick|SetActorTickEnabled false))

(event Custom|OnSafeComplete
  ;[0 1 0.2041] On Safe Minigame Completed
  (Input|DisableInput (Game|GetPlayerController 0))
  (bind _alpha (Timeline|TL_RotationHandle PlayFromStart)
    (:Update
      (Transformation|SetRelativeRotation (Variables|Default|GetPivotHandle) (Math|Rotator|Lerp(Rotator) "0, 0, 0" "0.000000,0.000000,-270.000000" _alpha) false false))
    (:Finished
      (Collision|SetCollisionResponsetoChannel (Variables|Default|GetStaticMesh) "ECC_GameTraceChannel2" "ECR_Ignore")
      (CallFunction|BacktoPlayerCamera)
      (bind _alpha_2 (Timeline|TL_RotationDoor PlayFromStart)
        (:Update
          (Transformation|SetRelativeRotation (Variables|Default|GetPivotDoor) (Math|Rotator|Lerp(Rotator) "0, 0, 0" "0.000000,-80.000000,0.000000" _alpha_2) false false))))))

(event Custom|BackToPlayerCamera
  (bind _startcameralocation (Variables|Default|GetStartCameraLocation))
  (Input|DisableInput (Game|GetPlayerController 0))
  (CameraFades|StartCameraFade :self (Game|GetPlayerCameraManager 0) :ToAlpha 1.0 :Duration (* (Variables|Default|GetCameraHalfFade) 2.0))
  (bind _alpha (Timeline|TL_ZoomOut PlayFromStart)
    (:Update
      (Transformation|SetActorLocation (Variables|Default|GetFixedCamera) (Math|Vector|Lerp(Vector) (+ _startcameralocation (* (Transformation|GetActorForwardVector (Variables|Default|GetFixedCamera)) 1e+01)) _startcameralocation _alpha) false true))
    (:Finished
      (Game|Player|SetViewTargetwithBlend (Game|GetPlayerController 0) (Game|Player|GetPlayerPawn 0) 0.0 "VTBlend_Linear" 0.0 false)
      (CameraFades|StartCameraFade :self (Game|GetPlayerCameraManager 0) :FromAlpha 1.0 :Duration (Variables|Default|GetCameraHalfFade))
      (Class|IPlayerUtils|SwitchInputContext(Message) (Game|Player|GetPlayerPawn 0) "/Game/Inputs/IMC_FirstPersonPlayer.IMC_FirstPersonPlayer" false)
      (Input|EnableInput (Game|Player|GetPlayerPawn 0) 0))))

(event Input|EnhancedActionEvents|EnhancedInputActionIA_Drop
  (params (ActionValue :type Boolean) (ElapsedSeconds :type Float%20%28double-precision%29) (TriggeredSeconds :type Float%20%28double-precision%29) (InputAction :type Input%20Action%20Object%20Reference :default "/Game/Inputs/Actions/IA_Drop.IA_Drop"))
  ;[1 0 0.1485] Keys
  ;;[1 1 1] Interact
  (:Started
    (CallFunction|BacktoPlayerCamera)))

(event Input|EnhancedActionEvents|EnhancedInputActionIA_Look
  (params (ActionValue :type Vector%202D%20Structure) (ElapsedSeconds :type Float%20%28double-precision%29) (TriggeredSeconds :type Float%20%28double-precision%29) (InputAction :type Input%20Action%20Object%20Reference :default "/Game/Inputs/Actions/IA_Look.IA_Look"))
  ;[1 0 0.1485] Keys
  (if (Variables|Default|GetIsMouseLeftClicked?)
    (Transformation|SetRelativeRotation (Variables|Default|GetPivotWheel) (Math|Rotator|CombineRotators (Variables|/Script/Engine.SceneComponent|GetRelativeRotation (Variables|Default|GetPivotWheel)) (Math|Rotator|MakeRotator (* (.x ActionValue) -1.0) 0.0 0.0)) false false)))

(event Input|EnhancedActionEvents|EnhancedInputActionIA_Interact
  (params (ActionValue :type Boolean) (ElapsedSeconds :type Float%20%28double-precision%29) (TriggeredSeconds :type Float%20%28double-precision%29) (InputAction :type Input%20Action%20Object%20Reference :default "/Game/Inputs/Actions/IA_Interact.IA_Interact"))
  ;[1 0 0.1485] Keys
  (:Started
    (Variables|Default|SetIsMouseLeftClicked? true))
  (:Canceled
    (Variables|Default|SetIsMouseLeftClicked? false :!label _label))
  (:Completed
    (goto _label)))

(event EventBeginPlay
  ;[1 1 1] Begin Play
  (Variables|Default|SetStartCameraLocation (Transformation|GetActorLocation (Variables|Default|GetFixedCamera)))
  (Transformation|SetActorRotation (Variables|Default|GetFixedCamera) (Class|KismetMathLibrary|NegateRotator (Transformation|GetActorRotation)))
  (bind _saveddata (Class|ISaveGame|GetGameData(Message) (Game|GetGameInstance)))
  (if (Utilities|Array|ContainsItem (.itemstaken (Variables|/Game/Blueprint/SaveGame/BP_GameData.BP_GameData_C|GetInventoryDiaryData _saveddata)) (Variables|Default|GetItemInsideRowName))
    (Collision|SetCollisionResponsetoChannel (Variables|Default|GetStaticMesh) "ECC_GameTraceChannel2" "ECR_Ignore")
    (Transformation|SetRelativeRotation (Variables|Default|GetPivotHandle) "0.000000,0.000000,-270.000000" false true)
    (Transformation|SetRelativeRotation (Variables|Default|GetPivotDoor) "0.000000,-80.000000,0.000000" false false)))

(event EventTick
  (params (DeltaSeconds :type Float%20%28single-precision%29))
  ;[1 1 1] Tick
  (bind _output_get (Variables|Default|SetCounterCheckCollision (- (Variables|Default|GetCounterCheckCollision) DeltaSeconds)))
  (if (< _output_get 0.0)
    (Actor|Tick|SetActorTickEnabled false)
    (Utilities|Array|RemoveIndex (Variables|Default|GetNumberBoxTags))
    (Audio|PlaySound2D "/Engine/VREditor/Sounds/VR_confirm.VR_confirm" 1.0 1.0 0.0 0 0)
    (if (== (Utilities|Array|Length (Variables|Default|GetNumberBoxTags)) 0)
      (CallFunction|OnSafeComplete))))

(event EventInteract
  (params (PlayerRef :type Actor%20Object%20Reference) (LookingComponent :type Primitive%20Component%20Object%20Reference))
  (bind _returnvalue (Game|GetPlayerController 0))
  (bind _startcameralocation (Variables|Default|GetStartCameraLocation))
  ;[1 0 0.1485] Keys
  ;;[1 1 1] Interact
  (Class|IPlayerUtils|SwitchInputContext(Message) (Game|Player|GetPlayerPawn 0) "/Game/Inputs/IMC_Inspect.IMC_Inspect" false)
  (Input|DisableInput PlayerRef _returnvalue)
  (Input|EnableInput _returnvalue)
  (CameraFades|StartCameraFade :self (Game|GetPlayerCameraManager 0) :ToAlpha 1.0 :Duration (Variables|Default|GetCameraHalfFade))
  (Utilities|FlowControl|Delay (Variables|Default|GetCameraHalfFade))
  (Game|Player|SetViewTargetwithBlend (Game|GetPlayerController 0) (Variables|Default|GetFixedCamera) 0.0 "VTBlend_Linear" 0.0 false)
  (CameraFades|StartCameraFade :self (Game|GetPlayerCameraManager 0) :FromAlpha 1.0 :ToAlpha 0.0 :Duration (Variables|Default|GetCameraHalfFade))
  (bind _alpha (Timeline|TL_ZoomInALittleBit PlayFromStart)
    (:Update
      (Transformation|SetActorLocation (Variables|Default|GetFixedCamera) (Math|Vector|Lerp(Vector) _startcameralocation (+ _startcameralocation (* (Transformation|GetActorForwardVector (Variables|Default|GetFixedCamera)) 1e+01)) _alpha) false true))))

(fn ConstructionScript)