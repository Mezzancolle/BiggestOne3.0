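; Triggerable light pole prop that ignites a fire and its point light when its ActivateLight event is called.
; Activation plays a fire-start sound at the Fire component and makes both Fire and PointLight visible through a shared visibility function.
; A timeline then fades the light in from zero, scaling its alpha by the Intensity variable.
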(event Custom|ActivateLight
  (Audio|PlaySoundatLocation "/Game/Audio/SFX/SFX_Misc/Lantern/SFX_Env_FireStart_Cue.SFX_Env_FireStart_Cue" (Transformation|GetWorldLocation (Variables|Default|GetFire)) "0, 0, 0" 1.0 1.0 0.0 "/Game/Audio/Settings/Attenuations/ATT_Audio3D.ATT_Audio3D" 0 0 0)
  (Rendering|Components|Light|SetIntensity (Variables|Default|GetPointLight) 0.0)
  (CallFunction|SetLightVisibility true)
  (bind _alpha (Timeline|Timeline PlayFromStart)
    (:Update
      (Rendering|Components|Light|SetIntensity (Variables|Default|GetPointLight) (* _alpha (Variables|Default|GetIntensity))))))

(fn ConstructionScript)

(fn SetLightVisibility
  (params (bNewVisibility :type Boolean))
  (Rendering|SetVisibility (Variables|Default|GetFire) bNewVisibility false)
  (Rendering|SetVisibility (Variables|Default|GetPointLight) bNewVisibility false))