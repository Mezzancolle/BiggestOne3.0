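; BP_FinalEnemy_Filippo is an enemy pawn for the ending sequence that, once activated, moves through patrol points and shoots at the player.
; At each point it fires timed line traces for a few seconds, applying damage to hit actors, then advances until the last point.
; Tick smoothly turns it toward the player while shooting.
; AnyDamage is empty; the health and defeat logic is disconnected and never runs.
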(event Custom|MoveToNextPoint
  (bind _movementresult (AI|AIMoveTo self "0, 0, 0" (Utilities|Array|Get(acopy) (Variables|Default|GetPatrolPoints) (Variables|Default|GetCurrentIndex)) 5.0 false)
    (:OnSuccess
      (Variables|Default|SetisShooting true)
      (bind _returnvalue (Utilities|Time|SetTimerbyEvent (delegate Custom|Shooting) 0.5 true))
      (bind _output_get (Variables|Default|SetShootTimerHandle _returnvalue))
      (Utilities|FlowControl|Delay 3.0)
      (Variables|Default|SetisShooting false)
      (Utilities|Time|ClearandInvalidateTimerbyHandle _output_get)
      (if (< (Variables|Default|GetCurrentIndex) (- (Utilities|Array|Length (Variables|Default|GetPatrolPoints)) 1))
        (Variables|Default|SetCurrentIndex (+ (Variables|Default|GetCurrentIndex) 1))
        (Utilities|FlowControl|Delay 0.5)
        (CallFunction|MovetoNextPoint)))
    (:OnFail
      (Development|PrintString (Utilities|String|EnumtoString _movementresult)))))

(event Custom|Shooting
  (bind (_outhit _returnvalue) (Collision|LineTraceByChannel (Transformation|GetActorLocation) (Transformation|GetActorLocation (Game|Player|GetPlayerPawn 0)) "TraceTypeQuery1" false 0 "ForDuration"))
  (Audio|SpawnSoundatLocation 0 "0, 0, 0" "0, 0, 0" 1.0 1.0 0.0 0 0)
  (Effects|SpawnEmitterAttached 0 (Variables|Default|GetGun) "Muzzle")
  (if _returnvalue
    (Game|Damage|ApplyDamage (.HitActor (Collision|BreakHitResult _outhit)) 0.0 0 0)))

(event EventTick
  (params (DeltaSeconds :type Float%20%28single-precision%29))
  (if (Variables|Default|GetisShooting)
    (Transformation|SetActorRotation (Math|Interpolation|RInterpTo (Transformation|GetActorRotation) (Math|Rotator|FindLookatRotation (Transformation|GetActorLocation) (Transformation|GetActorLocation (Game|Player|GetPlayerPawn 0))) DeltaSeconds 5.0))))

(event EventActivate
  (Utilities|FlowControl|DelayUntilNextTick)
  (CallFunction|MovetoNextPoint))

(event Game|Damage|EventAnyDamage
  (params (Damage :type Float%20%28single-precision%29) (DamageType :type Damage%20Type%20Object%20Reference) (InstigatedBy :type Controller%20Object%20Reference) (DamageCauser :type Actor%20Object%20Reference)))

(fn ConstructionScript)