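; BP_TriggerChangeLevel is a box trigger that sends the player to the next level.
; Its collision is off for the first five seconds after BeginPlay, then switches to query and physics.
; When a Player-tagged actor overlaps, it teleports that actor to NextTransform, saves NextLevel through the GameInstance and the player's game data synchronously, then opens NextLevel by name.
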(event OnComponentBeginOverlap(Box)
  (params (OverlappedComponent :type Primitive%20Component%20Object%20Reference) (OtherActor :type Actor%20Object%20Reference) (OtherComp :type Primitive%20Component%20Object%20Reference) (OtherBodyIndex :type Integer) (bFromSweep :type Boolean) (SweepResult :type Hit%20Result%20Structure%20%28by%20ref%29))
  (bind _nextlevel (Variables|Default|GetNextLevel))
  (if (Actor|ActorHasTag OtherActor "Player")
    (Transformation|SetActorTransform OtherActor (Variables|Default|GetNextTransform) false true)
    (Class|ISaveGame|SaveLevelData(Message) (Game|GetGameInstance) false _nextlevel)
    (Class|ISaveable|SavetoGameData(Message) OtherActor false)
    (Game|OpenLevel(byName) _nextlevel)))

(event EventBeginPlay
  (Collision|SetCollisionEnabled (Variables|Default|GetBox) "NoCollision")
  (Utilities|FlowControl|Delay 5.0)
  (Collision|SetCollisionEnabled (Variables|Default|GetBox) "QueryAndPhysics"))

(fn ConstructionScript)