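; BP_ListStaticMeshes is a utility Blueprint that builds a list of the unique static meshes used by StaticMeshActors in the level.
; A custom event calls NewFunction, which gathers those actors, then collects their mesh components behind a DoOnce.
; The event then stores each component's mesh asset in NewVar, using AddUnique to avoid duplicates.
; An older manual de-duplication pass remains disconnected, and BeginPlay, Tick and the construction script do nothing.
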(event Custom|asdasdasd
  (CallFunction|NewFunction)
  (for _array_element (Variables|Default|GetStatic%20Mesh%20Component_0)
    (Utilities|Array|AddUnique (Variables|Default|GetNewVar) (Variables|/Script/Engine.StaticMeshComponent|GetStaticMesh _array_element))))

(event EventBeginPlay)

(event Collision|EventActorBeginOverlap
  (params (OtherActor :type Actor%20Object%20Reference)))

(event EventTick
  (params (DeltaSeconds :type Float%20%28single-precision%29)))

(fn ConstructionScript)

(fn NewFunction
  (bind _static_mesh_component (Variables|Default|GetStatic%20Mesh%20Component))
  (bind _outactors (Actor|GetAllActorsOfClass "/Script/Engine.StaticMeshActor"))
  (for _array_element _outactors
    (Utilities|Array|AddUnique _static_mesh_component _array_element))
  (Utilities|FlowControl|DoOnce false
    (:Completed
      (for _array_element_2 _static_mesh_component
        (Utilities|Array|AddUnique (Variables|Default|GetStatic%20Mesh%20Component_0) (Variables|/Script/Engine.StaticMeshActor|GetStaticMeshComponent _array_element_2))))))