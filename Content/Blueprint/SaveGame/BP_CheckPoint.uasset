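; BP_CheckPoint is a checkpoint actor that saves game data when the player overlaps its box.
; BeginPlay caches the main character and every checkpoint in the level.
; On overlap it calls the player's save message, loops over the checkpoints' current flags, and marks itself as the current checkpoint.
; SpawnPlayer delegates to the character's SpawnAtCheckpoint, and a timed collision cooldown is left unconnected.
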(event OnComponentBeginOverlap(Box)
  (params (OverlappedComponent :type Primitive%20Component%20Object%20Reference) (OtherActor :type Actor%20Object%20Reference) (OtherComp :type Primitive%20Component%20Object%20Reference) (OtherBodyIndex :type Integer) (bFromSweep :type Boolean) (SweepResult :type Hit%20Result%20Structure%20%28by%20ref%29))
  (if (Actor|ActorHasTag OtherActor "Player")
    (Class|ISaveable|SavetoGameData(Message) OtherActor false)
    (for _array_element (Variables|Default|GetCheckpointsArray)
      (if (Variables|BP_CheckPoint_C|GetCurrentCheckpoint? _array_element)
        (Variables|Default|SetCurrentCheckpoint? false)))
    (Variables|Default|SetCurrentCheckpoint? true)))

(event Custom|SpawnPlayer
  ;[0.15 0.15 0.15 0.5] Spawn Player
  (Default|SpawnatCheckpoint (Variables|Default|GetPlayerCharacterRef)))

(event EventBeginPlay
  (bind _returnvalue (Actor|GetActorOfClass "/Game/Blueprint/Player/BP_MainCharacter.BP_MainCharacter_C"))
  (Variables|Default|SetPlayerCharacterRef _returnvalue)
  (bind _outactors (Actor|GetAllActorsOfClass "BP_CheckPoint_C"))
  (Variables|Default|SetCheckpointsArray _outactors))

(fn ConstructionScript)