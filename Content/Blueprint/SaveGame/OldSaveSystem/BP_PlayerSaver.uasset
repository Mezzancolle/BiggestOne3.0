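; BP_PlayerSaver, in the OldSaveSystem folder, saves player data to a save slot and calls LoadGame on BeginPlay.
; SaveGame loads or creates a BP_SavePlayerData, copies lantern and sprint flags from BP_MainCharacter, then writes the slot.
; Location and rotation are saved as zero vectors rather than the player's transform.
; LoadGame only caches the loaded data and character reference, without applying any saved values.
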(event EventBeginPlay
  (CallFunction|LoadGame))

(fn ConstructionScript)

(fn SaveGame
  (bind _returnvalue (SaveGame|DoesSaveGameExist (Variables|Default|GetSaveSlotName)))
  (if _returnvalue
    (bind _returnvalue_2 (SaveGame|LoadGamefromSlot (Variables|Default|GetSaveSlotName)))
    (bind _asbp_save_player_data (Utilities|Casting|CastToBP_SavePlayerData _returnvalue_2))
    (LocalVariables|SetSavedPlayerData _asbp_save_player_data)
    (else
      (bind _returnvalue_3 (SaveGame|CreateSaveGameObject "/Game/Blueprint/SaveGame/OldSaveSystem/BP_SavePlayerData.BP_SavePlayerData_C"))
      (LocalVariables|SetSavedPlayerData _returnvalue_3)))
  (Utilities|FlowControl|Sequence
    (:then_0
      (bind _asbp_main_character (Utilities|Casting|CastToBP_MainCharacter (Game|Player|GetPlayerPawn 0)))
      (LocalVariables|SetCurrentPlayer _asbp_main_character)
      ;[1 1 1] Player Position
      (Variables|/Game/Blueprint/SaveGame/OldSaveSystem/BP_SavePlayerData.BP_SavePlayerData_C|SetLocation (LocalVariables|GetSavedPlayerData) "0, 0, 0")
      ;[1 1 1] Player Rotation
      (Variables|/Game/Blueprint/SaveGame/OldSaveSystem/BP_SavePlayerData.BP_SavePlayerData_C|SetRotation (LocalVariables|GetSavedPlayerData) "0, 0, 0")
      ;[1 1 1] If has lantern and if is enabled
      (Variables|/Game/Blueprint/SaveGame/OldSaveSystem/BP_SavePlayerData.BP_SavePlayerData_C|SetHasLantern? (LocalVariables|GetSavedPlayerData) (Variables|/Game/Blueprint/Player/BP_MainCharacter.BP_MainCharacter_C|GetHasLantern? (LocalVariables|GetCurrentPlayer)))
      (Variables|/Game/Blueprint/SaveGame/OldSaveSystem/BP_SavePlayerData.BP_SavePlayerData_C|SetIsLanternEnabled? (LocalVariables|GetSavedPlayerData) (Variables|/Game/Blueprint/Player/BP_MainCharacter.BP_MainCharacter_C|GetIsLanternEnabled? (LocalVariables|GetCurrentPlayer)))
      ;[1 1 1] Can sprint?
      (Variables|/Game/Blueprint/SaveGame/OldSaveSystem/BP_SavePlayerData.BP_SavePlayerData_C|SetCanSprint? (LocalVariables|GetSavedPlayerData) (Variables|/Game/Blueprint/Player/BP_MainCharacter.BP_MainCharacter_C|GetCanSprint? (LocalVariables|GetCurrentPlayer))))
    (:then_1
      (SaveGame|SaveGametoSlot (LocalVariables|GetSavedPlayerData) (Variables|Default|GetSaveSlotName)))))

(fn LoadGame
  (bind _returnvalue (SaveGame|DoesSaveGameExist (Variables|Default|GetSaveSlotName)))
  (if _returnvalue
    (bind _returnvalue_2 (SaveGame|LoadGamefromSlot (Variables|Default|GetSaveSlotName)))
    (bind _asbp_save_player_data (Utilities|Casting|CastToBP_SavePlayerData _returnvalue_2))
    (LocalVariables|SetLoadPlayerData _asbp_save_player_data)
    (if true
      (bind _asbp_main_character (Utilities|Casting|CastToBP_MainCharacter (Game|Player|GetPlayerPawn 0)))
      (LocalVariables|SetCurrentPlayer _asbp_main_character))))