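; BP_InventorySaver saves and restores the diary's inventory through a BP_SaveInventoryData save slot.
; SaveGame loads the existing slot or creates a new save object, then copies ItemsTaken and InventoryItems from the diary's inventory widget and writes it to disk.
; LoadGame clears the item wrap box, restores both lists and re-adds each item by name.
; LoadGame also calls DestroyTakenItems, which is an empty stub.
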(fn ConstructionScript)

(fn SaveGame
  (params (WBP%20Diary :type WBP%20Diary%20Object%20Reference))
  (LocalVariables|SetWBP_Inventory (Variables|/Game/UserInterfaces/UIPauseMenu/WBP_Diary.WBP_Diary_C|GetWBP_Inventory WBP%20Diary))
  (bind _returnvalue (SaveGame|DoesSaveGameExist (Variables|Default|GetSaveSlotName)))
  (if _returnvalue
    (bind _returnvalue_2 (SaveGame|LoadGamefromSlot (Variables|Default|GetSaveSlotName)))
    (bind _asbp_save_inventory_data (Utilities|Casting|CastToBP_SaveInventoryData _returnvalue_2))
    (LocalVariables|SetSavedInventoryData _asbp_save_inventory_data)
    (else
      (bind _returnvalue_3 (SaveGame|CreateSaveGameObject "/Game/Blueprint/SaveGame/OldSaveSystem/Diary/BP_SaveInventoryData.BP_SaveInventoryData_C"))
      (LocalVariables|SetSavedInventoryData _returnvalue_3)))
  (Utilities|FlowControl|Sequence
    (:then_0
      (Variables|/Game/Blueprint/SaveGame/OldSaveSystem/Diary/BP_SaveInventoryData.BP_SaveInventoryData_C|SetItemsTaken (LocalVariables|GetSavedInventoryData) (Variables|/Game/UserInterfaces/UIPauseMenu/Inventory/WBP_Inventory.WBP_Inventory_C|GetItemsTaken (LocalVariables|GetWBP_Inventory)))
      (Variables|/Game/Blueprint/SaveGame/OldSaveSystem/Diary/BP_SaveInventoryData.BP_SaveInventoryData_C|SetInventoryItems (LocalVariables|GetSavedInventoryData) (Variables|/Game/UserInterfaces/UIPauseMenu/Inventory/WBP_Inventory.WBP_Inventory_C|GetInventoryItems (LocalVariables|GetWBP_Inventory))))
    (:then_1
      (SaveGame|SaveGametoSlot (LocalVariables|GetSavedInventoryData) (Variables|Default|GetSaveSlotName)))))

(fn LoadGame
  (params (Diary :type WBP%20Diary%20Object%20Reference))
  (bind _wbp_inventory (Variables|/Game/UserInterfaces/UIPauseMenu/WBP_Diary.WBP_Diary_C|GetWBP_Inventory Diary))
  (bind _returnvalue (SaveGame|DoesSaveGameExist (Variables|Default|GetSaveSlotName)))
  (if _returnvalue
    (bind _returnvalue_2 (SaveGame|LoadGamefromSlot (Variables|Default|GetSaveSlotName)))
    (bind _asbp_save_inventory_data (Utilities|Casting|CastToBP_SaveInventoryData _returnvalue_2))
    (bind _output_get (LocalVariables|SetLoadInventoryData _asbp_save_inventory_data))
    (Widget|Panel|ClearChildren (Variables|/Game/UserInterfaces/UIPauseMenu/Inventory/WBP_Inventory.WBP_Inventory_C|GetItemsWrapBox (Variables|/Game/UserInterfaces/UIPauseMenu/WBP_Diary.WBP_Diary_C|GetWBP_Inventory Diary)))
    (Variables|/Game/UserInterfaces/UIPauseMenu/Inventory/WBP_Inventory.WBP_Inventory_C|SetItemsTaken _wbp_inventory (Variables|/Game/Blueprint/SaveGame/OldSaveSystem/Diary/BP_SaveInventoryData.BP_SaveInventoryData_C|GetItemsTaken _output_get))
    (Variables|/Game/UserInterfaces/UIPauseMenu/Inventory/WBP_Inventory.WBP_Inventory_C|SetInventoryItems _wbp_inventory (Variables|/Game/Blueprint/SaveGame/OldSaveSystem/Diary/BP_SaveInventoryData.BP_SaveInventoryData_C|GetInventoryItems (LocalVariables|GetLoadInventoryData)))
    (CallFunction|DestroyTakenItems (LocalVariables|GetLoadInventoryData))
    (for _array_element (Variables|/Game/Blueprint/SaveGame/OldSaveSystem/Diary/BP_SaveInventoryData.BP_SaveInventoryData_C|GetInventoryItems (LocalVariables|GetLoadInventoryData))
      (Default|AddNewItembyName (Variables|/Game/UserInterfaces/UIPauseMenu/WBP_Diary.WBP_Diary_C|GetWBP_Inventory Diary) _array_element))))

(fn DestroyTakenItems
  (params (Target :type BP%20Save%20Inventory%20Data%20Object%20Reference%20%28by%20ref%29)))