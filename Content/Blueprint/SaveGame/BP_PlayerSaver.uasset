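; BP_PlayerSaver saves and restores the main character's state through a BP_SavePlayerData save slot.
; SaveGame reuses or creates the save object, then records transform, lantern ownership and on/off state, and sprint ability.
; LoadGame teleports player 0's pawn to the saved transform and reapplies those flags, activating the lantern if it was on.
; BeginPlay is empty and the event graph's LoadGame call is unwired, so nothing here triggers either function.
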(event EventBeginPlay)

(fn ConstructionScript)

(fn SaveGame
  (bind _returnvalue (SaveGame|DoesSaveGameExist (Variables|Default|GetSaveSlotName)))
  (if _returnvalue
    (bind _returnvalue_2 (SaveGame|LoadGamefromSlot (Variables|Default|GetSaveSlotName)))
    (bind _asbp_save_player_data (Utilities|Casting|CastToBP_SavePlayerData _returnvalue_2))
    (LocalVariables|SetSavedPlayerData _asbp_save_player_data)
    (else
      (bind _returnvalue_3 (SaveGame|CreateSaveGameObject "/Game/Blueprint/SaveGame/BP_SavePlayerData.BP_SavePlayerData_C"))
      (LocalVariables|SetSavedPlayerData _returnvalue_3)))
  (Utilities|FlowControl|Sequence
    (:then_0
      (bind _asbp_main_character (Utilities|Casting|CastToBP_MainCharacter (Game|Player|GetPlayerPawn 0)))
      (bind _output_get (LocalVariables|SetCurrentPlayer _asbp_main_character))
      ;[1 1 1] Player Position
      (Variables|/Game/Blueprint/SaveGame/BP_SavePlayerData.BP_SavePlayerData_C|SetLocation (LocalVariables|GetSavedPlayerData) (Transformation|GetActorLocation _output_get))
      ;[1 1 1] Player Rotation
      (Variables|/Game/Blueprint/SaveGame/BP_SavePlayerData.BP_SavePlayerData_C|SetRotation (LocalVariables|GetSavedPlayerData) (Transformation|GetActorRotation (LocalVariables|GetCurrentPlayer)))
      ;[1 1 1] If has lantern and if is enabled
      (Variables|/Game/Blueprint/SaveGame/BP_SavePlayerData.BP_SavePlayerData_C|SetHasLantern? (LocalVariables|GetSavedPlayerData) (Variables|/Game/Blueprint/Player/BP_MainCharacter.BP_MainCharacter_C|GetHasLantern? (LocalVariables|GetCurrentPlayer)))
      (Variables|/Game/Blueprint/SaveGame/BP_SavePlayerData.BP_SavePlayerData_C|SetIsLanternEnabled? (LocalVariables|GetSavedPlayerData) (Variables|/Game/Blueprint/Player/BP_MainCharacter.BP_MainCharacter_C|GetIsLanternEnabled? (LocalVariables|GetCurrentPlayer)))
      ;[1 1 1] Can sprint?
      (Variables|/Game/Blueprint/SaveGame/BP_SavePlayerData.BP_SavePlayerData_C|SetCanSprint? (LocalVariables|GetSavedPlayerData) (Variables|/Game/Blueprint/Player/BP_MainCharacter.BP_MainCharacter_C|GetCanSprint? (LocalVariables|GetCurrentPlayer))))
    (:then_1
      (SaveGame|SaveGametoSlot (LocalVariables|GetSavedPlayerData) (Variables|Default|GetSaveSlotName)))))

(fn LoadGame
  (bind _returnvalue (SaveGame|DoesSaveGameExist (Variables|Default|GetSaveSlotName)))
  (if _returnvalue
    (bind _returnvalue_2 (SaveGame|LoadGamefromSlot (Variables|Default|GetSaveSlotName)))
    (bind _asbp_save_player_data (Utilities|Casting|CastToBP_SavePlayerData _returnvalue_2))
    (LocalVariables|SetLoadPlayerData _asbp_save_player_data)
    (bind _asbp_main_character (Utilities|Casting|CastToBP_MainCharacter (Game|Player|GetPlayerPawn 0)))
    (bind _output_get (LocalVariables|SetCurrentPlayer _asbp_main_character))
    (Transformation|SetActorLocation _output_get (Variables|/Game/Blueprint/SaveGame/BP_SavePlayerData.BP_SavePlayerData_C|GetLocation (LocalVariables|GetLoadPlayerData)) false true)
    (Transformation|SetActorRotation (LocalVariables|GetCurrentPlayer) (Variables|/Game/Blueprint/SaveGame/BP_SavePlayerData.BP_SavePlayerData_C|GetRotation (LocalVariables|GetLoadPlayerData)) true)
    (Default|SetLanternPickup (LocalVariables|GetCurrentPlayer) (Variables|/Game/Blueprint/SaveGame/BP_SavePlayerData.BP_SavePlayerData_C|GetHasLantern? (LocalVariables|GetLoadPlayerData)))
    (Variables|/Game/Blueprint/Player/BP_MainCharacter.BP_MainCharacter_C|SetCanSprint? (LocalVariables|GetCurrentPlayer) (Variables|/Game/Blueprint/SaveGame/BP_SavePlayerData.BP_SavePlayerData_C|GetCanSprint? (LocalVariables|GetLoadPlayerData)))
    (if (Variables|/Game/Blueprint/SaveGame/BP_SavePlayerData.BP_SavePlayerData_C|GetIsLanternEnabled? (LocalVariables|GetLoadPlayerData))
      (Default|SetLanternOldWestActivate (LocalVariables|GetCurrentPlayer)))))