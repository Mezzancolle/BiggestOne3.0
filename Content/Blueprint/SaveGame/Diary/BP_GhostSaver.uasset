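; BP_GhostSaver saves and restores the ghost entries in the player's diary UI.
; SaveGame loads or creates a BP_SaveGhostData, refills its parallel arrays from the WBP_GhostSlot widgets and found-ghost list, then writes it to the slot.
; LoadGame rebuilds the ghost list through AddGhostByDataTable and restores completion and actual info, showing image and name for completed ghosts.
; Saved CorrectGhostInfo is not read back on load.
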(fn ConstructionScript)

(fn SaveGame
  (params (WBP%20Diary :type WBP%20Diary%20Object%20Reference))
  (LocalVariables|SetWBP_Ghosts (Variables|/Game/UserInterfaces/UIPauseMenu/WBP_Diary.WBP_Diary_C|GetWBP_Ghosts WBP%20Diary))
  (bind _returnvalue (SaveGame|DoesSaveGameExist (Variables|Default|GetSaveSlotName)))
  (if _returnvalue
    (bind _returnvalue_2 (SaveGame|LoadGamefromSlot (Variables|Default|GetSaveSlotName)))
    (bind _asbp_save_ghost_data (Utilities|Casting|CastToBP_SaveGhostData _returnvalue_2))
    (LocalVariables|SetSavedGhostData _asbp_save_ghost_data)
    (else
      (bind _returnvalue_3 (SaveGame|CreateSaveGameObject "/Game/Blueprint/SaveGame/Diary/BP_SaveGhostData.BP_SaveGhostData_C"))
      (LocalVariables|SetSavedGhostData _returnvalue_3)))
  (Utilities|FlowControl|Sequence
    (:then_0
      (Utilities|Array|Clear (Variables|/Game/Blueprint/SaveGame/Diary/BP_SaveGhostData.BP_SaveGhostData_C|GetActualGhostInfo (LocalVariables|GetSavedGhostData)))
      (Utilities|Array|Clear (Variables|/Game/Blueprint/SaveGame/Diary/BP_SaveGhostData.BP_SaveGhostData_C|GetCorrectGhostInfo (LocalVariables|GetSavedGhostData)))
      (Utilities|Array|Clear (Variables|/Game/Blueprint/SaveGame/Diary/BP_SaveGhostData.BP_SaveGhostData_C|GetCompletedGhost (LocalVariables|GetSavedGhostData)))
      (Utilities|Array|Clear (Variables|/Game/Blueprint/SaveGame/Diary/BP_SaveGhostData.BP_SaveGhostData_C|GetFoundGhosts (LocalVariables|GetSavedGhostData)))
      (for (_array_element _array_index) (Class|PanelWidget|GetAllChildren (Variables|/Game/UserInterfaces/UIPauseMenu/Ghosts/WBP_Ghosts.WBP_Ghosts_C|GetGhostVerticalBox (LocalVariables|GetWBP_Ghosts)))
        (bind _aswbp_ghost_slot (Utilities|Casting|CastToWBP_GhostSlot _array_element))
        (Utilities|Array|Add (Variables|/Game/Blueprint/SaveGame/Diary/BP_SaveGhostData.BP_SaveGhostData_C|GetActualGhostInfo (LocalVariables|GetSavedGhostData)) (Variables|/Game/UserInterfaces/UIPauseMenu/Ghosts/WBP_GhostSlot.WBP_GhostSlot_C|GetActualGhostInfo _aswbp_ghost_slot))
        (Utilities|Array|Add (Variables|/Game/Blueprint/SaveGame/Diary/BP_SaveGhostData.BP_SaveGhostData_C|GetCorrectGhostInfo (LocalVariables|GetSavedGhostData)) (Variables|/Game/UserInterfaces/UIPauseMenu/Ghosts/WBP_GhostSlot.WBP_GhostSlot_C|GetMyGhostInfo _aswbp_ghost_slot))
        (Utilities|Array|Add (Variables|/Game/Blueprint/SaveGame/Diary/BP_SaveGhostData.BP_SaveGhostData_C|GetCompletedGhost (LocalVariables|GetSavedGhostData)) (Variables|/Game/UserInterfaces/UIPauseMenu/Ghosts/WBP_GhostSlot.WBP_GhostSlot_C|GetIsGhostComplete? _aswbp_ghost_slot))
        (Utilities|Array|Add (Variables|/Game/Blueprint/SaveGame/Diary/BP_SaveGhostData.BP_SaveGhostData_C|GetFoundGhosts (LocalVariables|GetSavedGhostData)) (Utilities|Array|Get(acopy) (Variables|/Game/UserInterfaces/UIPauseMenu/Ghosts/WBP_Ghosts.WBP_Ghosts_C|GetFoundGhosts (LocalVariables|GetWBP_Ghosts)) _array_index))))
    (:then_1
      (SaveGame|SaveGametoSlot (LocalVariables|GetSavedGhostData) (Variables|Default|GetSaveSlotName)))))

(fn LoadGame
  (params (Diary :type WBP%20Diary%20Object%20Reference))
  (LocalVariables|SetWBP%20Diary Diary)
  (bind _returnvalue (SaveGame|DoesSaveGameExist (Variables|Default|GetSaveSlotName)))
  (if _returnvalue
    (bind _returnvalue_2 (SaveGame|LoadGamefromSlot (Variables|Default|GetSaveSlotName)))
    (bind _asbp_save_ghost_data (Utilities|Casting|CastToBP_SaveGhostData _returnvalue_2))
    (LocalVariables|SetLoadGhostData _asbp_save_ghost_data)
    (Widget|Panel|ClearChildren (Variables|/Game/UserInterfaces/UIPauseMenu/Ghosts/WBP_Ghosts.WBP_Ghosts_C|GetGhostVerticalBox (Variables|/Game/UserInterfaces/UIPauseMenu/WBP_Diary.WBP_Diary_C|GetWBP_Ghosts Diary)))
    (for (_array_element _array_index) (Variables|/Game/Blueprint/SaveGame/Diary/BP_SaveGhostData.BP_SaveGhostData_C|GetFoundGhosts (LocalVariables|GetLoadGhostData))
      (bind _ghostslotadded (Default|AddGhostbyDataTable (Variables|/Game/UserInterfaces/UIPauseMenu/WBP_Diary.WBP_Diary_C|GetWBP_Ghosts (LocalVariables|GetWBP%20Diary)) _array_element))
      (bind _output_get (Variables|/Game/UserInterfaces/UIPauseMenu/Ghosts/WBP_GhostSlot.WBP_GhostSlot_C|SetIsGhostComplete? _ghostslotadded (Utilities|Array|Get(acopy) (Variables|/Game/Blueprint/SaveGame/Diary/BP_SaveGhostData.BP_SaveGhostData_C|GetCompletedGhost (LocalVariables|GetLoadGhostData)) _array_index)))
      (bind _output_get_2 (Variables|/Game/UserInterfaces/UIPauseMenu/Ghosts/WBP_GhostSlot.WBP_GhostSlot_C|SetActualGhostInfo _ghostslotadded (Utilities|Array|Get(acopy) (Variables|/Game/Blueprint/SaveGame/Diary/BP_SaveGhostData.BP_SaveGhostData_C|GetActualGhostInfo (LocalVariables|GetLoadGhostData)) _array_index)))
      (if _output_get
        (Appearance|SetBrushfromTexture (Variables|/Game/UserInterfaces/UIPauseMenu/Ghosts/WBP_GhostSlot.WBP_GhostSlot_C|GetImage _ghostslotadded) (.bigimage _output_get_2) false)
        (Variables|/Script/UMG.TextBlock|SetText (Variables|/Game/UserInterfaces/UIPauseMenu/Ghosts/WBP_GhostSlot.WBP_GhostSlot_C|GetGhostName _ghostslotadded) (.name _output_get_2))))))