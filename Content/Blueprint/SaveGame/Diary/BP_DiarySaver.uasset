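; BP_DiarySaver is an actor that coordinates saving and loading of the player's diary.
; On BeginPlay it waits briefly, gets the diary widget from BP_MainCharacter, caches its inventory and ghost saver child actors, then loads automatically.
; SaveGame and LoadGame pass the diary to both child savers, BP_InventorySaver and BP_GhostSaver, which handle the actual work.
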(event EventBeginPlay
  (Utilities|FlowControl|Delay 0.4)
  (bind _asbp_main_character (Utilities|Casting|CastToBP_MainCharacter (Game|Player|GetPlayerPawn 0)))
  (bind _output_get (Variables|Default|SetCurrentPlayer _asbp_main_character))
  (Variables|Default|SetDiary (Variables|/Game/Blueprint/Player/BP_MainCharacter.BP_MainCharacter_C|GetWBP_Diary _output_get))
  (bind _asbp_inventory_saver (Utilities|Casting|CastToBP_InventorySaver (Variables|/Script/Engine.ChildActorComponent|GetChildActor (Variables|Default|GetInventorySaver))))
  (Variables|Default|SetAs%20BP%20Inventory%20Saver _asbp_inventory_saver)
  (bind _asbp_ghost_saver (Utilities|Casting|CastToBP_GhostSaver (Variables|/Script/Engine.ChildActorComponent|GetChildActor (Variables|Default|GetGhostSaver))))
  (Variables|Default|SetAs%20BP%20Ghost%20Saver _asbp_ghost_saver)
  (Development|PrintString "Can load game")
  (CallFunction|LoadGame))

(fn ConstructionScript)

(fn SaveGame
  (Default|SaveGame (Variables|Default|GetAs%20BP%20Inventory%20Saver) (Variables|Default|GetDiary))
  (Default|SaveGame (Variables|Default|GetAs%20BP%20Ghost%20Saver) (Variables|Default|GetDiary)))

(fn LoadGame
  (Default|LoadGame (Variables|Default|GetAs%20BP%20Inventory%20Saver) (Variables|Default|GetDiary))
  (Default|LoadGame (Variables|Default|GetAs%20BP%20Ghost%20Saver) (Variables|Default|GetDiary)))