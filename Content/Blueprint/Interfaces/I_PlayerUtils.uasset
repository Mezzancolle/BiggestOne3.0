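; I_PlayerUtils is a Blueprint interface exposing player functions to other actors without a direct cast.
; It covers inventory and item checks, item inspection with text UI, diary entries for notes and ghost details, and lantern power and access.
; It also exposes camera, held item and pocket getters, input context switching, sprint toggling, warp box rotation, and post-process control.
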(fn PlayerHasItem?
  (params (ItemRowName :type Name%20%28by%20ref%29))
  (return false))

(fn PlayerHasTakenItem?
  (params (ItemRowName :type Name%20%28by%20ref%29))
  (return false))

(fn AddDiaryGhostName
  (params (RowName :type Name%20%28by%20ref%29)))

(fn AddedItemtoInventoryManage
  (params (PreInspectDialogue :type Name) (PostInspectDialogue :type Name) (ItemRef :type Actor%20Object%20Reference%20%28by%20ref%29)))

(fn AddDiaryGhost
  (params (RowName :type Name%20%28by%20ref%29)))

(fn AddDiaryGhostWound
  (params (RowName :type Name%20%28by%20ref%29)))

(fn AddDiaryGhostWish
  (params (RowName :type Name%20%28by%20ref%29)))

(fn AddDiaryGhostCauseOfDeath
  (params (RowName :type Name%20%28by%20ref%29)))

(fn GetCamera
  (return 0))

(fn GetHoldingItem
  (return 0))

(fn CallonEndInteract
  (params (ItemCanBeAddedToInventory? :type Boolean) (ItemRowName :type Name)))

(fn SwitchInputContext
  (params (NewInputMappingContext :type Input%20Mapping%20Context%20Object%20Reference) (ShouldBlur? :type Boolean)))

(fn AddNotetoDiary
  (params (RowName :type Name)))

(fn SetSprint
  (params (CanSprint? :type Boolean)))

(fn InspectStaticMesh
  (params (ItemRowName :type Name%20%28by%20ref%29))
  (return))

(fn Open/CloseInventory)

(fn SetRotationWarpBox
  (params (TriggerPosition :type Vector)))

(fn SetWarpBoxPostProcess
  (params (Weight :type Float%20%28double-precision%29)))

(fn AddLanternPower)

(fn GetLanternActor
  (return 0))

(fn ChangePPDepthOfField
  (params (Value :type Float%20%28double-precision%29)))

(fn SetInspectText
  (params (Name :type Text%20%28by%20ref%29) (Description :type Text%20%28by%20ref%29)))

(fn GetPocket
  (return "0, 0, 0"))

(fn Open/CloseInspectTextUI
  (params (Open? :type Boolean)))