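; BP_ChurchBuilding_Trigger is an overlap trigger that switches the ambient audio as the player enters and leaves the church building.
; On begin and end overlap with the player character, it sets a new location index on MainAmbience and calls CheckLocation to apply it.
; It also enables ChurchAmbience sound effects on entry and disables them on exit.
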(event Collision|EventActorBeginOverlap
  (params (OtherActor :type Actor%20Object%20Reference))
  (bind _mainambience (Variables|Default|GetMainAmbience))
  (if (== OtherActor (Game|GetPlayerCharacter 0))
    (Variables|/Game/Blueprint/Audio/Ambience/BP_TownAmbience.BP_TownAmbience_C|SetNewLocation _mainambience 2)
    (Default|CheckLocation _mainambience)
    (Variables|/Game/Blueprint/BP_ChurchAmbience.BP_ChurchAmbience_C|SetCanPlaySFX (Variables|Default|GetChurchAmbience) true)))

(event Collision|EventActorEndOverlap
  (params (OtherActor :type Actor%20Object%20Reference))
  (bind _mainambience (Variables|Default|GetMainAmbience))
  (if (== OtherActor (Game|GetPlayerCharacter 0))
    (Variables|/Game/Blueprint/Audio/Ambience/BP_TownAmbience.BP_TownAmbience_C|SetNewLocation _mainambience 0)
    (Default|CheckLocation _mainambience)
    (Variables|/Game/Blueprint/BP_ChurchAmbience.BP_ChurchAmbience_C|SetCanPlaySFX (Variables|Default|GetChurchAmbience) false)))

(fn ConstructionScript)