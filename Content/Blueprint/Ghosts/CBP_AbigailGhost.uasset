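; Abigail ghost character Blueprint that adds idle variety and an emotional reaction to player interaction.
; On BeginPlay it randomly picks a look-around montage, a look-distance montage or nothing.
; A montage finishing or being interrupted re-rolls after a random delay, while the empty pick ends the loop.
; The first interaction plays a react montage followed by crying on completion, without explicitly stopping the idle loop.
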(event Custom|RandomizeIdle
  ;[0.15 0.15 0.15 0.5] Randomize Idle between Look Around/Look Distance/Idle
  (switch int (Math|Random|RandomIntegerinRange 1 3)
    (:2
      (Animation|Montage|PlayMontage (Variables|Default|GetSkeletalMesh) "/Game/Animations/NPC/Abigail/AM_LookAround.AM_LookAround"
        (:OnCompleted
          _)
        (:OnInterrupted
          _)))
    (:3
      (Animation|Montage|PlayMontage (Variables|Default|GetSkeletalMesh) "/Game/Animations/NPC/Abigail/AM_LookDistance.AM_LookDistance"
        (:OnCompleted
          _)
        (:OnInterrupted
          _))))
  (Utilities|FlowControl|Delay (Math|Random|RandomFloatinRange 5.0 15.0))
  (CallFunction|RandomizeIdle))

(event EventBeginPlay
  (|CallParentFunction)
  (CallFunction|RandomizeIdle))

(event EventInteract
  (params (LookingComponent :type Primitive%20Component%20Object%20Reference))
  ;[0.15 0.15 0.15 0.5] React when character talks to you the first time, then cry
  (|CallParentFunction LookingComponent)
  (Utilities|FlowControl|DoOnce false
    (:Completed
      (Animation|Montage|PlayMontage (Variables|Default|GetSkeletalMesh) "/Game/Animations/NPC/Abigail/AM_React.AM_React"
        (:OnCompleted
          (Animation|Montage|PlayMontage (Variables|Default|GetSkeletalMesh) "/Game/Animations/NPC/Adelaide/Retargeted/AM_Crying.AM_Crying"))))))

(fn ConstructionScript
  (|CallParentFunction))