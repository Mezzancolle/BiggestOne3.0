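; Ghost NPC Blueprint for Jane, built on a parent ghost class but using Timmy's montages and dialogue row.
; A looping animation event picks a montage from the current action state (idle, successful, unsuccessful, talking), then repeats after a random delay until the ghost completes.
; Singing audio plays on BeginPlay unless IsInsideSaves is set, and fades out on interaction.
; When fading ends, it notifies DemoChecker and queues a dialogue line.
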(event Custom|TimmyAnims
  (bind _skeletalmesh (Variables|Default|GetSkeletalMesh))
  (if (not (Variables|Default|GetIsCompleted?))
    (switch Utilities|FlowControl|Switch|SwitchonE_TimmyActions (Variables|Default|GetActions)
      (:NewEnumerator3
        (switch int (Math|Random|RandomIntegerinRange 1 2)
          (:1
            _)
          (:2
            (Animation|Montage|PlayMontage _skeletalmesh "/Game/Animations/NPC/Timmy/AM_Timmy_Looking_Idle1.AM_Timmy_Looking_Idle1"
              (:OnCompleted
                _)))))
      (:NewEnumerator2
        (Animation|Montage|PlayMontage _skeletalmesh "/Game/Animations/NPC/Timmy/AM_Timmy_Clap1.AM_Timmy_Clap1"
          (:OnCompleted
            _)))
      (:NewEnumerator1
        (Animation|Montage|PlayMontage _skeletalmesh "/Game/Animations/NPC/Timmy/AM_Timmy_NoNoNo1.AM_Timmy_NoNoNo1"
          (:OnCompleted
            _)))
      (:NewEnumerator0
        (Animation|Montage|PlayMontage _skeletalmesh "/Game/Animations/NPC/Timmy/Retargeted/AM_TimmyTalk.AM_TimmyTalk"
          (:OnCompleted
            _))))
    (Utilities|DelayandRestartAnims)))

(event EventBeginPlay
  (bind _singingaudio (Variables|Default|GetSingingAudio))
  (|CallParentFunction)
  (CallFunction|TimmyAnims)
  (if (Variables|Default|GetIsInsideSaves)
    (Audio|Components|Audio|Stop _singingaudio)
    (else
      (Audio|Components|Audio|Play _singingaudio 0.0))))

(event EventInteract
  (params (LookingComponent :type Primitive%20Component%20Object%20Reference))
  (|CallParentFunction LookingComponent)
  (Audio|Components|Audio|FadeOut (Variables|Default|GetSingingAudio) 1.0 0.0 "Linear" :!class /Script/Engine.AudioComponent))

(fn ConstructionScript
  (|CallParentFunction))

(fn OnEndFading
  (|CallParentFunction)
  (Class|IGhostable|OnGhostComplete(Message) (Variables|Default|GetDemoChecker))
  (Class|SNSNarrativeBlueprintFuncLib|EnqueueDialogue "/Game/Other/DataTables/Dialogues/DT_Ghosts_Dialogues.DT_Ghosts_Dialogues" "Timmy_4" false))