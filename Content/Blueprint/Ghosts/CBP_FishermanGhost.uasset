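; Fisherman ghost Blueprint that adds randomized idle animation to the behavior inherited from its parent.
; After the parent BeginPlay, TimmyAnims randomly either does nothing or plays Timmy's looking-idle montage on the skeletal mesh.
; Both branches, the montage one on completion, feed DelayandRestartAnims, which waits a random few seconds and calls TimmyAnims again, forming an endless loop.
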(event Custom|TimmyAnims
  (switch int (Math|Random|RandomIntegerinRange 1 2)
    (:1
      _)
    (:2
      (Animation|Montage|PlayMontage (Variables|Default|GetSkeletalMesh) "/Game/BO_VFX/Ghost/Ghost_Figo/Timmy/Anims/AM_Timmy_Looking_Idle.AM_Timmy_Looking_Idle"
        (:OnCompleted
          _))))
  (Utilities|DelayandRestartAnims))

(event EventBeginPlay
  (|CallParentFunction)
  (CallFunction|TimmyAnims))

(fn ConstructionScript
  (|CallParentFunction))