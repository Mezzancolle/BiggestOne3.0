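; Adelaide ghost Blueprint that plays crying, kneeling and praying montages and reports to DemoChecker when fading ends.
; From BeginPlay, Cry re-triggers itself after a random delay, looping the crying montage.
; KneelDown, Pray and StandUp events, not called here, set IsKneeling and IsPraying as montages complete, with Pray stopping itself after a random delay.
; The OnEndFading override runs the parent logic, then calls DemoChecker's OnGhostCompleteMessage.
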(event Custom|Cry
  (Animation|Montage|PlayMontage (Variables|Default|GetSkeletalMesh) "/Game/Animations/NPC/Adelaide/AM_Crying1.AM_Crying1"
    (:then
      (Utilities|FlowControl|Delay (Math|Random|RandomFloatinRange 7.0 15.0))
      (CallFunction|Cry))))

(event Custom|KneelDown
  (Animation|Montage|PlayMontage (Variables|Default|GetSkeletalMesh) "/Game/Animations/NPC/Adelaide/AM_KneelDown1.AM_KneelDown1"
    (:OnCompleted
      (Variables|Default|SetIsKneeling? true)
      (Utilities|FlowControl|Delay (Math|Random|RandomFloatinRange 5.0 15.0)))))

(event Custom|Pray
  (Animation|Montage|PlayMontage (Variables|Default|GetSkeletalMesh) "/Game/Animations/NPC/Adelaide/AM_StartPraying1.AM_StartPraying1"
    (:OnCompleted
      (Variables|Default|SetIsPraying? true)
      (Utilities|FlowControl|Delay (Math|Random|RandomFloatinRange 5.0 15.0))
      (Animation|Montage|PlayMontage (Variables|Default|GetSkeletalMesh) "/Game/Animations/NPC/Adelaide/AM_StopPraying1.AM_StopPraying1"
        (:OnCompleted
          (Variables|Default|SetIsPraying? false))))))

(event Custom|StandUp
  (Animation|Montage|PlayMontage (Variables|Default|GetSkeletalMesh) "/Game/Animations/NPC/Adelaide/AM_StandUp1.AM_StandUp1"
    (:OnCompleted
      (Variables|Default|SetIsKneeling? false))))

(event EventBeginPlay
  (|CallParentFunction)
  (CallFunction|Cry))

(fn ConstructionScript
  (|CallParentFunction))

(fn OnEndFading
  (|CallParentFunction)
  (Class|IGhostable|OnGhostComplete(Message) (Variables|Default|GetDemoChecker)))