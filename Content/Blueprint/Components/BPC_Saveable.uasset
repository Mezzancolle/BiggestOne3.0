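; Saveable actor component that records whether its owning actor's GUID exists in the map's save data.
; On BeginPlay it looks up the ID through the game instance and fires a found or not-in-saves callback, printing an error if the GUID is invalid.
; AddToSaves registers the ID and saves map data asynchronously.
; GenerateRandomGUID assigns an ID only when none is valid.
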(event EventBeginPlay
  (if (Guid|IsValidGuid (Variables|Default|GetID))
    (CallFunction|CheckFoundinSaves)
    (else
      (Development|PrintText (Utilities|Text|FormatText "{actor} has wrong GUID!" (Utilities|GetDisplayName (Components|GetOwner))) true true "(R=0.781250,G=0.000000,B=0.059085,A=1.000000)" 1e+01))))

(fn GenerateRandomGUID
  (if (not (Guid|IsValidGuid (Variables|Default|GetID)))
    (Variables|Default|SetID (Guid|NewGuid))))

(fn CheckFoundinSaves
  (bind _saveddata (Class|ISaveGame|GetGameData(Message) (Game|GetGameInstance)))
  (if (Utilities|Array|ContainsItem (Utilities|Struct|BreakS_MapSaveData (Variables|/Game/Blueprint/SaveGame/BP_GameData.BP_GameData_C|GetMapData _saveddata)) (Utilities|String|StringToName (Guid|ToString(Guid) (Variables|Default|GetID))))
    (Default|CallOnFoundinSaves)
    (else
      (Default|CallOnNotinSaves))))

(fn AddtoSaves
  (bind _returnvalue (Game|GetGameInstance))
  (bind _saveddata (Class|ISaveGame|GetGameData(Message) _returnvalue))
  (Utilities|Array|Add (Utilities|Struct|BreakS_MapSaveData (Variables|/Game/Blueprint/SaveGame/BP_GameData.BP_GameData_C|GetMapData _saveddata)) (Utilities|String|StringToName (Guid|ToString(Guid) (Variables|Default|GetID))))
  (bind _structout (Utilities|Struct|SetmembersinS_MapSaveData (Variables|/Game/Blueprint/SaveGame/BP_GameData.BP_GameData_C|GetMapData _saveddata) (Utilities|Struct|BreakS_MapSaveData (Variables|/Game/Blueprint/SaveGame/BP_GameData.BP_GameData_C|GetMapData _saveddata))))
  (Class|ISaveGame|SaveMapData(Message) _returnvalue true _structout))