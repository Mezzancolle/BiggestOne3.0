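; BPC_Floating is an actor component that makes its owning actor bob up and down.
; On BeginPlay it caches the owner's start location and turns off its tick if StartEnabled is false.
; Each tick it keeps X and Y fixed and offsets Z by a degree-based cosine of game time, shaped by Phase, Period and Amplitude.
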(event EventTick
  (params (DeltaSeconds :type Float%20%28single-precision%29))
  (bind _startposition (Variables|Default|GetStartPosition))
  (Transformation|SetActorLocation (Components|GetOwner) (Math|Vector|MakeVector (.x _startposition) (.y _startposition) (+ (.z _startposition) (* (Math|Trig|Cos(Degrees) (* (+ (Variables|Default|GetPhase) (Utilities|Time|GetTimeSeconds)) (Variables|Default|GetPeriod))) (Variables|Default|GetAmplitude)))) false false))

(event EventBeginPlay
  (Variables|Default|SetStartPosition (Transformation|GetActorLocation (Components|GetOwner)))
  (if (not (Variables|Default|GetStartEnabled?))
    (Components|Tick|SetComponentTickEnabled false)))