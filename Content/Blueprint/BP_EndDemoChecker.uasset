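; BP_EndDemoChecker swaps which actors are visible once enough ghosts are completed, apparently to mark the end of the demo.
; On BeginPlay it hides every actor in ToEnableActors.
; Each OnGhostComplete call increments the AbigailAndTimmy counter and, when the count reaches CurrentGhosts, hides ToDisableActors and reveals ToEnableActors.
; The swap only toggles hidden-in-game state, leaving collision and tick untouched.
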(event EventBeginPlay
  (for _array_element (Variables|Default|GetToEnableActors)
    (Rendering|SetActorHiddenInGame _array_element true)))

(event EventOnGhostComplete
  (bind _result (Math|Integer|IncrementInt (Variables|Default|GetAbigailAndTimmy))
    (:%20%20
      (if (>= _result (Variables|Default|GetCurrentGhosts))
        (for _array_element (Variables|Default|GetToDisableActors)
          (Rendering|SetActorHiddenInGame _array_element true))
        (for _array_element_2 (Variables|Default|GetToEnableActors)
          (Rendering|SetActorHiddenInGame _array_element_2 false))))))

(fn ConstructionScript)