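; BP_FixWestProps bulk-converts level StaticMeshActors into Old West or Present West prop actors.
; Each conversion spawns BP_OldWestActor or BP_PresentWestActor at the same transform with the same mesh, then hides and destroys the originals.
; DeleteAllCustomActors removes the spawned actors and attempts to re-show the originals.
; SetMaterialToWestMaterial rebuilds materials as sphere-mask dynamic instances, logging non-instance materials, but its calls are disconnected.
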(event Custom|SetAllToOldWest
  (Utilities|Array|Clear (Variables|Default|GetStaticMeshes))
  (bind _outactors (Actor|GetAllActorsOfClass "/Script/Engine.StaticMeshActor"))
  (for _array_element _outactors
    (Utilities|Array|Add (Variables|Default|GetStaticMeshes) _array_element)
    (bind _returnvalue (Game|SpawnActorfromClass "/Game/Blueprint/OldPresentWest/BP_OldWestActor.BP_OldWestActor_C" (Transformation|GetActorTransform _array_element) "AlwaysSpawn" "MultiplyWithRoot" 0 0))
    (Components|StaticMesh|SetStaticMesh (Variables|/Game/Blueprint/OldPresentWest/BP_OldWestActor.BP_OldWestActor_C|GetStaticMesh _returnvalue) (Variables|/Script/Engine.StaticMeshComponent|GetStaticMesh (Variables|/Script/Engine.StaticMeshActor|GetStaticMeshComponent _array_element)))
    (Utilities|Array|Add (Variables|Default|GetCustomActors) _returnvalue))
  (CallFunction|HideStaticMeshes))

(event Custom|SetAllToPresentWest
  (Utilities|Array|Clear (Variables|Default|GetStaticMeshes))
  (bind _outactors (Actor|GetAllActorsOfClass "/Script/Engine.StaticMeshActor"))
  (for _array_element _outactors
    (Utilities|Array|Add (Variables|Default|GetStaticMeshes) _array_element)
    (bind _returnvalue (Game|SpawnActorfromClass "/Game/Blueprint/OldPresentWest/BP_PresentWestActor.BP_PresentWestActor_C" (Transformation|GetActorTransform _array_element) "AlwaysSpawn" "MultiplyWithRoot" 0 0))
    (Components|StaticMesh|SetStaticMesh (Variables|/Game/Blueprint/OldPresentWest/BP_PresentWestActor.BP_PresentWestActor_C|GetStaticMesh _returnvalue) (Variables|/Script/Engine.StaticMeshComponent|GetStaticMesh (Variables|/Script/Engine.StaticMeshActor|GetStaticMeshComponent _array_element)))
    (Utilities|Array|Add (Variables|Default|GetCustomActors) _returnvalue))
  (CallFunction|HideStaticMeshes))

(event Custom|DeleteAllCustomActors
  (bind _customactors (Variables|Default|GetCustomActors))
  (for _array_element _customactors
    (Actor|DestroyActor _array_element))
  (Utilities|Array|Clear _customactors)
  (CallFunction|ShowStaticMeshes)
  (Utilities|Array|Clear (Variables|Default|GetWrongMaterial)))

(event Custom|ShowStaticMeshes
  (for _array_element (Variables|Default|GetStaticMeshes)
    (Rendering|SetActorHiddenInGame _array_element false)
    (Collision|SetActorEnableCollision _array_element true)))

(event Custom|HideStaticMeshes
  (for _array_element (Variables|Default|GetStaticMeshes)
    (Rendering|SetActorHiddenInGame _array_element true)
    (Collision|SetActorEnableCollision _array_element false)
    (Actor|DestroyActor _array_element)))

(fn ConstructionScript)

(fn SetMaterialtoWestMaterial
  (params (StaticMeshComponent :type Mesh%20Component%20Object%20Reference) (Parent :type Material%20Interface%20Object%20Reference) (WestActorMeshComponent :type Primitive%20Component%20Object%20Reference))
  (for (_array_element _array_index) (Rendering|Material|GetMaterials StaticMeshComponent)
    (bind _asmaterial_instance (Utilities|Casting|CastToMaterialInstance _array_element)
      (:then
        (bind _returnvalue (Rendering|Material|CreateDynamicMaterialInstance Parent "None" "None" :!class /Script/Engine.KismetMaterialLibrary))
        (Rendering|Material|SetTextureParameterValue _returnvalue "BaseTexture" (.parametervalue (Utilities|Array|Get(acopy) (Variables|/Script/Engine.MaterialInstance|GetTextureParameterValues _asmaterial_instance))))
        (Rendering|Material|SetTextureParameterValue _returnvalue "Normal" (.parametervalue (Utilities|Array|Get(acopy) (Variables|/Script/Engine.MaterialInstance|GetTextureParameterValues _asmaterial_instance) 1)))
        (Rendering|Material|SetTextureParameterValue _returnvalue "Metallic" (.parametervalue (Utilities|Array|Get(acopy) (Variables|/Script/Engine.MaterialInstance|GetTextureParameterValues _asmaterial_instance) 2)))
        (Rendering|Material|SetMaterial WestActorMeshComponent _array_index _returnvalue))
      (:CastFailed
        (Development|PrintString (Utilities|String|Append "NEED TO CHANGE " (Utilities|GetDisplayName _array_element) " MATERIAL"))
        (Utilities|Array|AddUnique (Variables|Default|GetWrongMaterial) (.AsMaterial (Utilities|Casting|CastToMaterial _array_element)))))))