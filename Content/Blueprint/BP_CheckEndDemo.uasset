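; Demo-ending controller that closes out the gym once enough ghosts are completed.
; Each OnGhostComplete call increments a counter, and reaching three starts a delayed ending sequence.
; The sequence fades the camera and audio out, shows the WB_EndGym widget, then loads the main menu map after a short pause.
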(event EventBeginPlay)

(event EventOnGhostComplete
  (bind _result (Math|Integer|IncrementInt (Variables|Default|GetGhostsCompleted))
    (:%20%20
      (if (>= _result 3)
        (Utilities|FlowControl|Delay 25.0)
        (CameraFades|StartCameraFade :self (Game|GetPlayerCameraManager 0) :ToAlpha 1.0 :Duration 5.0 :bShouldFadeAudio true :bHoldWhenFinished true)
        (bind _returnvalue (UserInterface|CreateWidget "/Game/UserInterfaces/WB_EndGym.WB_EndGym_C"))
        (UserInterface|Viewport|AddtoViewport _returnvalue 0)
        (Utilities|FlowControl|Delay 3.0)
        (Game|OpenLevel(byObjectReference) "/Game/Maps/Map_MainMenuNew.Map_MainMenuNew")))))

(fn ConstructionScript)