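; BP_DynamicBook is a dynamic event prop: a book that gets pushed and plays a drop sound as it falls.
; Activate applies an acceleration-style force to the book and starts a looping, delayed timer on CalculateFall.
; CalculateFall traces straight down from the book to a fixed world height, with debug drawing on.
; The first blocking hit pauses the timer and plays the drop sound at the hit point.
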(event EventActivate
  (Physics|AddForce (Variables|Default|GetBook) (Variables|Default|GetForce) "None" true)
  (bind _returnvalue (Utilities|Time|SetTimerbyFunctionName 0 "CalculateFall" 0.1 true false 1.0))
  (Variables|Default|SetTimerHandle _returnvalue))

(fn ConstructionScript)

(fn CalculateFall
  (bind _book (Variables|Default|GetBook))
  (bind _returnvalue (Transformation|GetWorldLocation _book))
  (bind _outhit (Collision|LineTraceByChannel (Math|Vector|MakeVector (.x _returnvalue) (.y _returnvalue) (.z _returnvalue)) (Math|Vector|MakeVector (.x _returnvalue) (.y _returnvalue) -2e+01) "TraceTypeQuery1" false 0 "ForDuration"))
  (if (.bblockinghit _outhit)
    (Utilities|FlowControl|DoOnce false
      (:Completed
        (Utilities|Time|PauseTimerbyHandle (Variables|Default|GetTimerHandle))
        (Audio|PlaySoundatLocation "/Game/Audio/SFX/SFX_Item/SFX_Items_BookDrop.SFX_Items_BookDrop" (.location _outhit) "0, 0, 0" 1.0 1.0 0.0 0 0 0 0)))))