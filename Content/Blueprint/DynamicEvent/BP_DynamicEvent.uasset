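; Placeable one-shot event that plays a timed sequence of camera shakes, sounds, Niagara effects and actor activations when the player enters its sphere or box trigger.
; A timer steps through DynamicElements, clearing each previous effect; activation can also change player walk speed.
; Optional horror or epic themes fade three distance-based audio layers until activation.
; Completion disables collisions and saves the event's GUID, though the destroy-if-saved check is never run.
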(event OnComponentBeginOverlap(Sphere)
  (params (OverlappedComponent :type Primitive%20Component%20Object%20Reference) (OtherActor :type Actor%20Object%20Reference) (OtherComp :type Primitive%20Component%20Object%20Reference) (OtherBodyIndex :type Integer) (bFromSweep :type Boolean) (SweepResult :type Hit%20Result%20Structure%20%28by%20ref%29))
  (if (Actor|ActorHasTag OtherActor "Player")
    (CallFunction|Activate)))

(event OnComponentBeginOverlap(Box)
  (params (OverlappedComponent :type Primitive%20Component%20Object%20Reference) (OtherActor :type Actor%20Object%20Reference) (OtherComp :type Primitive%20Component%20Object%20Reference) (OtherBodyIndex :type Integer) (bFromSweep :type Boolean) (SweepResult :type Hit%20Result%20Structure%20%28by%20ref%29))
  (if (Actor|ActorHasTag OtherActor "Player")
    (CallFunction|Activate)))

(event Custom|StartPlayingDynamicElements
  ;[0.15 0.15 0.15 0.5] Plays the first dynamic element
  (CallFunction|ManageCurrentDynamicElement))

(event Custom|ManageCurrentDynamicElement
  (CallFunction|ClearPreviousDynamicElement)
  (CallFunction|ExecuteDynamicElement (Utilities|Array|Get(acopy) (Variables|Default|GetDynamicElements) (Variables|Default|GetCurrentDynamicElementIndex)))
  (bind _result (Math|Integer|IncrementInt (Variables|Default|GetCurrentDynamicElementIndex))
    (:%20%20
      (if (>= _result (Utilities|Array|Length (Variables|Default|GetDynamicElements)))
        (Development|PrintString "Ended")
        (Utilities|Time|ClearandInvalidateTimerbyHandle (Variables|Default|GetTimerHandle))
        (CallFunction|DisableAllCollisions)
        (CallFunction|SaveDynamicEvent)
        (else
          (CallFunction|StartNextDynamicEvent))))))

(event Custom|StartNextDynamicEvent
  (Utilities|Time|ClearandInvalidateTimerbyHandle (Variables|Default|GetTimerHandle))
  (bind _returnvalue (Utilities|Time|SetTimerbyEvent (delegate Custom|ManageCurrentDynamicElement) (Utilities|Struct|BreakS_DynamicEventTiming (Utilities|Array|Get(acopy) (Variables|Default|GetDynamicElements) (Variables|Default|GetCurrentDynamicElementIndex)))))
  (Variables|Default|SetTimerHandle _returnvalue))

(event EventBeginPlay
  (CallFunction|SetTriggersCollisions))

(event EventActivate
  ;[0.15 0.15 0.15 0.5] Dynamic Elements
  (if (not (Variables|Default|GetbWasActivated?))
    (CallFunction|FadeOutAllAudios (Variables|Default|GetFadeAudioDuration))
    (CallFunction|StartPlayingDynamicElements)
    (Variables|Default|SetbWasActivated? true)
    (if (Variables|Default|GetbShouldChangePlayerVelocity?)
      (Class|IPlayerUtils|ForcePlayerWalkSpeed(Message) (Game|Player|GetPlayerPawn 0) (Variables|Default|GetNewPlayerVelocity) (Variables|Default|GetTimeToResetPlayerVelocity)))))

(event OnComponentEndOverlap(SphereInner)
  (params (OverlappedComponent :type Primitive%20Component%20Object%20Reference) (OtherActor :type Actor%20Object%20Reference) (OtherComp :type Primitive%20Component%20Object%20Reference) (OtherBodyIndex :type Integer))
  (CallFunction|FadeOutSphereAudio OtherActor (Variables|Default|GetAudioInner) (Variables|Default|GetFadeAudioDuration)))

(event OnComponentBeginOverlap(SphereMiddle)
  (params (OverlappedComponent :type Primitive%20Component%20Object%20Reference) (OtherActor :type Actor%20Object%20Reference) (OtherComp :type Primitive%20Component%20Object%20Reference) (OtherBodyIndex :type Integer) (bFromSweep :type Boolean) (SweepResult :type Hit%20Result%20Structure%20%28by%20ref%29))
  (CallFunction|FadeinSphereAudio OtherActor (Variables|Default|GetAudioMiddle) (Variables|Default|GetFadeAudioDuration)))

(event OnComponentBeginOverlap(SphereInner)
  (params (OverlappedComponent :type Primitive%20Component%20Object%20Reference) (OtherActor :type Actor%20Object%20Reference) (OtherComp :type Primitive%20Component%20Object%20Reference) (OtherBodyIndex :type Integer) (bFromSweep :type Boolean) (SweepResult :type Hit%20Result%20Structure%20%28by%20ref%29))
  (CallFunction|FadeinSphereAudio OtherActor (Variables|Default|GetAudioInner) (Variables|Default|GetFadeAudioDuration)))

(event OnComponentBeginOverlap(SphereOuter)
  (params (OverlappedComponent :type Primitive%20Component%20Object%20Reference) (OtherActor :type Actor%20Object%20Reference) (OtherComp :type Primitive%20Component%20Object%20Reference) (OtherBodyIndex :type Integer) (bFromSweep :type Boolean) (SweepResult :type Hit%20Result%20Structure%20%28by%20ref%29))
  (CallFunction|FadeinSphereAudio OtherActor (Variables|Default|GetAudioOuter) (Variables|Default|GetFadeAudioDuration)))

(event OnComponentEndOverlap(SphereMiddle)
  (params (OverlappedComponent :type Primitive%20Component%20Object%20Reference) (OtherActor :type Actor%20Object%20Reference) (OtherComp :type Primitive%20Component%20Object%20Reference) (OtherBodyIndex :type Integer))
  (CallFunction|FadeOutSphereAudio OtherActor (Variables|Default|GetAudioMiddle) (Variables|Default|GetFadeAudioDuration)))

(event OnComponentEndOverlap(SphereOuter)
  (params (OverlappedComponent :type Primitive%20Component%20Object%20Reference) (OtherActor :type Actor%20Object%20Reference) (OtherComp :type Primitive%20Component%20Object%20Reference) (OtherBodyIndex :type Integer))
  (CallFunction|FadeOutSphereAudio OtherActor (Variables|Default|GetAudioOuter) (Variables|Default|GetFadeAudioDuration)))

(fn ConstructionScript
  (CallFunction|SetTriggersSize)
  (CallFunction|SetTriggersCollisionandVisibility)
  (CallFunction|SetAudioSpheres)
  (CallFunction|GenerateRandomGUID))

(fn FadeOutAllAudios
  (params (FadeOutDuration :type Float%20%28single-precision%29))
  (Audio|Components|Audio|FadeOut (Variables|Default|GetAudioInner) FadeOutDuration 0.0 "Linear" :!class /Script/Engine.AudioComponent)
  (Audio|Components|Audio|FadeOut (Variables|Default|GetAudioMiddle) FadeOutDuration 0.0 "Linear" :!class /Script/Engine.AudioComponent)
  (Audio|Components|Audio|FadeOut (Variables|Default|GetAudioOuter) FadeOutDuration 0.0 "Linear" :!class /Script/Engine.AudioComponent))

(fn SetTriggersSize
  (Components|Sphere|SetSphereRadius (Variables|Default|GetSphere) (Variables|Default|GetSphere%20Trigger%20Radius) true)
  (Components|Box|SetBoxExtent (Variables|Default|GetBox) (Variables|Default|GetBox%20Trigger%20Radius) true))

(fn SetTriggersCollisionandVisibility
  (bind _box (Variables|Default|GetBox))
  (bind _sphere (Variables|Default|GetSphere))
  (if (Variables|Default|GetbIsCollider?)
    (if (Variables|Default|GetbIsBox?)
      (Rendering|SetVisibility _box true false)
      (Rendering|SetVisibility _sphere false false)
      (else
        (Rendering|SetVisibility _sphere true false)
        (Rendering|SetVisibility _box false false)))
    (else
      (CallFunction|HideCollision (Variables|Default|GetSphere))
      (CallFunction|HideCollision (Variables|Default|GetBox)))))

(fn FadeinSphereAudio
  (params (CollidedActor :type Actor%20Object%20Reference) (AudioToPlay :type Audio%20Component%20Object%20Reference) (FadeInDuration :type Float%20%28single-precision%29))
  (if (Actor|ActorHasTag CollidedActor "Player")
    (if (Components|Activation|IsActive AudioToPlay)
      _
      (else
        (Components|Activation|Activate AudioToPlay false)))
    (Audio|Components|Audio|FadeIn AudioToPlay FadeInDuration 1.0 0.0 "Logarithmic" :!class /Script/Engine.AudioComponent)))

(fn SetAudioSpheresSize
  (params (TriggerDistanceMultiplier :type Float%20%28double-precision%29))
  (Components|Sphere|SetSphereRadius (Variables|Default|GetSphereOuter) (* (Variables|Default|GetOuter%20Distance%20Trigger) TriggerDistanceMultiplier) true)
  (Components|Sphere|SetSphereRadius (Variables|Default|GetSphereMiddle) (* (Variables|Default|GetMiddle%20Distance%20Trigger) TriggerDistanceMultiplier) true)
  (Components|Sphere|SetSphereRadius (Variables|Default|GetSphereInner) (* (Variables|Default|GetInner%20Distance%20Trigger) TriggerDistanceMultiplier) true))

(fn SetAudioSoundsbyBool
  (if (Variables|Default|GetbIsHorrorTheme?)
    (Audio|Components|Audio|SetSound (Variables|Default|GetAudioInner) (Variables|Default|GetInner%20Horror%20Audio%20Media))
    (Audio|Components|Audio|SetSound (Variables|Default|GetAudioMiddle) (Variables|Default|GetMiddle%20Horror%20Audio%20Media))
    (Audio|Components|Audio|SetSound (Variables|Default|GetAudioOuter) (Variables|Default|GetOuter%20Horror%20Audio%20Media))
    (elif (Variables|Default|GetbIsEpicTheme?)
      (Audio|Components|Audio|SetSound (Variables|Default|GetAudioInner) (Variables|Default|GetInner%20Epic%20Audio%20Media))
      (Audio|Components|Audio|SetSound (Variables|Default|GetAudioMiddle) (Variables|Default|GetMiddle%20Epic%20Audio%20Media))
      (Audio|Components|Audio|SetSound (Variables|Default|GetAudioOuter) (Variables|Default|GetOuter%20Epic%20Audio%20Media)))))

(fn HideCollision
  (params (Primitive :type Primitive%20Component%20Object%20Reference))
  (Rendering|SetVisibility Primitive false false))

(fn ShowCollision
  (params (Primitive :type Primitive%20Component%20Object%20Reference))
  (Rendering|SetVisibility Primitive true false))

(fn SetAudioSpheres
  (if (or (Variables|Default|GetbIsHorrorTheme?) (Variables|Default|GetbIsEpicTheme?))
    (CallFunction|ShowCollision (Variables|Default|GetSphereMiddle))
    (CallFunction|ShowCollision (Variables|Default|GetSphereInner))
    (CallFunction|ShowCollision (Variables|Default|GetSphereOuter))
    (CallFunction|SetAudioSpheresSize 6e+02)
    (CallFunction|SetAudioSoundsbyBool)
    (else
      (CallFunction|HideCollision (Variables|Default|GetSphereMiddle))
      (CallFunction|HideCollision (Variables|Default|GetSphereInner))
      (CallFunction|HideCollision (Variables|Default|GetSphereOuter)))))

(fn SetTriggersCollisions
  (Utilities|FlowControl|Sequence
    (:then_0
      (if (not (Variables|Default|GetbIsCollider?))
        (Collision|SetCollisionEnabled (Variables|Default|GetSphere) "NoCollision")
        (Collision|SetCollisionEnabled (Variables|Default|GetBox) "NoCollision")
        (Collision|SetActorEnableCollision false)))
    (:then_1
      (if (not (or (Variables|Default|GetbIsHorrorTheme?) (Variables|Default|GetbIsEpicTheme?)))
        (Collision|SetCollisionEnabled (Variables|Default|GetSphereMiddle) "NoCollision")
        (Collision|SetCollisionEnabled (Variables|Default|GetSphereInner) "NoCollision")
        (Collision|SetCollisionEnabled (Variables|Default|GetSphereOuter) "NoCollision")))))

(fn FadeOutSphereAudio
  (params (CollidedActor :type Actor%20Object%20Reference) (AudioToPlay :type Audio%20Component%20Object%20Reference) (FadeInDuration :type Float%20%28single-precision%29))
  (if (Actor|ActorHasTag CollidedActor "Player")
    (if (Components|Activation|IsActive AudioToPlay)
      (Audio|Components|Audio|FadeOut AudioToPlay FadeInDuration 0.0 "Logarithmic" :!class /Script/Engine.AudioComponent))))

(fn DEShakeCamera
  (params (Condition :type Boolean) (ShakeClass :type Camera%20Shake%20Base%20Class%20Reference))
  (if Condition
    ;[0.15 0.15 0.15 0.5] Camera local or Based on dynamic event location?
    (bind _returnvalue (CameraShakes|StartCameraShake (Game|GetPlayerCameraManager 0) ShakeClass 1.0 "CameraLocal" "0, 0, 0"))
    (Variables|Default|SetPreviousCameraShake _returnvalue)))

(fn DEPlaySFX
  (params (SFX :type Sound%20Base%20Object%20Reference) (Condition :type Boolean))
  (Utilities|IsValid SFX
    (:Is%20Valid
      (if Condition
        (bind _returnvalue (Audio|SpawnSound2D SFX 1.0 1.0 0.0 0))
        (Variables|Default|SetPreviousAudioComponent _returnvalue)
        (else
          (bind _returnvalue_2 (Audio|SpawnSoundatLocation SFX (Transformation|GetActorLocation) "0, 0, 0" 1.0 1.0 0.0 "/Game/Audio/Settings/Attenuations/ATT_Audio3D.ATT_Audio3D" 0))
          (Variables|Default|SetPreviousAudioComponent _returnvalue_2))))))

(fn DESpawnVFX
  (params (VFX :type Niagara%20System%20Object%20Reference))
  (Utilities|IsValid VFX
    (:Is%20Valid
      (bind _returnvalue (Niagara|SpawnSystematLocation VFX (Transformation|GetActorLocation) "0, 0, 0" "1.000000,1.000000,1.000000" true true "AutoRelease"))
      (Variables|Default|SetPreviousNiagaraParticle _returnvalue))))

(fn ExecuteDynamicElement
  (params (S_DynamicEventTiming :type S%20Dynamic%20Event%20Timing%20Structure%20%28by%20ref%29))
  (bind (_timeduration _shouldcamerashake_ _camerashakestrength _sfx _forcesound2d _vfx _actorstointeract) (Utilities|Struct|BreakS_DynamicEventTiming S_DynamicEventTiming))
  (Utilities|FlowControl|Sequence
    (:then_0
      (CallFunction|DEShakeCamera _shouldcamerashake_ _camerashakestrength))
    (:then_1
      (CallFunction|DEPlaySFX _sfx _forcesound2d))
    (:then_2
      (CallFunction|DESpawnVFX _vfx))
    (:then_3
      (for _array_element _actorstointeract
        (Class|BPIDynamicEvent|Activate(Message) _array_element)))))

(fn ClearPreviousDynamicElement
  (Utilities|FlowControl|Sequence
    (:then_0
      (Utilities|IsValid (Variables|Default|GetPreviousCameraShake)
        (:Is%20Valid
          (CameraShakes|StopCameraShake (Game|GetPlayerCameraManager 0) (Variables|Default|GetPreviousCameraShake) true)
          (Variables|Default|SetPreviousCameraShake 0))))
    (:then_1
      (Utilities|IsValid (Variables|Default|GetPreviousAudioComponent)
        (:Is%20Valid
          (Audio|Components|Audio|FadeOut (Variables|Default|GetPreviousAudioComponent) (Variables|Default|GetFadeAudioDuration) 0.0 "Linear" :!class /Script/Engine.AudioComponent)
          (Variables|Default|SetPreviousAudioComponent 0))))
    (:then_2
      (Utilities|IsValid (Variables|Default|GetPreviousNiagaraParticle)
        (:Is%20Valid
          (Components|Activation|Deactivate (Variables|Default|GetPreviousNiagaraParticle))
          (Variables|Default|SetPreviousNiagaraParticle 0))))))

(fn DisableAllCollisions
  (Utilities|FlowControl|Sequence
    (:then_0
      (Collision|SetCollisionEnabled (Variables|Default|GetSphere) "NoCollision")
      (Collision|SetCollisionEnabled (Variables|Default|GetBox) "NoCollision")
      (Collision|SetActorEnableCollision false))
    (:then_1
      (Collision|SetCollisionEnabled (Variables|Default|GetSphereMiddle) "NoCollision")
      (Collision|SetCollisionEnabled (Variables|Default|GetSphereInner) "NoCollision")
      (Collision|SetCollisionEnabled (Variables|Default|GetSphereOuter) "NoCollision"))))

(fn GenerateRandomGUID
  (if (not (Guid|IsValidGuid (Variables|Default|GetID)))
    (Variables|Default|SetID (Guid|NewGuid))))

(fn SaveDynamicEvent
  (bind _returnvalue (Game|GetGameInstance))
  (bind _saveddata (Class|ISaveGame|GetGameData(Message) _returnvalue))
  (Utilities|Array|Add (.DynamicEventTriggered (Utilities|Struct|BreakS_MapSaveData (Variables|/Game/Blueprint/SaveGame/BP_GameData.BP_GameData_C|GetMapData _saveddata))) (Utilities|String|StringToName (Guid|ToString(Guid) (Variables|Default|GetID))))
  (bind _structout (Utilities|Struct|SetmembersinS_MapSaveData (Variables|/Game/Blueprint/SaveGame/BP_GameData.BP_GameData_C|GetMapData _saveddata) (.DynamicEventTriggered (Utilities|Struct|BreakS_MapSaveData (Variables|/Game/Blueprint/SaveGame/BP_GameData.BP_GameData_C|GetMapData _saveddata)))))
  (Class|ISaveGame|SaveMapData(Message) _returnvalue true _structout))

(fn DestroyifinSave
  (bind _saveddata (Class|ISaveGame|GetGameData(Message) (Game|GetGameInstance)))
  (if (Utilities|Array|ContainsItem (Utilities|Struct|BreakS_MapSaveData (Variables|/Game/Blueprint/SaveGame/BP_GameData.BP_GameData_C|GetMapData _saveddata)) (Utilities|String|StringToName (Guid|ToString(Guid) (Variables|Default|GetID))))
    (Actor|DestroyActor)))