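; BP_DynamicMargaret is a dynamic event actor whose static mesh appears on activation and later vanishes.
; Construction hides the mesh and disables its collision; Activate restores visibility only, then either follows the player or starts a timer, presumably to hide it.
; Following samples the player mesh's location once, and a timeline repeatedly lerps from the current position toward that point minus an offset, hiding the mesh when finished.
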(event Custom|SetInvisibility
  (bind _staticmesh (Variables|Default|GetStaticMesh))
  (Rendering|SetVisibility _staticmesh false false)
  (Collision|SetCollisionEnabled _staticmesh "NoCollision"))

(event Custom|Event%20FollowPlayer
  (Variables|Default|SetPlayerLocation (Transformation|GetWorldLocation (Variables|/Script/Engine.Character|GetMesh (Game|GetPlayerCharacter 0))))
  (bind _move (Timeline|MoveToLocation PlayFromStart)
    (:Update
      (Transformation|SetWorldLocation (Variables|Default|GetStaticMesh) (Math|Vector|Lerp(Vector) (Transformation|GetWorldLocation (Variables|Default|GetStaticMesh)) (- (Variables|Default|GetPlayerLocation) (Variables|Default|GetMoveOffset)) _move) false false))
    (:Finished
      (CallFunction|SetInvisibility))))

(event EventActivate
  (Rendering|SetVisibility (Variables|Default|GetStaticMesh) true false)
  (if (Variables|Default|GetbFollowPlayer?)
    (CallFunction|EventFollowPlayer)
    (else
      (Utilities|Time|SetTimerbyEvent (EventDispatchers|CreateEvent :!event Custom|SetInvisibility) (Variables|Default|GetTimetoInvisibility)))))

(fn ConstructionScript
  (CallFunction|SetInvisibility))