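; BP_GetAllMaterials is a level-design helper actor that gathers the materials recorded by the past and present material-check actors in the level.
; Its construction script finds every BP_PastCheckSameMaterial, then every BP_PresentCheckSameMaterial, and adds each entry of their AllMaterials arrays uniquely to AllAllMaterials.
; The result is one deduplicated material list, built at construction time with no active runtime event logic.
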(event EventBeginPlay)

(event Collision|EventActorBeginOverlap
  (params (OtherActor :type Actor%20Object%20Reference)))

(event EventTick
  (params (DeltaSeconds :type Float%20%28single-precision%29)))

(fn ConstructionScript
  (bind _allallmaterials (Variables|Default|GetAllAllMaterials))
  (Utilities|FlowControl|Sequence
    (:then_0
      (bind _outactors (Actor|GetAllActorsOfClass "/Game/Blueprint/OldPresentWest/BP_PastCheckSameMaterial.BP_PastCheckSameMaterial_C"))
      (for _array_element _outactors
        (for _array_element_2 (Variables|/Game/Blueprint/OldPresentWest/BP_PastCheckSameMaterial.BP_PastCheckSameMaterial_C|GetAllMaterials _array_element)
          (Utilities|Array|AddUnique _allallmaterials _array_element_2))))
    (:then_1
      (bind _outactors_2 (Actor|GetAllActorsOfClass "/Game/Blueprint/OldPresentWest/BP_PresentCheckSameMaterial.BP_PresentCheckSameMaterial_C"))
      (for _array_element_3 _outactors_2
        (for _array_element_4 (Variables|/Game/Blueprint/OldPresentWest/BP_PresentCheckSameMaterial.BP_PresentCheckSameMaterial_C|GetAllMaterials _array_element_3)
          (Utilities|Array|AddUnique _allallmaterials _array_element_4))))))