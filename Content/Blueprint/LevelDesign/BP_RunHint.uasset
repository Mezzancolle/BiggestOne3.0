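; Level design trigger that shows the sprint tutorial hint to the player.
; When an actor tagged Player overlaps the box, or Activate is called, it reads the tutorial data from the Game Instance.
; If the sprint tutorial is not yet closed, it tells the player pawn to show the run widget message, then destroys itself.
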(event OnComponentBeginOverlap(Box)
  (params (OverlappedComponent :type Primitive%20Component%20Object%20Reference) (OtherActor :type Actor%20Object%20Reference) (OtherComp :type Primitive%20Component%20Object%20Reference) (OtherBodyIndex :type Integer) (bFromSweep :type Boolean) (SweepResult :type Hit%20Result%20Structure%20%28by%20ref%29))
  (if (Actor|ActorHasTag OtherActor "Player")
    (bind _saveddata (Class|ISaveGame|GetGameData(Message) (Game|GetGameInstance)))
    (if (not (Utilities|Struct|BreakS_TutorialSave (Variables|/Game/Blueprint/SaveGame/BP_GameData.BP_GameData_C|GetTutorialData _saveddata)))
      (Class|IPlayerUtils|ShowRunWidget(Message) (Game|Player|GetPlayerPawn 0))
      (Actor|DestroyActor))))

(event EventBeginPlay)

(event EventActivate
  (bind _saveddata (Class|ISaveGame|GetGameData(Message) (Game|GetGameInstance)))
  (if (not (Utilities|Struct|BreakS_TutorialSave (Variables|/Game/Blueprint/SaveGame/BP_GameData.BP_GameData_C|GetTutorialData _saveddata)))
    (Class|IPlayerUtils|ShowRunWidget(Message) (Game|Player|GetPlayerPawn 0))
    (Actor|DestroyActor)))

(fn ConstructionScript)