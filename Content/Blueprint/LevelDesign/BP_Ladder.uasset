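; Climbable ladder that the player mounts by interacting and exits at either end.
; Interact disables input and timeline-lerps the pawn to the nearer top or bottom widget, turning the view to the ladder, then restores input and sends ClimbMessage.
; StartClimbBox overlap sends EndClimbMessage directly.
; EndClimbBox, for a flying (climbing) player, first lerps to a rotation-adjusted exit offset using separate forward and up curves.
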(event OnComponentBeginOverlap(StartClimbBox)
  (params (OverlappedComponent :type Primitive%20Component%20Object%20Reference) (OtherActor :type Actor%20Object%20Reference) (OtherComp :type Primitive%20Component%20Object%20Reference) (OtherBodyIndex :type Integer) (bFromSweep :type Boolean) (SweepResult :type Hit%20Result%20Structure%20%28by%20ref%29))
  ;[0.15 0.15 0.15 0.5] Climbing system
  (if (Actor|ActorHasTag OtherActor "Player")
    (Class|IClimb|EndClimb(Message) OtherActor)))

(event OnComponentBeginOverlap(EndClimbBox)
  (params (OverlappedComponent :type Primitive%20Component%20Object%20Reference) (OtherActor :type Actor%20Object%20Reference) (OtherComp :type Primitive%20Component%20Object%20Reference) (OtherBodyIndex :type Integer) (bFromSweep :type Boolean) (SweepResult :type Hit%20Result%20Structure%20%28by%20ref%29))
  (bind _returnvalue (Transformation|GetActorRotation))
  (bind _returnvalue_2 (Game|Player|GetPlayerPawn 0))
  (bind _returnvalue_3 (Game|Player|GetPlayerPawn 0))
  (bind _returnvalue_4 (Transformation|GetActorLocation))
  (bind _endtoplerpingposition (Variables|Default|GetEndTopLerpingPosition))
  (bind _returnvalue_5 (Math|Vector|UnrotateVector _endtoplerpingposition _returnvalue))
  ;[0.15 0.15 0.15 0.5] Climbing system
  (if (Actor|ActorHasTag OtherActor "Player")
    (if (and (Class|NavMovementComponent|IsFlying (Pawn|GetMovementComponent (Game|Player|GetPlayerPawn 0))) (not (Variables|Default|GetIsLerping?)))
      (Variables|Default|SetPreLerpPosition (Transformation|GetActorLocation _returnvalue_3))
      (Variables|Default|SetPreLerpRotation (Transformation|GetActorRotation _returnvalue_3))
      (Variables|Default|SetIsLerping? true)
      (bind (_direction _alphaforward _alphaup) (Timeline|TL_EndClimbing PlayFromStart)
        (:Update
          (Transformation|SetActorLocation _returnvalue_2 (Math|Vector|MakeVector (Math|Float|Lerp (.x (Variables|Default|GetPreLerpPosition)) (- (.x _returnvalue_4) (.x _returnvalue_5)) _alphaforward) (Math|Float|Lerp (.y (Variables|Default|GetPreLerpPosition)) (- (.y _returnvalue_4) (.y _returnvalue_5)) _alphaforward) (Math|Float|Lerp (.z (Variables|Default|GetPreLerpPosition)) (+ (.z _returnvalue_4) (.z _returnvalue_5)) _alphaup)) false false))
        (:Finished
          (Class|IClimb|EndClimb(Message) _returnvalue_2)
          (Variables|Default|SetIsLerping? false))))))

(event Custom|OnEndLerp
  (bind _returnvalue (Game|Player|GetPlayerPawn 0))
  (Input|EnableInput _returnvalue (Game|GetPlayerController 0))
  (Class|IClimb|Climb(Message) _returnvalue)
  (Variables|Default|SetIsLerping? false))

(event EventInteract
  (params (LookingComponent :type Primitive%20Component%20Object%20Reference))
  (bind _returnvalue (Game|Player|GetPlayerPawn 0))
  (bind _returnvalue_2 (Pawn|GetMovementComponent _returnvalue))
  (if (not (Math|Boolean|ORBoolean (Class|NavMovementComponent|IsFlying _returnvalue_2) (Variables|Default|GetIsLerping?) (AI|Components|NavMovement|IsFalling _returnvalue_2)))
    (Input|DisableInput _returnvalue (Game|GetPlayerController 0))
    (Variables|Default|SetPreLerpPosition (Transformation|GetActorLocation _returnvalue))
    (Variables|Default|SetPreLerpRotation (Transformation|GetActorRotation _returnvalue))
    (Variables|Default|SetIsLerping? true)
    (bind _isup_ (CallFunction|IsNearUpWidget?))
    (if _isup_
      (bind _movement_alpha (Timeline|TL_UpLadder PlayFromStart)
        (:Update
          (CallFunction|LerpPlayertoWidget (Variables|Default|GetTopWidget) _movement_alpha (Game|Player|GetPlayerPawn 0)))
        (:Finished
          (CallFunction|OnEndLerp)))
      (else
        (bind _movement_alpha_2 (Timeline|TL_DownLadder PlayFromStart)
          (:Update
            (CallFunction|LerpPlayertoWidget (Variables|Default|GetBottomWidget) _movement_alpha_2 (Game|Player|GetPlayerPawn 0)))
          (:Finished
            (CallFunction|OnEndLerp)))))))

(fn ConstructionScript)

(fn LerpPlayertoWidget
  (params (Widget :type Scene%20Component%20Object%20Reference) (Alpha :type Float%20%28double-precision%29) (Player :type Actor%20Object%20Reference))
  (Transformation|SetActorLocation Player (Math|Vector|Lerp(Vector) (Variables|Default|GetPreLerpPosition) (Transformation|GetWorldLocation Widget) Alpha) false false)
  (Pawn|SetControlRotation (Game|GetPlayerController 0) (Math|Rotator|Lerp(Rotator) (Variables|Default|GetPreLerpRotation) (Math|Conversions|RotationFromXVector (Math|Vector|NegateVector (Transformation|GetActorRightVector))) Alpha true)))

(fn IsNearUpWidget?
  (bind _returnvalue (Game|Player|GetPlayerPawn 0))
  (bind _returnvalue_2 (Transformation|GetActorLocation _returnvalue))
  (return (< (Class|KismetMathLibrary|VectorDistanceSquared _returnvalue_2 (Transformation|GetWorldLocation (Variables|Default|GetTopWidget))) (Class|KismetMathLibrary|VectorDistanceSquared _returnvalue_2 (Transformation|GetWorldLocation (Variables|Default|GetBottomWidget))))))