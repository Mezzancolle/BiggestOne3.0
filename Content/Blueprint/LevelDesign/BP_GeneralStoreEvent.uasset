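; General store scare-style event that starts ten seconds after play begins, blacking out the lights and briefly revealing Margareth.
; BeginEvent calls itself to switch off LightsArray in groups of four, pausing between groups.
; Margareth then jumps to MargTarget while a flip-flopped timeline fades FinalLight up to double its starting intensity and back down.
; Shortly after the fade-out begins, she returns to her original transform.
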(event Custom|BeginEvent
  (if (!= (Variables|Default|GetIndex) (Utilities|Array|Length (Variables|Default|GetLightsArray)))
    (Rendering|Components|Light|SetIntensity (Variables|/Game/ExternalPackages/Northwood/BP/BP_Light_Hanging_NN_01a.BP_Light_Hanging_NN_01a_C|GetPointLight1 (Utilities|Array|Get(acopy) (Variables|Default|GetLightsArray) (Variables|Default|GetIndex))) 0.0)
    (Math|Integer|IncrementInt (Variables|Default|GetIndex)
      (:%20%20
        (if (!= (Variables|Default|GetGroupingIndex) 3)
          (Math|Integer|IncrementInt (Variables|Default|GetGroupingIndex)
            (:%20%20
              _))
          (else
            (Variables|Default|SetGroupingIndex 0)
            (Utilities|FlowControl|Delay 0.75)))
        (CallFunction|BeginEvent)))
    (else
      (Utilities|FlowControl|Delay 0.2)
      (Transformation|SetActorTransform (Variables|Default|GetMargareth) (Transformation|GetWorldTransform (Variables|Default|GetMargTarget)))
      (Utilities|FlowControl|Delay 0.8)
      (CallFunction|FadeinLight)
      (Utilities|FlowControl|Delay 1.5)
      (CallFunction|FadeinLight)
      (Utilities|FlowControl|Delay 0.2)
      (Transformation|SetActorTransform (Variables|Default|GetMargareth) (Variables|Default|GetMargInitTransform)))))

(event Custom|FadeInLight
  (Utilities|FlowControl|FlipFlop
    (:A
      (bind _newtrack_0 (Timeline|FadeLight PlayFromStart)
        (:Update
          (Rendering|Components|Light|SetIntensity (Variables|/Game/ExternalPackages/Northwood/BP/BP_Light_Hanging_NN_01a.BP_Light_Hanging_NN_01a_C|GetPointLight1 (Variables|Default|GetFinalLight)) (Math|Float|Lerp 0.0 (Variables|Default|GetIntensity) _newtrack_0)))))
    (:B
      (Timeline|FadeLight ReverseFromEnd))))

(event EventBeginPlay
  (Variables|Default|SetIntensity (* (Variables|/Script/Engine.LightComponentBase|GetIntensity (Variables|/Game/ExternalPackages/Northwood/BP/BP_Light_Hanging_NN_01a.BP_Light_Hanging_NN_01a_C|GetPointLight1 (Variables|Default|GetFinalLight))) 2.0))
  (Variables|Default|SetMargInitTransform (Transformation|GetActorTransform (Variables|Default|GetMargareth)))
  (Utilities|FlowControl|Delay 1e+01)
  (CallFunction|BeginEvent))

(fn ConstructionScript)