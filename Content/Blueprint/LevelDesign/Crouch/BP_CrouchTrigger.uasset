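; BP_CrouchTrigger is a level-design trigger that automatically crouches and uncrouches the main character, found on BeginPlay.
; Entering the entrance volume sets IsCrouching and calls Crouch; the exit volume has no begin-overlap handler.
; The middle volume tracks whether the player is inside.
; Leaving the entrance or exit volume calls UncrouchLogic, which stands the player up only when outside the middle volume.
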(event OnComponentEndOverlap(ExitCrouchCollision)
  (params (OverlappedComponent :type Primitive%20Component%20Object%20Reference) (OtherActor :type Actor%20Object%20Reference) (OtherComp :type Primitive%20Component%20Object%20Reference) (OtherBodyIndex :type Integer))
  (CallFunction|UncrouchLogic OtherActor))

(event OnComponentBeginOverlap(EntranceCrouchCollision)
  (params (OverlappedComponent :type Primitive%20Component%20Object%20Reference) (OtherActor :type Actor%20Object%20Reference) (OtherComp :type Primitive%20Component%20Object%20Reference) (OtherBodyIndex :type Integer) (bFromSweep :type Boolean) (SweepResult :type Hit%20Result%20Structure%20%28by%20ref%29))
  (bind _playercharref (Variables|Default|GetPlayerCharRef))
  (if (== OtherActor _playercharref)
    (Variables|/Game/Blueprint/Player/BP_MainCharacter.BP_MainCharacter_C|SetIsCrouching? _playercharref true)
    (Character|Crouch _playercharref)))

(event OnComponentEndOverlap(EntranceCrouchCollision)
  (params (OverlappedComponent :type Primitive%20Component%20Object%20Reference) (OtherActor :type Actor%20Object%20Reference) (OtherComp :type Primitive%20Component%20Object%20Reference) (OtherBodyIndex :type Integer))
  (CallFunction|UncrouchLogic OtherActor))

(event OnComponentBeginOverlap(MidCollision)
  (params (OverlappedComponent :type Primitive%20Component%20Object%20Reference) (OtherActor :type Actor%20Object%20Reference) (OtherComp :type Primitive%20Component%20Object%20Reference) (OtherBodyIndex :type Integer) (bFromSweep :type Boolean) (SweepResult :type Hit%20Result%20Structure%20%28by%20ref%29))
  (if (== OtherActor (Variables|Default|GetPlayerCharRef))
    (Variables|Default|SetInMiddle? true)))

(event OnComponentEndOverlap(MidCollision)
  (params (OverlappedComponent :type Primitive%20Component%20Object%20Reference) (OtherActor :type Actor%20Object%20Reference) (OtherComp :type Primitive%20Component%20Object%20Reference) (OtherBodyIndex :type Integer))
  (if (== OtherActor (Variables|Default|GetPlayerCharRef))
    (Variables|Default|SetInMiddle? false)))

(event EventBeginPlay
  (bind _returnvalue (Actor|GetActorOfClass "/Game/Blueprint/Player/BP_MainCharacter.BP_MainCharacter_C"))
  (Variables|Default|SetPlayerCharRef _returnvalue))

(fn ConstructionScript)

(fn UncrouchLogic
  (params (Actor :type Actor%20Object%20Reference))
  (bind _playercharref (Variables|Default|GetPlayerCharRef))
  (if (and (not (Variables|Default|GetInMiddle?)) (== Actor _playercharref))
    (Variables|/Game/Blueprint/Player/BP_MainCharacter.BP_MainCharacter_C|SetIsCrouching? _playercharref false)
    (Character|UnCrouch _playercharref)))