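; BP_KillZone is a kill volume that sends the player back to a checkpoint on contact.
; BeginPlay caches the BP_MainCharacter reference through GetActorOfClass.
; When that character begins overlapping KillBox and is not InSequence, SpawnPlayer calls its SpawnAtCheckpoint.
; If the cached reference is invalid, the overlap only looks it up again, without respawning.
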(event OnComponentBeginOverlap(KillBox)
  (params (OverlappedComponent :type Primitive%20Component%20Object%20Reference) (OtherActor :type Actor%20Object%20Reference) (OtherComp :type Primitive%20Component%20Object%20Reference) (OtherBodyIndex :type Integer) (bFromSweep :type Boolean) (SweepResult :type Hit%20Result%20Structure%20%28by%20ref%29))
  ;[0.15 0.15 0.15 0.5] Respawn Player
  (bind _playercharacterref (Variables|Default|GetPlayerCharacterRef)
    (:then
      (if (and (== _playercharacterref OtherActor) (not (Variables|/Game/Blueprint/Player/BP_MainCharacter.BP_MainCharacter_C|GetInSequence? _playercharacterref)))
        (CallFunction|SpawnPlayer)))
    (:else
      ;[0.15 0.15 0.15 0.5] Initialize | Get Player Char Ref
      (bind _returnvalue (Actor|GetActorOfClass "/Game/Blueprint/Player/BP_MainCharacter.BP_MainCharacter_C"))
      (Variables|Default|SetPlayerCharacterRef _returnvalue))))

(event Custom|SpawnPlayer
  ;[0 1 0.2468 0.5] Spawn Player
  (Default|SpawnatCheckpoint (Variables|Default|GetPlayerCharacterRef)))

(event EventBeginPlay
  ;[0.15 0.15 0.15 0.5] Initialize | Get Player Char Ref
  (bind _returnvalue (Actor|GetActorOfClass "/Game/Blueprint/Player/BP_MainCharacter.BP_MainCharacter_C"))
  (Variables|Default|SetPlayerCharacterRef _returnvalue))

(fn ConstructionScript)