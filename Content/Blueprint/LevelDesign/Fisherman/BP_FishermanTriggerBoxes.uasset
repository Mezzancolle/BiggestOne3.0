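; Level trigger actor that relocates the fisherman ghost between house, docks and cargo spots as the player enters matching overlap boxes.
; BeginPlay caches the player and ghost, then each trigger snaps the ghost to its location component and starts fishing (house, docks) or card playing (cargo).
; A location enum gates each trigger but is only set at BeginPlay, so the docks trigger never passes its check here.
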(event OnComponentBeginOverlap(HouseTrigger)
  (params (OverlappedComponent :type Primitive%20Component%20Object%20Reference) (OtherActor :type Actor%20Object%20Reference) (OtherComp :type Primitive%20Component%20Object%20Reference) (OtherBodyIndex :type Integer) (bFromSweep :type Boolean) (SweepResult :type Hit%20Result%20Structure%20%28by%20ref%29))
  (if (and (== OtherActor (Variables|Default|GetPlayerCharRef)) (Utilities|Enum|NotEqual(Enum) (Variables|Default|GetCurrentLocations) "NewEnumerator0"))
    (Transformation|SetActorTransform (Variables|Default|GetFishermanRef) (Transformation|GetWorldTransform (Variables|Default|GetHouseLoc)))
    (Default|StartFishing (Variables|Default|GetFishermanRef))))

(event OnComponentBeginOverlap(DocksTrigger)
  (params (OverlappedComponent :type Primitive%20Component%20Object%20Reference) (OtherActor :type Actor%20Object%20Reference) (OtherComp :type Primitive%20Component%20Object%20Reference) (OtherBodyIndex :type Integer) (bFromSweep :type Boolean) (SweepResult :type Hit%20Result%20Structure%20%28by%20ref%29))
  (if (and (== OtherActor (Variables|Default|GetPlayerCharRef)) (Utilities|Enum|NotEqual(Enum) (Variables|Default|GetCurrentLocations) "NewEnumerator2"))
    (Transformation|SetActorTransform (Variables|Default|GetFishermanRef) (Transformation|GetWorldTransform (Variables|Default|GetDocksLoc)))
    (Default|StartFishing (Variables|Default|GetFishermanRef))))

(event OnComponentBeginOverlap(CargoTrigger)
  (params (OverlappedComponent :type Primitive%20Component%20Object%20Reference) (OtherActor :type Actor%20Object%20Reference) (OtherComp :type Primitive%20Component%20Object%20Reference) (OtherBodyIndex :type Integer) (bFromSweep :type Boolean) (SweepResult :type Hit%20Result%20Structure%20%28by%20ref%29))
  (if (and (== OtherActor (Variables|Default|GetPlayerCharRef)) (Utilities|Enum|NotEqual(Enum) (Variables|Default|GetCurrentLocations) "NewEnumerator1"))
    (Transformation|SetActorTransform (Variables|Default|GetFishermanRef) (Transformation|GetWorldTransform (Variables|Default|GetCargoLoc)))
    (Default|StartPlayingCards (Variables|Default|GetFishermanRef))))

(event EventBeginPlay
  (CallFunction|InitializeReferences)
  (Variables|Default|SetCurrentLocations "NewEnumerator2"))

(fn ConstructionScript
  (Variables|/Script/Engine.SceneComponent|SetbAbsoluteScale (Variables|Default|GetCargoLoc) true)
  (Variables|/Script/Engine.SceneComponent|SetbAbsoluteScale (Variables|Default|GetHouseLoc) true)
  (Variables|/Script/Engine.SceneComponent|SetbAbsoluteScale (Variables|Default|GetDocksLoc) true))

(fn InitializeReferences
  (bind _returnvalue (Actor|GetActorOfClass "/Game/Blueprint/Player/BP_MainCharacter.BP_MainCharacter_C"))
  (Variables|Default|SetPlayerCharRef _returnvalue)
  (bind _returnvalue_2 (Actor|GetActorOfClass "/Game/Blueprint/Ghosts/CBP_FishermanGhost.CBP_FishermanGhost_C"))
  (Variables|Default|SetFishermanRef _returnvalue_2))