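; Level-design tree that falls once when the player overlaps its trigger, optionally only if they hold a specified item.
; TreeEvent plays the falling sound and a timeline that lerps the mesh's relative pitch by a default or custom offset set in the construction script.
; If BreaksObject is set, near the end of the fall it calls BreakRoof once on a BP_DestructibleRoof found via GetActorOfClass.
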(event OnComponentBeginOverlap(EventTrigger1)
  (params (OverlappedComponent :type Primitive%20Component%20Object%20Reference) (OtherActor :type Actor%20Object%20Reference) (OtherComp :type Primitive%20Component%20Object%20Reference) (OtherBodyIndex :type Integer) (bFromSweep :type Boolean) (SweepResult :type Hit%20Result%20Structure%20%28by%20ref%29))
  (bind _itemrowname (Variables|Default|GetItemRowName))
  (if (not (Variables|Default|GetTreeFell?))
    (if (== OtherActor (Game|GetPlayerCharacter 0))
      (if (Variables|Default|GetItemDependentEvent?)
        (bind _isvalid_ (CallFunction|CheckValidRowName _itemrowname))
        (bind _hasitem_ (Class|IPlayerUtils|PlayerHasItem?(Message) (Game|Player|GetPlayerPawn 0) _itemrowname))
        (if (and _hasitem_ _isvalid_)
          (CallFunction|TreeEvent))
        (else
          (CallFunction|TreeEvent))))))

(event Custom|TreeEvent
  (bind _output_get (Variables|Default|SetCurrPitch (.pitch (Variables|/Script/Engine.SceneComponent|GetRelativeRotation (Variables|Default|GetSM_FallenTree)))))
  (Variables|Default|SetEndPitch (+ _output_get (Variables|Default|GetPitchAdditive)))
  (Variables|Default|SetTreeFell? true)
  (Audio|Components|Audio|Play (Variables|Default|GetSC_TreeFalling) 0.0)
  (bind _newtrack_0 (Timeline|Falling PlayFromStart)
    (:Update
      (Transformation|SetRelativeRotation (Variables|Default|GetSM_FallenTree) (Math|Rotator|MakeRotator 0.0 (Math|Float|Lerp (Variables|Default|GetCurrPitch) (Variables|Default|GetEndPitch) _newtrack_0) 0.0) false false)
      (if (and (> _newtrack_0 0.9) (Variables|Default|GetBreaksObject?))
        (Utilities|FlowControl|DoOnce false
          (:Completed
            (bind _returnvalue (Actor|GetActorOfClass "/Game/Meshes/DestructibleRoof/BP_DestructibleRoof.BP_DestructibleRoof_C"))
            (Default|BreakRoof _returnvalue)))))))

(fn ConstructionScript
  (if (Variables|Default|GetCustomPitch?)
    (Variables|Default|SetPitchAdditive (Variables|Default|GetCustomAdditive))
    (else
      (Variables|Default|SetPitchAdditive 77.0))))