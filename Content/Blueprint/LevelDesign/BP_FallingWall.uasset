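; Level design actor for a scripted wall that topples when the player walks into its trigger box.
; The overlap destroys the trigger and fires a one-time fall, where a timeline lerps the wall mesh's relative rotation along roll.
; When the timeline finishes, it activates an impact Niagara effect and plays a crash sound, then after a short delay tells a linked light pole trigger to turn on its lights.
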(event OnComponentBeginOverlap(TriggerBox)
  (params (OverlappedComponent :type Primitive%20Component%20Object%20Reference) (OtherActor :type Actor%20Object%20Reference) (OtherComp :type Primitive%20Component%20Object%20Reference) (OtherBodyIndex :type Integer) (bFromSweep :type Boolean) (SweepResult :type Hit%20Result%20Structure%20%28by%20ref%29))
  (if (== OtherActor (Game|GetPlayerCharacter 0))
    (CallFunction|StartFall)
    (Components|DestroyComponent (Variables|Default|GetTriggerBox))))

(event Custom|StartFall
  (Utilities|FlowControl|DoOnce false
    (:Completed
      (bind _output_get (Variables|Default|SetStartRot (Variables|/Script/Engine.SceneComponent|GetRelativeRotation (Variables|Default|GetSM_FallingWall))))
      (Variables|Default|SetEndRot (Math|Rotator|MakeRotator (- (.roll _output_get) 75.0) (.pitch _output_get) (.yaw _output_get)))
      (bind _newtrack_0 (Timeline|WallFalls PlayFromStart)
        (:Update
          (Transformation|SetRelativeRotation (Variables|Default|GetSM_FallingWall) (Math|Rotator|Lerp(Rotator) (Variables|Default|GetStartRot) (Variables|Default|GetEndRot) _newtrack_0) false false))
        (:Finished
          (Components|Activation|Activate (Variables|Default|GetNS_HouseImpact) false)
          (Audio|PlaySoundatLocation "/Game/Audio/SFX/SFX_Env/Church/SFX_Crash_Chandelier_Loud.SFX_Crash_Chandelier_Loud" (Transformation|GetActorLocation) "0, 0, 0" 1.0 1.0 0.0 0 0 0 0)
          (Utilities|FlowControl|Delay 1.5)
          (Default|TurnonLights (Variables|Default|GetLightPoleTrigger)))))))

(event EventBeginPlay)

(fn ConstructionScript)