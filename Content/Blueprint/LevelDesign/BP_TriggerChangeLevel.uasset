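; BP_TriggerChangeLevel is a trigger box that moves the player to NextLevel.
; Its collision stays off for five seconds after BeginPlay, then a DoOnce handles the first overlap by a Player-tagged actor.
; It shows a loading widget with a camera fade, sends sprint and save messages to the player and GameInstance, then calls LoadStreamLevel and OpenLevelByName.
; An unconnected teleport to NextTransform remains unused.
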(event OnComponentBeginOverlap(Box)
  (params (OverlappedComponent :type Primitive%20Component%20Object%20Reference) (OtherActor :type Actor%20Object%20Reference) (OtherComp :type Primitive%20Component%20Object%20Reference) (OtherBodyIndex :type Integer) (bFromSweep :type Boolean) (SweepResult :type Hit%20Result%20Structure%20%28by%20ref%29))
  (bind _nextlevel (Variables|Default|GetNextLevel))
  (if (Actor|ActorHasTag OtherActor "Player")
    (Utilities|FlowControl|DoOnce false
      (:Completed
        (bind _returnvalue (UserInterface|CreateWidget "/Game/UserInterfaces/WBP_Loading.WBP_Loading_C"))
        (bind _output_get (Variables|Default|SetWBP_Loading _returnvalue))
        (UserInterface|Viewport|AddtoViewport _returnvalue 0)
        (CameraFades|StartCameraFade (Game|GetPlayerCameraManager 0) 0.0 1.0 0.2 "(R=0.000000,G=0.000000,B=0.000000,A=1.000000)" true true)
        (Utilities|FlowControl|Delay 0.5)
        (Class|Border|SetBrushColor (Variables|/Game/UserInterfaces/WBP_Loading.WBP_Loading_C|GetBlackBackground (Variables|Default|GetWBP_Loading)) "(R=0.000000,G=0.000000,B=0.000000,A=1.000000)")
        (Class|IPlayerUtils|SetSprint(Message) OtherActor true)
        (Class|ISaveGame|SaveLevelData(Message) (Game|GetGameInstance) false _nextlevel)
        (Class|ISaveable|SavetoGameData(Message) OtherActor false)
        (Game|LoadStreamLevel(byName) _nextlevel true)
        (Game|OpenLevel(byName) _nextlevel)))))

(event EventBeginPlay
  (Collision|SetCollisionEnabled (Variables|Default|GetBox) "NoCollision")
  (Utilities|FlowControl|Delay 5.0)
  (Collision|SetCollisionEnabled (Variables|Default|GetBox) "QueryAndPhysics"))

(fn ConstructionScript)