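; BP_SoundTest is a level-design sound test Blueprint whose audio follows switches between the Present West and Old West states.
; Its Audio component starts playing at BeginPlay.
; OnOldWest fades the volume linearly to full and OnPresentWest fades it to silence, each over a short duration and with a debug print.
; The construction script does nothing, as its sound-assignment node is unwired.
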(event EventBeginPlay
  (Audio|Components|Audio|Play (Variables|Default|GetAudio) 0.0))

(event EventOnPresentWest
  (Audio|Components|Audio|AdjustVolume (Variables|Default|GetAudio) 1.0 0.0 "Linear" :!class /Script/Engine.AudioComponent)
  (Development|PrintString "Present West"))

(event EventOnOldWest
  (Audio|Components|Audio|AdjustVolume (Variables|Default|GetAudio) 1.0 1.0 "Linear" :!class /Script/Engine.AudioComponent)
  (Development|PrintString "Old West"))

(fn ConstructionScript)