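; A fog warp box child Blueprint that shows a Niagara effect over a box area and clears it once enough lights are activated.
; It extends the parent's inside-box setup by sizing the effect from the post-process box's horizontal extents, with a fixed height.
; Each light activation increments a counter; at the threshold, it deactivates the effect and collision once, then destroys itself after a short delay.
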(event EventBeginPlay
  (|CallParentFunction))

(event EventSetInsideBox
  (bind _postprocessbox (Variables|Default|GetPostProcessBox))
  (bind _boxextent (Variables|/Script/Engine.BoxComponent|GetBoxExtent _postprocessbox))
  (bind _returnvalue (* _boxextent "2.000000,2.000000,1.000000"))
  (bind (_x _y) (Math|Vector|BreakVector _returnvalue))
  (|CallParentFunction)
  (Effects|Components|ParticleSystem|SetVectorParameter (Variables|Default|GetNiagara) "Box Size" (Math|Vector|MakeVector _x _y 3e+02)))

(event EventOnLightActivation
  (bind _result (Math|Integer|IncrementInt (Variables|Default|GetIndexLight))
    (:%20%20
      (if (>= _result 2)
        (Utilities|FlowControl|DoOnce false
          (:Completed
            (Components|Activation|Deactivate (Variables|Default|GetNiagara))
            (Collision|SetActorEnableCollision false)
            (Utilities|FlowControl|Delay 3.0)
            (Actor|DestroyActor)))))))

(fn ConstructionScript
  (|CallParentFunction))