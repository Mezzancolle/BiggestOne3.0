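; BP_LightPoleTrigger is a level design Blueprint that switches on a series of light poles one after another.
; Its TurnOnLights event activates the pole at the current index, increments the index, waits a short delay, then calls itself again.
; The recursion stops once the index reaches the end of the LightPoles array, giving a staggered sequential lighting effect.
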(event Custom|TurnOnLights
  (if (!= (Variables|Default|GetIndex) (Utilities|Array|Length (Variables|Default|GetLightPoles)))
    (Default|ActivateLight (Utilities|Array|Get(acopy) (Variables|Default|GetLightPoles) (Variables|Default|GetIndex)))
    (Math|Integer|IncrementInt (Variables|Default|GetIndex)
      (:%20%20
        (Utilities|FlowControl|Delay 0.7)
        (CallFunction|TurnonLights)))))

(fn ConstructionScript)