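; BP_BG_SFX is a level-design Blueprint that controls background ambience and wind audio.
; BeginPlay initializes the ambience sound variable, plus the wind one when HasWind is set, with both assigned None here.
; StartAudio plays each idle Ambience and Wind component from a random start offset, and StopAduio calls a delayed stop and short fade-out on whichever is playing.
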(event Custom|StartAudio
  (bind _ambience (Variables|Default|GetAmbience))
  (bind _wind (Variables|Default|GetWind))
  ;[1 0.9779 0 0.5] Start Playing Audio
  (if (Audio|Components|Audio|IsPlaying _ambience)
    _
    (else
      (Audio|Components|Audio|Play _ambience (Math|Random|RandomFloatinRange 0.0 3e+01))))
  (if (not (Audio|Components|Audio|IsPlaying _wind))
    (Audio|Components|Audio|Play _wind (Math|Random|RandomFloatinRange 0.0 3e+01))))

(event Custom|StopAduio
  (bind _ambience (Variables|Default|GetAmbience))
  (bind _wind (Variables|Default|GetWind))
  ;[1 0.9779 0 0.5] Stop and Fade Out Audio
  (if (Audio|Components|Audio|IsPlaying _ambience)
    (Audio|Components|Audio|StopDelayed _ambience 0.5)
    (Audio|Components|Audio|FadeOut _ambience 0.5 0.0 "Linear" :!class /Script/Engine.AudioComponent))
  (if (Audio|Components|Audio|IsPlaying _wind)
    (Audio|Components|Audio|StopDelayed _wind 0.5)
    (Audio|Components|Audio|FadeOut _wind 0.5 0.0 "Linear" :!class /Script/Engine.AudioComponent)))

(event EventBeginPlay
  ;[0 0.15 0.02426 0.5] Initialize
  (Variables|Default|SetAmbienceSFX 0)
  (if (Variables|Default|GetHasWind?)
    (Variables|Default|SetWindSFX 0)))

(fn ConstructionScript)