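; Manager for a chandelier puzzle that checks whether the player lights the correct chandeliers.
; BindAllChandeliers hooks each chandelier's light-activation event to a shared check, which counts activations and clears an all-correct flag on any wrong one.
; At three activations the counter resets and a success message prints if the flag holds.
; Below three, every light turns off after a short delay, and the flag is never restored here.
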(event Custom|CheckCorrectChandeliers
  (params (Correct? :type Boolean))
  (bind _result (Math|Integer|IncrementInt (Variables|Default|GetCounterCheck))
    (:%20%20
      (if Correct?
        _
        (else
          (Variables|Default|SetAreAllCorrect? false)))
      (if (>= _result 3)
        (Variables|Default|SetCounterCheck 0)
        (if (Variables|Default|GetAreAllCorrect?)
          (Development|PrintString "Nice job!"))
        (else
          (Utilities|FlowControl|Delay 0.5)
          (for _array_element (Variables|Default|GetChandeliers)
            (Default|TurnOffLight _array_element)))))))

(event Custom|BindAllChandeliers
  (for _array_element (Variables|Default|GetChandeliers)
    (EventDispatchers|BindEventtoOnActivateLight _array_element (delegate Custom|CheckCorrectChandeliers))))

(fn ConstructionScript)