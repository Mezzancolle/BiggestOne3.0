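; Level trigger actor that plays a sound once when the player enters its box, then destroys itself.
; On overlap it marks its audio index in the saved misc data, saves asynchronously, and spawns the sound in 2D or at an offset with 3D attenuation.
; On BeginPlay it destroys itself if that index exists in the saved array, testing only index validity rather than the stored boolean.
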(event OnComponentBeginOverlap(Box)
  (params (OverlappedComponent :type Primitive%20Component%20Object%20Reference) (OtherActor :type Actor%20Object%20Reference) (OtherComp :type Primitive%20Component%20Object%20Reference) (OtherBodyIndex :type Integer) (bFromSweep :type Boolean) (SweepResult :type Hit%20Result%20Structure%20%28by%20ref%29))
  (bind _returnvalue (Game|GetGameInstance))
  (bind _sound (Variables|Default|GetSound))
  (bind _audiotransform (Variables|Default|GetAudioTransform))
  (if (Actor|ActorHasTag OtherActor "Player")
    (Utilities|FlowControl|DoOnce false
      (:Completed
        (bind _saveddata (Class|ISaveGame|GetGameData(Message) _returnvalue))
        (Utilities|Array|SetArrayElem (Utilities|Struct|BreakS_MiscSaveData (Variables|/Game/Blueprint/SaveGame/BP_GameData.BP_GameData_C|GetMiscData _saveddata)) (Variables|Default|GetAudioIndexSaveData) true true)
        (bind _structout (Utilities|Struct|SetmembersinS_MiscSaveData (Variables|/Game/Blueprint/SaveGame/BP_GameData.BP_GameData_C|GetMiscData _saveddata) (Utilities|Struct|BreakS_MiscSaveData (Variables|/Game/Blueprint/SaveGame/BP_GameData.BP_GameData_C|GetMiscData _saveddata))))
        (Class|ISaveGame|SaveMiscData(Message) _returnvalue true _structout)
        (if (Variables|Default|GetAudio3D?)
          (Audio|SpawnSoundatLocation _sound (+ (Transformation|GetActorLocation) (Math|Vector|RotateVector (.location _audiotransform) (Transformation|GetActorRotation))) (.rotation _audiotransform) (Variables|Default|GetVolume%20Multiplier) (Variables|Default|GetPitch%20Multiplier) (Variables|Default|GetStart%20Time) "/Game/Audio/Settings/Attenuations/ATT_Audio3D.ATT_Audio3D" 0)
          (else
            (Audio|SpawnSound2D _sound (Variables|Default|GetVolume%20Multiplier) (Variables|Default|GetPitch%20Multiplier) (Variables|Default|GetStart%20Time) 0)))
        (Actor|DestroyActor)))))

(event EventBeginPlay
  (bind _saveddata (Class|ISaveGame|GetGameData(Message) (Game|GetGameInstance)))
  (if (Utilities|Array|IsValidIndex (Utilities|Struct|BreakS_MiscSaveData (Variables|/Game/Blueprint/SaveGame/BP_GameData.BP_GameData_C|GetMiscData _saveddata)) (Variables|Default|GetAudioIndexSaveData))
    (Actor|DestroyActor)))

(fn ConstructionScript)