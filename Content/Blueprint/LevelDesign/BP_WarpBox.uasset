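; BP_WarpBox is a level-design volume that sends the player a warp rotation message and plays a random bark on entering its inner WarpBox.
; A surrounding PostProcessBox, matched to WarpBox in X and Z, drives warp post-process intensity from the player's local-Y proximity to the actor.
; Timelines blend the effect in and out, while Tick, active inside, also scales choir, scream and ambience volumes.
; Exiting stops camera shakes and fades the audio.
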(event OnComponentBeginOverlap(WarpBox)
  (params (OverlappedComponent :type Primitive%20Component%20Object%20Reference) (OtherActor :type Actor%20Object%20Reference) (OtherComp :type Primitive%20Component%20Object%20Reference) (OtherBodyIndex :type Integer) (bFromSweep :type Boolean) (SweepResult :type Hit%20Result%20Structure%20%28by%20ref%29))
  (if (and (Utilities|DoesObjectImplementInterface OtherActor "/Game/Blueprint/Interfaces/I_PlayerUtils.I_PlayerUtils_C") (Actor|ActorHasTag OtherActor "Player"))
    (Class|IPlayerUtils|SetRotationWarpBox(Message) OtherActor (Math|Vector|GetRightVector (Variables|Default|GetWarpBox)))
    (Utilities|PlayRandomBark (Variables|Default|GetDialogues%20Rown%20Name) (Variables|Default|GetTime%20to%20Play%20Dialogue))))

(event OnComponentBeginOverlap(PostProcessBox)
  (params (OverlappedComponent :type Primitive%20Component%20Object%20Reference) (OtherActor :type Actor%20Object%20Reference) (OtherComp :type Primitive%20Component%20Object%20Reference) (OtherBodyIndex :type Integer) (bFromSweep :type Boolean) (SweepResult :type Hit%20Result%20Structure%20%28by%20ref%29))
  (if (and (Utilities|DoesObjectImplementInterface OtherActor "/Game/Blueprint/Interfaces/I_PlayerUtils.I_PlayerUtils_C") (Actor|ActorHasTag OtherActor "Player"))
    (bind _alpha (Timeline|TL_LerpIn PlayFromStart)
      (:Update
        (bind _returnvalue (CallFunction|CalculateAmount))
        (Class|IPlayerUtils|SetWarpBoxPostProcess(Message) (Game|Player|GetPlayerPawn 0) (Math|Float|Lerp 0.0 _returnvalue _alpha)))
      (:Finished
        (Actor|Tick|SetActorTickEnabled true)
        (Audio|Components|Audio|Play (Variables|Default|GetAmbienceAudio) 0.0)
        (Audio|Components|Audio|Play (Variables|Default|GetScreamAudio) 0.0)
        (Audio|Components|Audio|Play (Variables|Default|GetChoirAudio) 0.0)))))

(event OnComponentEndOverlap(PostProcessBox)
  (params (OverlappedComponent :type Primitive%20Component%20Object%20Reference) (OtherActor :type Actor%20Object%20Reference) (OtherComp :type Primitive%20Component%20Object%20Reference) (OtherBodyIndex :type Integer))
  (if (and (Utilities|DoesObjectImplementInterface OtherActor "/Game/Blueprint/Interfaces/I_PlayerUtils.I_PlayerUtils_C") (Actor|ActorHasTag OtherActor "Player"))
    (Actor|Tick|SetActorTickEnabled false)
    (CameraShake|StopAllCameraShakes (Game|GetPlayerCameraManager 0) true)
    (bind _alpha (Timeline|TL_LerpOut PlayFromStart)
      (:Update
        (bind _returnvalue (CallFunction|CalculateAmount))
        (Class|IPlayerUtils|SetWarpBoxPostProcess(Message) (Game|Player|GetPlayerPawn 0) (Math|Float|Lerp _returnvalue 0.0 _alpha))
        (CallFunction|SetAudio (Math|Float|Lerp _returnvalue 0.0 _alpha)))
      (:Finished
        (Audio|Components|Audio|Stop (Variables|Default|GetScreamAudio))
        (Audio|Components|Audio|Stop (Variables|Default|GetAmbienceAudio))
        (Audio|Components|Audio|Stop (Variables|Default|GetChoirAudio))))))

(event Custom|SetInsideBox
  (bind _warpbox (Variables|Default|GetWarpBox))
  (bind _boxextent (Variables|/Script/Engine.BoxComponent|GetBoxExtent _warpbox))
  (Components|Box|SetBoxExtent (Variables|Default|GetPostProcessBox) (Math|Vector|MakeVector (.x _boxextent) (.y (Variables|/Script/Engine.BoxComponent|GetBoxExtent (Variables|Default|GetPostProcessBox))) (.z _boxextent)) true))

(event EventTick
  (params (DeltaSeconds :type Float%20%28single-precision%29))
  (bind _returnvalue (CallFunction|CalculateAmount))
  (Class|IPlayerUtils|SetWarpBoxPostProcess(Message) (Game|Player|GetPlayerPawn 0) _returnvalue)
  (CallFunction|SetAudio _returnvalue))

(event EventBeginPlay
  (CallFunction|SetInsideBox)
  (Audio|Components|Audio|Stop (Variables|Default|GetChoirAudio))
  (Audio|Components|Audio|Stop (Variables|Default|GetScreamAudio))
  (Audio|Components|Audio|Stop (Variables|Default|GetAmbienceAudio))
  (Variables|Default|SetDivider (* (.y (Variables|/Script/Engine.BoxComponent|GetBoxExtent (Variables|Default|GetPostProcessBox))) 2.0)))

(fn ConstructionScript)

(fn CalculateAmount
  (Utilities|IsValid (Game|Player|GetPlayerPawn 0)
    (:Is%20Valid
      (return (- 1.0 (Math|Float|Min(Float) (Math|Float|Max(Float) (/ (Math|Float|Absolute(Float) (.y (Math|Vector|UnrotateVector (- (Transformation|GetActorLocation) (Transformation|GetActorLocation (Game|Player|GetPlayerPawn 0))) (Transformation|GetActorRotation)))) (Variables|Default|GetDivider)) 0.0) 1.0))))))

(fn SetAudio
  (params (AudioValue :type Float%20%28double-precision%29))
  (Audio|Components|Audio|SetVolumeMultiplier (Variables|Default|GetScreamAudio) (* AudioValue 0.3) :!class /Script/Engine.AudioComponent)
  (Audio|Components|Audio|SetVolumeMultiplier (Variables|Default|GetAmbienceAudio) (* AudioValue 0.05) :!class /Script/Engine.AudioComponent)
  (Audio|Components|Audio|SetVolumeMultiplier (Variables|Default|GetChoirAudio) (* AudioValue 1.0) :!class /Script/Engine.AudioComponent))