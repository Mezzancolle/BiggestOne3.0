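; Level generator for the chandeliers enigma that spawns graves and their matching chandeliers on BeginPlay.
; Shuffles position and mesh indices on first run and saves them through the game instance, reusing the saved layout afterwards.
; Graves take shuffled positions and meshes with index-ordered reading texts, and chandeliers follow the same positions, scaled and offset.
; The first three shuffled entries are flagged correct, and all chandeliers are bound through a spawned BP_ChandeliersManager.
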(event EventBeginPlay
  (Utilities|FlowControl|Sequence
    (:then_0
      (CallFunction|GenerateRandomGraves))
    (:then_1
      (bind _returnvalue (Game|SpawnActorfromClass "/Game/Blueprint/LevelDesign/BP_ChandeliersManager.BP_ChandeliersManager_C" (Math|Transform|MakeTransform "0, 0, 0" "0, 0, 0" "1.000000,1.000000,1.000000") "Undefined" "MultiplyWithRoot" 0 0))
      (Variables|Default|SetChandeliersManager _returnvalue))
    (:then_2
      (CallFunction|GenerateChandeliers))
    (:then_3
      (Default|BindAllChandeliers (Variables|Default|GetChandeliersManager)))))

(fn ConstructionScript)

(fn GenerateRandomGraves
  (bind _saveddata (Class|ISaveGame|GetGameData(Message) (Game|GetGameInstance)))
  (if (== (Utilities|Array|Length (.chandeliersenigma_positionsindexes (Variables|/Game/Blueprint/SaveGame/BP_GameData.BP_GameData_C|GetEnigmasData _saveddata))) 0)
    (Utilities|Array|Shuffle (Variables|Default|GetChandeliersMeshesIndexes))
    (Utilities|Array|Shuffle (Variables|Default|GetChandeliersPositionIndexes))
    (Class|ISaveGame|SaveEnigmasData(Message) (Game|GetGameInstance) true (Utilities|Struct|MakeS_EnigmasSaveData (Variables|Default|GetChandeliersPositionIndexes) (Variables|Default|GetChandeliersMeshesIndexes) false false))
    (else
      (Variables|Default|SetChandeliersMeshesIndexes (.chandeliersenigma_staticmeshesindexes (Variables|/Game/Blueprint/SaveGame/BP_GameData.BP_GameData_C|GetEnigmasData _saveddata)))
      (Variables|Default|SetChandeliersPositionIndexes (.chandeliersenigma_positionsindexes (Variables|/Game/Blueprint/SaveGame/BP_GameData.BP_GameData_C|GetEnigmasData _saveddata)))))
  (for _index (range 0 (- (Utilities|Array|Length (Variables|Default|GetChandeliersPositionIndexes)) 1))
    (bind _returnvalue (Game|SpawnActorfromClass "/Game/Blueprint/Interactable/SceneInteraction/BPC_Grave.BPC_Grave_C" (Math|Transform|MakeTransform (+ (Transformation|GetActorLocation) (Utilities|Array|Get(acopy) (Variables|Default|GetGravesPositions) (Utilities|Array|Get(acopy) (Variables|Default|GetChandeliersPositionIndexes) _index))) "0, 0, 0" "1.000000,1.000000,1.000000") "Undefined" "MultiplyWithRoot" 0 "Default" (Utilities|Array|Get(acopy) (Variables|Default|GetReading%20Panel%20Texts) _index) 0))
    (Components|StaticMesh|SetStaticMesh (Variables|/Game/Blueprint/Interactable/Interactable/BP_InteractableParent.BP_InteractableParent_C|GetStaticMesh _returnvalue) (Utilities|Array|Get(acopy) (Variables|Default|GetGravesStaticMeshes) (Utilities|Array|Get(acopy) (Variables|Default|GetChandeliersMeshesIndexes) _index)))))

(fn GenerateChandeliers
  (for (_array_element _array_index) (Variables|Default|GetChandeliersPositionIndexes)
    (bind _returnvalue (Game|SpawnActorfromClass "/Game/Blueprint/Interactable/Interactable/CBP_Chandelier.CBP_Chandelier_C" (Math|Transform|MakeTransform (+ (Transformation|GetActorLocation) (* (Utilities|Array|Get(acopy) (Variables|Default|GetGravesPositions) _array_element) (Variables|Default|GetMultiplyGravesPosition)) (Variables|Default|GetOffsetFromGraves)) "0, 0, 0" "1.000000,1.000000,1.000000") "Undefined" "MultiplyWithRoot" 0 (< _array_index 3) 0))
    (Utilities|Array|Add (Variables|/Game/Blueprint/LevelDesign/BP_ChandeliersManager.BP_ChandeliersManager_C|GetChandeliers (Variables|Default|GetChandeliersManager)) _returnvalue)))