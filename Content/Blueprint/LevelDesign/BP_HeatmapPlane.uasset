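; BP_HeatmapPlane is a level design plane that records a heatmap of the player character's position.
; Each tick it line-traces from the player down past the plane, looking for hits on itself.
; Hit locations are converted to plane-local coordinates scaled by resolution, then passed to a dynamic M_Heatmap material that is drawn into a runtime render target.
; Debug traces and print strings remain active.
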(event Custom|DrawToTarget
  (params (Location :type Vector) (Strength :type Float%20%28double-precision%29) (Size :type Float%20%28double-precision%29))
  (bind _dmi_heatmap (Variables|Default|GetDMI_Heatmap))
  (Rendering|Material|SetScalarParameterValue _dmi_heatmap "Strength" Strength :!class /Script/Engine.MaterialInstanceDynamic)
  (Rendering|Material|SetScalarParameterValue _dmi_heatmap "Size" Size :!class /Script/Engine.MaterialInstanceDynamic)
  (Rendering|Material|SetVectorParameterValue _dmi_heatmap "Position" (Math|Conversions|ToLinearColor(Vector) (/ (Math|Transform|TransformLocation (Math|Transform|InvertTransform (Transformation|GetWorldTransform (Variables|Default|GetPlane))) Location) (Variables|Default|GetResolution))) :!class /Script/Engine.MaterialInstanceDynamic)
  (Rendering|DrawMaterialtoRenderTarget (Variables|Default|GetRenderTargetRuntime) _dmi_heatmap)
  (Development|PrintString "DrewHeatmap"))

(event EventBeginPlay
  (Actor|GetActorOfClass "/Game/Blueprint/Player/BP_MainCharacter.BP_MainCharacter_C")
  (Variables|Default|SetPlayerRef (Game|GetPlayerCharacter 0)))

(event EventTick
  (params (DeltaSeconds :type Float%20%28single-precision%29))
  (bind _playerref (Variables|Default|GetPlayerRef))
  (bind _returnvalue (Transformation|GetActorLocation _playerref))
  (bind (_x _y) (Math|Vector|BreakVector _returnvalue))
  (Utilities|IsValid _playerref
    (:Is%20Valid
      (bind _outhits (Class|KismetSystemLibrary|LineTraceMultiforObjects _returnvalue (Math|Vector|MakeVector _x _y (- (.z (Transformation|GetWorldLocation (Variables|Default|GetPlane))) 2e+02)) (Utilities|Array|MakeArray "ObjectTypeQuery1" "ObjectTypeQuery2") false 0 "ForDuration" true "(R=1.000000,G=0.000000,B=0.000000,A=1.000000)" "(R=0.000000,G=1.000000,B=0.000000,A=1.000000)" 0.1))
      (for _array_element _outhits
        (if (and (.bBlockingHit (Collision|BreakHitResult _array_element)) (== (.HitActor (Collision|BreakHitResult _array_element)) self))
          (CallFunction|DrawtoTarget (.Location (Collision|BreakHitResult _array_element)) 1.0 1.0)
          (Development|PrintString "Triggered")
          (else
            (Development|PrintString (Utilities|String|ToString(Boolean) (== (.HitActor (Collision|BreakHitResult _array_element)) self)))
            (Development|PrintString "NotTriggered")))))))

(fn ConstructionScript
  (bind _returnvalue (Rendering|Material|CreateDynamicMaterialInstance "/Game/Blueprint/LevelDesign/M_Heatmap.M_Heatmap" "None" "None" :!class /Script/Engine.KismetMaterialLibrary))
  (Variables|Default|SetDMI_Heatmap _returnvalue))