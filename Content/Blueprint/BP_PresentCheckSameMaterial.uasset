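; BP_PresentCheckSameMaterial is a tool Blueprint that steps through BP_PresentWestActor instances in groups sharing identical static mesh materials.
; NewCheck gathers all those actors and extracts the first group.
; Each ContinueCheck clears the current group, then moves actors matching the first remaining one out of the pool, storing their material list and advancing CurrentIndex.
; Replacenewmaterial writes the Materials array back onto every mesh in the current group.
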(event Custom|Continue%20Check
  (Utilities|Array|Clear (Variables|Default|GetCurrent%20Actors))
  (Utilities|Array|Clear (Variables|Default|GetMaterials))
  (if (Utilities|Array|IsEmpty (stale Custom|New%20Check _output_get))
    (Variables|Default|SetCurrent%20Index 0)
    (else
      (bind (_arrayindex _arrayelement) (Utilities|Array|ReverseforEachLoop (stale Custom|New%20Check _output_get))
        (:LoopBody
          (if (Utilities|Array|Identical (Rendering|Material|GetMaterials (Variables|/Game/Blueprint/Abstacts/BP_PresentWestActor.BP_PresentWestActor_C|GetStaticMesh (Utilities|Array|Get(acopy) (stale Custom|New%20Check _output_get)))) (Rendering|Material|GetMaterials (Variables|/Game/Blueprint/Abstacts/BP_PresentWestActor.BP_PresentWestActor_C|GetStaticMesh _arrayelement)))
            (Utilities|Array|Add (Variables|Default|GetCurrent%20Actors) _arrayelement)
            (Utilities|Array|RemoveIndex (stale Custom|New%20Check _output_get) _arrayindex)))
        (:Completed
          (Math|Integer|IncrementInt (Variables|Default|GetCurrent%20Index)
            (:%20%20
              (Variables|Default|SetMaterials (Rendering|Material|GetMaterials (Variables|/Game/Blueprint/Abstacts/BP_PresentWestActor.BP_PresentWestActor_C|GetStaticMesh (Utilities|Array|Get(acopy) (Variables|Default|GetCurrent%20Actors))))))))))))

(event Custom|Replace%20new%20material
  (for _array_element (Variables|Default|GetCurrent%20Actors)
    (for (_ _array_index) (Rendering|Material|GetMaterials (Variables|/Game/Blueprint/Abstacts/BP_PresentWestActor.BP_PresentWestActor_C|GetStaticMesh _array_element))
      (Rendering|Material|SetMaterial (Variables|/Game/Blueprint/Abstacts/BP_PresentWestActor.BP_PresentWestActor_C|GetStaticMesh _array_element) _array_index (Utilities|Array|Get(acopy) (Variables|Default|GetMaterials) _array_index)))))

(event Custom|New%20Check
  (bind _outactors (Actor|GetAllActorsOfClass "/Game/Blueprint/Abstacts/BP_PresentWestActor.BP_PresentWestActor_C"))
  (bind _output_get (Variables|Default|SetAll%20Present%20Actor _outactors))
  (if (Utilities|Array|IsEmpty _output_get)
    (Variables|Default|SetCurrent%20Index 0)
    (else
      (bind (_arrayindex _arrayelement) (Utilities|Array|ReverseforEachLoop _output_get)
        (:LoopBody
          (if (Utilities|Array|Identical (Rendering|Material|GetMaterials (Variables|/Game/Blueprint/Abstacts/BP_PresentWestActor.BP_PresentWestActor_C|GetStaticMesh (Utilities|Array|Get(acopy) _output_get))) (Rendering|Material|GetMaterials (Variables|/Game/Blueprint/Abstacts/BP_PresentWestActor.BP_PresentWestActor_C|GetStaticMesh _arrayelement)))
            (Utilities|Array|Add (Variables|Default|GetCurrent%20Actors) _arrayelement)
            (Utilities|Array|RemoveIndex _output_get _arrayindex)))
        (:Completed
          (Math|Integer|IncrementInt (Variables|Default|GetCurrent%20Index)
            (:%20%20
              (Variables|Default|SetMaterials (Rendering|Material|GetMaterials (Variables|/Game/Blueprint/Abstacts/BP_PresentWestActor.BP_PresentWestActor_C|GetStaticMesh (Utilities|Array|Get(acopy) (Variables|Default|GetCurrent%20Actors))))))))))))

(event EventBeginPlay)

(event Collision|EventActorBeginOverlap
  (params (OtherActor :type Actor%20Object%20Reference)))

(event EventTick
  (params (DeltaSeconds :type Float%20%28single-precision%29)))

(fn ConstructionScript)