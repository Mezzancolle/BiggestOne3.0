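; Parent interactable that only succeeds when the player carries a required item.
; Interact checks the player's diary inventory for ItemToHave and fires either the successfully-interact or cannot-interact dispatcher.
; BeginPlay creates a dynamic material on the static mesh and binds both dispatchers to debug handlers that tint it green or red.
; LookAt returns a fixed "locked!" message with the player and hit component.
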(event Custom|OnNoItem
  (params (PlayerRef :type BP%20Main%20Character%20Object%20Reference))
  (Rendering|Material|SetVectorParameterValue (Variables|Default|GetDynamicMaterial) "Color" "(R=1.000000,G=0.045656,B=0.000000,A=1.000000)" :!class /Script/Engine.MaterialInstanceDynamic))

(event Custom|DebugTest
  (params (PlayerRef :type BP%20Main%20Character%20Object%20Reference))
  (Rendering|Material|SetVectorParameterValue (Variables|Default|GetDynamicMaterial) "Color" "(R=0.176222,G=1.000000,B=0.000000,A=1.000000)" :!class /Script/Engine.MaterialInstanceDynamic))

(event EventInteract
  (params (PlayerRef :type BP%20Main%20Character%20Object%20Reference) (LookingComponent :type Primitive%20Component%20Object%20Reference))
  (if (Utilities|Array|ContainsItem (Variables|/Game/UserInterfaces/UIPauseMenu/Inventory/WBP_Inventory.WBP_Inventory_C|GetInventoryItems (Variables|/Game/UserInterfaces/UIPauseMenu/WBP_Diary.WBP_Diary_C|GetWBP_Inventory (Variables|/Game/Blueprint/Player/BP_MainCharacter.BP_MainCharacter_C|GetWBP_Diary PlayerRef))) (Variables|Default|GetItemToHave))
    (Default|CallOnSuccessfullyInteract PlayerRef)
    (else
      (Default|CallOnCannotInteract PlayerRef))))

(event EventBeginPlay
  (bind _returnvalue (Rendering|Material|CreateDynamicMaterialInstance (Variables|Default|GetStaticMesh) 0 (Rendering|Material|GetMaterial (Variables|Default|GetStaticMesh) 0) "None" :!class /Script/Engine.PrimitiveComponent))
  (Variables|Default|SetDynamicMaterial _returnvalue)
  (Rendering|Material|SetMaterial (Variables|Default|GetStaticMesh) 0 _returnvalue)
  (EventDispatchers|BindEventtoOnSuccessfullyInteract (delegate Custom|DebugTest))
  (EventDispatchers|BindEventtoOnCannotInteract (delegate Custom|OnNoItem)))

(fn ConstructionScript
  (|CallParentFunction))

(fn Lookat
  (params (Player%20Ref :type BP%20Main%20Character%20Object%20Reference) (Hit%20Component :type Primitive%20Component%20Object%20Reference))
  (return Player%20Ref Hit%20Component "locked!"))