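; Interactable hatch that the player swings open and closed, optionally locked behind a key item looked up by KeyRowName.
; Interact is ignored when StuckOpen, plays a closed-door sound without the key, or toggles a timeline that lerps the door mesh's pitch forward or in reverse.
; Toggle sounds use random pitch and a short DoOnce cooldown.
; LookAt reports the locked state, which SetDoorStatus sets and OnGhostComplete clears.
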(event Custom|SetDoorStatus
  (params (NewStatus :type Boolean))
  (Variables|Default|SetIsLocked NewStatus))

(event Custom|PlaySound
  (params (SoundToPlay :type Sound%20Base%20Object%20Reference))
  ;[1 1 1] Add Impact SFX
  (Utilities|FlowControl|DoOnce false :!label _label
    (:Completed
      (Audio|SpawnSoundatLocation SoundToPlay (Transformation|GetActorLocation) "0, 0, 0" 1.0 (Math|Random|RandomFloatinRange 0.85 1.2) 0.0 "/Game/Audio/Settings/Attenuations/ATT_Audio3D.ATT_Audio3D" 0)
      (Utilities|FlowControl|Delay 0.4)
      (goto _label Reset))))

(event Custom|Open
  (bind _sm_building_door1 (Variables|Default|GetSM_Building_Door1))
  (bind _returnvalue (Transformation|GetWorldRotation _sm_building_door1))
  (CallFunction|PlaySound "/Game/Audio/SFX/SFX_Env/Door/SFX_Env_Door_Close.SFX_Env_Door_Close")
  (Variables|Default|SetIsOpen? true)
  (bind _alpha (Timeline|TL_OpenDoor Play)
    (:Update
      (Transformation|SetWorldRotation _sm_building_door1 (Math|Rotator|MakeRotator (.roll _returnvalue) (Math|Float|Lerp (Variables|Default|GetClosedRotation) (Variables|Default|GetOpenedRotation) _alpha) (.yaw _returnvalue)) false false))))

(event Custom|Close
  (bind _sm_building_door1 (Variables|Default|GetSM_Building_Door1))
  (bind _returnvalue (Transformation|GetWorldRotation _sm_building_door1))
  (CallFunction|PlaySound "/Game/Audio/SFX/SFX_Env/Door/SFX_Env_Door_Close_1.SFX_Env_Door_Close_1")
  (Variables|Default|SetIsOpen? false)
  (bind _alpha (Timeline|TL_OpenDoor Reverse)
    (:Update
      (Transformation|SetWorldRotation _sm_building_door1 (Math|Rotator|MakeRotator (.roll _returnvalue) (Math|Float|Lerp (Variables|Default|GetClosedRotation) (Variables|Default|GetOpenedRotation) _alpha) (.yaw _returnvalue)) false false))))

(event EventOnGhostComplete
  (Variables|Default|SetIsLocked false))

(event EventInteract
  (params (LookingComponent :type Primitive%20Component%20Object%20Reference))
  (if (not (Variables|Default|GetStuckOpen?))
    (if (Variables|Default|GetIsLocked)
      (bind _hasitem_ (Class|IPlayerUtils|PlayerHasTakenItem?(Message) (Game|Player|GetPlayerPawn 0) (Variables|Default|GetKeyRowName)))
      (if _hasitem_
        (if (not (Variables|Default|GetIsOpen?)) :!label _label
          (CallFunction|Open)
          (else
            (CallFunction|Close)))
        (else
          (Audio|PlaySoundatLocation "/Game/Audio/SFX/SFX_Misc/Door/SFX_DoorClosed.SFX_DoorClosed" (Transformation|GetActorLocation) "0, 0, 0" 1.0 1.0 0.0 "/Game/Audio/Settings/Attenuations/ATT_Audio3D.ATT_Audio3D" 0 0 0)))
      (else
        (goto _label)))))

(event EventBeginPlay
  (bind _output_get (Variables|Default|SetClosedRotation (.pitch (Transformation|GetWorldRotation (Variables|Default|GetSM_Building_Door1)))))
  (Variables|Default|SetOpenedRotation (+ _output_get (Variables|Default|GetOpeningDegrees))))

(fn ConstructionScript)

(fn Lookat
  (params (Player%20Ref :type Actor%20Object%20Reference) (Hit%20Component :type Primitive%20Component%20Object%20Reference))
  (if (Variables|Default|GetIsLocked)
    (bind _hasitem_ (Class|IPlayerUtils|PlayerHasTakenItem?(Message) Player%20Ref (Variables|Default|GetKeyRowName)))
    (return Player%20Ref Hit%20Component "" (not _hasitem_))
    (else
      (return Player%20Ref Hit%20Component "" false))))