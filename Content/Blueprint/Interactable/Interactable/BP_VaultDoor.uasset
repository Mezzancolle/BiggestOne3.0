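; Vault door interactable that plays a one-time opening sequence when the player character overlaps its trigger.
; Chained timelines spin the dial, then both knobs, then swing the hinge open after a short pause.
; An AudioManager macro handles timed, faded sound cues, while UnlatchDoor re-calls itself to play one spaced unlatch sound per bar.
; LookAt reports a locked state from the player's taken-item check, which the trigger ignores.
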(event OnComponentBeginOverlap(EventTrigger)
  (params (OverlappedComponent :type Primitive%20Component%20Object%20Reference) (OtherActor :type Actor%20Object%20Reference) (OtherComp :type Primitive%20Component%20Object%20Reference) (OtherBodyIndex :type Integer) (bFromSweep :type Boolean) (SweepResult :type Hit%20Result%20Structure%20%28by%20ref%29))
  ;[0.15 0.15 0.15 0.5] Opening Vault Door Event
  ;;[0.15 0.15 0.15 0.5] Trigger Event
  (if (== OtherActor (Game|GetPlayerCharacter 0))
    (Utilities|FlowControl|DoOnce false
      (:Completed
        (CallFunction|RotateAcc)))))

(event Custom|UnlatchDoor
  (if (== (Variables|Default|GetBarIndex) 0)
    (Variables|Default|SetBarDelayTime (/ (Variables|Default|GetUnlatchTime?) (Variables|Default|GetTotalBars))))
  (if (!= (Variables|Default|GetBarIndex) (Variables|Default|GetTotalBars))
    (Utilities|AudioManager (Variables|Default|GetSC_Safe_Unlatch) 0.1 0.1 0.7
      (:OutPin
        (Utilities|FlowControl|Delay (Variables|Default|GetBarDelayTime))
        (Math|Integer|IncrementInt (Variables|Default|GetBarIndex)
          (:%20%20
            (CallFunction|UnlatchDoor)))))))

(event Custom|Open
  (bind _hingepin (Variables|Default|GetHingepin))
  (bind _returnvalue (Transformation|GetWorldRotation _hingepin))
  ;[0.15 0.15 0.15 0.5] Opening Vault Door Event
  ;;[0.15 0.15 0.15 0.5] Open Door (3 Seconds)
  (Audio|SpawnSoundatLocation "/Game/Audio/SFX/SFX_Misc/Safe/SFX_Safe_Open_Large.SFX_Safe_Open_Large" (Transformation|GetActorLocation) "0, 0, 0" 1.0 1.0 0.0 0 0)
  (bind _alpha (Timeline|TL_OpenDoor PlayFromStart)
    (:Update
      (Transformation|SetRelativeRotation _hingepin (Math|Rotator|MakeRotator (.roll _returnvalue) (.pitch _returnvalue) (Math|Float|Lerp (Variables|Default|GetClosedRotation) (Variables|Default|GetOpenedRotation) _alpha)) false false))))

(event Custom|RotateAcc
  ;[0.15 0.15 0.15 0.5] Opening Vault Door Event
  ;;[0.15 0.15 0.15 0.5] Rotate Dial and Knobs (4 seconds)
  (Utilities|AudioManager (Variables|Default|GetSFX_DialTurn) 0.25 0.25 1.75
    (:OutPin
      (bind _newtrack_0 (Timeline|RotateDial PlayFromStart)
        (:Update
          (Transformation|SetRelativeRotation (Variables|Default|GetDial) (Math|Rotator|Lerp(Rotator) "0, 0, 0" "0.000000,0.000000,360.000000" _newtrack_0) false false))
        (:Finished
          (Utilities|AudioManager (Variables|Default|GetSC_Safe_Unlock) 0.05 0.05 0.4
            (:OutPin
              (CallFunction|UnlatchDoor)
              (bind _newtrack_0_2 (Timeline|RotateKnobs PlayFromStart)
                (:Update
                  (Transformation|SetRelativeRotation (Variables|Default|GetKnob1) (Math|Rotator|Lerp(Rotator) "0, 0, 0" "0.000000,0.000000,360.000000" _newtrack_0_2) false false))
                (:Finished
                  (Utilities|FlowControl|Delay 0.5)
                  (CallFunction|Open))))))))))

(event EventBeginPlay
  ;[0.15 0.15 0.15 0.5] Begin Play
)

(fn ConstructionScript)

(fn Lookat
  (params (Player%20Ref :type Actor%20Object%20Reference) (Hit%20Component :type Primitive%20Component%20Object%20Reference))
  (if true
    (bind _hasitem_ (Class|IPlayerUtils|PlayerHasTakenItem?(Message) Player%20Ref "None"))
    (return Player%20Ref Hit%20Component "" (not _hasitem_))
    (else
      (return Player%20Ref Hit%20Component "" false))))