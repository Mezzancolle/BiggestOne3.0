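; Door variant that, going by its name, closes behind the player and locks once they have passed through from the front.
; An outside collision overlap by an actor tagged Player records a front entry.
; A later inside overlap by the player then fires once, setting the door locked and calling ForceOpen.
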(event OnComponentBeginOverlap(OutsideCollision)
  (params (OverlappedComponent :type Primitive%20Component%20Object%20Reference) (OtherActor :type Actor%20Object%20Reference) (OtherComp :type Primitive%20Component%20Object%20Reference) (OtherBodyIndex :type Integer) (bFromSweep :type Boolean) (SweepResult :type Hit%20Result%20Structure%20%28by%20ref%29))
  (if (Actor|ActorHasTag OtherActor "Player")
    (Variables|Default|SetEnteredFromFront true)))

(event OnComponentBeginOverlap(InsideCollision)
  (params (OverlappedComponent :type Primitive%20Component%20Object%20Reference) (OtherActor :type Actor%20Object%20Reference) (OtherComp :type Primitive%20Component%20Object%20Reference) (OtherBodyIndex :type Integer) (bFromSweep :type Boolean) (SweepResult :type Hit%20Result%20Structure%20%28by%20ref%29))
  (if (and (Actor|ActorHasTag OtherActor "Player") (Variables|Default|GetEnteredFromFront))
    (Utilities|FlowControl|DoOnce false
      (:Completed
        (Variables|Default|SetIsLocked true)
        (CallFunction|ForceOpen)))))

(fn ConstructionScript)