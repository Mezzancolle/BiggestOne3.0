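; Interactable pair of cellar doors that swing open and closed, optionally locked behind a key item.
; On interact, DoorSFX checks the lock and player's key, then flip-flops between playing and reversing a timeline that lerps both doors' roll, or plays a locked sound.
; LookAt reports the lock state, while SetDoorStatus and OnGhostComplete change it.
; Open and close sounds use random pitch and a DoOnce-plus-delay throttle.
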(event Custom|SetDoorStatus
  (params (NewStatus :type Boolean))
  ;[0.15 0.15 0.15 0.5] Initialize Variables
  (Variables|Default|SetIsLocked NewStatus))

(event Custom|PlaySound
  (params (SoundToPlay :type Sound%20Base%20Object%20Reference))
  ;[1 1 1] Add Impact SFX
  (Utilities|FlowControl|DoOnce false :!label _label
    (:Completed
      (Audio|SpawnSoundatLocation SoundToPlay (Transformation|GetActorLocation) "0, 0, 0" 1.0 (Math|Random|RandomFloatinRange 0.85 1.2) 0.0 "/Game/Audio/Settings/Attenuations/ATT_Audio3D.ATT_Audio3D" 0)
      (Utilities|FlowControl|Delay 0.4)
      (goto _label Reset))))

(event EventOnGhostComplete
  ;[0.15 0.15 0.15 0.5] Initialize Variables
  (Variables|Default|SetIsLocked false))

(event EventInteract
  (params (LookingComponent :type Primitive%20Component%20Object%20Reference))
  ;[0 0.15 0.04013 0.5] Interact Event
  (Utilities|DoorSFX
    (:Opening
      (bind _alpha (Timeline|TL_OpenDoor Play)
        (:Update
          (CallFunction|SetDoorRotation _alpha))))
    (:Closing
      (Timeline|TL_OpenDoor Reverse))))

(event EventBeginPlay
  ;[0.15 0.15 0.15 0.5] Initialize Variables
  (Components|Timeline|SetPlayRate (Variables|Default|GetTL_OpenDoor) (/ 1.0 (Variables|Default|GetTimelineLength))))

(fn ConstructionScript)

(fn SetDoorRotation
  (params (Alpha :type Float%20%28single-precision%29))
  (bind _l_door (Variables|Default|GetL_Door))
  (bind _r_door (Variables|Default|GetR_Door))
  (bind _relativerotation (Variables|/Script/Engine.SceneComponent|GetRelativeRotation _r_door))
  (bind _relativerotation_2 (Variables|/Script/Engine.SceneComponent|GetRelativeRotation _l_door))
  (Transformation|SetRelativeRotation _l_door (Math|Rotator|MakeRotator (Math|Float|Lerp (Variables|Default|GetL_StartRot) (Variables|Default|GetL_EndRot) Alpha) (.pitch _relativerotation_2) (.yaw _relativerotation_2)) false false)
  (Transformation|SetRelativeRotation _r_door (Math|Rotator|MakeRotator (Math|Float|Lerp (Variables|Default|GetR_StartRot) (Variables|Default|GetR_EndRot) Alpha) (.pitch _relativerotation) (.yaw _relativerotation)) false false))

(fn Lookat
  (params (Player%20Ref :type Actor%20Object%20Reference) (Hit%20Component :type Primitive%20Component%20Object%20Reference))
  (if (Variables|Default|GetIsLocked)
    (bind _hasitem_ (Class|IPlayerUtils|PlayerHasTakenItem?(Message) Player%20Ref (Variables|Default|GetKeyRowName)))
    (return Player%20Ref Hit%20Component "" (not _hasitem_))
    (else
      (return Player%20Ref Hit%20Component "" false))))