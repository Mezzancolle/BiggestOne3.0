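; BP_WindTrigger is a sphere trigger, with a radius set in the construction script, that plays a dynamic sound and optional effect for the player.
; On overlap by a Player-tagged actor, if DynamicSFX is set, it plays the cue and spawns any optional VFX.
; The one-shot flag is set only on the VFX path, so sound-only triggers can repeat.
; Leaving stops the audio and deactivates the VFX.
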(event OnComponentBeginOverlap(Sphere)
  (params (OverlappedComponent :type Primitive%20Component%20Object%20Reference) (OtherActor :type Actor%20Object%20Reference) (OtherComp :type Primitive%20Component%20Object%20Reference) (OtherBodyIndex :type Integer) (bFromSweep :type Boolean) (SweepResult :type Hit%20Result%20Structure%20%28by%20ref%29))
  (bind _audio (Variables|Default|GetAudio))
  (bind _optionalvfxtemplate (Variables|Default|GetOptionalVFXTemplate))
  (if (Actor|ActorHasTag OtherActor "Player")
    (if (not (Variables|Default|GetbHasAlreadyActivated))
      (if (Variables|Default|GetbDynamicSFX)
        (Audio|Components|Audio|SetSound _audio (Variables|Default|GetDynamicSFXCue))
        (Audio|Components|Audio|Play _audio 0.0)
        (if (Utilities|IsValid _optionalvfxtemplate)
          (bind _returnvalue (Niagara|SpawnSystematLocation _optionalvfxtemplate (Transformation|GetActorLocation)))
          (Variables|Default|SetSpawnedVFX _returnvalue)
          (Transformation|AttachComponentToComponent (Variables|Default|GetDefaultSceneRoot) "None" "KeepRelative" "KeepRelative" "KeepRelative" true)
          (Variables|Default|SetbHasAlreadyActivated true))))))

(event OnComponentEndOverlap(Sphere)
  (params (OverlappedComponent :type Primitive%20Component%20Object%20Reference) (OtherActor :type Actor%20Object%20Reference) (OtherComp :type Primitive%20Component%20Object%20Reference) (OtherBodyIndex :type Integer))
  (if (Actor|ActorHasTag OtherActor "Player")
    (Audio|Components|Audio|Stop (Variables|Default|GetAudio))
    (if (Utilities|IsValid (Variables|Default|GetOptionalVFXTemplate))
      (Components|Activation|Deactivate (Variables|Default|GetSpawnedVFX)))))

(fn ConstructionScript
  (Components|Sphere|SetSphereRadius (Variables|Default|GetSphere) (Variables|Default|GetSphereRadius) true))