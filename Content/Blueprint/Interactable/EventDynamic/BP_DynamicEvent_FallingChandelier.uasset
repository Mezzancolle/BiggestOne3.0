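; Horror dynamic event where a church chandelier falls and a pair of doors slams shut near the player.
; While the player is inside the sphere, a looping timer picks one of three distance zones and spawns its ambient audio on each zone change.
; Entering the box fades that audio and runs a one-shot timeline sequence: chandelier drop, broken-mesh swap, camera shake and door shut with sounds.
; The finished sequence disables the event's triggers.
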(event OnComponentBeginOverlap(Sphere)
  (params (OverlappedComponent :type Primitive%20Component%20Object%20Reference) (OtherActor :type Actor%20Object%20Reference) (OtherComp :type Primitive%20Component%20Object%20Reference) (OtherBodyIndex :type Integer) (bFromSweep :type Boolean) (SweepResult :type Hit%20Result%20Structure%20%28by%20ref%29))
  (if (Actor|ActorHasTag OtherActor "Player")
    (if (and (Variables|Default|GetbHorrorEnabled) (Variables|Default|GetbDynamicEventActive%20))
      (Variables|Default|SetPlayerRef OtherActor)
      (Variables|Default|SetSphereRadius (Components|Sphere|GetScaledSphereRadius (Variables|Default|GetSphere)))
      (Variables|Default|SetCurrentZone 0)
      (bind _returnvalue (Utilities|Time|SetTimerbyFunctionName 0 "CheckPlayerDistance" 0.2 true))
      (Variables|Default|SetCheckPlayerDistanceTimerHandle _returnvalue))))

(event OnComponentBeginOverlap(Box)
  (params (OverlappedComponent :type Primitive%20Component%20Object%20Reference) (OtherActor :type Actor%20Object%20Reference) (OtherComp :type Primitive%20Component%20Object%20Reference) (OtherBodyIndex :type Integer) (bFromSweep :type Boolean) (SweepResult :type Hit%20Result%20Structure%20%28by%20ref%29))
  (if (Actor|ActorHasTag OtherActor "Player")
    (if (== (Variables|Default|GetbTriggered) false)
      (Variables|Default|SetbTriggered true)
      (CallFunction|StopAllAmbientAudios)
      (CallFunction|SequenceEffects)
      (CallFunction|FadeOutCurrentAudio))))

(event OnComponentEndOverlap(Box)
  (params (OverlappedComponent :type Primitive%20Component%20Object%20Reference) (OtherActor :type Actor%20Object%20Reference) (OtherComp :type Primitive%20Component%20Object%20Reference) (OtherBodyIndex :type Integer))
  (bind _activevfx_ (Variables|Default|GetActiveVFX%20))
  (Utilities|Time|ClearandInvalidateTimerbyHandle (Variables|Default|GetCheckPlayerDistanceTimerHandle))
  (if (Variables|Default|GetIsSequenceActive)
    (Game|Feedback|ClientStopCameraShake (Game|GetPlayerController 0) 0 true)
    (Variables|Default|SetIsSequenceActive false)
    (if (Variables|Default|GetisDebuggingEvent)
      (Variables|Default|SetbTriggered false))
    (Utilities|IsValid (Variables|Default|GetPrincipaleHorrorAudioReference)
      (:Is%20Valid
        (Audio|Components|Audio|FadeOut (Variables|Default|GetPrincipaleHorrorAudioReference) (Variables|Default|GetFadeOutDuration%20) 0.0 "Linear" :!class /Script/Engine.AudioComponent)))
    (else
      (Utilities|IsValid _activevfx_
        (:Is%20Valid
          (Components|Activation|Deactivate _activevfx_))))))

(event OnComponentEndOverlap(Sphere)
  (params (OverlappedComponent :type Primitive%20Component%20Object%20Reference) (OtherActor :type Actor%20Object%20Reference) (OtherComp :type Primitive%20Component%20Object%20Reference) (OtherBodyIndex :type Integer))
  (CallFunction|FadeOutCurrentAudio)
  (Utilities|Time|ClearandInvalidateTimerbyHandle (Variables|Default|GetCheckPlayerDistanceTimerHandle))
  (if (Variables|Default|GetisDebuggingEvent)
    (Variables|Default|SetbTriggered false)))

(event Custom|SoundEvent
  (params (Sound :type Sound%20Base%20Object%20Reference) (Location :type Vector) (VolumeMultiplier :type Float%20%28single-precision%29))
  (Audio|PlaySoundatLocation Sound Location "0, 0, 0" VolumeMultiplier 1.0 0.0 0 0 0 0))

(event Custom|DisableDynamicEvent
  (Utilities|Time|ClearandInvalidateTimerbyHandle (Variables|Default|GetCheckPlayerDistanceTimerHandle))
  (Variables|Default|SetbDynamicEventActive%20 false)
  (Collision|SetCollisionEnabled (Variables|Default|GetSphere) "NoCollision")
  (Collision|SetCollisionEnabled (Variables|Default|GetBox) "NoCollision"))

(event Custom|SequenceEffects
  (Variables|Default|SetIsSequenceActive true)
  (CallFunction|SoundEvent "/Game/Audio/SFX/SFX_Env/Sheriffs/SFX_Chains_4.SFX_Chains_4" (Transformation|GetWorldLocation (Variables|Default|GetSM_Church_Chandelier)) 1.0)
  (Utilities|FlowControl|Delay 0.5)
  (CallFunction|SoundEvent "/Game/Audio/SFX/SFX_Env/Church/SFX_Snap_Chandelier.SFX_Snap_Chandelier" (Transformation|GetWorldLocation (Variables|Default|GetSM_Church_Chandelier)) 1.0)
  (bind _newtrack_0 (Timeline|AnimazioneProva Play)
    (:Update
      (Transformation|SetRelativeLocation (Variables|Default|GetSM_Church_Chandelier) _newtrack_0 false false))
    (:Finished
      (Components|StaticMesh|SetStaticMesh (Variables|Default|GetSM_Church_Chandelier) "/Game/ExternalPackages/Chandelier/SM_Church_Chandelier_Broken.SM_Church_Chandelier_Broken")
      (Camera|PlayWorldCameraShake "/Game/Blueprint/LevelDesign/DynamicEvents/BP_CameraShake_Church.BP_CameraShake_Church_C" (Transformation|GetActorLocation (.AsBP%20Main%20Character (Utilities|Casting|CastToBP_MainCharacter (Game|GetPlayerCharacter 0)))) 0.0 5e+02 0.0 true)
      (CallFunction|SoundEvent "/Game/Audio/SFX/SFX_Env/Church/SFX_Crash_Chandelier.SFX_Crash_Chandelier" (Transformation|GetWorldLocation (Variables|Default|GetSM_Church_Chandelier)) 1.0)
      (Utilities|FlowControl|Delay 1.0)
      (bind _rotation (Timeline|DoorShut Play)
        (:Update
          (Transformation|SetRelativeRotation (Variables|Default|GetDoor_A) (Math|Rotator|MakeRotator 0.0 0.0 _rotation) false false)
          (Transformation|SetRelativeRotation (Variables|Default|GetDoor_B) (Math|Rotator|MakeRotator 0.0 0.0 _rotation) false false))
        (:Finished
          (CallFunction|SoundEvent "/Game/Audio/SFX/SFX_Env/Church/SFX_Door_Shut.SFX_Door_Shut" (Transformation|GetWorldLocation (Variables|Default|GetDoor_A)) 2.0)
          (CallFunction|SoundEvent "/Game/Audio/SFX/SFX_Env/Saloon/SFX_Env_Steps_1.SFX_Env_Steps_1" (Transformation|GetWorldLocation (Variables|Default|GetDefaultSceneRoot)) 2.0)
          (Variables|Default|SetIsSequenceActive false)
          (CallFunction|DisableDynamicEvent))))))

(event EventBeginPlay
  (Utilities|Array|Clear (Variables|Default|GetAudioComponents))
  (Collision|SetCollisionEnabled (Variables|Default|GetSphere) "QueryOnly")
  (Collision|SetCollisionEnabled (Variables|Default|GetBox) "QueryOnly"))

(fn ConstructionScript
  (Components|Sphere|SetSphereRadius (Variables|Default|GetSphere) (Variables|Default|GetSphereRadius) true)
  (Components|Box|SetBoxExtent (Variables|Default|GetBox) (Variables|Default|GetBoxDimension) true))

(fn CheckPlayerDistance
  (if (<= (Math|Vector|VectorLength (- (Transformation|GetActorLocation (Variables|Default|GetPlayerRef)) (Transformation|GetActorLocation))) (* (Variables|Default|GetSphereRadius) 0.33))
    (Variables|Default|SetDesiredZone 1)
    (elif (<= (Math|Vector|VectorLength (- (Transformation|GetActorLocation (Variables|Default|GetPlayerRef)) (Transformation|GetActorLocation))) (* (Variables|Default|GetSphereRadius) 0.66))
      (Variables|Default|SetDesiredZone 2)
      (else
        (Variables|Default|SetDesiredZone 3))))
  (if (!= (Variables|Default|GetCurrentZone) (Variables|Default|GetDesiredZone))
    (CallFunction|SetNewAudioZone (Utilities|Select :Index (- (Variables|Default|GetDesiredZone) 1) :Option%200 (Variables|Default|GetAudioMedia1) :Option%201 (Variables|Default|GetAudioMedia2) :Option%202 (Variables|Default|GetAudioMedia3)) (- (Variables|Default|GetDesiredZone) 1) (Math|Float|Lerp (Variables|Default|GetVolumeEnded) (Variables|Default|GetVolumeStart) (Math|Float|Clamp(Float) (/ (Math|Vector|VectorLength (- (Transformation|GetActorLocation (Variables|Default|GetPlayerRef)) (Transformation|GetActorLocation))) (Variables|Default|GetSphereRadius)))))))

(fn FadeOutCurrentAudio
  (bind _audiocomponents (Variables|Default|GetAudioComponents))
  (bind _currentzone (Variables|Default|GetCurrentZone))
  (bind _returnvalue (- _currentzone 1))
  (bind _output (Utilities|Array|Get(acopy) _audiocomponents _returnvalue))
  (if (and (>= (Variables|Default|GetCurrentZone) 0) (<= (Variables|Default|GetCurrentZone) (Utilities|Array|Length (Variables|Default|GetAudioComponents))))
    (if (Utilities|IsValid _output)
      (Audio|Components|Audio|FadeOut _output (Variables|Default|GetFadeOutDuration%20) 0.0 "Linear" :!class /Script/Engine.AudioComponent))))

(fn SetNewAudioZone
  (params (Sound :type Sound%20Base%20Object%20Reference) (Index :type Integer) (SetVolume :type Float%20%28double-precision%29))
  (bind _audiocomponents (Variables|Default|GetAudioComponents))
  (Utilities|FlowControl|Sequence
    (:then_0
      (if (Variables|Default|GetbIs2DSound)
        (bind _returnvalue (Audio|SpawnSound2D Sound 1.0 1.0 0.0 0))
        (Utilities|Array|SetArrayElem _audiocomponents Index _returnvalue true)
        (else
          (bind _returnvalue_2 (Audio|SpawnSoundAttached Sound (Variables|Default|GetDefaultSceneRoot) "None" "0, 0, 0" "0, 0, 0" "KeepRelativeOffset" false 1.0 1.0 0.0 0 0))
          (Audio|Components|Audio|SetVolumeMultiplier _returnvalue_2 SetVolume :!class /Script/Engine.AudioComponent)
          (Utilities|Array|SetArrayElem _audiocomponents Index _returnvalue_2 true))))
    (:then_1
      (Variables|Default|SetCurrentZone (Variables|Default|GetDesiredZone)))))

(fn StopAllAmbientAudios
  (for _array_element (Variables|Default|GetAudioComponents)
    (Utilities|IsValid _array_element
      (:Is%20Valid
        (Audio|Components|Audio|FadeOut _array_element 0.3 0.0 "Linear" :!class /Script/Engine.AudioComponent)))))