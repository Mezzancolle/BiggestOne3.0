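; Interactable horror event that layers proximity-based audio around a one-shot scare sound, played either 2D or attached.
; When the player enters the sphere with horror enabled and the event active, a looping timer polls distance and swaps between three radius-based audio zones, fading out the previous one.
; Entering the box plays the principal sound once and, if horror is enabled, fades zone audio and disables the event.
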(event OnComponentBeginOverlap(Sphere)
  (params (OverlappedComponent :type Primitive%20Component%20Object%20Reference) (OtherActor :type Actor%20Object%20Reference) (OtherComp :type Primitive%20Component%20Object%20Reference) (OtherBodyIndex :type Integer) (bFromSweep :type Boolean) (SweepResult :type Hit%20Result%20Structure%20%28by%20ref%29))
  (if (Actor|ActorHasTag OtherActor "Player")
    (if (and (Variables|Default|GetbHorrorEnabled) (Variables|Default|GetbDynamicEventActive%20))
      (Variables|Default|SetPlayerRef OtherActor)
      (Variables|Default|SetSphereRadius (Components|Sphere|GetScaledSphereRadius (Variables|Default|GetSphere)))
      (Variables|Default|SetCurrentZone 0)
      (bind _returnvalue (Utilities|Time|SetTimerbyFunctionName 0 "CheckPlayerDistance" 0.2 true))
      (Variables|Default|SetCheckPlayerDistanceTimerHandle _returnvalue))))

(event OnComponentBeginOverlap(Box)
  (params (OverlappedComponent :type Primitive%20Component%20Object%20Reference) (OtherActor :type Actor%20Object%20Reference) (OtherComp :type Primitive%20Component%20Object%20Reference) (OtherBodyIndex :type Integer) (bFromSweep :type Boolean) (SweepResult :type Hit%20Result%20Structure%20%28by%20ref%29))
  (if (Actor|ActorHasTag OtherActor "Player")
    (if (== (Variables|Default|GetbTriggered) false)
      (Variables|Default|SetbTriggered true)
      (CallFunction|PrincipleHorrorSound)
      (if (Variables|Default|GetbHorrorEnabled)
        (CallFunction|FadeOutCurrentAudio)
        (CallFunction|DisableDynamicEvent)))))

(event OnComponentEndOverlap(Box)
  (params (OverlappedComponent :type Primitive%20Component%20Object%20Reference) (OtherActor :type Actor%20Object%20Reference) (OtherComp :type Primitive%20Component%20Object%20Reference) (OtherBodyIndex :type Integer))
  (Utilities|Time|ClearandInvalidateTimerbyHandle (Variables|Default|GetCheckPlayerDistanceTimerHandle))
  (Utilities|IsValid (Variables|Default|GetPrincipaleHorrorAudioReference)
    (:Is%20Valid
      (Audio|Components|Audio|FadeOut (Variables|Default|GetPrincipaleHorrorAudioReference) (Variables|Default|GetFadeOutDuration%20) 0.0 "Linear" :!class /Script/Engine.AudioComponent))))

(event OnComponentEndOverlap(Sphere)
  (params (OverlappedComponent :type Primitive%20Component%20Object%20Reference) (OtherActor :type Actor%20Object%20Reference) (OtherComp :type Primitive%20Component%20Object%20Reference) (OtherBodyIndex :type Integer))
  (CallFunction|FadeOutCurrentAudio)
  (Utilities|Time|ClearandInvalidateTimerbyHandle (Variables|Default|GetCheckPlayerDistanceTimerHandle)))

(event Custom|PrincipleHorrorSound
  (if (Variables|Default|GetbIs2DSound)
    (Audio|PlaySound2D (Variables|Default|GetPrincipaleHorrorThemeSound) 1.0 1.0 0.0 0 0)
    (else
      (bind _returnvalue (Audio|SpawnSoundAttached (Variables|Default|GetPrincipaleHorrorThemeSound) (Variables|Default|GetDefaultSceneRoot) "None" "0, 0, 0" "0, 0, 0" "KeepRelativeOffset" false 1.0 1.0 0.0 "/Game/Audio/Settings/Attenuations/ATT_Audio3D.ATT_Audio3D" 0))
      (Audio|Components|Audio|SetVolumeMultiplier _returnvalue (Variables|Default|GetPrincipalAudioThemeVolume) :!class /Script/Engine.AudioComponent)
      (Variables|Default|SetPrincipaleHorrorAudioReference _returnvalue))))

(event Custom|DisableDynamicEvent
  (Utilities|Time|ClearandInvalidateTimerbyHandle (Variables|Default|GetCheckPlayerDistanceTimerHandle))
  (Variables|Default|SetbDynamicEventActive%20 false)
  (Collision|SetCollisionEnabled (Variables|Default|GetSphere) "NoCollision")
  (Collision|SetCollisionEnabled (Variables|Default|GetBox) "NoCollision"))

(event EventBeginPlay
  (Utilities|Array|Clear (Variables|Default|GetAudioComponents))
  (Collision|SetCollisionEnabled (Variables|Default|GetSphere) "QueryOnly")
  (Collision|SetCollisionEnabled (Variables|Default|GetBox) "QueryOnly"))

(fn ConstructionScript
  (Components|Sphere|SetSphereRadius (Variables|Default|GetSphere) (Variables|Default|GetSphereRadius) true)
  (Components|Box|SetBoxExtent (Variables|Default|GetBox) (Variables|Default|GetBoxDimension) true))

(fn CheckPlayerDistance
  (if (<= (Math|Vector|VectorLength (- (Transformation|GetActorLocation (Variables|Default|GetPlayerRef)) (Transformation|GetActorLocation))) (* (Variables|Default|GetSphereRadius) 0.33))
    (Variables|Default|SetDesiredZone 1)
    (elif (<= (Math|Vector|VectorLength (- (Transformation|GetActorLocation (Variables|Default|GetPlayerRef)) (Transformation|GetActorLocation))) (* (Variables|Default|GetSphereRadius) 0.66))
      (Variables|Default|SetDesiredZone 2)
      (else
        (Variables|Default|SetDesiredZone 3))))
  (if (!= (Variables|Default|GetCurrentZone) (Variables|Default|GetDesiredZone))
    (CallFunction|SetNewAudioZone (Utilities|Select :Index (- (Variables|Default|GetDesiredZone) 1) :Option%200 (Variables|Default|GetAudioMedia1) :Option%201 (Variables|Default|GetAudioMedia2) :Option%202 (Variables|Default|GetAudioMedia3)) (- (Variables|Default|GetDesiredZone) 1) (Utilities|Select :Index (- (Variables|Default|GetDesiredZone) 1) :Option%200 (Variables|Default|GetThemeVolumeAudio1) :Option%201 (Variables|Default|GetThemeVolumeAudio2) :Option%202 (Variables|Default|GetThemeVolumeAudio3)))))

(fn FadeOutCurrentAudio
  (bind _audiocomponents (Variables|Default|GetAudioComponents))
  (bind _currentzone (Variables|Default|GetCurrentZone))
  (bind _returnvalue (- _currentzone 1))
  (bind _output (Utilities|Array|Get(acopy) _audiocomponents _returnvalue))
  (if (and (>= (Variables|Default|GetCurrentZone) 0) (<= (Variables|Default|GetCurrentZone) (Utilities|Array|Length (Variables|Default|GetAudioComponents))))
    (if (Utilities|IsValid _output)
      (Audio|Components|Audio|FadeOut _output (Variables|Default|GetFadeOutDuration%20) 0.0 "Linear" :!class /Script/Engine.AudioComponent))))

(fn SetNewAudioZone
  (params (Sound :type Sound%20Base%20Object%20Reference) (Index :type Integer) (SetVolume :type Float%20%28double-precision%29))
  (bind _audiocomponents (Variables|Default|GetAudioComponents))
  (Utilities|FlowControl|Sequence
    (:then_0
      (CallFunction|FadeOutCurrentAudio)
      (if (Variables|Default|GetbIs2DSound)
        (bind _returnvalue (Audio|SpawnSound2D Sound 1.0 1.0 0.0 0))
        (Utilities|Array|SetArrayElem _audiocomponents Index _returnvalue true)
        (else
          (bind _returnvalue_2 (Audio|SpawnSoundAttached Sound (Variables|Default|GetDefaultSceneRoot) "None" "0, 0, 0" "0, 0, 0" "KeepRelativeOffset" false 1.0 1.0 0.0 0 0))
          (Audio|Components|Audio|SetVolumeMultiplier _returnvalue_2 SetVolume :!class /Script/Engine.AudioComponent)
          (Utilities|Array|SetArrayElem _audiocomponents Index _returnvalue_2 true))))
    (:then_1
      (Variables|Default|SetCurrentZone (Variables|Default|GetDesiredZone)))))