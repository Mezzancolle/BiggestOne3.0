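; Base Blueprint for an interactable drawer that slides open and closed and can hold a configurable child actor.
; Construction caches the start location, derives the open position by adding OpenOffset along world Y, and assigns ChildClass to the InsideObject child actor component.
; Interact uses a FlipFlop to alternately play and reverse a Timeline, whose Alpha lerps the whole actor between the two positions.
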(event EventInteract
  (params (PlayerRef :type BP%20Main%20Character%20Object%20Reference) (LookingComponent :type Primitive%20Component%20Object%20Reference))
  (Utilities|FlowControl|FlipFlop
    (:A
      (bind _alpha (Timeline|Timeline Play)
        (:Update
          (Transformation|SetActorLocation (Math|Vector|Lerp(Vector) (Variables|Default|GetStartPos) (Variables|Default|GetEndPos) _alpha) false false))))
    (:B
      (Timeline|Timeline Reverse))))

(fn ConstructionScript
  (|CallParentFunction)
  (CallFunction|SetVariables))

(fn SetVariables
  (bind _output_get (Variables|Default|SetStartPos (Transformation|GetActorLocation)))
  (Variables|Default|SetEndPos (+ _output_get (Math|Vector|MakeVector 0.0 (Variables|Default|GetOpenOffset) 0.0)))
  (ChildActorComponent|SetChildActorClass (Variables|Default|GetInsideObject) (Variables|Default|GetChildClass)))