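; Base inspectable item, configured from DT_Items by row name, that destroys itself if already taken.
; Pickup hands input to the item and lerps it on Tick before the player camera.
; While inspected it supports rotation, description toggling and cursor traces against tagged message/action boxes, with empty hooks for custom behavior.
; Dropping lerps it back, animates it into the player's pocket as inventory, or destroys it if already an inventory item.
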(event Custom|ManagePickUp
  ;[1 1 1] PICKUP INTERFACE
  (Development|SetHiddeninGame (Variables|Default|GetGhostOverlayMesh) true false)
  (Variables|Default|SetHasPickupLerpEnded? false)
  (Audio|PlaySound2D (Variables|Customization|GetInteractSound) 1.0 1.0 0.0 0 0)
  (CallFunction|EnableInputto self)
  (if (Variables|Default|GetIsAnInventoryItem?)
    _
    (else
      (bind _itemactorcomponent (Class|IPlayerUtils|GetHoldingItem(Message) (Game|Player|GetPlayerPawn 0)))
      (Transformation|AttachComponentToComponent _itemactorcomponent "None" "KeepWorld" "KeepWorld" "KeepWorld" false)))
  (CallFunction|SetInspectionVariables)
  (bind _output_get (Variables|Animation|SetIsInspecting? true))
  (CallFunction|SetCollisions _output_get)
  (CallFunction|PlayLerpingAnimation (Variables|Camera|GetInspectPosition) (Variables|Camera|GetInspectRotation))
  (EventDispatchers|BindEventtoOnFinishedInspectionLerping (delegate Custom|CanViewDescriptionEvent)))

(event Custom|SetItemToDefaultState
  ;[1 1 1] DROP ITEM TO THE GROUND
  (Actor|Tick|SetActorTickEnabled false)
  (CallFunction|SetCollisions (Variables|Animation|GetIsInspecting?))
  (Class|IPlayerUtils|CallonEndInteract(Message) (Game|Player|GetPlayerPawn 0) false (Variables|Customization|GetItemsRowName))
  (EventDispatchers|UnbindEventfromOnFinishedInspectionLerping (delegate Custom|SetItemToDefaultState)))

(event Custom|CanViewDescriptionEvent
  (bind _returnvalue (Game|GetPlayerController 0))
  ;[1 1 1] PICKUP INTERFACE
  (EventDispatchers|UnbindEventfromOnFinishedInspectionLerping (delegate Custom|CanViewDescriptionEvent))
  (Variables|Animation|SetCanViewDescription? true)
  (Input|SetInputModeGameandUI _returnvalue 0 "DoNotLock" true false)
  (Variables|/Script/Engine.PlayerController|SetbShowMouseCursor _returnvalue true)
  (Variables|Default|SetHasPickupLerpEnded? true))

(event Custom|DropByEvent
  (bind _returnvalue (Game|Player|GetPlayerPawn 0))
  (bind _returnvalue_2 (Game|GetPlayerController 0))
  ;[1 1 1] DROP ITEM TO THE GROUND
  (if (and (Variables|Other|GetCanBeDropped?) (Variables|Default|GetHasPickupLerpEnded?))
    (Actor|Tick|SetActorTickEnabled false)
    (Variables|Animation|SetCanViewDescription? false)
    (bind _msgwidget (Variables|Other|GetMsgWidget)
      (:then
        (Widget|RemovefromParent _msgwidget)
        (Variables|Other|SetMsgWidget 0))
      (:else
        _))
    (if (Variables|Other|GetIsVisibleDescription?)
      (CallFunction|ViewItemDescription))
    (CallFunction|EnableInputto _returnvalue)
    (if (Variables|Default|GetIsAnInventoryItem?)
      (Class|IPlayerUtils|Open/CloseInspectTextUI(Message) (Game|Player|GetPlayerPawn 0) false)
      (CallFunction|EnableInteractUI)
      (CallFunction|OnDropInventoryItem)
      (Actor|DestroyActor)
      (else
        (Class|IPlayerUtils|SwitchInputContext(Message) _returnvalue "/Game/Inputs/IMC_FirstPersonPlayer.IMC_FirstPersonPlayer" false)
        (Transformation|DetachFromActor "KeepWorld" "KeepWorld" "KeepWorld")
        (Variables|Animation|SetIsInspecting? false)
        (Variables|/Script/Engine.PlayerController|SetbShowMouseCursor _returnvalue_2 false)
        (Input|SetInputModeGameOnly _returnvalue_2 true)
        (if (.CanBeAddedToInventory? (Utilities|Struct|BreakS_DataItem (Variables|Other|GetMyItemData)))
          ;;[0.5011 1 0.06198] Add Item To Inventory
          (Audio|PlaySound2D (Variables|Customization|GetPickupSound) 1.0 1.0 0.0 0 0)
          (CallFunction|AddItemtoInventory)
          (bind _alpha (Timeline|TL_AddToInventoryAnimation PlayFromStart)
            (:Update
              (CallFunction|FromCameratoInsidePlayer _alpha))
            (:Finished
              (Utilities|IsValid self
                (:Is%20Valid
                  (Actor|DestroyActor)))))
          (else
            (CallFunction|PlayLerpingAnimation (Variables|Transformation|GetStartPos) (Variables|Transformation|GetStartRot))
            (EventDispatchers|BindEventtoOnFinishedInspectionLerping (delegate Custom|SetItemToDefaultState))))))
    (else
      (Class|SNSNarrativeBlueprintFuncLib|EnqueueDialogue "/Game/Other/DataTables/Dialogues/DT_Items_Dialogues.DT_Items_Dialogues" "InspectionNotFinished" false))))

(event Custom|ForceGoToPocketItem
  ;[1 1 1] DROP ITEM TO THE GROUND
  ;;[0.5011 1 0.06198] Add Item To Inventory
  (bind _alpha (Timeline|TL_AddToInventoryAnimation PlayFromStart)
    (:Update
      (CallFunction|FromCameratoInsidePlayer _alpha))
    (:Finished
      (Utilities|IsValid self
        (:Is%20Valid
          (Actor|DestroyActor))))))

(event Custom|PutInPocket
  (params (Target :type Scene%20Component%20Object%20Reference))
  (bind _output_get (Variables|Default|SetPutInPocketLocation (Transformation|GetWorldLocation Target)))
  (bind _alpha (Timeline|TL_PutInPocket PlayFromStart)
    (:Update
      (bind _pocketlocation (Class|IPlayerUtils|GetPocket(Message) (Game|Player|GetPlayerPawn 0)))
      (Transformation|SetWorldLocation Target (Math|Vector|Lerp(Vector) _output_get _pocketlocation _alpha) false false)
      (CallFunction|TickPutinPocket _alpha))
    (:Finished
      (Rendering|SetVisibility Target false true)
      (CallFunction|EndPutinPocket))))

(event Custom|Enable%20Interact%20UI
  ;[1 1 1] DROP ITEM TO THE GROUND
  (Collision|SetCollisionProfileName (Variables|Default|GetInventoryWidgetComponent) "UI" true :!class /Script/Engine.PrimitiveComponent))

(event Input|EnhancedActionEvents|EnhancedInputActionIA_Drop
  (params (ActionValue :type Boolean) (ElapsedSeconds :type Float%20%28double-precision%29) (TriggeredSeconds :type Float%20%28double-precision%29) (InputAction :type Input%20Action%20Object%20Reference :default "/Game/Inputs/Actions/IA_Drop.IA_Drop"))
  (bind _returnvalue (Game|Player|GetPlayerPawn 0))
  (bind _returnvalue_2 (Game|GetPlayerController 0))
  ;[1 1 1] DROP ITEM TO THE GROUND
  (if (and (Variables|Other|GetCanBeDropped?) (Variables|Default|GetHasPickupLerpEnded?))
    (Actor|Tick|SetActorTickEnabled false)
    (Variables|Animation|SetCanViewDescription? false)
    (bind _msgwidget (Variables|Other|GetMsgWidget)
      (:then
        (Widget|RemovefromParent _msgwidget)
        (Variables|Other|SetMsgWidget 0))
      (:else
        _))
    (if (Variables|Other|GetIsVisibleDescription?)
      (CallFunction|ViewItemDescription))
    (CallFunction|EnableInputto _returnvalue)
    (if (Variables|Default|GetIsAnInventoryItem?)
      (Class|IPlayerUtils|Open/CloseInspectTextUI(Message) (Game|Player|GetPlayerPawn 0) false)
      (CallFunction|EnableInteractUI)
      (CallFunction|OnDropInventoryItem)
      (Actor|DestroyActor)
      (else
        (Class|IPlayerUtils|SwitchInputContext(Message) _returnvalue "/Game/Inputs/IMC_FirstPersonPlayer.IMC_FirstPersonPlayer" false)
        (Transformation|DetachFromActor "KeepWorld" "KeepWorld" "KeepWorld")
        (Variables|Animation|SetIsInspecting? false)
        (Variables|/Script/Engine.PlayerController|SetbShowMouseCursor _returnvalue_2 false)
        (Input|SetInputModeGameOnly _returnvalue_2 true)
        (if (.CanBeAddedToInventory? (Utilities|Struct|BreakS_DataItem (Variables|Other|GetMyItemData)))
          ;;[0.5011 1 0.06198] Add Item To Inventory
          (Audio|PlaySound2D (Variables|Customization|GetPickupSound) 1.0 1.0 0.0 0 0)
          (CallFunction|AddItemtoInventory)
          (bind _alpha (Timeline|TL_AddToInventoryAnimation PlayFromStart)
            (:Update
              (CallFunction|FromCameratoInsidePlayer _alpha))
            (:Finished
              (Utilities|IsValid self
                (:Is%20Valid
                  (Actor|DestroyActor)))))
          (else
            (CallFunction|PlayLerpingAnimation (Variables|Transformation|GetStartPos) (Variables|Transformation|GetStartRot))
            (EventDispatchers|BindEventtoOnFinishedInspectionLerping (delegate Custom|SetItemToDefaultState))))))
    (else
      (Class|SNSNarrativeBlueprintFuncLib|EnqueueDialogue "/Game/Other/DataTables/Dialogues/DT_Items_Dialogues.DT_Items_Dialogues" "InspectionNotFinished" false))))

(event EventTick
  (params (DeltaSeconds :type Float%20%28single-precision%29))
  ;[1 1 1] Tick
  (if (Variables|Animation|GetIsPlayingAnimation?)
    (CallFunction|LoopLerpingAnimation DeltaSeconds)
    (else
      (CallFunction|SetCursorInspection))))

(event EventSetCanbeDropped
  (params (NewDroppability :type Boolean))
  (Variables|Other|SetCanBeDropped? NewDroppability))

(event EventBeginPlay
  ;[1 1 1] BEGIN PLAY
  (CallFunction|CheckifAlreadyTaken (Variables|Customization|GetItemsRowName))
  (CallFunction|SetVariablesfromDataTable)
  (if (Variables|Default|GetIsAnInventoryItem?)
    (Development|PrintString (Utilities|GetDisplayName self))))

(event Input|EnhancedActionEvents|EnhancedInputActionIA_Look
  (params (ActionValue :type Vector%202D%20Structure) (ElapsedSeconds :type Float%20%28double-precision%29) (TriggeredSeconds :type Float%20%28double-precision%29) (InputAction :type Input%20Action%20Object%20Reference :default "/Game/Inputs/Actions/IA_Look.IA_Look"))
  ;[1 1 1] Mouse Inspect
  (if (Variables|Other|GetCanRotateItem?)
    (if (Math|Boolean|ANDBoolean (Variables|Animation|GetIsInspecting?) (Variables|Input|GetIsMouseLeftClicked?) (not (Variables|Other|GetIsVisibleDescription?)) (not (Variables|Other|GetIsMouseCollidingWithBoxes?)))
      (CallFunction|MouseRotateMesh ActionValue))
    (else
      (CallFunction|OnNotRotating ActionValue))))

(event Input|EnhancedActionEvents|EnhancedInputActionIA_ViewObject
  (params (ActionValue :type Vector%202D%20Structure) (ElapsedSeconds :type Float%20%28double-precision%29) (TriggeredSeconds :type Float%20%28double-precision%29) (InputAction :type Input%20Action%20Object%20Reference :default "/Game/Inputs/Actions/IA_ViewObject.IA_ViewObject"))
  (bind _returnvalue (Game|GetPlayerController 0))
  (bind (_locationx _locationy) (Game|Player|GetMousePosition _returnvalue))
  (Class|PlayerController|SetMouseLocation (Game|GetPlayerController 0) (Math|Float|Round (+ (* (.x ActionValue) 5.0) _locationx)) (Math|Float|Round (+ (* (.y ActionValue) -5.0) _locationy))))

(event Input|EnhancedActionEvents|EnhancedInputActionIA_Interact
  (params (ActionValue :type Boolean) (ElapsedSeconds :type Float%20%28double-precision%29) (TriggeredSeconds :type Float%20%28double-precision%29) (InputAction :type Input%20Action%20Object%20Reference :default "/Game/Inputs/Actions/IA_Interact.IA_Interact"))
  (bind _returnvalue (Game|GetPlayerController 0))
  (bind _returnvalue_2 (Game|GetPlayerController 0))
  (bind _returnvalue_3 (Viewport|GetViewportSize))
  (bind _preinspectmouseposition (Variables|Other|GetPreInspectMousePosition))
  (bind _returnvalue_4 (* _returnvalue_3 "(X=0.500000,Y=0.500000)"))
  ;[1 0.2083 0.2182] ON INTERACT
  (:Triggered
    (if (not (Variables|/Script/Engine.PlayerController|GetbShowMouseCursor _returnvalue_2))
      (Class|PlayerController|SetMouseLocation _returnvalue_2 (Math|Float|Truncate (.x _returnvalue_4)) (Math|Float|Truncate (.y _returnvalue_4)))))
  (:Started
    (Variables|Input|SetIsMouseLeftClicked? true)
    (CallFunction|CheckifMouseonInteractionTrigger))
  (:Canceled
    (Variables|Input|SetIsMouseLeftClicked? false :!label _label)
    (if (Variables|Other|GetIsMouseCollidingWithBoxes?)
      (Variables|Other|SetIsMouseCollidingWithBoxes? false)
      (Class|PlayerController|SetMouseLocation _returnvalue (Math|Float|Truncate (.x _preinspectmouseposition)) (Math|Float|Truncate (.y _preinspectmouseposition)))
      (Variables|/Script/Engine.PlayerController|SetbShowMouseCursor _returnvalue true)))
  (:Completed
    (goto _label)))

(event Input|EnhancedActionEvents|EnhancedInputActionIA_ReadItem
  (params (ActionValue :type Boolean) (ElapsedSeconds :type Float%20%28double-precision%29) (TriggeredSeconds :type Float%20%28double-precision%29) (InputAction :type Input%20Action%20Object%20Reference :default "/Game/Inputs/Actions/IA_ReadItem.IA_ReadItem"))
  ;[1 1 1] Read Item Decription
  (:Started
    (if (Variables|Animation|GetCanViewDescription?)
      (CallFunction|ViewItemDescription)
      (Class|WidgetBlueprintLibrary|SetHardwareCursor "Default" "T_WestCursor" "(X=0.000000,Y=0.000000)"))))

(event Input|EnhancedActionEvents|EnhancedInputActionIA_GamePadInspect
  (params (ActionValue :type Vector%202D%20Structure) (ElapsedSeconds :type Float%20%28double-precision%29) (TriggeredSeconds :type Float%20%28double-precision%29) (InputAction :type Input%20Action%20Object%20Reference :default "/Game/Inputs/Actions/IA_GamePadInspect.IA_GamePadInspect"))
  (bind (_x _y) (Math|Vector2D|BreakVector2D ActionValue))
  (bind _joypadrotationdeadzone (Variables|Default|GetJoypadRotationDeadzone))
  (if (and (Variables|Other|GetCanRotateItem?) (or (> (Math|Float|Absolute(Float) _x) _joypadrotationdeadzone) (> (Math|Float|Absolute(Float) _y) _joypadrotationdeadzone)))
    (if (Math|Boolean|ANDBoolean (Variables|Animation|GetIsInspecting?) (not (Variables|Other|GetIsVisibleDescription?)) (not (Variables|Other|GetIsMouseCollidingWithBoxes?)))
      (CallFunction|MouseRotateMesh ActionValue))))

(fn ConstructionScript
  (Utilities|FlowControl|Sequence
    (:then_0
      (if (Variables|Customization|GetOverrideDataTableMesh?)
        _
        (else
          (bind _returnvalue (Utilities|GetDataTableRow "/Game/Other/DataTables/DT_Items.DT_Items" (Variables|Customization|GetItemsRowName))
            (:then
              (bind _output_get (Variables|Other|SetMyItemData _returnvalue))
              (bind _returnvalue_2 (Utilities|LoadAssetBlocking (.StaticMesh (Utilities|Struct|BreakS_DataItem _output_get))))
              (Components|StaticMesh|SetStaticMesh (Variables|Default|GetStaticMesh) (.AsStatic%20Mesh (Utilities|Casting|CastToStaticMesh _returnvalue_2)))))))
      (if (Variables|Customization|GetHasMSGBox?)
        _
        (else
          (Components|DestroyComponent (Variables|Default|GetMessageInteractionBox))))
      (if (not (Variables|Customization|GetHasActionBox?))
        (Components|DestroyComponent (Variables|Default|GetActionInteractionBox))))
    (:then_1
      (Components|StaticMesh|SetStaticMesh (Variables|Default|GetGhostOverlayMesh) (Variables|/Script/Engine.StaticMeshComponent|GetStaticMesh (Variables|Default|GetStaticMesh))))))

(fn CheckifAlreadyTaken
  (params (ItemToHave :type Name%20%28by%20ref%29))
  (bind _saveddata (Class|ISaveGame|GetGameData(Message) (Game|GetGameInstance)))
  (if (Utilities|Array|ContainsItem (.itemstaken (Variables|/Game/Blueprint/SaveGame/BP_GameData.BP_GameData_C|GetInventoryDiaryData _saveddata)) ItemToHave)
    (Utilities|IsValid self
      (:Is%20Valid
        (Actor|DestroyActor)))))

(fn EnableInputto
  (params (Actor :type Actor%20Object%20Reference))
  (bind _returnvalue (Game|GetPlayerController 0))
  (Input|DisableInput _returnvalue)
  (Input|DisableInput (Game|Player|GetPlayerPawn 0) _returnvalue)
  (Input|EnableInput Actor _returnvalue))

(fn SetInspectionVariables
  (bind _inspectionrotationoffset (Variables|Customization|GetInspectionRotationOffset))
  (bind _playercamera (Variables|Default|GetPlayerCamera))
  (bind (_roll _pitch _yaw) (Math|Rotator|BreakRotator _inspectionrotationoffset))
  (bind _returnvalue (Math|Vector|GetForwardVector _playercamera))
  (bind _returnvalue_2 (* _returnvalue -1))
  (bind _returnvalue_3 (Math|Conversions|RotationFromXVector _returnvalue_2))
  (bind (_roll_2 _pitch_2 _yaw_2) (Math|Rotator|BreakRotator _returnvalue_3))
  (Variables|Camera|SetInspectPosition (+ (Transformation|GetWorldLocation _playercamera) (* (Math|Vector|GetForwardVector _playercamera) (Variables|Customization|GetInspectionDistance))))
  (Variables|Camera|SetInspectRotation (Math|Rotator|MakeRotator (+ _roll_2 _roll) (+ _pitch_2 _pitch) (+ _yaw_2 _yaw))))

(fn PlayLerpingAnimation
  (params (NextPosition :type Vector) (NextRotation :type Rotator))
  (Actor|Tick|SetActorTickEnabled true)
  (Variables|Camera|SetEndAnimationPos NextPosition)
  (Variables|Camera|SetStartAnimationPos (Transformation|GetWorldLocation (Variables|Default|GetPivot)))
  (Variables|Camera|SetEndAnimationRot NextRotation)
  (Variables|Camera|SetStartAnimationRot (Transformation|GetWorldRotation (Variables|Default|GetPivot)))
  (Variables|Animation|SetIsPlayingAnimation? true)
  (Variables|Animation|SetCounterInspectLerp 0.0))

(fn LoopLerpingAnimation
  (params (DeltaTime :type Float%20%28double-precision%29))
  (Variables|Animation|SetCounterInspectLerp (+ DeltaTime (Variables|Animation|GetCounterInspectLerp)))
  (Transformation|SetWorldLocationAndRotation (Variables|Default|GetPivot) (Math|Vector|Lerp(Vector) (Variables|Camera|GetStartAnimationPos) (Variables|Camera|GetEndAnimationPos) (/ (Variables|Animation|GetCounterInspectLerp) (Variables|Animation|GetTimerInspectLerp))) (Math|Rotator|Lerp(Rotator) (Variables|Camera|GetStartAnimationRot) (Variables|Camera|GetEndAnimationRot) (/ (Variables|Animation|GetCounterInspectLerp) (Variables|Animation|GetTimerInspectLerp)) true) false false)
  ;[1 1 1] OnFinishLerping
  (if (> (Variables|Animation|GetCounterInspectLerp) (Variables|Animation|GetTimerInspectLerp))
    (Variables|Animation|SetCounterInspectLerp 0.0)
    (Variables|Animation|SetIsPlayingAnimation? false)
    (Default|CallOnFinishedInspectionLerping)))

(fn FromCameratoInsidePlayer
  (params (Alpha :type Float%20%28single-precision%29))
  (bind _pocketlocation (Class|IPlayerUtils|GetPocket(Message) (Game|Player|GetPlayerPawn 0)))
  (Transformation|SetActorLocation (Math|Vector|Lerp(Vector) (Variables|Camera|GetInspectPosition) _pocketlocation Alpha) false false))

(fn AddItemtoInventory
  (Class|IPlayerUtils|CallonEndInteract(Message) (Game|Player|GetPlayerPawn 0) true (Variables|Customization|GetItemsRowName)))

(fn ViewItemDescription
  (bind _myitemdata (Variables|Other|GetMyItemData))
  (bind (_name _description) (Utilities|Struct|BreakS_DataItem _myitemdata))
  (Class|IPlayerUtils|SetInspectText(Message) (Game|Player|GetPlayerPawn 0) _name _description)
  (Variables|Other|SetIsVisibleDescription? (not (Variables|Other|GetIsVisibleDescription?))))

(fn MouseRotateMesh
  (params (ActionValue :type Vector%202D%20Structure))
  (bind _returnvalue (* (.y ActionValue) 2.0))
  (bind _playercamera (Variables|Default|GetPlayerCamera))
  (bind _returnvalue_2 (Math|Vector|GetRightVector _playercamera))
  (bind _returnvalue_3 (* _returnvalue (.x _returnvalue_2)))
  (bind _returnvalue_4 (* _returnvalue (.y _returnvalue_2)))
  (bind _returnvalue_5 (Math|Rotator|MakeRotator _returnvalue_3 _returnvalue_4 0.0))
  (Class|Actor|AddActorWorldRotation (Math|Rotator|MakeRotator (.roll _returnvalue_5) (.pitch _returnvalue_5) (* (.x ActionValue) -2.0))))

(fn SetVariablesfromDataTable
  (bind _pivot (Variables|Default|GetPivot))
  (bind _returnvalue (Utilities|GetDataTableRow "/Game/Other/DataTables/DT_Items.DT_Items" (Variables|Customization|GetItemsRowName))
    (:then
      (Variables|Other|SetMyItemData _returnvalue)
      (Variables|Transformation|SetStartScale (Transformation|GetActorScale3D))
      (Variables|Transformation|SetStartPos (Transformation|GetWorldLocation _pivot))
      (Variables|Transformation|SetStartRot (Transformation|GetWorldRotation _pivot))
      (if (Utilities|IsValidSoftObjectReference (.StaticMesh (Utilities|Struct|BreakS_DataItem (Variables|Other|GetMyItemData))))
        (if (Variables|Customization|GetLoadItemFromDataTable?)
          (CallFunction|SetValuesfromDataTable (Variables|Other|GetMyItemData)))
        (else
          (Development|PrintString (Utilities|String|Append "ERROR 404: ITEM " (Utilities|String|ToString(Name) (Variables|Customization|GetItemsRowName)) " NOT FOUND") true true "(R=1.000000,G=0.000000,B=0.034441,A=1.000000)")
          (Actor|DestroyActor))))
    (:RowNotFound
      (Development|PrintString "NOT FOUND ITEM ROW NAME IN DT_ITEMS" true true "(R=1.000000,G=0.029169,B=0.000000,A=1.000000)"))))

(fn CheckifMouseonInteractionTrigger
  (bind _returnvalue (Game|GetPlayerController 0))
  (bind _hitresult (Game|Player|GetHitResultUnderCursorbyChannel _returnvalue "TraceTypeQuery3" false))
  (if (Math|Boolean|ANDBoolean (not (Variables|Other|GetIsVisibleDescription?)) (.bblockinghit _hitresult) (Utilities|Array|ContainsItem (Components|GetChildrenComponents (Variables|Default|GetPivot) true) (.hitcomponent _hitresult)))
    (if (Components|ComponentHasTag (.hitcomponent _hitresult) "MessageBox")
      (Variables|Other|SetIsMouseCollidingWithBoxes? true)
      (CallFunction|OnClickMessageBox)
      (CallFunction|OnClickSaveMousePosition :!label _label)
      (elif (Components|ComponentHasTag (.hitcomponent _hitresult) "ActionBox")
        (Variables|Other|SetIsMouseCollidingWithBoxes? true)
        (CallFunction|OnClickActionBox (.hitcomponent _hitresult))
        (goto _label)))))

(fn SetCursorInspection
  (bind _returnvalue (Game|GetPlayerController 0))
  (bind _hitresult (Game|Player|GetHitResultUnderCursorbyChannel _returnvalue "TraceTypeQuery3" false))
  (if (not (Variables|Other|GetIsVisibleDescription?))
    (Variables|Default|SetSelectedComponent (.hitcomponent _hitresult))
    (Utilities|IsValid (.hitcomponent _hitresult)
      (:Is%20Valid
        (if (and (.bblockinghit _hitresult) (or (Components|ComponentHasTag (.hitcomponent _hitresult) "MessageBox") (Components|ComponentHasTag (.hitcomponent _hitresult) "ActionBox")))
          (Class|WidgetBlueprintLibrary|SetHardwareCursor "Default" "T_CursorLens" "(X=0.200000,Y=0.200000)")
          (else
            (Class|WidgetBlueprintLibrary|SetHardwareCursor "Default" "T_WestCursor" "(X=0.000000,Y=0.000000)" :!label _label))))
      (:Is%20Not%20Valid
        (goto _label)))))

(fn SetCollisions
  (params (Inspecting? :type Boolean))
  (bind _messageinteractionbox (Variables|Default|GetMessageInteractionBox))
  (bind _actioninteractionbox (Variables|Default|GetActionInteractionBox))
  (bind _staticmesh (Variables|Default|GetStaticMesh))
  (bind _hasmsgbox_ (Variables|Customization|GetHasMSGBox?))
  (bind _hasactionbox_ (Variables|Customization|GetHasActionBox?))
  (if Inspecting?
    (Collision|SetCollisionEnabled _staticmesh "QueryOnly")
    (if _hasmsgbox_
      (Collision|SetCollisionEnabled _messageinteractionbox "QueryOnly"))
    (if _hasactionbox_
      (Collision|SetCollisionEnabled _actioninteractionbox "QueryOnly"))
    (else
      (Collision|SetCollisionEnabled _staticmesh "QueryOnly")
      (if _hasmsgbox_
        (Collision|SetCollisionEnabled _messageinteractionbox "NoCollision"))
      (if _hasactionbox_
        (Collision|SetCollisionEnabled _actioninteractionbox "NoCollision")))))

(fn OnClickMessageBox
  (Development|PrintString "MSG BOX")
  (bind _msgwidget (Variables|Other|GetMsgWidget)
    (:then
      (Default|FlipFlopFadeAnimation _msgwidget))
    (:else
      (bind _returnvalue (UserInterface|CreateWidget "/Game/UserInterfaces/Inspect/WBP_SceneInteractionWindow.WBP_SceneInteractionWindow_C" 0 (Variables|Customization|GetReading%20Panel%20Position) (Variables|Customization|GetReading%20Panel%20Text)))
      (UserInterface|Viewport|AddtoViewport _returnvalue 0)
      (Variables|Other|SetMsgWidget _returnvalue))))

(fn OnClickActionBox
  (params (ActionActorClicked :type Actor%20Component%20Object%20Reference)))

(fn OnClickSaveMousePosition
  (bind _returnvalue (Game|GetPlayerController 0))
  (bind (_locationx _locationy) (Game|Player|GetMousePosition _returnvalue))
  (Variables|Other|SetPreInspectMousePosition (Math|Vector2D|MakeVector2D _locationx _locationy)))

(fn OnNotRotating
  (params (Action%20Value :type Vector%202D%20Structure%20%28by%20ref%29)))

(fn SetValuesfromDataTable
  (params (S_DataItem :type S%20Data%20Item%20Structure%20%28by%20ref%29))
  (bind (_staticmesh _staticmeshpositionoffsetfrompivot _staticmeshrotationoffset _staticmeshscale _inspectiondistance _interactsound _pickupsound _readingpaneltext _readingpanelpos) (Utilities|Struct|BreakS_DataItem S_DataItem))
  (Transformation|SetRelativeLocationAndRotation (Variables|Default|GetStaticMesh) _staticmeshpositionoffsetfrompivot _staticmeshrotationoffset false false)
  (Variables|Customization|SetInspectionDistance _inspectiondistance)
  (Variables|Customization|SetReading%20Panel%20Text _readingpaneltext)
  (Variables|Customization|SetReading%20Panel%20Position _readingpanelpos)
  (Utilities|LoadAssetBlocking _interactsound)
  (Variables|Customization|SetInteractSound (Utilities|ResolveSoftReference _interactsound))
  (Utilities|LoadAssetBlocking _pickupsound)
  (Variables|Customization|SetPickupSound (Utilities|ResolveSoftReference _pickupsound))
  (Transformation|SetRelativeScale3D (Variables|Default|GetStaticMesh) _staticmeshscale))

(fn TickPutinPocket
  (params (Alpha :type Float%20%28double-precision%29)))

(fn EndPutinPocket)

(fn OnDropInventoryItem)

(fn PickUp
  (bind _returnvalue (Game|Player|GetPlayerPawn 0))
  (bind _itemsrowname (Variables|Customization|GetItemsRowName))
  (bind _cameraactorcomponent (Class|IPlayerUtils|GetCamera(Message) _returnvalue))
  (Variables|Default|SetPlayerCamera _cameraactorcomponent)
  (CallFunction|ManagePickUp)
  (if (or (== _itemsrowname "Default") (== _itemsrowname ""))
    _
    (else
      (Class|IPlayerUtils|AddedItemtoInventoryManage(Message) _returnvalue (Variables|Customization|GetPreInspectDialogue) (Variables|Customization|GetPostInspectDialogue) self)))
  (return (Variables|Other|GetMyItemData)))