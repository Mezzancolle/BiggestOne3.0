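; Inspectable picture frame holding Adelaide's picture, opened by removing three screws and sliding off the back.
; Cursor traces against tagged boxes fire click dispatchers that play one-shot timeline animations for each part.
; Pressing all three screw boxes enables the back's box.
; After the back slides away, the item calls PutInPocket, switches to the picture's row name and becomes inventory-eligible.
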(event Custom|Screw1Animation
  (bind _screw1 (Variables|Default|GetScrew1))
  (Variables|Default|SetCanBeDropped? false)
  (EventDispatchers|UnbindEventfromOnClickonActionBox (delegate Custom|Screw1Animation))
  (bind _alpha (Timeline|RotationScrew1 PlayFromStart)
    (:Update
      (Transformation|SetRelativeRotation _screw1 (Math|Rotator|Lerp(Rotator) (Variables|/Script/Engine.SceneComponent|GetRelativeRotation _screw1) "0, 0, 0" _alpha) false false)
      (CallFunction|OnAllScrewOpened))
    (:Finished
      (Collision|SetCollisionEnabled (Variables|Default|GetActionInteractionBox) "NoCollision"))))

(event Custom|Screw2Animation
  (bind _screw2 (Variables|Default|GetScrew2))
  (Variables|Default|SetCanBeDropped? false)
  (EventDispatchers|UnbindEventfromOnClickonActionBox1 (delegate Custom|Screw2Animation))
  (bind _alpha (Timeline|RotationScraw2 PlayFromStart)
    (:Update
      (Transformation|SetRelativeRotation _screw2 (Math|Rotator|Lerp(Rotator) (Variables|/Script/Engine.SceneComponent|GetRelativeRotation _screw2) "0, 0, 0" _alpha) false false)
      (CallFunction|OnAllScrewOpened))
    (:Finished
      (Collision|SetCollisionEnabled (Variables|Default|GetActionInteractionBox1) "NoCollision"))))

(event Custom|Screw3Animation
  (bind _screw3 (Variables|Default|GetScrew3))
  (Variables|Default|SetCanBeDropped? false)
  (EventDispatchers|UnbindEventfromOnClickonActionBox2 (delegate Custom|Screw3Animation))
  (bind _alpha (Timeline|RotationScrew3 PlayFromStart)
    (:Update
      (Transformation|SetRelativeRotation _screw3 (Math|Rotator|Lerp(Rotator) (Variables|/Script/Engine.SceneComponent|GetRelativeRotation _screw3) "0.000000,0.000000,90.000000" _alpha) false false)
      (CallFunction|OnAllScrewOpened))
    (:Finished
      (Collision|SetCollisionEnabled (Variables|Default|GetActionInteractionBox2) "NoCollision"))))

(event Custom|OnAllScrewOpened
  (if (Math|Boolean|ANDBoolean (Variables|Default|GetIsActionInteractionBoxPressed?) (Variables|Default|GetIsActionInteractionBox1Pressed?) (Variables|Default|GetIsActionInteractionBox2Pressed?))
    (Collision|SetCollisionEnabled (Variables|Default|GetActionInteractionBox3) "QueryOnly")))

(event Custom|BackAnimation
  (bind _back (Variables|Default|GetBack))
  (EventDispatchers|UnbindEventfromOnClickonActionBox3 (delegate Custom|BackAnimation))
  (Collision|SetCollisionEnabled (Variables|Default|GetStaticMesh) "NoCollision")
  (Variables|Default|SetCanRotateItem? false)
  (bind _alpha (Timeline|BackAnimationTimeline PlayFromStart)
    (:Update
      (Transformation|SetRelativeLocation _back (.location (Math|Transform|Lerp(Transform) (Transformation|GetRelativeTransform _back) (Math|Transform|MakeTransform "130.000000,-60.000000,-5.000000" "0, 0, 0" "1.000000,1.000000,1.000000") _alpha)) false false))
    (:Finished
      (CallFunction|PutinPocket (Variables|Default|GetStaticMesh))
      (Variables|Default|SetCanRotateItem? true)
      (Variables|Default|SetCanBeDropped? true)
      (Variables|Default|SetItemsRowName (Variables|Default|GetPictureRawName))
      (Utilities|Struct|SetmembersinS_DataItem (Variables|Default|GetMyItemData) true))))

(event EventBeginPlay
  (|CallParentFunction)
  (CallFunction|CheckifAlreadyTaken (Variables|Default|GetPictureRawName))
  (EventDispatchers|BindEventtoOnClickonActionBox (delegate Custom|Screw1Animation))
  (EventDispatchers|BindEventtoOnClickonActionBox1 (delegate Custom|Screw2Animation))
  (EventDispatchers|BindEventtoOnClickonActionBox2 (delegate Custom|Screw3Animation))
  (EventDispatchers|BindEventtoOnClickonActionBox3 (delegate Custom|BackAnimation)))

(event EventTick
  (params (DeltaSeconds :type Float%20%28single-precision%29))
  (|CallParentFunction DeltaSeconds))

(fn ConstructionScript
  (|CallParentFunction)
  (Collision|SetActorEnableCollision (Variables|/Script/Engine.ChildActorComponent|GetChildActor (Variables|Default|GetAdelaidePicture)) false))

(fn OnClickActionBox
  (|CallParentFunction)
  (Variables|Default|SetIsActionInteractionBoxPressed? true)
  (Default|CallOnClickonActionBox))

(fn CheckifMouseonInteractionTrigger
  (bind _returnvalue (Game|GetPlayerController 0))
  (bind _hitresult (Game|Player|GetHitResultUnderCursorbyChannel _returnvalue "TraceTypeQuery3" false))
  (if (and (not (Variables|Default|GetIsVisibleDescription?)) (.bblockinghit _hitresult))
    (if (Components|ComponentHasTag (.hitcomponent _hitresult) "MessageBox")
      (Variables|Default|SetIsMouseCollidingWithBoxes? true)
      (CallFunction|OnClickMessageBox)
      (CallFunction|OnClickSaveMousePosition :!label _label)
      (elif (Components|ComponentHasTag (.hitcomponent _hitresult) "ActionBox")
        (Variables|Default|SetIsMouseCollidingWithBoxes? true)
        (CallFunction|OnClickActionBox)
        (goto _label)
        (elif (Components|ComponentHasTag (.hitcomponent _hitresult) "ActionBox1")
          (Variables|Default|SetIsMouseCollidingWithBoxes? true)
          (CallFunction|OnClickActionBox1)
          (goto _label)
          (elif (Components|ComponentHasTag (.hitcomponent _hitresult) "ActionBox2")
            (Variables|Default|SetIsMouseCollidingWithBoxes? true)
            (CallFunction|OnClickActionBox2)
            (goto _label)
            (elif (Components|ComponentHasTag (.hitcomponent _hitresult) "ActionBox3")
              (Variables|Default|SetIsMouseCollidingWithBoxes? true)
              (CallFunction|OnClickActionBox3)
              (goto _label))))))))

(fn OnClickActionBox2
  (Variables|Default|SetIsActionInteractionBox2Pressed? true)
  (Default|CallOnClickonActionBox2))

(fn OnClickActionBox1
  (Variables|Default|SetIsActionInteractionBox1Pressed? true)
  (Default|CallOnClickonActionBox1))

(fn SetCollisions
  (params (Inspecting? :type Boolean))
  (bind _messageinteractionbox (Variables|Default|GetMessageInteractionBox))
  (bind _actioninteractionbox (Variables|Default|GetActionInteractionBox))
  (bind _staticmesh (Variables|Default|GetStaticMesh))
  (bind _hasmsgbox_ (Variables|Default|GetHasMSGBox?))
  (bind _hasactionbox_ (Variables|Default|GetHasActionBox?))
  (if Inspecting?
    (Collision|SetCollisionEnabled _staticmesh "NoCollision")
    (if _hasmsgbox_
      (Collision|SetCollisionEnabled _messageinteractionbox "QueryOnly"))
    (if _hasactionbox_
      (Collision|SetCollisionEnabled _actioninteractionbox "QueryOnly"))
    (else
      (Collision|SetCollisionEnabled _staticmesh "QueryAndPhysics")
      (if _hasmsgbox_
        (Collision|SetCollisionEnabled _messageinteractionbox "NoCollision"))
      (if _hasactionbox_
        (Collision|SetCollisionEnabled _actioninteractionbox "NoCollision")))))

(fn SetCursorInspection
  (bind _returnvalue (Game|GetPlayerController 0))
  (bind _hitresult (Game|Player|GetHitResultUnderCursorbyChannel _returnvalue "TraceTypeQuery3" false))
  (if (not (Variables|Default|GetIsVisibleDescription?))
    (Utilities|IsValid (.hitcomponent _hitresult)
      (:Is%20Valid
        (if (and (.bblockinghit _hitresult) (or (Components|ComponentHasTag (.hitcomponent _hitresult) "MessageBox") (Math|Boolean|ORBoolean (Components|ComponentHasTag (.hitcomponent _hitresult) "ActionBox") (Components|ComponentHasTag (.hitcomponent _hitresult) "ActionBox1") (Components|ComponentHasTag (.hitcomponent _hitresult) "ActionBox2"))))
          (Class|WidgetBlueprintLibrary|SetHardwareCursor "Default" "T_CursorLens" "(X=0.200000,Y=0.200000)")
          (else
            (Class|WidgetBlueprintLibrary|SetHardwareCursor "Default" "T_Cursor" "(X=0.500000,Y=0.500000)" :!label _label))))
      (:Is%20Not%20Valid
        (goto _label)))))

(fn OnClickActionBox3
  (Default|CallOnClickonActionBox3))