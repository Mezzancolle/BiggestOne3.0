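; Trigger volume that queues a subtitled dialogue line from DT_Trigger_Dialogues when the player overlaps it.
; One-shot triggers also update Abigail's hints through AbigailManager, flag their ID in the map data, save it asynchronously and destroy themselves.
; On BeginPlay, a trigger whose ID is already flagged destroys itself, while Repeatable triggers only queue the line and stay active.
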(event OnComponentBeginOverlap(BoxTrigger)
  (params (OverlappedComponent :type Primitive%20Component%20Object%20Reference) (OtherActor :type Actor%20Object%20Reference) (OtherComp :type Primitive%20Component%20Object%20Reference) (OtherBodyIndex :type Integer) (bFromSweep :type Boolean) (SweepResult :type Hit%20Result%20Structure%20%28by%20ref%29))
  (bind _returnvalue (Game|GetGameInstance))
  (if (Actor|ActorHasTag OtherActor "Player")
    (Class|SNSNarrativeBlueprintFuncLib|EnqueueDialogue "/Game/Other/DataTables/Dialogues/DT_Trigger_Dialogues.DT_Trigger_Dialogues" (Variables|Default|GetAudio%20Row%20Name) false)
    (if (not (Variables|Default|GetRepeatable?))
      (Default|UpdateHints (Variables|Default|GetAbigailManager) "Abigail")
      (bind _saveddata (Class|ISaveGame|GetGameData(Message) _returnvalue))
      (Utilities|Array|SetArrayElem (.triggerboxsubtitlesabigail (Variables|/Game/Blueprint/SaveGame/BP_GameData.BP_GameData_C|GetMapData _saveddata)) (Variables|Default|GetID) true)
      (Class|ISaveGame|SaveMapData(Message) _returnvalue true (Variables|/Game/Blueprint/SaveGame/BP_GameData.BP_GameData_C|GetMapData _saveddata))
      (Actor|DestroyActor))))

(event EventBeginPlay
  ;[0.15 0.15 0.15 0.5] Check if the box was already picked
  (bind _saveddata (Class|ISaveGame|GetGameData(Message) (Game|GetGameInstance)))
  (if (Utilities|Array|Get(acopy) (.triggerboxsubtitlesabigail (Variables|/Game/Blueprint/SaveGame/BP_GameData.BP_GameData_C|GetMapData _saveddata)) (Variables|Default|GetID))
    (Actor|DestroyActor)))

(fn ConstructionScript)