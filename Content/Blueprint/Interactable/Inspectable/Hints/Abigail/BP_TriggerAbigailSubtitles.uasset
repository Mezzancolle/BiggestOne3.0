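; Trigger box that plays Abigail dialogue subtitles when the player walks into it.
; On player overlap it validates the audio row name and enqueues that row from the trigger dialogue table without stopping other dialogue.
; Non-repeatable boxes then update AbigailManager hints by ID and destroy themselves.
; On BeginPlay, boxes already flagged in the GameInstance's map data update hints and self-destroy.
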(event OnComponentBeginOverlap(BoxTrigger)
  (params (OverlappedComponent :type Primitive%20Component%20Object%20Reference) (OtherActor :type Actor%20Object%20Reference) (OtherComp :type Primitive%20Component%20Object%20Reference) (OtherBodyIndex :type Integer) (bFromSweep :type Boolean) (SweepResult :type Hit%20Result%20Structure%20%28by%20ref%29))
  (bind _audio_row_name (Variables|Default|GetAudio%20Row%20Name))
  (if (Actor|ActorHasTag OtherActor "Player")
    (bind _isvalid_ (CallFunction|CheckValidRowName _audio_row_name))
    (if _isvalid_
      (Class|SNSNarrativeBlueprintFuncLib|EnqueueDialogue "/Game/Other/DataTables/Dialogues/DT_Trigger_Dialogues.DT_Trigger_Dialogues" _audio_row_name false))
    (if (not (Variables|Default|GetRepeatable?))
      (Default|UpdateHints (Variables|Default|GetAbigailManager) (Variables|Default|GetID))
      (Actor|DestroyActor))))

(event EventBeginPlay
  ;[0.15 0.15 0.15 0.5] Check if the box was already picked
  (|CallParentFunction)
  (bind _saveddata (Class|ISaveGame|GetGameData(Message) (Game|GetGameInstance)))
  (if (Utilities|Array|Get(acopy) (.triggerboxsubtitlesabigail (Variables|/Game/Blueprint/SaveGame/BP_GameData.BP_GameData_C|GetMapData _saveddata)) (Variables|Default|GetID))
    (Default|UpdateHints (Variables|Default|GetAbigailManager) (Variables|Default|GetID))
    (Actor|DestroyActor)))

(fn ConstructionScript
  (|CallParentFunction))