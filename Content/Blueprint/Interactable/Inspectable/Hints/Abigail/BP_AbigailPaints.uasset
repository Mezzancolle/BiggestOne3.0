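; Inspectable hint actor for Abigail's paintings, where a click identifies the right, center or left painting.
; Each click adds the ghost's name message to the player's diary, then dismisses an open interaction window or creates a new one.
; The painting is picked by converting the cursor trace impact into the mesh's local space and thresholding its Y, with placeholder-like Italian text shown for each.
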(event EventBeginPlay
  (|CallParentFunction) ; This node is disabled and will not be called.\nDrag off pins to build functionality.
)

(event Collision|EventActorBeginOverlap
  (params (OtherActor :type Actor%20Object%20Reference)))

(event EventTick
  (params (DeltaSeconds :type Float%20%28single-precision%29))
  (|CallParentFunction DeltaSeconds) ; This node is disabled and will not be called.\nDrag off pins to build functionality.
)

(fn ConstructionScript
  (|CallParentFunction))

(fn OnClickonMouseInteractionTrigger
  (|CallParentFunction)
  (Class|IPlayerUtils|AddDiaryGhostName(Message) (Game|Player|GetPlayerPawn 0) (Variables|Default|GetGhostRowName))
  (Variables|Default|GetWBP_InteractionWindow
    (:then
      (Default|FlipFlopFadeAnimation (Variables|Default|GetWBP_InteractionWindow))
      (Variables|Default|SetWBP_InteractionWindow 0))
    (:else
      (bind _output_get (Variables|Default|SetLocalClick (Math|Vector|MakeVector 0.0 (.y (Math|Transform|InverseTransformLocation (Transformation|GetWorldTransform (Variables|Default|GetStaticMesh)) (.ImpactPoint (Collision|BreakHitResult (.HitResult (Game|Player|GetHitResultUnderCursorbyChannel (Game|GetPlayerController 0) "TraceTypeQuery3" true)))))) 0.0)))
      (if (< (.y _output_get) -1e+01)
        (bind _returnvalue (UserInterface|CreateWidget "/Game/UserInterfaces/Inspect/WBP_SceneInteractionWindow.WBP_SceneInteractionWindow_C" 0 "(X=150.000000,Y=-200.000000)" "Hai cliccato il quadro DESTRO"))
        (UserInterface|Viewport|AddtoViewport _returnvalue 0)
        (Variables|Default|SetWBP_InteractionWindow _returnvalue)
        (elif (> (.y _output_get) 1e+01)
          (bind _returnvalue_2 (UserInterface|CreateWidget "/Game/UserInterfaces/Inspect/WBP_SceneInteractionWindow.WBP_SceneInteractionWindow_C" 0 "(X=150.000000,Y=-200.000000)" "Hai cliccato il quadro SINISTRO"))
          (UserInterface|Viewport|AddtoViewport _returnvalue_2 0)
          (Variables|Default|SetWBP_InteractionWindow _returnvalue_2)
          (else
            (bind _returnvalue_3 (UserInterface|CreateWidget "/Game/UserInterfaces/Inspect/WBP_SceneInteractionWindow.WBP_SceneInteractionWindow_C" 0 "(X=150.000000,Y=-200.000000)" "Hai cliccato il quadro CENTRALE"))
            (UserInterface|Viewport|AddtoViewport _returnvalue_3 0)
            (Variables|Default|SetWBP_InteractionWindow _returnvalue_3)))))))