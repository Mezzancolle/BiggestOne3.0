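; BPC_Grave is a scene-interaction grave that shows a reading panel and sends its ghost name to the player's diary.
; A click without a live window calls the pawn's diary message with GhostRowName and creates the panel from ReadingPanelText.
; Later clicks flip-flop that panel's fade animation.
; Before control returns to the player, it removes and clears the widget, then forces garbage collection.
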(fn ConstructionScript
  (|CallParentFunction))

(fn OnClickonMouseInteractionTrigger
  (|CallParentFunction)
  (Variables|Default|GetWBP_InteractionWindow
    (:then
      (Default|FlipFlopFadeAnimation (Variables|Default|GetWBP_InteractionWindow)))
    (:else
      (Class|IPlayerUtils|AddDiaryGhostName(Message) (Game|Player|GetPlayerPawn 0) (Variables|Default|GetGhostRowName))
      (bind _returnvalue (UserInterface|CreateWidget "/Game/UserInterfaces/Inspect/WBP_SceneInteractionWindow.WBP_SceneInteractionWindow_C" 0 "(X=150.000000,Y=-200.000000)" (Variables|Default|GetReading%20Panel%20Text)))
      (UserInterface|Viewport|AddtoViewport _returnvalue 0)
      (Variables|Default|SetWBP_InteractionWindow _returnvalue))))

(fn BeforeBacktoPlayer
  (|CallParentFunction)
  (Utilities|IsValid (Variables|Default|GetWBP_InteractionWindow)
    (:Is%20Valid
      (Widget|RemovefromParent (Variables|Default|GetWBP_InteractionWindow))
      (Variables|Default|SetWBP_InteractionWindow 0)
      (Utilities|Platform|CollectGarbage))))