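; BP_SymbolLockElement is a single rotatable element of a symbol lock that advances to the next symbol when interacted with, unless rotation is disabled.
; The construction script divides a full turn by the symbol count to get the step angle.
; Each rotation increments and wraps the symbol index, then snaps the mesh pitch to that step.
; SetSettings applies a given index and locked state, then refreshes the rotation.
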(event EventInteract
  (params (LookingComponent :type Primitive%20Component%20Object%20Reference))
  (if (not (Variables|Default|GetCannotRotate?))
    (CallFunction|Rotate)))

(fn ConstructionScript
  (Variables|Default|SetRotateValue (/ 3.6e+02 (+ (Variables|Default|GetMaxSymbolIndex) 1))))

(fn Rotate
  (Utilities|FlowControl|Sequence
    (:then_0
      (Math|Integer|IncrementInt (Variables|Default|GetCurrentSymbolIndex)
        (:%20%20
          (if (> (Variables|Default|GetCurrentSymbolIndex) (Variables|Default|GetMaxSymbolIndex))
            (Variables|Default|SetCurrentSymbolIndex 0)))))
    (:then_1
      (CallFunction|SetRotationbyIndex))))

(fn SetRotationbyIndex
  (Transformation|SetRelativeRotation (Variables|Default|GetMesh) (Math|Rotator|MakeRotator 0.0 (* (Variables|Default|GetCurrentSymbolIndex) (Variables|Default|GetRotateValue) 1) 0.0) false false))

(fn SetSettings
  (params (Settings :type S%20Symbol%20Data%20Structure))
  (Variables|Default|SetCurrentSymbolIndex (.value Settings))
  (Variables|Default|SetCannotRotate? (.locked? Settings))
  (CallFunction|SetRotationbyIndex))