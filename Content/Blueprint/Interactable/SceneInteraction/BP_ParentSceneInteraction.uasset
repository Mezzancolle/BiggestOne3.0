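; Base actor for scene inspections: on Interact it fades to its own camera with a short zoom, swaps to inspect input and shows the cursor.
; Tick traces under the cursor to show a lens over tagged points of interest.
; Clicking one checks for a required key item and queues dialogue before calling an overridable click hook.
; Drop fades back to the player, with overridable hooks around transitions.
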(event Custom|DelayDialogueActivation
  (Variables|Default|SetCanSkipDialogue? false)
  (Utilities|FlowControl|Delay 0.2)
  (Variables|Default|SetCanSkipDialogue? true))

(event Custom|BackToPlayerCamera
  (bind _returnvalue (Game|GetPlayerController 0))
  (bind _camerahalffade (Variables|Default|GetCameraHalfFade))
  (bind _startcameralocation (Variables|Default|GetStartCameraLocation))
  (CallFunction|BeforeBacktoPlayer)
  (Variables|/Script/Engine.PlayerController|SetbShowMouseCursor _returnvalue false)
  (Input|DisableInput _returnvalue)
  ;[1 1 1] camera back  to player's one
  (Collision|SetCollisionEnabled (Variables|Default|GetMouseInteractionTrigger) "NoCollision")
  (Collision|SetCollisionEnabled (Variables|Default|GetInteractionBox) "QueryOnly")
  (Variables|/Script/Engine.PlayerController|SetbShowMouseCursor (Game|GetPlayerController 0) false)
  (Variables|Default|SetIsMouseLeftClicked? false)
  (Variables|Default|SetIsGamePadButtonClicked? false)
  (Variables|Default|SetIsMouseColliding? false)
  (CameraFades|StartCameraFade :self (Game|GetPlayerCameraManager 0) :ToAlpha 1.0 :Duration (* (Variables|Default|GetCameraHalfFade) 2.0))
  (bind _alpha (Timeline|TL_ZoomOut PlayFromStart)
    (:Update
      (Transformation|SetWorldLocation (Variables|Default|GetCamera) (Math|Vector|Lerp(Vector) (+ _startcameralocation (* (Math|Vector|GetForwardVector (Variables|Default|GetCamera)) 1e+01)) _startcameralocation _alpha) false true))
    (:Finished
      (Game|Player|SetViewTargetwithBlend (Game|GetPlayerController 0) (Game|Player|GetPlayerPawn 0) 0.0 "VTBlend_Linear" 0.0 false)
      (CallFunction|PreDropFadein)
      (CameraFades|StartCameraFade :self (Game|GetPlayerCameraManager 0) :FromAlpha 1.0 :Duration _camerahalffade)
      (Class|IPlayerUtils|SwitchInputContext(Message) (Game|Player|GetPlayerPawn 0) "/Game/Inputs/IMC_FirstPersonPlayer.IMC_FirstPersonPlayer" false)
      (Input|EnableInput (Game|Player|GetPlayerPawn 0) 0)
      (Utilities|FlowControl|Delay _camerahalffade)
      (CallFunction|PostDropFadein))))

(event Custom|OnStartInteract)

(event Custom|OnSceneInteractionCompleted
  ;[0 1 0.2041] OnSceneInteractionCompleted
  (Input|DisableInput (Game|GetPlayerController 0))
  (Variables|Default|SetIsCompleted? true))

(event Input|EnhancedActionEvents|EnhancedInputActionIA_Drop
  (params (ActionValue :type Boolean) (ElapsedSeconds :type Float%20%28double-precision%29) (TriggeredSeconds :type Float%20%28double-precision%29) (InputAction :type Input%20Action%20Object%20Reference :default "/Game/Inputs/Actions/IA_Drop.IA_Drop"))
  ;[1 1 1] On player interaction with this object change player camera to this object's camera
  (:Started
    (if (CallFunction|CanCloseInspection)
      (CallFunction|BacktoPlayerCamera))))

(event Input|EnhancedActionEvents|EnhancedInputActionIA_ViewObject
  (params (ActionValue :type Vector%202D%20Structure) (ElapsedSeconds :type Float%20%28double-precision%29) (TriggeredSeconds :type Float%20%28double-precision%29) (InputAction :type Input%20Action%20Object%20Reference :default "/Game/Inputs/Actions/IA_ViewObject.IA_ViewObject"))
  (CallFunction|MoveMousewithGamepad (Variables|Default|GetCanGamepadMoveMouse?) ActionValue (Game|GetPlayerController 0)))

(event Input|EnhancedActionEvents|EnhancedInputActionIA_Interact
  (params (ActionValue :type Boolean) (ElapsedSeconds :type Float%20%28double-precision%29) (TriggeredSeconds :type Float%20%28double-precision%29) (InputAction :type Input%20Action%20Object%20Reference :default "/Game/Inputs/Actions/IA_Interact.IA_Interact"))
  (bind _returnvalue (Game|GetPlayerController 0))
  (bind _returnvalue_2 (Game|GetPlayerController 0))
  (bind _preinspectmouseposition (Variables|Default|GetPreInspectMousePosition))
  (bind (_locationx _locationy) (Game|Player|GetMousePosition _returnvalue_2))
  ;[1 0.2083 0.2182] ON INTERACT
  (:Triggered
    (if (not (and (not (Variables|Default|GetShouldLockMouse?)) (Variables|/Script/Engine.PlayerController|GetbShowMouseCursor _returnvalue_2)))
      (Class|PlayerController|SetMouseLocation _returnvalue_2 (Math|Float|Truncate _locationx) (Math|Float|Truncate _locationy))))
  (:Started
    (Variables|Default|SetIsMouseLeftClicked? true)
    (CallFunction|CheckifMouseonInteractionTrigger (not (Variables|Default|GetShouldLockMouse?)))
    (CallFunction|OnStartInteract))
  (:Canceled
    (Variables|Default|SetIsMouseLeftClicked? false :!label _label)
    (if (and (Variables|Default|GetIsMouseColliding?) (Variables|Default|GetShouldLockMouse?))
      (Variables|Default|SetIsMouseColliding? false)
      (Class|PlayerController|SetMouseLocation _returnvalue (Math|Float|Truncate (.x _preinspectmouseposition)) (Math|Float|Truncate (.y _preinspectmouseposition)))
      (Variables|/Script/Engine.PlayerController|SetbShowMouseCursor _returnvalue true)))
  (:Completed
    (goto _label)))

(event EventBeginPlay
  ;[1 1 1] Begin Play
  (Variables|Default|SetStartCameraLocation (Transformation|GetWorldLocation (Variables|Default|GetCamera)))
  (bind _saveddata (Class|ISaveGame|GetGameData(Message) (Game|GetGameInstance)))
  (if (Utilities|Array|ContainsItem (.itemstaken (Variables|/Game/Blueprint/SaveGame/BP_GameData.BP_GameData_C|GetInventoryDiaryData _saveddata)) (Variables|Default|GetUnlockableItemRowName))
    (CallFunction|OnKeyItemAlreadyGot)))

(event EventInteract
  (params (LookingComponent :type Primitive%20Component%20Object%20Reference))
  (bind _returnvalue (Game|Player|GetPlayerPawn 0))
  (bind _shouldlockmouse_ (Variables|Default|GetShouldLockMouse?))
  (bind _startcameralocation (Variables|Default|GetStartCameraLocation))
  ;[1 1 1] On player interaction with this object change player camera to this object's camera
  (Class|IPlayerUtils|SwitchInputContext(Message) _returnvalue "/Game/Inputs/IMC_Inspect.IMC_Inspect" true)
  (Collision|SetCollisionEnabled (Variables|Default|GetInteractionBox) "NoCollision")
  (Input|DisableInput _returnvalue (Game|GetPlayerController 0))
  (CameraFades|StartCameraFade :self (Game|GetPlayerCameraManager 0) :ToAlpha 1.0 :Duration (Variables|Default|GetCameraHalfFade))
  (Utilities|FlowControl|Delay (Variables|Default|GetCameraHalfFade))
  (CallFunction|PreInspectFadein)
  (Game|Player|SetViewTargetwithBlend (Game|GetPlayerController 0) self 0.0 "VTBlend_Linear" 0.0 false)
  (CameraFades|StartCameraFade :self (Game|GetPlayerCameraManager 0) :FromAlpha 1.0 :Duration (Variables|Default|GetCameraHalfFade))
  (bind _alpha (Timeline|TL_ZoomInALittleBit PlayFromStart)
    (:Update
      (Transformation|SetWorldLocation (Variables|Default|GetCamera) (Math|Vector|Lerp(Vector) _startcameralocation (+ _startcameralocation (* (Math|Vector|GetForwardVector (Variables|Default|GetCamera)) 1e+01)) _alpha) false true))
    (:Finished
      (Variables|/Script/Engine.PlayerController|SetbShowMouseCursor (Game|GetPlayerController 0) true)
      (Collision|SetCollisionEnabled (Variables|Default|GetMouseInteractionTrigger) "QueryAndPhysics")
      (Input|EnableInput (Game|GetPlayerController 0))
      (Actor|Tick|SetActorTickEnabled true)
      (Input|SetInputModeGameandUI (Game|GetPlayerController 0) 0 (select _shouldlockmouse_ "DoNotLock" "LockOnCapture") _shouldlockmouse_ true)
      (CallFunction|PostInspectFadein))))

(event EventTick
  (params (DeltaSeconds :type Float%20%28single-precision%29))
  (CallFunction|SetCursorInspection))

(fn ConstructionScript)

(fn OnKeyItemAlreadyGot
  (bind _camera (Variables|Default|GetCamera))
  (Transformation|SetRelativeLocation (Variables|Default|GetMouseInteractionTrigger) (+ (Variables|/Script/Engine.SceneComponent|GetRelativeLocation _camera) (* (Math|Vector|GetForwardVector _camera) -1e+01)) false false))

(fn CheckifMouseonInteractionTrigger
  (params (Show%20Mouse%20Cursor :type Boolean))
  (bind _returnvalue (Game|GetPlayerController 0))
  (bind _returnvalue_2 (Game|GetPlayerController 0))
  (bind _dialoguerownameonnotousekeyitem (Variables|Default|GetDialogueRowNameOnNoToUseKeyItem))
  (bind _dialoguerownameonusekeyitem (Variables|Default|GetDialogueRowNameOnUseKeyItem))
  (bind _hitresult (Game|Player|GetHitResultUnderCursorbyChannel _returnvalue "TraceTypeQuery3" false))
  (bind (_locationx _locationy) (Game|Player|GetMousePosition _returnvalue_2))
  (Utilities|IsValid (.hitcomponent _hitresult)
    (:Is%20Valid
      (if (and (.bblockinghit _hitresult) (Components|ComponentHasTag (.hitcomponent _hitresult) "ScenePointOfInterestTrigger"))
        (Variables|Default|SetIsMouseColliding? true)
        (if Show%20Mouse%20Cursor
          _
          (else
            (Variables|Default|SetPreInspectMousePosition (Math|Vector2D|MakeVector2D _locationx _locationy))))
        (if (== (Variables|Default|GetToUseItemRowName) "")
          (CallFunction|OnClickonMouseInteractionTrigger (.hitcomponent _hitresult) :!label _label)
          (else
            (bind _hasitem_ (Class|IPlayerUtils|PlayerHasItem?(Message) (Game|Player|GetPlayerPawn 0) (Variables|Default|GetToUseItemRowName)))
            (if _hasitem_
              (bind _isvalid_ (CallFunction|CheckValidRowName _dialoguerownameonusekeyitem))
              (if _isvalid_
                (Class|SNSNarrativeBlueprintFuncLib|EnqueueDialogue "/Game/Other/DataTables/Dialogues/DT_Items_Dialogues.DT_Items_Dialogues" _dialoguerownameonusekeyitem false)
                (goto _label)
                (else
                  (goto _label)))
              (else
                (bind _isvalid__2 (CallFunction|CheckValidRowName _dialoguerownameonnotousekeyitem))
                (if _isvalid__2
                  (Class|SNSNarrativeBlueprintFuncLib|EnqueueDialogue "/Game/Other/DataTables/Dialogues/DT_Barks.DT_Barks" _dialoguerownameonnotousekeyitem false)
                  (CallFunction|DelayDialogueActivation))))))
        (else
          (Variables|Default|SetIsMouseLeftClicked? false :!label _label_2)
          (Variables|Default|SetIsMouseColliding? false)
          (Variables|Default|SetIsGamePadButtonClicked? false))))
    (:Is%20Not%20Valid
      (goto _label_2))))

(fn OnClickonMouseInteractionTrigger
  (params (ComponentClicked :type Actor%20Component%20Object%20Reference)))

(fn BeforeBacktoPlayer
  (Input|SetInputModeGameOnly (Game|GetPlayerController 0) true)
  (Actor|Tick|SetActorTickEnabled false))

(fn SetCursorInspection
  (bind _returnvalue (Game|GetPlayerController 0))
  (bind _hitresult (Game|Player|GetHitResultUnderCursorbyChannel _returnvalue "TraceTypeQuery3" true))
  (Utilities|IsValid (.hitcomponent _hitresult)
    (:Is%20Valid
      (if (and (.bblockinghit _hitresult) (Components|ComponentHasTag (.hitcomponent _hitresult) "ScenePointOfInterestTrigger"))
        (Class|WidgetBlueprintLibrary|SetHardwareCursor "Default" "T_CursorLens" "(X=0.200000,Y=0.200000)")
        (Variables|Default|SetUnderMousePOIComponent (.hitcomponent _hitresult))
        (else
          (Class|WidgetBlueprintLibrary|SetHardwareCursor "Default" "T_Cursor" "(X=0.500000,Y=0.500000)" :!label _label)
          (Variables|Default|SetUnderMousePOIComponent 0))))
    (:Is%20Not%20Valid
      (goto _label))))

(fn PreInspectFadein
  (Rendering|SetVisibility (Variables|Default|GetLight) true false))

(fn PreDropFadein
  (Rendering|SetVisibility (Variables|Default|GetLight) false false))

(fn PostDropFadein)

(fn PostInspectFadein)

(fn CanCloseInspection
  (return (Variables|Default|GetCanExitInspection?)))