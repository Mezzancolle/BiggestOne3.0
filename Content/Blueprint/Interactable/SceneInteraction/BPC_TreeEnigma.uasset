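; Scene-interaction puzzle where the player saws through a tree rope to release a rope item.
; Clicking reveals the saw via timeline, then held-click mouse look drags it within clamped bounds, counting alternating strokes with sound.
; After enough strokes, a timeline moves the rope, then returns the player camera, saves completion and reveals the rope item.
; On BeginPlay, saved completion hides rope and saw and disables interaction.
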(event Custom|MakeRopeFall
  (bind _returnvalue (Game|GetGameInstance))
  (bind _ropebottom (Variables|Default|GetROPEBOTTOM))
  (bind _ropeitembp (Variables|Default|GetRopeItemBP))
  (bind _relativelocation (Variables|/Script/Engine.SceneComponent|GetRelativeLocation _ropebottom))
  (bind _alpha (Timeline|TL_FallingRope PlayFromStart)
    (:Update
      (Transformation|SetRelativeLocation (Variables|Default|GetROPEBOTTOM) (Math|Vector|MakeVector (Math|Float|Lerp 125.0 3.5e+02 _alpha) (.y _relativelocation) (.z _relativelocation)) false false))
    (:Finished
      (Audio|PlaySound2D "/Game/Audio/SFX/SFX_Item/SFX_Items_RopeFalling.SFX_Items_RopeFalling" 1.0 1.0 0.0 0 0)
      (CallFunction|BacktoPlayerCamera)
      (bind _saveddata (Class|ISaveGame|GetGameData(Message) _returnvalue))
      (bind _structout (Utilities|Struct|SetmembersinS_EnigmasSaveData (Variables|/Game/Blueprint/SaveGame/BP_GameData.BP_GameData_C|GetEnigmasData _saveddata) true))
      (Class|ISaveGame|SaveEnigmasData(Message) _returnvalue true _structout)
      (Development|SetHiddeninGame (Variables|Default|GetROPEBOTTOM) true false)
      (Development|SetHiddeninGame (Variables|Default|GetSaw) true false)
      (Collision|SetCollisionEnabled (Variables|Default|GetInteractionBox) "NoCollision")
      (Utilities|IsValid _ropeitembp
        (:Is%20Valid
          (Rendering|SetActorHiddenInGame _ropeitembp false))
        (:Is%20Not%20Valid
          (Development|PrintString "CANNOT CHANGE ROPE ITEM HIDDEN IN GAME PROPERTY"))))))

(event Custom|StartCutting
  (Development|SetHiddeninGame (Variables|Default|GetSaw) false false)
  (bind _movementalpha (Timeline|TL_MovingSaw PlayFromStart)
    (:Update
      (Transformation|SetRelativeLocation (Variables|Default|GetSaw) (Math|Vector|MakeVector (Math|Float|Lerp -46.0 -55.0 0.0) (Math|Float|Lerp -41.0 -25.0 0.0) (Math|Float|Lerp 0.0 82.0 _movementalpha)) false false))))

(event Input|EnhancedActionEvents|EnhancedInputActionIA_Look
  (params (ActionValue :type Vector%202D%20Structure) (ElapsedSeconds :type Float%20%28double-precision%29) (TriggeredSeconds :type Float%20%28double-precision%29) (InputAction :type Input%20Action%20Object%20Reference :default "/Game/Inputs/Actions/IA_Look.IA_Look"))
  (bind _x (Math|Vector2D|BreakVector2D ActionValue))
  (bind _saw (Variables|Default|GetSaw))
  (bind _mousespeedmultiplier (Variables|Default|GetMouseSpeedMultiplier))
  (bind _saw_2 (Variables|Default|GetSaw))
  (bind _cutcounts (Variables|Default|GetCutCounts))
  (bind _returnvalue (Math|Vector|GetUpVector _saw_2))
  (bind _returnvalue_2 (* _x _mousespeedmultiplier))
  (bind _relativelocation (Variables|/Script/Engine.SceneComponent|GetRelativeLocation _saw))
  (bind _relativerotation (Variables|/Script/Engine.SceneComponent|GetRelativeRotation _saw_2))
  (bind _returnvalue_3 (Math|Vector|RotateVector _returnvalue _relativerotation))
  (bind _returnvalue_4 (* _returnvalue_3 _returnvalue_2))
  (if (and (Variables|Default|GetIsCutting?) (Variables|Default|GetIsMouseLeftClicked?))
    (Transformation|AddRelativeLocation _saw_2 (Math|Vector|MakeVector (.x _returnvalue_4) (.y _returnvalue_4) 0.0) false false)
    (Transformation|SetRelativeLocation _saw (Math|Vector|MakeVector (Math|Float|Clamp(Float) (.x _relativelocation) -56.0 -43.0) (Math|Float|Clamp(Float) (.y _relativelocation) -45.0 -22.0) (.z _relativelocation)) false false)
    (if (Variables|Default|GetCuttingWay)
      (if (> (.y _relativelocation) -25.0)
        (Utilities|FlowControl|FlipFlop :!label _label
          (:A
            ;[1 0 0] TODO: random sound + pitch with sound cue
            (Audio|PlaySound2D "/Game/Audio/SFX/SFX_Item/Saw/SFX_Items_Saw_Upstroke_Cue.SFX_Items_Saw_Upstroke_Cue" 1.0 1.0 0.0 0 0))
          (:B
            (Audio|PlaySound2D "/Game/Audio/SFX/SFX_Item/Saw/SFX_Items_Saw_Downstroke_Cue.SFX_Items_Saw_Downstroke_Cue" 1.0 1.0 0.0 0 0)))
        (Variables|Default|SetCuttingWay (not (Variables|Default|GetCuttingWay)))
        (Math|Integer|IncrementInt _cutcounts
          (:%20%20
            (if (> _cutcounts 4)
              (CallFunction|MakeRopeFall)
              (CallFunction|OnSceneInteractionCompleted)))))
      (elif (< (.y _relativelocation) -4e+01)
        (goto _label)))))

(event EventBeginPlay
  (|CallParentFunction)
  (bind _saveddata (Class|ISaveGame|GetGameData(Message) (Game|GetGameInstance)))
  (if (Utilities|Struct|BreakS_EnigmasSaveData (Variables|/Game/Blueprint/SaveGame/BP_GameData.BP_GameData_C|GetEnigmasData _saveddata))
    (CallFunction|OnKeyItemAlreadyGot)))

(fn ConstructionScript
  (|CallParentFunction))

(fn OnClickonMouseInteractionTrigger
  (|CallParentFunction)
  (if (not (Variables|Default|GetIsCutting?))
    (Variables|Default|SetIsCutting? true)
    (CallFunction|StartCutting)))

(fn OnKeyItemAlreadyGot
  (|CallParentFunction)
  (Development|SetHiddeninGame (Variables|Default|GetROPEBOTTOM) true false)
  (Development|SetHiddeninGame (Variables|Default|GetSaw) true false)
  (Collision|SetCollisionEnabled (Variables|Default|GetInteractionBox) "NoCollision"))