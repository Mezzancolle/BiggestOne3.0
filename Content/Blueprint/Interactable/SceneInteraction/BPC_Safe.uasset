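; Combination safe puzzle built on a scene interaction parent, where look input rotates the dial with click sounds while the mouse is colliding.
; Holding the red arrow over the next tagged number box for a countdown removes that tag, advancing the ordered combination.
; The last number triggers chained handle and door timelines, returns the player camera and registers with BPCSaveable.
; Saved or already-looted safes snap open with interaction disabled.
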(event OnComponentBeginOverlap(RedArrow)
  (params (OverlappedComponent :type Primitive%20Component%20Object%20Reference) (OtherActor :type Actor%20Object%20Reference) (OtherComp :type Primitive%20Component%20Object%20Reference) (OtherBodyIndex :type Integer) (bFromSweep :type Boolean) (SweepResult :type Hit%20Result%20Structure%20%28by%20ref%29))
  ;[1 1 1] CollisionCheck
  (if (> (Utilities|Array|Length (Variables|Default|GetNumberBoxTags)) 0)
    (if (Components|ComponentHasTag OtherComp (Utilities|Array|Get(acopy) (Variables|Default|GetNumberBoxTags)))
      (Variables|Default|SetIsCounterEnabled? true)
      (Variables|Default|SetCounterCheckCollision (Variables|Default|GetTimerCheckCollision)))))

(event OnComponentEndOverlap(RedArrow)
  (params (OverlappedComponent :type Primitive%20Component%20Object%20Reference) (OtherActor :type Actor%20Object%20Reference) (OtherComp :type Primitive%20Component%20Object%20Reference) (OtherBodyIndex :type Integer))
  ;[1 1 1] CollisionCheck
  (Variables|Default|SetIsCounterEnabled? false))

(event OnFoundinSaves(BPC_Saveable)
  (Transformation|SetRelativeRotation (Variables|Default|GetPivotHandle) "0.000000,0.000000,-270.000000" false false)
  (Transformation|SetRelativeRotation (Variables|Default|GetPivotDoor) "0.000000,-80.000000,0.000000" false false)
  (Collision|SetCollisionResponsetoChannel (Variables|Default|GetSafe_safe_door) "ECC_GameTraceChannel2" "ECR_Ignore")
  (Collision|SetCollisionResponsetoChannel (Variables|Default|GetStaticMesh) "ECC_GameTraceChannel2" "ECR_Ignore")
  (Collision|SetCollisionResponsetoChannel (Variables|Default|GetInteractionBox) "ECC_GameTraceChannel2" "ECR_Ignore"))

(event Input|EnhancedActionEvents|EnhancedInputActionIA_Look
  (params (ActionValue :type Vector%202D%20Structure) (ElapsedSeconds :type Float%20%28double-precision%29) (TriggeredSeconds :type Float%20%28double-precision%29) (InputAction :type Input%20Action%20Object%20Reference :default "/Game/Inputs/Actions/IA_Look.IA_Look"))
  (bind _returnvalue (Utilities|String|ToString(Float) (.x ActionValue)))
  (bind _pivotwheel (Variables|Default|GetPivotWheel))
  (bind _relativerotation (Variables|/Script/Engine.SceneComponent|GetRelativeRotation _pivotwheel))
  (:Triggered
    ;[1 0 0.1485] ONLY SAFE Keys
    (Development|PrintString _returnvalue)
    (CallFunction|SetCursorInspection)
    (if (Variables|Default|GetIsMouseColliding?)
      (Transformation|SetRelativeRotation (Variables|Default|GetPivotWheel) (Math|Rotator|CombineRotators (Variables|/Script/Engine.SceneComponent|GetRelativeRotation (Variables|Default|GetPivotWheel)) (Math|Rotator|MakeRotator (* (.x ActionValue) -1.0) 0.0 0.0)) false false)
      (if (> (Math|Float|Absolute(Float) (- (.roll _relativerotation) (Variables|Default|GetLastWheelRotation))) (Variables|Default|GetDifferenceInRotationToMakeSound))
        (Audio|PlaySound2D "/Game/Audio/SFX/SFX_Misc/Safe/SFX_Safe_Turn_Cue.SFX_Safe_Turn_Cue" 1.0 1.0 0.8 0 0)
        (Variables|Default|SetLastWheelRotation (.roll _relativerotation)))))
  (:Started
    (Development|PrintString _returnvalue :!label _label))
  (:Ongoing
    (goto _label))
  (:Canceled
    (goto _label))
  (:Completed
    (goto _label)))

(event EventTick
  (params (DeltaSeconds :type Float%20%28single-precision%29))
  (|CallParentFunction DeltaSeconds)
  ;[1 1 1] Tick
  (if (Variables|Default|GetIsCounterEnabled?)
    (bind _output_get (Variables|Default|SetCounterCheckCollision (- (Variables|Default|GetCounterCheckCollision) DeltaSeconds)))
    (if (< _output_get 0.0)
      (Variables|Default|SetIsCounterEnabled? false)
      (Utilities|Array|RemoveIndex (Variables|Default|GetNumberBoxTags))
      (Audio|PlaySound2D "/Game/Audio/SFX/SFX_Misc/Safe/SFX_Safe_CorrectNumber.SFX_Safe_CorrectNumber" 1.0 1.0 0.0 0 0)
      (if (== (Utilities|Array|Length (Variables|Default|GetNumberBoxTags)) 0)
        (CallFunction|OnSceneInteractionCompleted)
        (Default|AddtoSaves (Variables|Default|GetBPC_Saveable))))))

(event EventOnSceneInteractionCompleted
  ;[0 1 0.2041] OnSceneInteractionCompleted
  (|CallParentFunction)
  (Audio|PlaySound2D "/Game/Audio/SFX/SFX_Misc/Safe/SFX_Safe_Handle.SFX_Safe_Handle" 2.0 1.0 0.0 0 0)
  (bind _alpha (Timeline|TL_Opening1 PlayFromStart)
    (:Update
      (Transformation|SetRelativeRotation (Variables|Default|GetPivotHandle) (Math|Rotator|Lerp(Rotator) "0, 0, 0" "0.000000,0.000000,-270.000000" _alpha) false false))
    (:Finished
      (Collision|SetCollisionResponsetoChannel (Variables|Default|GetInteractionBox) "ECC_GameTraceChannel2" "ECR_Ignore")
      (CallFunction|BacktoPlayerCamera)
      (Audio|SpawnSoundatLocation "/Game/Audio/SFX/SFX_Misc/Safe/SFX_Safe_Open.SFX_Safe_Open" (Transformation|GetActorLocation) "0, 0, 0" 1.0 1.0 0.0 0 0)
      (bind _alpha_2 (Timeline|TL_Opening2 PlayFromStart)
        (:Update
          (Transformation|SetRelativeRotation (Variables|Default|GetPivotDoor) (Math|Rotator|Lerp(Rotator) "0, 0, 0" "0.000000,-80.000000,0.000000" _alpha_2) false false))
        (:Finished
          (Transformation|SetRelativeRotation (Variables|Default|GetPivotHandle) "0.000000,0.000000,-270.000000" false false)
          (Transformation|SetRelativeRotation (Variables|Default|GetPivotDoor) "0.000000,-80.000000,0.000000" false false)
          (Collision|SetCollisionResponsetoChannel (Variables|Default|GetSafe_safe_door) "ECC_GameTraceChannel2" "ECR_Ignore")
          (Collision|SetCollisionResponsetoChannel (Variables|Default|GetStaticMesh) "ECC_GameTraceChannel2" "ECR_Ignore")
          (Collision|SetCollisionResponsetoChannel (Variables|Default|GetInteractionBox) "ECC_GameTraceChannel2" "ECR_Ignore"))))))

(fn ConstructionScript
  (Default|GenerateRandomGUID (Variables|Default|GetBPC_Saveable)))

(fn OnKeyItemAlreadyGot
  (|CallParentFunction)
  (Collision|SetCollisionResponsetoChannel (Variables|Default|GetInteractionBox) "ECC_GameTraceChannel2" "ECR_Ignore")
  (Transformation|SetRelativeRotation (Variables|Default|GetPivotHandle) "0.000000,0.000000,-270.000000" false true)
  (Transformation|SetRelativeRotation (Variables|Default|GetPivotDoor) "0.000000,-80.000000,0.000000" false false))