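; Parent inspectable item actor, configured from a DT_Items row, that self-destroys if game data lists it as taken.
; Pickup attaches it to the player, takes over input and lerps it before the camera for drag rotation, zoom and description viewing.
; Tick drives the move animation, or zoom smoothing with distance-based depth of field.
; Dropping either returns it to its start transform or stores it, shrinking it into the player via timeline before destruction.
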(event Custom|ManagePickUp
  ;[0 1 0.01716] PICKUP INTERFACE
  (Components|Activation|Deactivate (Variables|Default|GetNiagara))
  (Audio|PlaySound2D (Variables|Default|GetInteractSound) 1.0 1.0 0.0 0 0)
  (CallFunction|EnableInputto self)
  (bind _itemactorcomponent (Class|IPlayerUtils|GetHoldingItem(Message) (Variables|Default|GetPlayer%20Ref)))
  (Transformation|AttachComponentToComponent _itemactorcomponent "None" "KeepWorld" "KeepWorld" "KeepWorld" false)
  (Collision|SetActorEnableCollision false)
  (CallFunction|SetInspectionVariables)
  (Variables|Inspect|SetIsInspecting? true)
  (CallFunction|SetOffsetInspection 1.0)
  (CallFunction|PlayLerpingAnimation (Variables|Inspect|GetInspectPosition) (Variables|Inspect|GetInspectRotation))
  (Utilities|FlowControl|Delay 0.2)
  (Variables|Default|SetCanViewDescription? true))

(event Custom|SetItemToDefaultState
  ;[1 1 1] Comment
  ;;[1 1 1] DROP ITEM TO THE GROUND
  (Actor|Tick|SetActorTickEnabled false)
  (Components|Activation|Activate (Variables|Default|GetNiagara) true)
  (Collision|SetActorEnableCollision true)
  (Class|IPlayerUtils|CallonEndInteract(Message) (Variables|Default|GetPlayer%20Ref) false (Variables|Default|GetItemsRowName))
  (EventDispatchers|UnbindEventfromOnFinishedInspectionAnimation (delegate Custom|SetItemToDefaultState)))

(event Input|EnhancedActionEvents|EnhancedInputActionIA_Drop
  (params (ActionValue :type Boolean) (ElapsedSeconds :type Float%20%28double-precision%29) (TriggeredSeconds :type Float%20%28double-precision%29) (InputAction :type Input%20Action%20Object%20Reference :default "/Game/Inputs/Actions/IA_Drop.IA_Drop"))
  (bind _player_ref (Variables|Default|GetPlayer%20Ref))
  ;[1 1 1] Comment
  ;;[1 1 1] DROP ITEM TO THE GROUND
  (:Started
    (Actor|Tick|SetActorTickEnabled false)
    (Variables|Default|SetCanViewDescription? false)
    (Class|IPlayerUtils|ChangePPDepthOfField(Message) (Game|Player|GetPlayerPawn 0) 0.0)
    (if (Variables|Default|GetIsVisibleDescription?)
      (CallFunction|ViewItemDescription))
    (CallFunction|EnableInputto _player_ref)
    (Class|IPlayerUtils|SwitchInputContext(Message) _player_ref "/Game/Inputs/IMC_FirstPersonPlayer.IMC_FirstPersonPlayer" false)
    (Transformation|DetachFromActor "KeepWorld" "KeepWorld" "KeepWorld")
    (if (not (.CanBeAddedToInventory? (Utilities|Struct|BreakS_DataItem (Variables|Default|GetItemData))))
      (Variables|Inspect|SetIsInspecting? false)
      (CallFunction|PlayLerpingAnimation (Variables|Inspect|GetStartPos) (Variables|Inspect|GetStartRot))
      (EventDispatchers|BindEventtoOnFinishedInspectionAnimation (delegate Custom|SetItemToDefaultState))
      (else
        ;;;[0.5011 1 0.06198] Add Item To Inventory
        (Audio|PlaySound2D (Variables|Default|GetPickupSound) 1.0 1.0 0.0 0 0)
        (CallFunction|AddItemtoInventory)
        (bind _alpha (Timeline|TL_AddToInventoryAnimation PlayFromStart)
          (:Update
            (Transformation|SetActorScale3D (Math|Vector|Lerp(Vector) (Variables|Default|GetStartScale) "0, 0, 0" _alpha))
            (CallFunction|FromCameratoInsidePlayer _alpha))
          (:Finished
            (Utilities|IsValid self
              (:Is%20Valid
                (Actor|DestroyActor)))))))))

(event EventTick
  (params (DeltaSeconds :type Float%20%28single-precision%29))
  ;[0 1 0.01749] Tick
  (if (Variables|Default|GetIsPlayingAnimation?)
    (CallFunction|LoopLerpingAnimation DeltaSeconds)
    (else
      (CallFunction|ManageLerpZoom DeltaSeconds)
      (CallFunction|ManageFieldOfView))))

(event EventBeginPlay
  (bind _itemsrowname (Variables|Default|GetItemsRowName))
  (bind _pivot (Variables|Default|GetPivot))
  ;[0 1 0.0377] BEGIN PLAY
  (CallFunction|CheckifAlreadyTaken)
  (Variables|Default|SetStartScale (Transformation|GetActorScale3D))
  (Variables|Inspect|SetStartPos (Transformation|GetWorldLocation _pivot))
  (Variables|Inspect|SetStartRot (Transformation|GetWorldRotation _pivot))
  (bind _returnvalue (Utilities|GetDataTableRow "/Game/Other/DataTables/DT_Items.DT_Items" _itemsrowname)
    (:then
      (Variables|Default|SetItemData _returnvalue))
    (:RowNotFound
      (Development|PrintString (Utilities|String|Append "ERROR 404: ITEM " (Utilities|String|ToString(Name) _itemsrowname) " NOT FOUND") true true "(R=1.000000,G=0.000000,B=0.034441,A=1.000000)")
      (Utilities|IsValid self
        (:Is%20Valid
          (Actor|DestroyActor))))))

(event Input|EnhancedActionEvents|EnhancedInputActionIA_Look
  (params (ActionValue :type Vector%202D%20Structure) (ElapsedSeconds :type Float%20%28double-precision%29) (TriggeredSeconds :type Float%20%28double-precision%29) (InputAction :type Input%20Action%20Object%20Reference :default "/Game/Inputs/Actions/IA_Look.IA_Look"))
  ;[1 1 1] Mouse Inspect
  (if (Variables|Inspect|GetIsInspecting?)
    (if (Variables|Default|GetIsMouseLeftClicked?)
      (CallFunction|MouseRotateMesh ActionValue))))

(event Input|EnhancedActionEvents|EnhancedInputActionIA_ZoomInspect
  (params (ActionValue :type Float%20%28double-precision%29) (ElapsedSeconds :type Float%20%28double-precision%29) (TriggeredSeconds :type Float%20%28double-precision%29) (InputAction :type Input%20Action%20Object%20Reference :default "/Game/Inputs/Actions/IA_ZoomInspect.IA_ZoomInspect"))
  ;[0.5339 0.5245 1] Zoom Inspect
  (if (Variables|Inspect|GetIsInspecting?)
    (CallFunction|SetOffsetInspection (* ActionValue -2.0))))

(event Input|EnhancedActionEvents|EnhancedInputActionIA_Interact
  (params (ActionValue :type Boolean) (ElapsedSeconds :type Float%20%28double-precision%29) (TriggeredSeconds :type Float%20%28double-precision%29) (InputAction :type Input%20Action%20Object%20Reference :default "/Game/Inputs/Actions/IA_Interact.IA_Interact"))
  ;[1 1 1] Grab Item to move
  (:Started
    (Variables|Default|SetIsMouseLeftClicked? true))
  (:Canceled
    (Variables|Default|SetIsMouseLeftClicked? false :!label _label))
  (:Completed
    (goto _label)))

(event Input|EnhancedActionEvents|EnhancedInputActionIA_ReadItem
  (params (ActionValue :type Boolean) (ElapsedSeconds :type Float%20%28double-precision%29) (TriggeredSeconds :type Float%20%28double-precision%29) (InputAction :type Input%20Action%20Object%20Reference :default "/Game/Inputs/Actions/IA_ReadItem.IA_ReadItem"))
  ;[1 1 1] Read Item Decription
  (:Started
    (if (Variables|Default|GetCanViewDescription?)
      (CallFunction|ViewItemDescription))))

(fn ConstructionScript
  (Components|StaticMesh|SetStaticMesh (Variables|Default|GetStaticMesh) (Variables|Default|GetInspectMesh)))

(fn CheckFinishedTimeline
  (if (not (Variables|Default|GetIsPlayingAnimation?))
    (if (Variables|Inspect|GetIsInspecting?)
      (Variables|Default|SetCanViewDescription? true)
      (else
        (Variables|Default|SetCanViewDescription? false)
        (Components|Activation|Activate (Variables|Default|GetNiagara) true)
        (Collision|SetCollisionEnabled (Variables|Default|GetStaticMesh) "QueryAndPhysics")
        (Class|IPlayerUtils|CallonEndInteract(Message) (Variables|Default|GetPlayer%20Ref) (.CanBeAddedToInventory? (Utilities|Struct|BreakS_DataItem (Variables|Default|GetItemData))) (Variables|Default|GetItemsRowName))))))

(fn CheckifAlreadyTaken
  (bind _saveddata (Class|ISaveGame|GetGameData(Message) (Game|GetGameInstance)))
  (if (Utilities|Array|ContainsItem (.itemstaken (Variables|/Game/Blueprint/SaveGame/BP_GameData.BP_GameData_C|GetInventoryDiaryData _saveddata)) (Variables|Default|GetItemsRowName))
    (Utilities|IsValid self
      (:Is%20Valid
        (Actor|DestroyActor)))))

(fn FromCameratoInsidePlayer
  (params (Alpha :type Float%20%28single-precision%29))
  (bind _playercamera (Variables|Default|GetPlayerCamera))
  (bind _returnvalue (Math|Vector|GetForwardVector _playercamera))
  (Transformation|SetActorLocation (Math|Vector|Lerp(Vector) (Transformation|GetActorLocation) (- (+ (Transformation|GetWorldLocation _playercamera) _returnvalue) (Math|Vector|MakeVector (* (Math|Float|Sign(Float) (.X (Math|Vector|BreakVector _returnvalue))) 5e+01) 0.0 5e+01)) Alpha) false false))

(fn AddItemtoInventory
  (Variables|Inspect|SetIsInspecting? false)
  (Class|IPlayerUtils|CallonEndInteract(Message) (Variables|Default|GetPlayer%20Ref) (.CanBeAddedToInventory? (Utilities|Struct|BreakS_DataItem (Variables|Default|GetItemData))) (Variables|Default|GetItemsRowName)))

(fn EnableInputto
  (params (Actor :type Actor%20Object%20Reference))
  (bind _returnvalue (Game|GetPlayerController 0))
  (Input|DisableInput (Variables|Default|GetPlayer%20Ref) _returnvalue)
  (Input|EnableInput Actor _returnvalue))

(fn ViewItemDescription
  (bind _itemdata (Variables|Default|GetItemData))
  (bind (_name _description) (Utilities|Struct|BreakS_DataItem _itemdata))
  (Class|IPlayerUtils|SetInspectText(Message) (Variables|Default|GetPlayer%20Ref) _name _description)
  (Variables|Default|SetIsVisibleDescription? (not (Variables|Default|GetIsVisibleDescription?))))

(fn SetInspectionVariables
  (bind _playercamera (Variables|Default|GetPlayerCamera))
  (bind _output_get (Variables|Inspect|SetInspectPosition (+ (Transformation|GetWorldLocation _playercamera) (* (Math|Vector|GetForwardVector _playercamera) (+ (.InspectionDistance (Utilities|Struct|BreakS_DataItem (Variables|Default|GetItemData))) (Variables|Inspect|GetStartInspectDistance))))))
  (Variables|Default|SetNextZoomLerpPos _output_get)
  (Variables|Inspect|SetInspectRotation (Math|Conversions|RotationFromXVector (* (Math|Vector|GetForwardVector _playercamera) -1))))

(fn ManageLerpZoom
  (params (DeltaTime :type Float%20%28double-precision%29))
  (Transformation|SetActorLocation (Math|Vector|Lerp(Vector) (Transformation|GetActorLocation) (Variables|Default|GetNextZoomLerpPos) (* DeltaTime (Variables|Default|GetZoomLerpSpeed))) false false))

(fn ManageFieldOfView
  (Class|IPlayerUtils|ChangePPDepthOfField(Message) (Game|Player|GetPlayerPawn 0) (* (* (Math|Vector|Distance(Vector) (Transformation|GetWorldLocation (Variables|Default|GetPivot)) (Transformation|GetWorldLocation (Variables|Default|GetPlayerCamera))) 0.5) 1.6)))

(fn PlayLerpingAnimation
  (params (NextPosition :type Vector) (NextRotation :type Rotator))
  (Actor|Tick|SetActorTickEnabled true)
  (Variables|Default|SetEndAnimationPos NextPosition)
  (Variables|Default|SetStartAnimationPos (Transformation|GetWorldLocation (Variables|Default|GetPivot)))
  (Variables|Default|SetEndAnimationRot NextRotation)
  (Variables|Default|SetStartAnimationRot (Transformation|GetWorldRotation (Variables|Default|GetPivot)))
  (Variables|Default|SetIsPlayingAnimation? true)
  (Variables|Default|SetCounterInspectAnimation 0.0))

(fn LoopLerpingAnimation
  (params (DeltaTime :type Float%20%28double-precision%29))
  (Variables|Default|SetCounterInspectAnimation (+ (Variables|Default|GetCounterInspectAnimation) DeltaTime))
  (Transformation|SetWorldLocationAndRotation (Variables|Default|GetPivot) (Math|Vector|Lerp(Vector) (Variables|Default|GetStartAnimationPos) (Variables|Default|GetEndAnimationPos) (/ (Variables|Default|GetCounterInspectAnimation) (Variables|Default|GetTimerInspectAnimation))) (Math|Rotator|Lerp(Rotator) (Variables|Default|GetStartAnimationRot) (Variables|Default|GetEndAnimationRot) (/ (Variables|Default|GetCounterInspectAnimation) (Variables|Default|GetTimerInspectAnimation)) true) false false)
  (if (> (Variables|Default|GetCounterInspectAnimation) (Variables|Default|GetTimerInspectAnimation))
    (Default|CallOnFinishedInspectionAnimation)
    (Variables|Default|SetCounterInspectAnimation 0.0)
    (Variables|Default|SetIsPlayingAnimation? false)))

(fn ManageRotationLerp
  (params (DeltaTime :type Float%20%28double-precision%29))
  (Transformation|SetActorRotation (Math|Rotator|Lerp(Rotator) (Transformation|GetActorRotation) (Variables|Default|GetNextLerpedRotation) 1.0 true)))

(fn MouseRotateMesh
  (params (ActionValue :type Vector%202D%20Structure))
  (bind _returnvalue (* (.y ActionValue) 2.0))
  (bind _playercamera (Variables|Default|GetPlayerCamera))
  (bind _returnvalue_2 (Math|Vector|GetRightVector _playercamera))
  (bind _returnvalue_3 (* _returnvalue (.x _returnvalue_2)))
  (bind _returnvalue_4 (* _returnvalue (.y _returnvalue_2)))
  (bind _returnvalue_5 (Math|Rotator|MakeRotator _returnvalue_3 _returnvalue_4 0.0))
  (Class|Actor|AddActorWorldRotation (Math|Rotator|MakeRotator (.roll _returnvalue_5) (.pitch _returnvalue_5) (* (.x ActionValue) -2.0))))

(fn SetOffsetInspection
  (params (Value :type Float%20%28double-precision%29))
  (bind _playercamera (Variables|Default|GetPlayerCamera))
  (Variables|Inspect|SetStartInspectDistance (Math|Float|Clamp(Float) (+ Value (Variables|Inspect|GetStartInspectDistance)) (Variables|Inspect|GetMinInspectDistance) (Variables|Inspect|GetMaxInspectDistance)))
  (Variables|Default|SetNextZoomLerpPos (+ (Transformation|GetWorldLocation _playercamera) (* (Math|Vector|GetForwardVector _playercamera) (Variables|Inspect|GetStartInspectDistance)))))

(fn PickUp
  (params (PlayerRef :type Actor%20Object%20Reference))
  (bind _output_get (Variables|Default|SetPlayer%20Ref PlayerRef))
  (bind _cameraactorcomponent (Class|IPlayerUtils|GetCamera(Message) _output_get))
  (Variables|Default|SetPlayerCamera _cameraactorcomponent)
  (CallFunction|ManagePickUp)
  (if (== (Variables|Default|GetItemsRowName) "Default")
    _
    (else
      (Class|IPlayerUtils|AddedItemtoInventoryManage(Message) PlayerRef (Variables|Default|GetPreInspectDialogue) (Variables|Default|GetPostInspectDialogue) self)))
  (return (Variables|Default|GetItemData)))