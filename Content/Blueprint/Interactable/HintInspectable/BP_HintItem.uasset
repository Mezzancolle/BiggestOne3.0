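; Inspectable hint item whose mesh, text and inventory flag come from a DT_Items row, destroying itself if already taken.
; On pickup it takes over input and lerps in front of the player camera for rotation, zoom and description viewing.
; Tick drives the lerps and distance-based depth of field.
; On drop, it either joins the inventory with a shrink timeline before destruction, or lerps back and resets.
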(event Custom|ManagePickUp
  ;[1 1 1] PICKUP INTERFACE
  (Components|Activation|Deactivate (Variables|Default|GetNiagara))
  (Audio|PlaySound2D (Variables|Customization|GetInteractSound) 1.0 1.0 0.0 0 0)
  (CallFunction|EnableInputto self)
  (bind _itemactorcomponent (Class|IPlayerUtils|GetHoldingItem(Message) (Game|Player|GetPlayerPawn 0)))
  (Transformation|AttachComponentToComponent _itemactorcomponent "None" "KeepWorld" "KeepWorld" "KeepWorld" false)
  (Collision|SetActorEnableCollision false)
  (CallFunction|SetInspectionVariables)
  (Variables|Animation|SetIsInspecting? true)
  (CallFunction|SetOffsetInspection 1.0)
  (CallFunction|PlayLerpingAnimation (Variables|Camera|GetInspectPosition) (Variables|Camera|GetInspectRotation))
  ;;[1 0 0] TODO: add this when lerping animation ends
  (Utilities|FlowControl|Delay 0.2)
  (Variables|Animation|SetCanViewDescription? true))

(event Custom|SetItemToDefaultState
  ;[1 1 1] DROP ITEM TO THE GROUND
  (Actor|Tick|SetActorTickEnabled false)
  (Components|Activation|Activate (Variables|Default|GetNiagara) true)
  (Collision|SetActorEnableCollision true)
  (Class|IPlayerUtils|CallonEndInteract(Message) (Game|Player|GetPlayerPawn 0) false (Variables|Customization|GetItemsRowName))
  (EventDispatchers|UnbindEventfromOnFinishedInspectionLerping (delegate Custom|SetItemToDefaultState)))

(event Input|EnhancedActionEvents|EnhancedInputActionIA_Drop
  (params (ActionValue :type Boolean) (ElapsedSeconds :type Float%20%28double-precision%29) (TriggeredSeconds :type Float%20%28double-precision%29) (InputAction :type Input%20Action%20Object%20Reference :default "/Game/Inputs/Actions/IA_Drop.IA_Drop"))
  (bind _returnvalue (Game|Player|GetPlayerPawn 0))
  ;[1 1 1] DROP ITEM TO THE GROUND
  (Actor|Tick|SetActorTickEnabled false)
  (Variables|Animation|SetCanViewDescription? false)
  (Class|IPlayerUtils|ChangePPDepthOfField(Message) (Game|Player|GetPlayerPawn 0) 0.0)
  (if (Variables|Other|GetIsVisibleDescription?)
    (CallFunction|ViewItemDescription))
  (CallFunction|EnableInputto _returnvalue)
  (Class|IPlayerUtils|SwitchInputContext(Message) _returnvalue "/Game/Inputs/IMC_FirstPersonPlayer.IMC_FirstPersonPlayer" false)
  (Transformation|DetachFromActor "KeepWorld" "KeepWorld" "KeepWorld")
  (Variables|Animation|SetIsInspecting? false)
  (if (.CanBeAddedToInventory? (Utilities|Struct|BreakS_DataItem (Variables|Other|GetMyItemData)))
    ;;[0.5011 1 0.06198] Add Item To Inventory
    (Audio|PlaySound2D (Variables|Customization|GetPickupSound) 1.0 1.0 0.0 0 0)
    (CallFunction|AddItemtoInventory)
    (bind _alpha (Timeline|TL_AddToInventoryAnimation PlayFromStart)
      (:Update
        ;;;[1 0.3287 0.8674] TODO: add to tick / remove scale?
        (Transformation|SetActorScale3D (Math|Vector|Lerp(Vector) (Variables|Transformation|GetStartScale) "0, 0, 0" _alpha))
        ;;;[1 0 0] TODO: fix (read inside)
        (CallFunction|FromCameratoInsidePlayer _alpha))
      (:Finished
        (Utilities|IsValid self
          (:Is%20Valid
            (Actor|DestroyActor)))))
    (else
      (CallFunction|PlayLerpingAnimation (Variables|Transformation|GetStartPos) (Variables|Transformation|GetStartRot))
      (EventDispatchers|BindEventtoOnFinishedInspectionLerping (delegate Custom|SetItemToDefaultState)))))

(event EventTick
  (params (DeltaSeconds :type Float%20%28single-precision%29))
  ;[1 1 1] Tick
  (if (Variables|Animation|GetIsPlayingAnimation?)
    (CallFunction|LoopLerpingAnimation DeltaSeconds)
    (else
      (CallFunction|ManageLerpZoom DeltaSeconds)
      (CallFunction|ManageFieldOfView))))

(event EventBeginPlay
  ;[1 1 1] BEGIN PLAY
  (CallFunction|CheckifAlreadyTaken)
  (CallFunction|SetVariablesfromDataTable))

(event Input|EnhancedActionEvents|EnhancedInputActionIA_Look
  (params (ActionValue :type Vector%202D%20Structure) (ElapsedSeconds :type Float%20%28double-precision%29) (TriggeredSeconds :type Float%20%28double-precision%29) (InputAction :type Input%20Action%20Object%20Reference :default "/Game/Inputs/Actions/IA_Look.IA_Look"))
  ;[1 1 1] Mouse Inspect
  (if (Variables|Animation|GetIsInspecting?)
    (if (Variables|Input|GetIsMouseLeftClicked?)
      (CallFunction|MouseRotateMesh ActionValue))))

(event Input|EnhancedActionEvents|EnhancedInputActionIA_ZoomInspect
  (params (ActionValue :type Float%20%28double-precision%29) (ElapsedSeconds :type Float%20%28double-precision%29) (TriggeredSeconds :type Float%20%28double-precision%29) (InputAction :type Input%20Action%20Object%20Reference :default "/Game/Inputs/Actions/IA_ZoomInspect.IA_ZoomInspect"))
  ;[0.5339 0.5245 1] Zoom Inspect
  (if (Variables|Animation|GetIsInspecting?)
    (CallFunction|SetOffsetInspection (* ActionValue -2.0))))

(event Input|EnhancedActionEvents|EnhancedInputActionIA_Interact
  (params (ActionValue :type Boolean) (ElapsedSeconds :type Float%20%28double-precision%29) (TriggeredSeconds :type Float%20%28double-precision%29) (InputAction :type Input%20Action%20Object%20Reference :default "/Game/Inputs/Actions/IA_Interact.IA_Interact"))
  ;[1 1 1] Grab Item to move
  (:Started
    (Variables|Input|SetIsMouseLeftClicked? true))
  (:Canceled
    (Variables|Input|SetIsMouseLeftClicked? false :!label _label))
  (:Completed
    (goto _label)))

(event Input|EnhancedActionEvents|EnhancedInputActionIA_ReadItem
  (params (ActionValue :type Boolean) (ElapsedSeconds :type Float%20%28double-precision%29) (TriggeredSeconds :type Float%20%28double-precision%29) (InputAction :type Input%20Action%20Object%20Reference :default "/Game/Inputs/Actions/IA_ReadItem.IA_ReadItem"))
  ;[1 1 1] Read Item Decription
  (:Started
    (if (Variables|Animation|GetCanViewDescription?)
      (CallFunction|ViewItemDescription))))

(fn ConstructionScript
  (bind _returnvalue (Utilities|GetDataTableRow "/Game/Other/DataTables/DT_Items.DT_Items" (Variables|Customization|GetItemsRowName))
    (:then
      (bind _output_get (Variables|Other|SetMyItemData _returnvalue))
      (bind _returnvalue_2 (Utilities|LoadAssetBlocking (.StaticMesh (Utilities|Struct|BreakS_DataItem _output_get))))
      (Components|StaticMesh|SetStaticMesh (Variables|Default|GetStaticMesh) (.AsStatic%20Mesh (Utilities|Casting|CastToStaticMesh _returnvalue_2))))))

(fn CheckifAlreadyTaken
  (bind _saveddata (Class|ISaveGame|GetGameData(Message) (Game|GetGameInstance)))
  (if (Utilities|Array|ContainsItem (.itemstaken (Variables|/Game/Blueprint/SaveGame/BP_GameData.BP_GameData_C|GetInventoryDiaryData _saveddata)) (Variables|Customization|GetItemsRowName))
    (Utilities|IsValid self
      (:Is%20Valid
        (Actor|DestroyActor)))))

(fn EnableInputto
  (params (Actor :type Actor%20Object%20Reference))
  (bind _returnvalue (Game|GetPlayerController 0))
  (Input|DisableInput (Game|Player|GetPlayerPawn 0) _returnvalue)
  (Input|EnableInput Actor _returnvalue))

(fn SetInspectionVariables
  (bind _playercamera (Variables|Default|GetPlayerCamera))
  (bind _output_get (Variables|Camera|SetInspectPosition (+ (Transformation|GetWorldLocation _playercamera) (* (Math|Vector|GetForwardVector _playercamera) (+ (.NearInspectDistanceOffset (Utilities|Struct|BreakS_DataItem (Variables|Other|GetMyItemData))) (Variables|Customization|GetCurrentInspectDistance))))))
  (Variables|Camera|SetNextZoomLerpPos _output_get)
  (Variables|Camera|SetInspectRotation (Math|Conversions|RotationFromXVector (* (Math|Vector|GetForwardVector _playercamera) -1))))

(fn PlayLerpingAnimation
  (params (NextPosition :type Vector) (NextRotation :type Rotator))
  (Actor|Tick|SetActorTickEnabled true)
  (Variables|Camera|SetEndAnimationPos NextPosition)
  (Variables|Camera|SetStartAnimationPos (Transformation|GetWorldLocation (Variables|Default|GetPivot)))
  (Variables|Camera|SetEndAnimationRot NextRotation)
  (Variables|Camera|SetStartAnimationRot (Transformation|GetWorldRotation (Variables|Default|GetPivot)))
  (Variables|Animation|SetIsPlayingAnimation? true)
  (Variables|Animation|SetCounterInspectLerp 0.0))

(fn SetOffsetInspection
  (params (Value :type Float%20%28double-precision%29))
  (bind _playercamera (Variables|Default|GetPlayerCamera))
  (Variables|Customization|SetCurrentInspectDistance (Math|Float|Clamp(Float) (+ Value (Variables|Customization|GetCurrentInspectDistance)) (Variables|Customization|GetNearInspectDistance) (Variables|Customization|GetFarInspectDistance)))
  (Variables|Camera|SetNextZoomLerpPos (+ (Transformation|GetWorldLocation _playercamera) (* (Math|Vector|GetForwardVector _playercamera) (Variables|Customization|GetCurrentInspectDistance)))))

(fn ManageLerpZoom
  (params (DeltaTime :type Float%20%28double-precision%29))
  (Transformation|SetActorLocation (Math|Vector|Lerp(Vector) (Transformation|GetActorLocation) (Variables|Camera|GetNextZoomLerpPos) (* DeltaTime (Variables|Animation|GetZoomLerpSpeed))) false false))

(fn ManageFieldOfView
  (Class|IPlayerUtils|ChangePPDepthOfField(Message) (Game|Player|GetPlayerPawn 0) (+ (Math|Float|MapRangeClamped (Math|Vector|Distance(Vector) (Transformation|GetWorldLocation (Variables|Default|GetPlayerCamera)) (Transformation|GetWorldLocation (Variables|Default|GetPivot))) (Variables|Customization|GetNearInspectDistance) (Variables|Customization|GetFarInspectDistance) 0.0 1.0) (Variables|Default|GetFocalDistanceOffset))))

(fn LoopLerpingAnimation
  (params (DeltaTime :type Float%20%28double-precision%29))
  (Variables|Animation|SetCounterInspectLerp (+ DeltaTime (Variables|Animation|GetCounterInspectLerp)))
  (Transformation|SetWorldLocationAndRotation (Variables|Default|GetPivot) (Math|Vector|Lerp(Vector) (Variables|Camera|GetStartAnimationPos) (Variables|Camera|GetEndAnimationPos) (/ (Variables|Animation|GetCounterInspectLerp) (Variables|Animation|GetTimerInspectLerp))) (Math|Rotator|Lerp(Rotator) (Variables|Camera|GetStartAnimationRot) (Variables|Camera|GetEndAnimationRot) (/ (Variables|Animation|GetCounterInspectLerp) (Variables|Animation|GetTimerInspectLerp)) true) false false)
  ;[1 1 1] OnFinishLerping
  (if (> (Variables|Animation|GetCounterInspectLerp) (Variables|Animation|GetTimerInspectLerp))
    (Variables|Animation|SetCounterInspectLerp 0.0)
    (Variables|Animation|SetIsPlayingAnimation? false)
    (Default|CallOnFinishedInspectionLerping)))

(fn FromCameratoInsidePlayer
  (params (Alpha :type Float%20%28single-precision%29))
  (bind _playercamera (Variables|Default|GetPlayerCamera))
  (bind _returnvalue (Math|Vector|GetForwardVector _playercamera))
  (Transformation|SetActorLocation (Math|Vector|Lerp(Vector) (Transformation|GetActorLocation) (- (+ (Transformation|GetWorldLocation _playercamera) _returnvalue) (Math|Vector|MakeVector (* (Math|Float|Sign(Float) (.X (Math|Vector|BreakVector _returnvalue))) 5e+01) 0.0 5e+01)) Alpha) false false))

(fn AddItemtoInventory
  (Class|IPlayerUtils|CallonEndInteract(Message) (Game|Player|GetPlayerPawn 0) true (Variables|Customization|GetItemsRowName)))

(fn ViewItemDescription
  (bind _myitemdata (Variables|Other|GetMyItemData))
  (bind (_name _description) (Utilities|Struct|BreakS_DataItem _myitemdata))
  (Class|IPlayerUtils|SetInspectText(Message) (Game|Player|GetPlayerPawn 0) _name _description)
  (Variables|Other|SetIsVisibleDescription? (not (Variables|Other|GetIsVisibleDescription?))))

(fn MouseRotateMesh
  (params (ActionValue :type Vector%202D%20Structure))
  (bind _returnvalue (* (.y ActionValue) 2.0))
  (bind _playercamera (Variables|Default|GetPlayerCamera))
  (bind _returnvalue_2 (Math|Vector|GetRightVector _playercamera))
  (bind _returnvalue_3 (* _returnvalue (.x _returnvalue_2)))
  (bind _returnvalue_4 (* _returnvalue (.y _returnvalue_2)))
  (bind _returnvalue_5 (Math|Rotator|MakeRotator _returnvalue_3 _returnvalue_4 0.0))
  (Class|Actor|AddActorWorldRotation (Math|Rotator|MakeRotator (.roll _returnvalue_5) (.pitch _returnvalue_5) (* (.x ActionValue) -2.0))))

(fn SetVariablesfromDataTable
  (bind _pivot (Variables|Default|GetPivot))
  (bind _returnvalue (Utilities|GetDataTableRow "/Game/Other/DataTables/DT_Items.DT_Items" (Variables|Customization|GetItemsRowName))
    (:then
      (Variables|Other|SetMyItemData _returnvalue)
      (Variables|Customization|SetCurrentInspectDistance (* (+ (Variables|Customization|GetNearInspectDistance) (Variables|Customization|GetFarInspectDistance)) 0.5))
      (Variables|Transformation|SetStartScale (Transformation|GetActorScale3D))
      (Variables|Transformation|SetStartPos (Transformation|GetWorldLocation _pivot))
      (Variables|Transformation|SetStartRot (Transformation|GetWorldRotation _pivot))
      (if (not (Utilities|IsValidSoftObjectReference (.StaticMesh (Utilities|Struct|BreakS_DataItem (Variables|Other|GetMyItemData)))))
        (Development|PrintString (Utilities|String|Append "ERROR 404: ITEM " (Utilities|String|ToString(Name) (Variables|Customization|GetItemsRowName)) " NOT FOUND") true true "(R=1.000000,G=0.000000,B=0.034441,A=1.000000)")
        (Actor|DestroyActor)))))

(fn PickUp
  (params (PlayerRef :type Actor%20Object%20Reference))
  (bind _itemsrowname (Variables|Customization|GetItemsRowName))
  (bind _cameraactorcomponent (Class|IPlayerUtils|GetCamera(Message) PlayerRef))
  (Variables|Default|SetPlayerCamera _cameraactorcomponent)
  (CallFunction|ManagePickUp)
  (if (Math|Boolean|ORBoolean (== _itemsrowname "Default") (== _itemsrowname "") (== _itemsrowname ""))
    _
    (else
      (Class|IPlayerUtils|AddedItemtoInventoryManage(Message) PlayerRef (Variables|Customization|GetPreInspectDialogue) (Variables|Customization|GetPostInspectDialogue) self)))
  (return (Variables|Other|GetMyItemData)))