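; Interactable chest Blueprint whose lid toggles open and closed each time it is interacted with.
; A FlipFlop on the Interact event alternately plays and reverses a timeline, whose alpha lerps the TopChest component's relative rotation between start and end rotators.
; The construction script derives both rotators from the lid's world roll, offsetting the end by 70 degrees and zeroing the other two axes.
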(event EventInteract
  (params (PlayerRef :type BP%20Main%20Character%20Object%20Reference) (LookingComponent :type Primitive%20Component%20Object%20Reference))
  (Utilities|FlowControl|FlipFlop
    (:A
      (bind _alpha (Timeline|TL_ChestAnim Play)
        (:Update
          (Transformation|SetRelativeRotation (Variables|Default|GetTopChest) (Math|Rotator|Lerp(Rotator) (Variables|Default|GetStartRot) (Variables|Default|GetLastRot) _alpha) false false))))
    (:B
      (Timeline|TL_ChestAnim Reverse))))

(fn ConstructionScript
  (bind _topchest (Variables|Default|GetTopChest))
  (bind _returnvalue (Transformation|GetWorldRotation _topchest))
  (|CallParentFunction)
  (Variables|Default|SetStartRot (Math|Rotator|MakeRotator (.roll _returnvalue) 0.0 0.0))
  (Variables|Default|SetLastRot (Math|Rotator|MakeRotator (- (.roll _returnvalue) 7e+01) 0.0 0.0)))