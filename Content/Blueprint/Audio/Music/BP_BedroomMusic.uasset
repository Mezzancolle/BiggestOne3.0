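; BP_BedroomMusic is a music actor that plays the guitar house theme while the player is in its overlap area.
; The first player entry starts the track; later overlaps fade it up on entry and down to near silence on exit with S-curves, rather than stopping it.
; A Lantern event alternates between adding and clearing submix effects through a FlipFlop.
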(event Custom|Lantern
  (Utilities|FlowControl|FlipFlop
    (:A
      (Class|AudioMixerBlueprintLibrary|AddSubmixEffect))
    (:B
      (Class|AudioMixerBlueprintLibrary|ClearSubmixEffects))))

(event Collision|EventActorBeginOverlap
  (params (OtherActor :type Actor%20Object%20Reference))
  (bind _housetheme_guitar (Variables|Default|GetHouseTheme_Guitar))
  (if (Actor|ActorHasTag OtherActor "Player")
    (if (Variables|Default|GetPlaying)
      (Audio|Components|Audio|AdjustVolume _housetheme_guitar 3.0 1.0 "SCurve" :!class /Script/Engine.AudioComponent)
      (else
        (Audio|Components|Audio|Play _housetheme_guitar 0.0)
        (Variables|Default|SetPlaying true)))))

(event Collision|EventActorEndOverlap
  (params (OtherActor :type Actor%20Object%20Reference))
  (if (Actor|ActorHasTag OtherActor "Player")
    (Audio|Components|Audio|AdjustVolume (Variables|Default|GetHouseTheme_Guitar) 4.0 0.002 "SCurve" :!class /Script/Engine.AudioComponent)))

(fn ConstructionScript)