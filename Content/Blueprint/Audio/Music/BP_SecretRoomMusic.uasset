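; Secret room music trigger that plays a violin house theme when the main character overlaps it.
; The first entry starts playback, and later entries fade the track back up with an S-curve.
; Leaving fades it to near silence rather than stopping it, so it keeps running.
; A Lantern event alternates between adding an age filter effect to the music submix and clearing that submix's effects.
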(event Custom|Lantern
  (Utilities|FlowControl|FlipFlop
    (:A
      (Class|AudioMixerBlueprintLibrary|AddSubmixEffect "/Engine/EngineSounds/Submixes/MusicSubmix.MusicSubmix" "/Engine/EngineSounds/Submixes/MusicAgeFilterSubmixPreset.MusicAgeFilterSubmixPreset"))
    (:B
      (Class|AudioMixerBlueprintLibrary|ClearSubmixEffects "/Engine/EngineSounds/Submixes/MusicSubmix.MusicSubmix"))))

(event Collision|EventActorBeginOverlap
  (params (OtherActor :type Actor%20Object%20Reference))
  (bind _housetheme_violin (Variables|Default|GetHouseTheme_Violin))
  (Utilities|Casting|CastToBP_MainCharacter OtherActor)
  (if (Variables|Default|GetPlaying)
    (Audio|Components|Audio|AdjustVolume _housetheme_violin 3.0 1.0 "SCurve" :!class /Script/Engine.AudioComponent)
    (else
      (Audio|Components|Audio|Play _housetheme_violin 0.0)
      (Variables|Default|SetPlaying true))))

(event Collision|EventActorEndOverlap
  (params (OtherActor :type Actor%20Object%20Reference))
  (Utilities|Casting|CastToBP_MainCharacter OtherActor)
  (Audio|Components|Audio|AdjustVolume (Variables|Default|GetHouseTheme_Violin) 4.0 0.002 "SCurve" :!class /Script/Engine.AudioComponent))

(fn ConstructionScript)