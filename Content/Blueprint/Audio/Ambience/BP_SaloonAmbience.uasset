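; Saloon ambience actor that plays an audio bed and random footstep sounds, audible while the lantern is active.
; The audio component fades in almost silent on BeginPlay, then lantern changes ramp its volume up or down and pause or resume a looping SFX timer.
; Each timer event adds a random delay, a chance roll and lantern/CanPlaySFX checks before playing steps at a random offset around SaloonLocator.
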(event Custom|AmbienceSFX
  ;[0.1373 0.1373 0.1373] SFX Random delay and chance
  (Utilities|FlowControl|Delay (Math|Random|RandomFloatinRange 3.0 15.0))
  (if (== (Math|Random|RandomIntegerinRange 0 3) 0)
    (if (Variables|Default|GetIs%20Lantern%20Enabled)
      (if (Variables|Default|GetCanPlaySFX)
        (Audio|PlaySoundatLocation "/Game/Audio/SFX/SFX_Env/Saloon/SFX_Env_Steps_CUE.SFX_Env_Steps_CUE" (+ (Transformation|GetActorLocation (Variables|Default|GetSaloonLocator)) (Math|Vector|MakeVector (Math|Random|RandomFloatinRange -5e+02 5e+02) (Math|Random|RandomFloatinRange -6e+02 6e+02) (Math|Random|RandomFloatinRange -2e+02 2e+02))) "0, 0, 0" 1.0 1.0 0.0 0 0 0 0)))))

(event Custom|OnLanternActive
  (params (IsLanternEnabled :type Boolean))
  (bind _randomsfx (Variables|Default|GetRandomSFX))
  (Variables|Default|SetIs%20Lantern%20Enabled IsLanternEnabled)
  (if (Variables|Default|GetIs%20Lantern%20Enabled)
    (Audio|Components|Audio|AdjustVolume (Variables|Components|GetAudioComponent) 1.5 1.0 "Linear" :!class /Script/Engine.AudioComponent)
    (Utilities|Time|UnpauseTimerbyHandle _randomsfx)
    (else
      (Audio|Components|Audio|AdjustVolume (Variables|Components|GetAudioComponent) 1.5 0.001 "Linear" :!class /Script/Engine.AudioComponent)
      (Utilities|Time|PauseTimerbyHandle _randomsfx))))

(event EventBeginPlay
  (Audio|Components|Audio|FadeIn (Variables|Components|GetAudioComponent) 1.0 0.002 0.0 "Linear" :!class /Script/Engine.AudioComponent)
  (bind _returnvalue (Utilities|Time|SetTimerbyEvent (delegate Custom|AmbienceSFX) 3.0 true))
  (Variables|Default|SetRandomSFX _returnvalue))

(fn ConstructionScript)