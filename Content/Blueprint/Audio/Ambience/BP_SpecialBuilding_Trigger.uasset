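; Trigger volume that switches the ambience audio when the player enters or leaves a special building.
; On begin and end overlap with player character 0, it sets NewLocation on the referenced Ambience object to a hardcoded location index for the building or back to the default of zero.
; It then calls CheckLocation on Ambience, which is left to handle the change.
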(event Collision|EventActorBeginOverlap
  (params (OtherActor :type Actor%20Object%20Reference))
  (bind _ambience (Variables|Default|GetAmbience))
  (if (== OtherActor (Game|GetPlayerCharacter 0))
    (Variables|/Game/Blueprint/Audio/Ambience/BP_TownAmbience.BP_TownAmbience_C|SetNewLocation _ambience 2)
    (Default|CheckLocation _ambience)))

(event Collision|EventActorEndOverlap
  (params (OtherActor :type Actor%20Object%20Reference))
  (bind _ambience (Variables|Default|GetAmbience))
  (if (== OtherActor (Game|GetPlayerCharacter 0))
    (Variables|/Game/Blueprint/Audio/Ambience/BP_TownAmbience.BP_TownAmbience_C|SetNewLocation _ambience 0)
    (Default|CheckLocation _ambience)))

(fn ConstructionScript)