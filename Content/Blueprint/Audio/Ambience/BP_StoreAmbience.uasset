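; BP_StoreAmbience is an ambient sound actor for a store, with loudness tied to whether a lantern is active.
; It fades its AudioComponent in at a near-silent level on BeginPlay.
; OnLanternActive stores the lantern state and linearly adjusts the volume up to full when enabled, or back to near silence when disabled.
; A RandomFloatPosNeg graph holds unused random-sign float logic.
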(event Custom|OnLanternActive
  (params (IsLanternEnabled :type Boolean))
  (Variables|Default|SetIs%20Lantern%20Enabled IsLanternEnabled)
  (if (Variables|Default|GetIs%20Lantern%20Enabled)
    (Audio|Components|Audio|AdjustVolume (Variables|Components|GetAudioComponent) 1.5 1.0 "Linear" :!class /Script/Engine.AudioComponent)
    (else
      (Audio|Components|Audio|AdjustVolume (Variables|Components|GetAudioComponent) 1.5 0.001 "Linear" :!class /Script/Engine.AudioComponent))))

(event EventBeginPlay
  (Audio|Components|Audio|FadeIn (Variables|Components|GetAudioComponent) 1.0 0.002 0.0 "Linear" :!class /Script/Engine.AudioComponent))

(fn ConstructionScript)