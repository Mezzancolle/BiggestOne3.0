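; Ambience controller for the Parris House, layering base, wooden room, guitar and violin audio with random creaks and thumps.
; Player overlaps with the indoor collision alternate through a FlipFlop between fading the layers in and lowering them to near silence.
; An active lantern leaves only the base layer audible and pauses the looping SFX timer.
; Leaving does not stop that timer, and lantern changes re-apply the mix without checking player presence.
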(event OnComponentBeginOverlap(IndoorCollision)
  (params (OverlappedComponent :type Primitive%20Component%20Object%20Reference) (OtherActor :type Actor%20Object%20Reference) (OtherComp :type Primitive%20Component%20Object%20Reference) (OtherBodyIndex :type Integer) (bFromSweep :type Boolean) (SweepResult :type Hit%20Result%20Structure%20%28by%20ref%29))
  (if (Actor|ActorHasTag OtherActor "Player")
    (Utilities|FlowControl|FlipFlop
      (:A
        (CallFunction|Triggered))
      (:B
        (CallFunction|Left)))))

(event Custom|Triggered
  (Utilities|FlowControl|Sequence
    (:then_0
      (Audio|Components|Audio|FadeIn (Variables|Default|GetAmb_House_Base) 1.0 1.0 0.0 "Linear" :!class /Script/Engine.AudioComponent)
      (Audio|Components|Audio|FadeIn (Variables|Default|GetAmb_WoodenRoom) 1.0 0.3 0.0 "Linear" :!class /Script/Engine.AudioComponent)
      (Audio|Components|Audio|FadeIn (Variables|Default|GetAmb_House_Guitar) 1.0 0.3 0.0 "Linear" :!class /Script/Engine.AudioComponent)
      (Audio|Components|Audio|FadeIn (Variables|Default|GetAmb_House_Violin) 1.0 0.002 0.0 "Linear" :!class /Script/Engine.AudioComponent)
      (bind _returnvalue (Utilities|Time|SetTimerbyEvent (delegate Custom|AmbienceSFX) 1.0 true))
      (Variables|Default|SetRandomSFX _returnvalue))
    (:then_1
      (if (Variables|Default|GetIs%20Lantern%20Enabled)
        (Utilities|FlowControl|Sequence
          (:then_0
            (Audio|Components|Audio|AdjustVolume (Variables|Default|GetAmb_House_Base) 1.5 1.0 "Sin" :!class /Script/Engine.AudioComponent)
            (Utilities|Time|PauseTimerbyHandle (Variables|Default|GetRandomSFX)))
          (:then_1
            (Audio|Components|Audio|AdjustVolume (Variables|Default|GetAmb_House_Guitar) 1.5 0.001 "Sin" :!class /Script/Engine.AudioComponent))
          (:then_2
            (Audio|Components|Audio|AdjustVolume (Variables|Default|GetAmb_WoodenRoom) 1.5 0.001 "Sin" :!class /Script/Engine.AudioComponent))
          (:then_3
            (Audio|Components|Audio|AdjustVolume (Variables|Default|GetAmb_House_Violin) 1.5 0.001 "Sin" :!class /Script/Engine.AudioComponent)))
        (else
          (Utilities|FlowControl|Sequence
            (:then_0
              (Audio|Components|Audio|AdjustVolume (Variables|Default|GetAmb_House_Base) 1.5 1.0 "Sin" :!class /Script/Engine.AudioComponent)
              (Utilities|Time|UnpauseTimerbyHandle (Variables|Default|GetRandomSFX)))
            (:then_1
              (Audio|Components|Audio|AdjustVolume (Variables|Default|GetAmb_House_Guitar) 1.5 1.0 "Sin" :!class /Script/Engine.AudioComponent))
            (:then_2
              (Audio|Components|Audio|AdjustVolume (Variables|Default|GetAmb_WoodenRoom) 1.5 0.5 "Sin" :!class /Script/Engine.AudioComponent))
            (:then_3
              (Audio|Components|Audio|AdjustVolume (Variables|Default|GetAmb_House_Violin) 1.5 1.0 "Sin" :!class /Script/Engine.AudioComponent))))))))

(event Custom|AmbienceSFX
  (bind _returnvalue (Transformation|GetActorLocation))
  (Utilities|FlowControl|Sequence
    (:then_0
      ;[0.1373 0.1373 0.1373] SFX Random delay and chance
      (Utilities|FlowControl|Delay (Math|Random|RandomFloatinRange 2.0 8.0))
      (if (== (Math|Random|RandomIntegerinRange 0 1) 0)
        (if (not (Variables|Default|GetIs%20Lantern%20Enabled))
          (if (Variables|Default|GetCanPlaySFX)
            (Audio|PlaySoundatLocation "/Game/Audio/SFX/SFX_Env/Misc/Wood/SFX_Env_WoodCreaking_Cue.SFX_Env_WoodCreaking_Cue" (+ _returnvalue (Math|Vector|MakeVector (Math|Random|RandomFloatinRange -4e+02 4e+02) (Math|Random|RandomFloatinRange -3.5e+02 3.5e+02) (Math|Random|RandomFloatinRange -2e+02 2e+02))) "0, 0, 0" 1.0 1.0 0.0 0 0 0 0)))))
    (:then_1
      (Utilities|FlowControl|Delay (Math|Random|RandomFloatinRange 5.0 15.0))
      (if (== (Math|Random|RandomIntegerinRange 0 1) 0)
        (if (not (Variables|Default|GetIs%20Lantern%20Enabled))
          (if (Variables|Default|GetCanPlaySFX)
            (Audio|PlaySoundatLocation "/Game/Audio/SFX/SFX_Env/Misc/Wood/SFX_Env_WoodThump_Cue.SFX_Env_WoodThump_Cue" (+ _returnvalue (Math|Vector|MakeVector (Math|Random|RandomFloatinRange -4e+02 4e+02) (Math|Random|RandomFloatinRange -3.5e+02 3.5e+02) (Math|Random|RandomFloatinRange -2e+02 2e+02))) "0, 0, 0" 1.0 1.0 0.0 0 0 0 0)))))))

(event Custom|OnLanternActive
  (params (IsLanternEnabled :type Boolean))
  (bind _randomsfx (Variables|Default|GetRandomSFX))
  (Variables|Default|SetIs%20Lantern%20Enabled IsLanternEnabled)
  (if (Variables|Default|GetIs%20Lantern%20Enabled)
    (Utilities|FlowControl|Sequence
      (:then_0
        (Audio|Components|Audio|AdjustVolume (Variables|Default|GetAmb_House_Base) 1.5 1.0 "Sin" :!class /Script/Engine.AudioComponent)
        (Utilities|Time|PauseTimerbyHandle _randomsfx))
      (:then_1
        (Audio|Components|Audio|AdjustVolume (Variables|Default|GetAmb_House_Guitar) 1.5 0.001 "Sin" :!class /Script/Engine.AudioComponent))
      (:then_2
        (Audio|Components|Audio|AdjustVolume (Variables|Default|GetAmb_WoodenRoom) 1.5 0.001 "Sin" :!class /Script/Engine.AudioComponent))
      (:then_3
        (Audio|Components|Audio|AdjustVolume (Variables|Default|GetAmb_House_Violin) 1.5 0.001 "Sin" :!class /Script/Engine.AudioComponent)))
    (else
      (Utilities|FlowControl|Sequence
        (:then_0
          (Audio|Components|Audio|AdjustVolume (Variables|Default|GetAmb_House_Base) 1.5 1.0 "Sin" :!class /Script/Engine.AudioComponent)
          (Utilities|Time|UnpauseTimerbyHandle _randomsfx))
        (:then_1
          (Audio|Components|Audio|AdjustVolume (Variables|Default|GetAmb_House_Guitar) 1.5 1.0 "Sin" :!class /Script/Engine.AudioComponent))
        (:then_2
          (Audio|Components|Audio|AdjustVolume (Variables|Default|GetAmb_WoodenRoom) 1.5 0.5 "Sin" :!class /Script/Engine.AudioComponent))
        (:then_3
          (Audio|Components|Audio|AdjustVolume (Variables|Default|GetAmb_House_Violin) 1.5 1.0 "Sin" :!class /Script/Engine.AudioComponent))))))

(event Custom|Left
  (Audio|Components|Audio|AdjustVolume (Variables|Default|GetAmb_House_Base) 0.3 0.001 "Sin" :!class /Script/Engine.AudioComponent)
  (Audio|Components|Audio|AdjustVolume (Variables|Default|GetAmb_WoodenRoom) 0.3 0.001 "Sin" :!class /Script/Engine.AudioComponent)
  (Audio|Components|Audio|AdjustVolume (Variables|Default|GetAmb_House_Guitar) 0.3 0.001 "Sin" :!class /Script/Engine.AudioComponent)
  (Audio|Components|Audio|AdjustVolume (Variables|Default|GetAmb_House_Violin) 0.3 0.001 "Sin" :!class /Script/Engine.AudioComponent))

(event Collision|EventActorBeginOverlap
  (params (OtherActor :type Actor%20Object%20Reference)))

(event EventTick
  (params (DeltaSeconds :type Float%20%28single-precision%29)))

(fn ConstructionScript)