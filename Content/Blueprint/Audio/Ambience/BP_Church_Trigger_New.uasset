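; BP_Church_Trigger_New is an audio trigger that toggles church ambience when the player character overlaps it.
; On each overlap it reads the current location from MainAmbience, switching location 0 to 2 and either 1 or 2 back to 0.
; It then has MainAmbience re-check its location and tells ChurchAmbience to enable SFX and trigger on entry, or disable SFX and leave on exit.
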(event Collision|EventActorBeginOverlap
  (params (OtherActor :type Actor%20Object%20Reference))
  (bind _mainambience (Variables|Default|GetMainAmbience))
  (bind _mainambience_2 (Variables|Default|GetMainAmbience))
  (bind _churchambience (Variables|Default|GetChurchAmbience))
  (if (== OtherActor (Game|GetPlayerCharacter 0))
    (switch int (Variables|/Game/Blueprint/Audio/Ambience/BP_TownAmbience.BP_TownAmbience_C|GetCurrentLocation (Variables|Default|GetMainAmbience))
      (:0
        (Variables|/Game/Blueprint/Audio/Ambience/BP_TownAmbience.BP_TownAmbience_C|SetNewLocation _mainambience_2 2)
        (Default|CheckLocation _mainambience_2)
        (Variables|/Game/Blueprint/Audio/Ambience/BP_Church_Amb.BP_Church_Amb_C|SetCanPlaySFX _churchambience true)
        (Default|Triggered _churchambience))
      (:1
        (Variables|/Game/Blueprint/Audio/Ambience/BP_TownAmbience.BP_TownAmbience_C|SetNewLocation _mainambience 0 :!label _label)
        (Default|CheckLocation _mainambience)
        (Variables|/Game/Blueprint/Audio/Ambience/BP_Church_Amb.BP_Church_Amb_C|SetCanPlaySFX _churchambience false)
        (Default|Left _churchambience))
      (:2
        (goto _label)))))

(fn ConstructionScript)