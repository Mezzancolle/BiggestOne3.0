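; Town ambience actor for the past setting that fades in outdoor and indoor 2D beds on BeginPlay, the indoor one nearly silent.
; CheckLocation crossfades the beds when NewLocation changes, enabling random SFX outdoors and blocking them indoors.
; AmbienceSFX rolls delayed chances to play bird, dog and fly sounds offset around the player.
; The looping timer meant to drive AmbienceSFX is disconnected, so this graph never starts it.
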(event Custom|CheckLocation
  (bind _amb_outdoor (Variables|Default|GetAmb_Outdoor))
  (bind _amb_indoor (Variables|Default|GetAmb_indoor))
  (bind _fade_duration (Variables|Default|GetFade_Duration))
  (bind _fade_curve (Variables|Default|GetFade_Curve))
  (bind _randomsfxtimer (Variables|Default|GetRandomSFXTimer))
  (bind _newlocation (Variables|Default|GetNewLocation))
  ;[0.1373 0.1373 0.1373] IndoorSwitch
  (if (!= (Variables|Default|GetCurrentLocation) _newlocation)
    (switch int _newlocation
      (:0
        (Audio|Components|Audio|AdjustVolume _amb_outdoor _fade_duration 1.0 _fade_curve :!class /Script/Engine.AudioComponent)
        (Audio|Components|Audio|AdjustVolume _amb_indoor _fade_duration 0.001 _fade_curve :!class /Script/Engine.AudioComponent)
        (Variables|Default|SetCurrentLocation 0)
        (Utilities|Time|UnpauseTimerbyHandle _randomsfxtimer)
        (Variables|Default|SetCanPlaySFX true))
      (:1
        (Audio|Components|Audio|AdjustVolume _amb_outdoor _fade_duration 0.001 _fade_curve :!class /Script/Engine.AudioComponent)
        (Audio|Components|Audio|AdjustVolume _amb_indoor _fade_duration 1.0 _fade_curve :!class /Script/Engine.AudioComponent)
        (Variables|Default|SetCurrentLocation 1)
        (Utilities|Time|PauseTimerbyHandle _randomsfxtimer)
        (Variables|Default|SetCanPlaySFX false)))))

(event Custom|AmbienceSFX
  (bind _returnvalue (Game|GetPlayerCharacter 0))
  (bind _canplaysfx (Variables|Default|GetCanPlaySFX))
  (bind _returnvalue_2 (Transformation|GetActorLocation _returnvalue))
  (Utilities|FlowControl|Sequence
    (:then_0
      ;[0.1373 0.1373 0.1373] SFX Random delay and chance
      (Utilities|FlowControl|Delay (Math|Random|RandomFloatinRange 5.0 1e+01))
      (if (== (Math|Random|RandomIntegerinRange 0 2) 0)
        (if _canplaysfx
          (Audio|PlaySoundatLocation "/Game/Audio/SFX/SFX_Env/Town/SFX_Env_Birds_CUE.SFX_Env_Birds_CUE" (+ _returnvalue_2 (Math|Vector|MakeVector (Utilities|RandomFloatPosNeg 8e+02 2e+03) (Utilities|RandomFloatPosNeg 8e+02 2e+03) (Math|Random|RandomFloatinRange 8e+02 2e+03))) "0, 0, 0" 1.0 1.0 0.0 0 0 0 0))))
    (:then_1
      (Utilities|FlowControl|Delay (Math|Random|RandomFloatinRange 5.0 15.0))
      (if (== (Math|Random|RandomIntegerinRange 0 3) 0)
        (if _canplaysfx
          (Audio|PlaySoundatLocation "/Game/Audio/SFX/SFX_Env/Town/SFX_Env_Dogs_CUE.SFX_Env_Dogs_CUE" (+ _returnvalue_2 (Math|Vector|MakeVector (Utilities|RandomFloatPosNeg 5e+03 8e+03) (Utilities|RandomFloatPosNeg 5e+03 8e+03) 0.0)) "0, 0, 0" 1.0 1.0 0.0 0 0 0 0))))
    (:then_2
      (Utilities|FlowControl|Delay (Math|Random|RandomFloatinRange 7.0 12.0))
      (if (== (Math|Random|RandomIntegerinRange 0 2) 0)
        (if _canplaysfx
          (Audio|PlaySoundatLocation "/Game/Audio/SFX/SFX_Env/Town/SFX_Env_Fly_CUE.SFX_Env_Fly_CUE" (+ _returnvalue_2 (Math|Vector|MakeVector (Utilities|RandomFloatPosNeg 0.0 2e+02) (Utilities|RandomFloatPosNeg 0.0 2e+02) 0.0)) "0, 0, 0" 1.0 1.0 0.0 0 0 0 0))))))

(event EventBeginPlay
  (Utilities|FlowControl|Sequence
    (:then_0
      (bind _returnvalue (Audio|SpawnSound2D "/Game/Audio/Ambience/Amb_TownPast.Amb_TownPast" 1.0 1.0 0.0 0))
      (bind _output_get (Variables|Default|SetAmb_Outdoor _returnvalue))
      (Audio|Components|Audio|FadeIn _output_get 5.0 1.0 0.0 "SCurve" :!class /Script/Engine.AudioComponent))
    (:then_1
      (bind _returnvalue_2 (Audio|SpawnSound2D "/Game/Audio/Ambience/Amb_TownPast_Indoor.Amb_TownPast_Indoor" 1.0 1.0 0.0 0))
      (bind _output_get_2 (Variables|Default|SetAmb_indoor _returnvalue_2))
      (Audio|Components|Audio|FadeIn _output_get_2 1.0 0.002 0.0 "Linear" :!class /Script/Engine.AudioComponent))))

(fn ConstructionScript)