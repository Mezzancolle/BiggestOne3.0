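; Sheriff's ambience actor that raises its audio bed while the lantern is active and fades it nearly silent otherwise.
; BeginPlay starts the bed very quietly and a looping timer, which lantern toggles pause or resume.
; The timer feeds a random delay and coin flip that, when lantern and CanPlaySFX flags allow, plays chain sounds at random offsets around a Locator actor.
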(event Custom|AmbienceSFX
  ;[0.1373 0.1373 0.1373] SFX Random delay and chance
  (Utilities|FlowControl|Delay (Math|Random|RandomFloatinRange 1.0 1e+01))
  (if (== (Math|Random|RandomIntegerinRange 0 1) 0)
    (if (Variables|Default|GetIs%20Lantern%20Enabled)
      (if (Variables|Default|GetCanPlaySFX)
        (Audio|PlaySoundatLocation "/Game/Audio/SFX/SFX_Env/Sheriffs/SFX_Chains_CUE.SFX_Chains_CUE" (+ (Transformation|GetActorLocation (Variables|Default|GetLocator)) (Math|Vector|MakeVector (Math|Random|RandomFloatinRange -2e+02 2e+02) (Math|Random|RandomFloatinRange -4e+02 4e+02) (Math|Random|RandomFloatinRange -2e+02 2e+02))) "0, 0, 0" 1.0 1.0 0.0 0 0 0 0)))))

(event Custom|OnLanternActive
  (params (IsLanternEnabled :type Boolean))
  (bind _randomsfx (Variables|Default|GetRandomSFX))
  (Variables|Default|SetIs%20Lantern%20Enabled IsLanternEnabled)
  (if (Variables|Default|GetIs%20Lantern%20Enabled)
    (Audio|Components|Audio|AdjustVolume (Variables|Components|GetAudioComponent) 1.5 1.0 "Linear" :!class /Script/Engine.AudioComponent)
    (Utilities|Time|UnpauseTimerbyHandle _randomsfx)
    (else
      (Audio|Components|Audio|AdjustVolume (Variables|Components|GetAudioComponent) 1.5 0.001 "Linear" :!class /Script/Engine.AudioComponent)
      (Utilities|Time|PauseTimerbyHandle _randomsfx))))

(event EventBeginPlay
  (Audio|Components|Audio|FadeIn (Variables|Components|GetAudioComponent) 1.0 0.002 0.0 "Linear" :!class /Script/Engine.AudioComponent)
  (bind _returnvalue (Utilities|Time|SetTimerbyEvent (delegate Custom|AmbienceSFX) 0.1 true))
  (Variables|Default|SetRandomSFX _returnvalue))

(fn ConstructionScript)