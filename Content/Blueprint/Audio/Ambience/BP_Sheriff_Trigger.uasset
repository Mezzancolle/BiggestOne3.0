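; BP_Sheriff_Trigger is a trigger actor that switches ambient audio as the player enters or leaves the sheriff area.
; On player overlap begin and end, it sets the location index on MainAmbience and calls CheckLocation to update the ambience.
; It also toggles SheriffAmbience's CanPlaySFX flag, so sheriff-specific sound effects are allowed only while the player is inside.
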(event Collision|EventActorBeginOverlap
  (params (OtherActor :type Actor%20Object%20Reference))
  (bind _mainambience (Variables|Default|GetMainAmbience))
  (if (== OtherActor (Game|GetPlayerCharacter 0))
    (Variables|/Game/Blueprint/Audio/Ambience/BP_TownAmbience.BP_TownAmbience_C|SetNewLocation _mainambience 1)
    (Default|CheckLocation _mainambience)
    (Variables|/Game/Blueprint/Audio/Ambience/BP_SheriffsAmbience.BP_SheriffsAmbience_C|SetCanPlaySFX (Variables|Default|GetSheriffAmbience) true)))

(event Collision|EventActorEndOverlap
  (params (OtherActor :type Actor%20Object%20Reference))
  (bind _mainambience (Variables|Default|GetMainAmbience))
  (if (== OtherActor (Game|GetPlayerCharacter 0))
    (Variables|/Game/Blueprint/Audio/Ambience/BP_TownAmbience.BP_TownAmbience_C|SetNewLocation _mainambience 0)
    (Default|CheckLocation _mainambience)
    (Variables|/Game/Blueprint/Audio/Ambience/BP_SheriffsAmbience.BP_SheriffsAmbience_C|SetCanPlaySFX (Variables|Default|GetSheriffAmbience) false)))

(fn ConstructionScript)