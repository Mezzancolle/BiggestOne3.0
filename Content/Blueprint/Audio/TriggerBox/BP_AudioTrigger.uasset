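; Audio trigger actor that plays its Audio component's sound and provides events to fade it out or remove the trigger.
; Play starts the sound, waits for its duration, then calls FadeAndStopAudio, which fades and stops it only if IsPlayerInside is false after the delay.
; DestroyTrigger runs the same fade and destroys the actor after the fade time.
; No overlap handling or setter for IsPlayerInside appears here.
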(event Custom|FadeAndStopAudio
  (params (FadeOutDuration :type Float%20%28single-precision%29))
  (bind _audio (Variables|Default|GetAudio))
  (Audio|Components|Audio|FadeOut _audio FadeOutDuration 0.0 "Linear" :!class /Script/Engine.AudioComponent)
  (Utilities|FlowControl|Delay FadeOutDuration)
  (if (not (Variables|Default|GetIsPlayerInside?))
    (Audio|Components|Audio|Stop _audio)))

(event Custom|DestroyTrigger
  (params (FadeOutDuration :type Float%20%28single-precision%29))
  (Variables|Default|SetIsDestroying? false)
  (CallFunction|FadeandStopAudio FadeOutDuration)
  (Utilities|FlowControl|Delay FadeOutDuration)
  (Actor|DestroyActor))

(event Custom|Play
  (bind _audio (Variables|Default|GetAudio))
  (Audio|Components|Audio|Play _audio 0.0)
  (Utilities|FlowControl|Delay (Variables|/Script/Engine.SoundBase|GetDuration (Variables|/Script/Engine.AudioComponent|GetSound _audio)))
  (CallFunction|FadeandStopAudio 1.0))

(fn ConstructionScript)

(fn NewFunction)