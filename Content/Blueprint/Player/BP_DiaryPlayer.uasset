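; The player's inspectable 3D diary, an animated book with Whispers, Ghosts and Inventory sections.
; Each Tick copies the section widgets' render targets into dynamic page materials on the book mesh.
; Arrow clicks or input actions call TurnPage, which checks cooldown and CanBeClosed, drives ABP_Book and switches widget messages and collision.
; It also spawns inventory items for inspection while scaling the book, and forwards save/load to the widgets.
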(event Custom|GhostsSection
  (CallFunction|TurnPage 1)
  (CallFunction|WaittoChangePage))

(event Custom|InventorySection
  (CallFunction|TurnPage 2)
  (CallFunction|WaittoChangePage))

(event Custom|Close
  (bind _diaryanimationbp (Variables|Default|GetDiaryAnimationBP))
  (bind _ghostlyoverlay (Variables|Default|GetGhostlyOverlay))
  (Utilities|FlowControl|Sequence
    (:then_0
      (Default|ResetSelection (Variables|Default|GetWBP%20Arrows))
      (Variables|Default|SetCurrentWidget 0)
      (Collision|SetActorEnableCollision false)
      (Variables|/Game/Assets/Models/Book/Anims/ABP_Book.ABP_Book_C|SetPage%20Number (Variables|Default|GetDiaryAnimationBP) 0)
      (Variables|/Game/Assets/Models/Book/Anims/ABP_Book.ABP_Book_C|SetInteracting? _diaryanimationbp false)
      (Variables|/Game/Assets/Models/Book/Anims/ABP_Book.ABP_Book_C|SetClosing? _diaryanimationbp true)
      (Class|ISwitchUIDiaryWidget|OnExit(Message) (UserInterface|GetUserWidgetObject (Variables|Default|GetWBP_Inventory)))
      (Class|ISwitchUIDiaryWidget|OnExit(Message) (UserInterface|GetUserWidgetObject (Variables|Default|GetWBP_Ghosts)))
      (Class|ISwitchUIDiaryWidget|OnExit(Message) (UserInterface|GetUserWidgetObject (Variables|Default|GetWBP_Whispers)))
      (Class|IPlayerUtils|SetInsideDiary(Message) (Game|Player|GetPlayerPawn 0) false))
    (:then_1
      (Development|SetHiddeninGame _ghostlyoverlay true true)
      (Rendering|SetVisibility _ghostlyoverlay true true))))

(event Custom|BackToDiaryInventory
  (params (DestroyedActor :type Actor%20Object%20Reference))
  (Utilities|FlowControl|Sequence
    (:then_0
      (Variables|Default|SetIsGoingBackFromInspection? true))
    (:then_1
      (bind _alpha (Timeline|TL_BackDiary ReverseFromEnd)
        (:Update
          (Transformation|SetRelativeScale3D (Variables|Default|GetDiary) (Math|Vector|MakeVector (Math|Float|Lerp 0.11 0.09 _alpha) (Math|Float|Lerp 0.11 0.09 _alpha) (Math|Float|Lerp 0.11 0.09 _alpha))))
        (:Finished
          (if (Variables|Default|GetIsGoingBackFromInspection?)
            (Variables|Default|SetIsGoingBackFromInspection? false)
            (Development|SetHiddeninGame (Variables|Default|GetWBP_Arrows) false false)))))
    (:then_2
      (Development|SetHiddeninGame (Variables|Default|GetBGInspections) true false)
      (Collision|SetCollisionEnabled (Variables|Default|GetWBP_Inventory) "QueryAndPhysics"))
    (:then_3
      (Class|ISwitchUIDiaryWidget|OnEnter(Message) (UserInterface|GetUserWidgetObject (Variables|Default|GetWBP_Inventory))))))

(event Custom|WhispersSection
  (CallFunction|TurnPage)
  (CallFunction|WaittoChangePage))

(event Custom|WaitToChangePage
  (Utilities|FlowControl|Delay 0.5)
  (Variables|Default|SetCanTurnPage? true))

(event Custom|Open
  (params (LookingComponent :type Primitive%20Component%20Object%20Reference))
  (bind _widgets (Variables|Default|GetWidgets))
  (bind _output (Utilities|Array|Get(acopy) _widgets))
  (Utilities|FlowControl|Sequence
    (:then_0
      (Collision|SetActorEnableCollision true)
      (Collision|SetCollisionEnabled (Variables|Default|GetWBP_GhostSelection) "NoCollision")
      (Collision|SetCollisionEnabled (Variables|Default|GetWBP_ItemSelection) "NoCollision")
      (Collision|SetCollisionEnabled (Variables|Default|GetWBP_WhispersSelection) "QueryOnly")
      (Variables|/Game/Assets/Models/Book/Anims/ABP_Book.ABP_Book_C|SetClosing? (Variables|Default|GetDiaryAnimationBP) false)
      (Transformation|SetRelativeTransform (Variables|Default|GetCamera) (Variables|Default|GetStartCameraLocalTransform) false true)
      (Variables|Default|SetStartCameraLocation (Transformation|GetWorldLocation (Variables|Default|GetCamera)))
      (CallFunction|Interact)
      (CallFunction|LoadfromGameData)
      (Variables|/Game/Assets/Models/Book/Anims/ABP_Book.ABP_Book_C|SetPage%20Number (Variables|Default|GetDiaryAnimationBP) 0)
      (Variables|/Game/Assets/Models/Book/Anims/ABP_Book.ABP_Book_C|SetInteracting? (Variables|Default|GetDiaryAnimationBP) true)
      (Class|WidgetBlueprintLibrary|SetHardwareCursor "Default" "T_WestCursor" "(X=0.000000,Y=0.000000)")
      (Variables|Default|SetCanExitInspection? false)
      (Collision|SetCollisionEnabled (Utilities|Array|Get(acopy) (Variables|Default|GetWidgets) 1) "NoCollision")
      (Collision|SetCollisionEnabled _output "QueryOnly")
      (Class|ISwitchUIDiaryWidget|OnEnter(Message) (UserInterface|GetWidget _output))
      (Collision|SetCollisionEnabled (Utilities|Array|Get(acopy) (Variables|Default|GetWidgets) 2) "NoCollision"))
    (:then_1
      (Utilities|FlowControl|Delay 1.0)
      (bind _wbp_tutorialdiary (Variables|Default|GetWBP_TutorialDiary)
        (:then
          (switch Utilities|FlowControl|Switch|SwitchonESlateVisibility (Variables|/Script/UMG.Widget|GetVisibility _wbp_tutorialdiary)
            (:Visible
              _)
            (:HitTestInvisible
              _)
            (:SelfHitTestInvisible
              _))
          (UserInterface|Viewport|AddtoViewport _wbp_tutorialdiary 0))
        (:else)))))

(event Input|EnhancedActionEvents|EnhancedInputActionIA_ChangeDiaryPageRight
  (params (ActionValue :type Boolean) (ElapsedSeconds :type Float%20%28double-precision%29) (TriggeredSeconds :type Float%20%28double-precision%29) (InputAction :type Input%20Action%20Object%20Reference :default "/Game/Inputs/Actions/IA_ChangeDiaryPageRight.IA_ChangeDiaryPageRight"))
  (:Started
    (if (Variables|Default|GetCanTurnPage?)
      (CallFunction|TurnPage (Math|Integer|Clamp(Integer) (+ (Variables|Default|GetCurrentWidget) 1) 0 (- (Utilities|Array|Length (Variables|Default|GetWidgets)) 1)))
      (CallFunction|WaittoChangePage))))

(event Input|EnhancedActionEvents|EnhancedInputActionIA_ChangeDiaryPageLeft
  (params (ActionValue :type Boolean) (ElapsedSeconds :type Float%20%28double-precision%29) (TriggeredSeconds :type Float%20%28double-precision%29) (InputAction :type Input%20Action%20Object%20Reference :default "/Game/Inputs/Actions/IA_ChangeDiaryPageLeft.IA_ChangeDiaryPageLeft"))
  (:Started
    (if (Variables|Default|GetCanTurnPage?)
      (CallFunction|TurnPage (Math|Integer|Clamp(Integer) (- (Variables|Default|GetCurrentWidget) 1) 0 (- (Utilities|Array|Length (Variables|Default|GetWidgets)) 1)))
      (CallFunction|WaittoChangePage))))

(event Input|EnhancedActionEvents|EnhancedInputActionIA_ViewObject
  (params (ActionValue :type Vector%202D%20Structure) (ElapsedSeconds :type Float%20%28double-precision%29) (TriggeredSeconds :type Float%20%28double-precision%29) (InputAction :type Input%20Action%20Object%20Reference :default "/Game/Inputs/Actions/IA_ViewObject.IA_ViewObject"))
  (CallFunction|MoveMousewithGamepad true ActionValue (Game|GetPlayerController 0)))

(event EventInteract
  (params (LookingComponent :type Primitive%20Component%20Object%20Reference))
  (if (not (Variables|/Game/Assets/Models/Book/Anims/ABP_Book.ABP_Book_C|GetInteracting? (Variables|Default|GetDiaryAnimationBP)))
    (|CallParentFunction LookingComponent)))

(event EventTick
  (params (DeltaSeconds :type Float%20%28single-precision%29))
  (Rendering|Material|SetTextureParameterValue (Variables|Default|GetDMI_PagePrimary) "Widget" (Class|WidgetComponent|GetRenderTarget (Utilities|Array|Get(acopy) (Variables|Default|GetWidgets))))
  (Rendering|Material|SetTextureParameterValue (Variables|Default|GetDMI_PageSecondary) "Widget" (Class|WidgetComponent|GetRenderTarget (Utilities|Array|Get(acopy) (Variables|Default|GetWidgets) 1)))
  (Rendering|Material|SetTextureParameterValue (Variables|Default|GetDMI%20Page%20Third) "Widget" (Class|WidgetComponent|GetRenderTarget (Utilities|Array|Get(acopy) (Variables|Default|GetWidgets) 2))))

(event EventLoadfromGameData
  (Class|ISaveable|LoadfromGameData(Message) (UserInterface|GetWidget (Variables|Default|GetWBP_Ghosts)))
  (Class|ISaveable|LoadfromGameData(Message) (UserInterface|GetWidget (Variables|Default|GetWBP_Inventory)))
  (Class|ISaveable|LoadfromGameData(Message) (UserInterface|GetWidget (Variables|Default|GetWBP_Whispers))))

(event EventSavetoGameData
  (params (Async :type Boolean))
  (Class|ISaveable|SavetoGameData(Message) (UserInterface|GetWidget (Variables|Default|GetWBP_Ghosts)) Async)
  (Class|ISaveable|SavetoGameData(Message) (UserInterface|GetWidget (Variables|Default|GetWBP_Inventory)) Async))

(event EventInspectMesh
  (params (ItemRowName :type Name%20%28by%20ref%29 :default "None"))
  (bind _ispectingitemposition (Variables|Default|GetIspectingItemPosition))
  (bind _returnvalue (Transformation|GetWorldTransform _ispectingitemposition))
  (Utilities|FlowControl|Sequence
    (:then_0
      (Development|SetHiddeninGame (Variables|Default|GetBGInspections) false false)
      (Development|SetHiddeninGame (Variables|Default|GetWBP_Arrows) true false)
      (Collision|SetCollisionEnabled (Variables|Default|GetWBP_Inventory) "NoCollision")
      (bind _returnvalue_2 (Game|SpawnActorfromClass "/Game/Blueprint/Interactable/Inspectable/CBP_InventoryItem.CBP_InventoryItem_C" (Math|Transform|MakeTransform (.location _returnvalue) (.rotation _returnvalue) "1.000000,1.000000,1.000000") "AlwaysSpawn" "MultiplyWithRoot" 0 (Variables|Default|GetCamera) (Variables|Default|GetWBP_Inventory) ItemRowName 0))
      (Game|BindEventtoOnDestroyed _returnvalue_2 (delegate Custom|BackToDiaryInventory))
      (Default|EnableInspectUi _returnvalue_2)
      (Class|IPickUp|PickUp(Message) _returnvalue_2)
      (Class|IPlayerUtils|SwitchInputContext(Message) (Game|Player|GetPlayerPawn 0) "/Game/Inputs/IMC_Inspect.IMC_Inspect" false)
      (Class|IPlayerUtils|Open/CloseInspectTextUI(Message) (Game|Player|GetPlayerPawn 0) true))
    (:then_1
      (bind _alpha (Timeline|TL_BackDiary PlayFromStart)
        (:Update
          (Transformation|SetRelativeScale3D (Variables|Default|GetDiary) (Math|Vector|MakeVector (Math|Float|Lerp 0.11 0.09 _alpha) (Math|Float|Lerp 0.11 0.09 _alpha) (Math|Float|Lerp 0.11 0.09 _alpha))))
        (:Finished
          (if (Variables|Default|GetIsGoingBackFromInspection?)
            (Variables|Default|SetIsGoingBackFromInspection? false)
            (Development|SetHiddeninGame (Variables|Default|GetWBP_Arrows) false false)))))))

(event EventBeginPlay
  (Rendering|SetVisibility (Variables|Default|GetDiary) false true)
  (Variables|Default|SetStartCameraLocalTransform (Transformation|GetRelativeTransform (Variables|Default|GetCamera)))
  (|CallParentFunction)
  (CallFunction|DynamicMaterialCreation)
  (CallFunction|CreatingWidgetsArray)
  (CallFunction|LoadfromGameData)
  (bind _asabp_book (Utilities|Casting|CastToABP_Book (Components|SkeletalMesh|GetAnimInstance (Variables|Default|GetDiary))))
  (Variables|Default|SetDiaryAnimationBP _asabp_book)
  (bind _aswbp_arrows (Utilities|Casting|CastToWBP_Arrows (UserInterface|GetUserWidgetObject (Variables|Default|GetWBP_Arrows))))
  (Variables|Default|SetWBP%20Arrows _aswbp_arrows)
  (EventDispatchers|BindEventtoOnGhostsClicked _aswbp_arrows (delegate Custom|GhostsSection))
  (EventDispatchers|BindEventtoOnInventoryClicked _aswbp_arrows (delegate Custom|InventorySection))
  (EventDispatchers|BindEventtoOnWhispersClicked _aswbp_arrows (delegate Custom|WhispersSection)))

(event Input|KeyboardEvents|DebugKeyU
  (params (Key :type Key%20Structure :default "None") (ActionValue :type Input%20Action%20Value%20Structure))
  (:Pressed
    (bind _isa (Utilities|FlowControl|FlipFlop)
      (:A
        _)
      (:B
        _))
    (Development|SetHiddeninGame (Variables|Default|GetDiary) _isa false)))

(event Input|KeyboardEvents|DebugKeyH
  (params (Key :type Key%20Structure :default "None") (ActionValue :type Input%20Action%20Value%20Structure))
  (bind _returnvalue (Game|GetPlayerController 0))
  (bind _hitresult (Game|Player|GetHitResultUnderCursorbyChannel _returnvalue "TraceTypeQuery1" true))
  (:Pressed
    (if (.bblockinghit _hitresult)
      (Development|PrintText (Utilities|Text|FormatText "Hitted {component} in {actor}" (Utilities|GetDisplayName (.hitcomponent _hitresult)) (Utilities|GetDisplayName (.hitactor _hitresult)))))))

(event Input|KeyboardEvents|Multiply
  (params (Key :type Key%20Structure :default "None"))
  (bind _wbp_itemselection (Variables|Default|GetWBP_ItemSelection))
  (bind _wbp_whispersselection (Variables|Default|GetWBP_WhispersSelection))
  (bind _wbp_ghostselection (Variables|Default|GetWBP_GhostSelection))
  (:Pressed
    (Development|PrintText (Utilities|Text|FormatText "Whispers Selection Collisons {bool}" (Math|Boolean|ORBoolean (Class|PrimitiveComponent|IsCollisionEnabled _wbp_whispersselection) (Class|PrimitiveComponent|IsPhysicsCollisionEnabled _wbp_whispersselection) (Class|PrimitiveComponent|IsQueryCollisionEnabled _wbp_whispersselection))))
    (Development|PrintText (Utilities|Text|FormatText "Item Selection Collisons {bool}" (Math|Boolean|ORBoolean (Class|PrimitiveComponent|IsCollisionEnabled _wbp_itemselection) (Class|PrimitiveComponent|IsPhysicsCollisionEnabled _wbp_itemselection) (Class|PrimitiveComponent|IsQueryCollisionEnabled _wbp_itemselection))))
    (Development|PrintText (Utilities|Text|FormatText "Ghost Selection Collisons {bool}" (Math|Boolean|ORBoolean (Class|PrimitiveComponent|IsCollisionEnabled _wbp_ghostselection) (Class|PrimitiveComponent|IsPhysicsCollisionEnabled _wbp_ghostselection) (Class|PrimitiveComponent|IsQueryCollisionEnabled _wbp_ghostselection))))))

(fn ConstructionScript)

(fn CreatingWidgetsArray
  (bind _wbp_itemselection (Variables|Default|GetWBP_ItemSelection))
  (bind _wbp_inventory (Variables|Default|GetWBP_Inventory))
  (bind _wbp_ghosts (Variables|Default|GetWBP_Ghosts))
  (bind _wbp_whispers (Variables|Default|GetWBP_Whispers))
  (bind _returnvalue (UserInterface|GetUserWidgetObject _wbp_inventory))
  (bind _returnvalue_2 (UserInterface|GetWidget _wbp_itemselection))
  (bind _aswbp_inventory (Utilities|Casting|CastToWBP_Inventory _returnvalue))
  (bind _aswbp_item_selection (Utilities|Casting|CastToWBP_ItemSelection _returnvalue_2))
  (Utilities|FlowControl|Sequence
    (:then_0
      (Utilities|FlowControl|Sequence
        (:then_0
          (Utilities|Array|Add (Variables|Default|GetWidgets) _wbp_whispers)
          (Collision|SetCollisionEnabled _wbp_whispers "NoCollision")
          (bind _aswbp_whispers (Utilities|Casting|CastToWBP_Whispers (UserInterface|GetWidget _wbp_whispers)))
          (Variables|Default|SetWBP%20Whispers _aswbp_whispers)
          (bind _aswbp_whisper_selection (Utilities|Casting|CastToWBP_WhisperSelection (UserInterface|GetWidget (Variables|Default|GetWBP_WhispersSelection))))
          (Variables|/Game/UserInterfaces/DiaryUI/Whispers/WBP_Whispers.WBP_Whispers_C|SetWhispersSelection _aswbp_whispers _aswbp_whisper_selection))
        (:then_1
          (Utilities|Array|Add (Variables|Default|GetWidgets) _wbp_ghosts)
          (bind _aswbp_ghosts (Utilities|Casting|CastToWBP_Ghosts (UserInterface|GetWidget _wbp_ghosts)))
          (Variables|Default|SetWBP%20Ghosts _aswbp_ghosts)
          (bind _aswbp_ghost_slection (Utilities|Casting|CastToWBP_GhostSlection (UserInterface|GetWidget (Variables|Default|GetWBP_GhostSelection))))
          (Variables|/Game/UserInterfaces/DiaryUI/Ghosts/WBP_Ghosts.WBP_Ghosts_C|SetGhostSelection _aswbp_ghosts _aswbp_ghost_slection))
        (:then_2
          (Utilities|Array|Add (Variables|Default|GetWidgets) _wbp_inventory)
          (Collision|SetCollisionEnabled (Variables|Default|GetWBP_Inventory) "NoCollision")
          (Variables|Default|SetWBP_Inventorys _aswbp_inventory)
          (bind _output_get (Variables|/Game/UserInterfaces/DiaryUI/Inventory/WBP_Inventory.WBP_Inventory_C|SetItemSelection _aswbp_inventory _aswbp_item_selection))
          (Variables|/Game/UserInterfaces/DiaryUI/Inventory/WBP_ItemSelection.WBP_ItemSelection_C|SetDiaryInspector _output_get self)
          (Widget|SetVisibility _aswbp_item_selection "Collapsed"))))
    (:then_1
      (Variables|Default|SetWidgetSelections (Utilities|Array|MakeArray (Variables|Default|GetWBP_WhispersSelection) (Variables|Default|GetWBP_GhostSelection) (Variables|Default|GetWBP_ItemSelection))))))

(fn DynamicMaterialCreation
  (bind _diary (Variables|Default|GetDiary))
  (bind _returnvalue (Rendering|Material|CreateDynamicMaterialInstance _diary 2 "/Game/Assets/Models/NewestBook/M_WidgetDiaryPage.M_WidgetDiaryPage" "None" :!class /Script/Engine.PrimitiveComponent))
  (Variables|Default|SetDMI_PagePrimary _returnvalue)
  (bind _returnvalue_2 (Rendering|Material|CreateDynamicMaterialInstance _diary 3 "/Game/Assets/Models/NewestBook/M_WidgetDiaryPage.M_WidgetDiaryPage" "None" :!class /Script/Engine.PrimitiveComponent))
  (Variables|Default|SetDMI_PageSecondary _returnvalue_2)
  (bind _returnvalue_3 (Rendering|Material|CreateDynamicMaterialInstance _diary 4 "/Game/Assets/Models/NewestBook/M_WidgetDiaryPage.M_WidgetDiaryPage" "None" :!class /Script/Engine.PrimitiveComponent))
  (Variables|Default|SetDMI%20Page%20Third _returnvalue_3))

(fn PreInspectFadein
  (|CallParentFunction)
  (Rendering|SetVisibility (Variables|Default|GetDiary) true true))

(fn PostDropFadein)

(fn PreDropFadein
  (|CallParentFunction)
  (Rendering|SetVisibility (Variables|Default|GetDiary) false true)
  (CallFunction|Close))

(fn PostInspectFadein
  (|CallParentFunction)
  (Development|SetHiddeninGame (Variables|Default|GetWBP_Arrows) false false))

(fn BeforeBacktoPlayer
  (|CallParentFunction)
  (Development|SetHiddeninGame (Variables|Default|GetWBP_Arrows) true false))

(fn TurnPage
  (params (NextPage :type Integer))
  (if (Math|Boolean|ANDBoolean (Variables|Default|GetCanTurnPage?) (!= NextPage (Variables|Default|GetCurrentWidget)) (CallFunction|CanCloseInspection))
    (Utilities|FlowControl|Sequence
      (:then_0
        (Variables|/Game/Assets/Models/Book/Anims/ABP_Book.ABP_Book_C|SetReverse%20Page%20Turn? (Variables|Default|GetDiaryAnimationBP) (> (Class|KismetMathLibrary|SignOfInteger (- NextPage (Variables|Default|GetCurrentWidget))) 0))
        (Collision|SetCollisionEnabled (Utilities|Array|Get(acopy) (Variables|Default|GetWidgets) (Variables|Default|GetCurrentWidget)) "NoCollision")
        (Default|SetSelectedWidget (Variables|Default|GetWBP%20Arrows) NextPage)
        (bind _output_get (LocalVariables|SetNextCurrentWidget NextPage))
        (if (== _output_get (Variables|Default|GetCurrentWidget))
          (return)
          (else
            (Class|ISwitchUIDiaryWidget|OnExit(Message) (UserInterface|GetUserWidgetObject (Utilities|Array|Get(acopy) (Variables|Default|GetWidgets) (Variables|Default|GetCurrentWidget))))
            (Class|ISwitchUIDiaryWidget|OnEnter(Message) (UserInterface|GetUserWidgetObject (Utilities|Array|Get(acopy) (Variables|Default|GetWidgets) (LocalVariables|GetNextCurrentWidget))))
            (Collision|SetCollisionEnabled (Utilities|Array|Get(acopy) (Variables|Default|GetWidgets) (Variables|Default|GetCurrentWidget)) "NoCollision")
            (Collision|SetCollisionEnabled (Utilities|Array|Get(acopy) (Variables|Default|GetWidgets) (LocalVariables|GetNextCurrentWidget)) "QueryOnly")
            (bind _output_get_2 (Variables|Default|SetCurrentWidget (LocalVariables|GetNextCurrentWidget)))
            (Collision|SetCollisionEnabled (Utilities|Array|Get(acopy) (Variables|Default|GetWidgets) _output_get_2) "QueryOnly")
            (bind _output_get_3 (Variables|/Game/Assets/Models/Book/Anims/ABP_Book.ABP_Book_C|SetPage%20Number (Variables|Default|GetDiaryAnimationBP) _output_get_2))
            (for (_array_element _array_index) (Variables|Default|GetWidgetSelections)
              (if (== _array_index _output_get_3)
                (Collision|SetCollisionEnabled _array_element "QueryOnly")
                (else
                  (Collision|SetCollisionEnabled _array_element "NoCollision")))))))
      (:then_1
        (Variables|Default|SetCanTurnPage? false)))
    (else
      (Default|SetSelectedWidget (Variables|Default|GetWBP%20Arrows) (Variables|Default|GetCurrentWidget)))))

(fn SetArrowsCollisions
  (params (Enabled? :type Boolean))
  (bind _wbp_arrows (Variables|Default|GetWBP_Arrows))
  (if Enabled?
    (Collision|SetCollisionEnabled _wbp_arrows "QueryOnly")
    (else
      (Collision|SetCollisionEnabled _wbp_arrows "NoCollision"))))

(fn CanCloseInspection
  (bind _value (Default|CanbeClosed (Variables|Default|GetWBP%20Whispers)))
  (bind _value_2 (Default|CanbeClosed (Variables|Default|GetWBP%20Ghosts)))
  (bind _value_3 (Default|CanbeClosed (Variables|Default|GetWBP_Inventorys)))
  (return (Math|Boolean|ANDBoolean _value_3 _value_2 _value)))