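; Interactive player diary actor that shows Option, Inventory and Ghosts widgets as pages on an animated mesh; Interact enables mouse UI input.
; Each Tick copies primary and secondary widget render targets into two dynamic page materials.
; Arrow-widget clicks cycle the wrapping indices and play one flip animation, forward for left, reversed for right.
; Collision profiles are swapped during flips to move UI interaction to the new page.
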(event Custom|OnLeftClicked
  (bind _diary (Variables|Default|GetDiary))
  (bind _diary_2 (Variables|Default|GetDiary))
  (if (not (Audio|Components|Audio|IsPlaying (Variables|Default|GetDiary)))
    (Collision|SetCollisionProfileName (Utilities|Array|Get(acopy) (Variables|Default|GetWidgets) (Variables|Default|GetWidgetIndexSecondary)) "NoCollision" false :!class /Script/Engine.PrimitiveComponent)
    (CallFunction|SetNewSecondaryIndex -1)
    (Collision|SetCollisionProfileName (Utilities|Array|Get(acopy) (Variables|Default|GetWidgets) (Variables|Default|GetWidgetIndexSecondary)) "UI" false :!class /Script/Engine.PrimitiveComponent)
    (Components|Timeline|SetPlayRate _diary 1.0)
    (Audio|Components|Audio|Play _diary false)
    (Utilities|FlowControl|Delay (Animation|GetPlayLength (.animtoplay (Variables|/Script/Engine.SkeletalMeshComponent|GetAnimationData _diary))))
    (Components|Animation|SetPosition _diary_2 0.0 true)
    (Audio|Components|Audio|Stop _diary_2)
    (Variables|Default|SetWidgetIndexPrimary (Variables|Default|GetWidgetIndexSecondary))))

(event Custom|OnRightClicked
  (bind _diary (Variables|Default|GetDiary))
  (bind _diary_2 (Variables|Default|GetDiary))
  (bind _animationdata (Variables|/Script/Engine.SkeletalMeshComponent|GetAnimationData _diary))
  (bind _returnvalue (Animation|GetPlayLength (.animtoplay _animationdata)))
  (if (not (Audio|Components|Audio|IsPlaying (Variables|Default|GetDiary)))
    (Variables|Default|SetWidgetIndexSecondary (Variables|Default|GetWidgetIndexPrimary))
    (Collision|SetCollisionProfileName (Utilities|Array|Get(acopy) (Variables|Default|GetWidgets) (Variables|Default|GetWidgetIndexPrimary)) "NoCollision" false :!class /Script/Engine.PrimitiveComponent)
    (CallFunction|SetNewPrimaryIndex 1)
    (Collision|SetCollisionProfileName (Utilities|Array|Get(acopy) (Variables|Default|GetWidgets) (Variables|Default|GetWidgetIndexPrimary)) "UI" false :!class /Script/Engine.PrimitiveComponent)
    (Components|Animation|SetPosition _diary _returnvalue true)
    (Components|Timeline|SetPlayRate _diary -1.0)
    (Audio|Components|Audio|Play _diary false)
    (Utilities|FlowControl|Delay _returnvalue)
    (Audio|Components|Audio|Stop _diary_2)
    (Components|Animation|SetPosition _diary_2 0.0 true)))

(event EventBeginPlay
  (CallFunction|DynamicMaterialCreation)
  (CallFunction|CreatingWidgetsArray)
  (bind _aswbp_arrows (Utilities|Casting|CastToWBP_Arrows (UserInterface|GetUserWidgetObject (Variables|Default|GetWBP_Arrows))))
  (EventDispatchers|BindEventtoOnLeftClicked _aswbp_arrows (delegate Custom|OnLeftClicked))
  (EventDispatchers|BindEventtoOnRightClicked _aswbp_arrows (delegate Custom|OnRightClicked)))

(event EventTick
  (params (DeltaSeconds :type Float%20%28single-precision%29))
  (Rendering|Material|SetTextureParameterValue (Variables|Default|GetDMI_PagePrimary) "Widget" (Class|WidgetComponent|GetRenderTarget (Utilities|Array|Get(acopy) (Variables|Default|GetWidgets) (Variables|Default|GetWidgetIndexPrimary))))
  (Rendering|Material|SetTextureParameterValue (Variables|Default|GetDMI_PageSecondary) "Widget" (Class|WidgetComponent|GetRenderTarget (Utilities|Array|Get(acopy) (Variables|Default|GetWidgets) (Variables|Default|GetWidgetIndexSecondary)))))

(event EventInteract
  (params (LookingComponent :type Primitive%20Component%20Object%20Reference))
  (bind _returnvalue (Game|GetPlayerController 0))
  (Input|SetInputModeGameandUI _returnvalue (UserInterface|GetWidget (Variables|Default|GetWBP_Arrows)) "DoNotLock" false true)
  (Variables|/Script/Engine.PlayerController|SetbShowMouseCursor _returnvalue true))

(fn ConstructionScript)

(fn DynamicMaterialCreation
  (bind _diary (Variables|Default|GetDiary))
  (bind _returnvalue (Rendering|Material|CreateDynamicMaterialInstance _diary 1 "/Game/Assets/Models/Diary/M_DiaryPages.M_DiaryPages" "None" :!class /Script/Engine.PrimitiveComponent))
  (Variables|Default|SetDMI_PageSecondary _returnvalue)
  (bind _returnvalue_2 (Rendering|Material|CreateDynamicMaterialInstance _diary 2 "/Game/Assets/Models/Diary/M_DiaryPages.M_DiaryPages" "None" :!class /Script/Engine.PrimitiveComponent))
  (Variables|Default|SetDMI_PagePrimary _returnvalue_2))

(fn CreatingWidgetsArray
  (Utilities|Array|Add (Variables|Default|GetWidgets) (Variables|Default|GetWBP_Option))
  (Utilities|Array|Add (Variables|Default|GetWidgets) (Variables|Default|GetWBP_Inventory))
  (Utilities|Array|Add (Variables|Default|GetWidgets) (Variables|Default|GetWBP_Ghosts)))

(fn SetNewSecondaryIndex
  (params (Offset :type Integer))
  (bind _widgets (Variables|Default|GetWidgets))
  (bind _widgetindexprimary (Variables|Default|GetWidgetIndexPrimary))
  (bind _returnvalue (Utilities|Array|Length _widgets))
  (bind _returnvalue_2 (+ _widgetindexprimary Offset))
  (bind _returnvalue_3 (Math|Integer|%(Integer) _returnvalue_2 _returnvalue))
  (if (< _returnvalue_3 0)
    (Variables|Default|SetWidgetIndexSecondary (- _returnvalue 1))
    (else
      (Variables|Default|SetWidgetIndexSecondary _returnvalue_3))))

(fn SetNewPrimaryIndex
  (params (Offset :type Integer))
  (bind _widgets (Variables|Default|GetWidgets))
  (bind _widgetindexsecondary (Variables|Default|GetWidgetIndexSecondary))
  (bind _returnvalue (Utilities|Array|Length _widgets))
  (bind _returnvalue_2 (+ _widgetindexsecondary Offset))
  (bind _returnvalue_3 (Math|Integer|%(Integer) _returnvalue_2 _returnvalue))
  (if (< _returnvalue_3 0)
    (Variables|Default|SetWidgetIndexPrimary (- _returnvalue 1))
    (else
      (Variables|Default|SetWidgetIndexPrimary _returnvalue_3))))