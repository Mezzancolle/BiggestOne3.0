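; BP_Diary is the player's diary, an animated book that shows the option and inventory widgets on its pages.
; Each tick it copies both widgets' render targets into dynamic M_DiaryPages materials on the two page slots.
; Clicks on the WBP_Arrows widget play the diary animation, with play rate sign setting the direction.
; Interact shows the mouse cursor and switches input to game and UI, focused on the arrows.
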(event Custom|OnLeftClicked
  (bind _diary (Variables|Default|GetDiary))
  (bind _diary_2 (Variables|Default|GetDiary))
  (if (Audio|Components|Audio|IsPlaying _diary_2)
    (Audio|Components|Audio|Stop _diary_2)
    (Components|Timeline|SetPlayRate _diary_2 1.0)
    (Audio|Components|Audio|Play _diary_2 false)
    (else
      (if (== (Components|Animation|GetPlayRate _diary) 1.0)
        _
        (else
          (Components|Timeline|SetPlayRate _diary 1.0)))
      (Audio|Components|Audio|Play _diary_2 false))))

(event Custom|OnRightClicked
  (bind _diary (Variables|Default|GetDiary))
  (bind _diary_2 (Variables|Default|GetDiary))
  (if (Audio|Components|Audio|IsPlaying _diary_2)
    (Audio|Components|Audio|Stop _diary_2)
    (Components|Timeline|SetPlayRate _diary_2 -1.0)
    (Audio|Components|Audio|Play _diary_2 false)
    (else
      (if (== (Components|Animation|GetPlayRate _diary) -1.0)
        _
        (else
          (Components|Timeline|SetPlayRate _diary -1.0)))
      (Audio|Components|Audio|Play _diary_2 false))))

(event EventBeginPlay
  (bind _diary (Variables|Default|GetDiary))
  (bind _returnvalue (Rendering|Material|CreateDynamicMaterialInstance _diary 1 "/Game/Assets/Models/Diary/M_DiaryPages.M_DiaryPages" "None" :!class /Script/Engine.PrimitiveComponent))
  (Variables|Default|SetDMI_PageDown _returnvalue)
  (bind _returnvalue_2 (Rendering|Material|CreateDynamicMaterialInstance _diary 2 "/Game/Assets/Models/Diary/M_DiaryPages.M_DiaryPages" "None" :!class /Script/Engine.PrimitiveComponent))
  (Variables|Default|SetDMI_PageUp _returnvalue_2)
  (Audio|Components|Audio|Stop (Variables|Default|GetDiary))
  (bind _aswbp_arrows (Utilities|Casting|CastToWBP_Arrows (UserInterface|GetUserWidgetObject (Variables|Default|GetWBP_Arrows))))
  (EventDispatchers|BindEventtoOnLeftClicked _aswbp_arrows (delegate Custom|OnLeftClicked))
  (EventDispatchers|BindEventtoOnRightClicked _aswbp_arrows (delegate Custom|OnRightClicked)))

(event EventTick
  (params (DeltaSeconds :type Float%20%28single-precision%29))
  (Rendering|Material|SetTextureParameterValue (Variables|Default|GetDMI_PageUp) "Widget" (Class|WidgetComponent|GetRenderTarget (Variables|Default|GetWBP_Option)))
  (Rendering|Material|SetTextureParameterValue (Variables|Default|GetDMI_PageDown) "Widget" (Class|WidgetComponent|GetRenderTarget (Variables|Default|GetWBP_Inventory))))

(event EventInteract
  (params (LookingComponent :type Primitive%20Component%20Object%20Reference))
  (bind _returnvalue (Game|GetPlayerController 0))
  (Input|SetInputModeGameandUI _returnvalue (UserInterface|GetWidget (Variables|Default|GetWBP_Arrows)) "DoNotLock" false true)
  (Variables|/Script/Engine.PlayerController|SetbShowMouseCursor _returnvalue true))

(fn ConstructionScript)