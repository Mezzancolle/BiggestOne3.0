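; BP_WallLantern is a wall lantern prop for WesterTown that can be lit or unlit through the LightOn flag.
; The flag sets the visibility of the SpotLight and Niagara components together, without propagating to their children.
; The Construction Script and BeginPlay repeat the same check, so the state is applied both at construction and when play begins.
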(event EventBeginPlay
  (bind _spotlight (Variables|Default|GetSpotLight))
  (if (Variables|Default|GetLightOn)
    (Rendering|SetVisibility _spotlight true false)
    (else
      (Rendering|SetVisibility _spotlight false false))))

(event Collision|EventActorBeginOverlap
  (params (OtherActor :type Actor%20Object%20Reference)))

(fn ConstructionScript
  (bind _spotlight (Variables|Default|GetSpotLight))
  (if (Variables|Default|GetLightOn)
    (Rendering|SetVisibility _spotlight true false)
    (else
      (Rendering|SetVisibility _spotlight false false))))