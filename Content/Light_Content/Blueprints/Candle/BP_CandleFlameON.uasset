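; BP_CandleFlameON is a candle flame Blueprint that can be switched between lit and extinguished.
; The LightOut event sets the PointLight intensity to zero and hides both flame card components, while Light_In restores a fixed bright intensity and shows them.
; It has no logic on begin play, overlap, tick or construction, and nothing in its own graph calls either event.
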(event Custom|LightOut
  (Rendering|Components|Light|SetIntensity (Variables|Default|GetPointLight) 0.0)
  (Rendering|SetVisibility (Variables|Default|GetFlameCard) false false))

(event Custom|Light_In
  (Rendering|Components|Light|SetIntensity (Variables|Default|GetPointLight) 3e+04)
  (Rendering|SetVisibility (Variables|Default|GetFlameCard) true false))

(event EventBeginPlay)

(event Collision|EventActorBeginOverlap
  (params (OtherActor :type Actor%20Object%20Reference)))

(event EventTick
  (params (DeltaSeconds :type Float%20%28single-precision%29)))

(fn ConstructionScript)